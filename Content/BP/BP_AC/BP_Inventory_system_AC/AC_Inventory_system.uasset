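; Inventory component that holds the current items as BP_inventorn_object instances and adds to or checks them.
; AddInventoryData stacks existing non-unique items up to their maximum; unique or unfound items become new objects from matching T_inventory_table rows.
; CheckInventoryEnough matches name, index and type, then calls the still-empty RemoveInventoryData for each sufficient item.
; FindByIndex returns on the first element, so lookups only test that one.
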(event EventBeginPlay)

(event EventTick
  (params (DeltaSeconds :type Float%20%28single-precision%29)))

(fn AddInventoryData
  (params (RowName :type Name) (inventory_info :type Array%20of%20St%20Inventory%20Number%20Structures))
  (for _array_element inventory_info
    (bind (_array_element_2 _is_vaild) (B1|FindbyIndex (Variables|Default|GetCurrent%20inventory) (Utilities|Struct|BreakST_Inventory_lite_info (.inventory_info (Utilities|Struct|Breakst_inventory_number _array_element)))))
    (if _is_vaild ; 是否存在
      (if (.unique (Utilities|Struct|BreakST_Inventory_base_info (Variables|/Game/BP/BP_AC/BP_Inventory_system_AC/BP_inventorn_object.BP_inventorn_object_C|Getbase_info _array_element_2))) ; 是否唯一
        (bind _returnvalue (Utilities|GetDataTableRow "/Game/Struct/Inventory_system/T_inventory_table.T_inventory_table" RowName :!label _label)
          (:then
            (if (and (== (.Inventory_name (Utilities|Struct|BreakST_Inventory_base_info _returnvalue)) (.Inventory_name (Utilities|Struct|BreakST_Inventory_lite_info (Utilities|Struct|Breakst_inventory_number _array_element)))) (== (.Inventory_index (Utilities|Struct|BreakST_Inventory_base_info _returnvalue)) (.Inventory_index (Utilities|Struct|BreakST_Inventory_lite_info (Utilities|Struct|Breakst_inventory_number _array_element)))))
              (bind _returnvalue_2 (Game|ConstructObjectfromClass "/Game/BP/BP_AC/BP_Inventory_system_AC/BP_inventorn_object.BP_inventorn_object_C"))
              (Default|Initialization _returnvalue_2 _returnvalue)
              (Utilities|Array|Add (Variables|Default|GetCurrent%20inventory) _returnvalue_2))))
        (elif (> (+ (Variables|/Game/BP/BP_AC/BP_Inventory_system_AC/BP_inventorn_object.BP_inventorn_object_C|Getcurrent_number _array_element_2) (.number (Utilities|Struct|Breakst_inventory_number _array_element))) (.maximum (Utilities|Struct|BreakST_Inventory_base_info (Variables|/Game/BP/BP_AC/BP_Inventory_system_AC/BP_inventorn_object.BP_inventorn_object_C|Getbase_info _array_element_2)))) ; 检查数量
          (Variables|/Game/BP/BP_AC/BP_Inventory_system_AC/BP_inventorn_object.BP_inventorn_object_C|Setcurrent_number _array_element_2 (.maximum (Utilities|Struct|BreakST_Inventory_base_info (Variables|/Game/BP/BP_AC/BP_Inventory_system_AC/BP_inventorn_object.BP_inventorn_object_C|Getbase_info _array_element_2))))
          (Utilities|Array|SetArrayElem (Variables|Default|GetCurrent%20inventory) 0 _array_element_2)
          (else
            (Variables|/Game/BP/BP_AC/BP_Inventory_system_AC/BP_inventorn_object.BP_inventorn_object_C|Setcurrent_number _array_element_2 (+ (Variables|/Game/BP/BP_AC/BP_Inventory_system_AC/BP_inventorn_object.BP_inventorn_object_C|Getcurrent_number _array_element_2) (.number (Utilities|Struct|Breakst_inventory_number _array_element))))
            (Utilities|Array|SetArrayElem (Variables|Default|GetCurrent%20inventory) 0 _array_element_2))))
      (else
        (goto _label)))))

(fn RemoveInventoryData)

(fn CheckInventoryEnough
  (params (inventory :type Array%20of%20St%20Inventory%20Number%20Structures))
  (for _array_element (Variables|Default|GetCurrent%20inventory)
    (for _array_element_2 inventory
      (if (Math|Boolean|ANDBoolean (== (.Inventory_name (Utilities|Struct|BreakST_Inventory_lite_info (.inventory_info (Utilities|Struct|Breakst_inventory_number _array_element_2)))) (.Inventory_name (Utilities|Struct|BreakST_Inventory_base_info (Variables|/Game/BP/BP_AC/BP_Inventory_system_AC/BP_inventorn_object.BP_inventorn_object_C|Getbase_info _array_element)))) (== (.Inventory_index (Utilities|Struct|BreakST_Inventory_lite_info (.inventory_info (Utilities|Struct|Breakst_inventory_number _array_element_2)))) (.Inventory_index (Utilities|Struct|BreakST_Inventory_base_info (Variables|/Game/BP/BP_AC/BP_Inventory_system_AC/BP_inventorn_object.BP_inventorn_object_C|Getbase_info _array_element)))) (Utilities|Enum|Equal(Enum) (.Inventory_type (Utilities|Struct|BreakST_Inventory_lite_info (.inventory_info (Utilities|Struct|Breakst_inventory_number _array_element_2)))) (.Inventory_type (Utilities|Struct|BreakST_Inventory_base_info (Variables|/Game/BP/BP_AC/BP_Inventory_system_AC/BP_inventorn_object.BP_inventorn_object_C|Getbase_info _array_element)))))
        (if (>= (Variables|/Game/BP/BP_AC/BP_Inventory_system_AC/BP_inventorn_object.BP_inventorn_object_C|Getcurrent_number _array_element) (.number (Utilities|Struct|Breakst_inventory_number _array_element_2)))
          (CallFunction|RemoveInventoryData))))))

(fn FindbyIndex
  (params (current_inventpry :type Array%20of%20BP%20Inventorn%20Object%20Object%20References) (index :type Integer))
  (for _array_element current_inventpry
    (if (== (.Inventory_index (Utilities|Struct|BreakST_Inventory_base_info (Variables|/Game/BP/BP_AC/BP_Inventory_system_AC/BP_inventorn_object.BP_inventorn_object_C|Getbase_info _array_element))) index)
      (return _array_element true)
      (else
        (return 0 false)))))