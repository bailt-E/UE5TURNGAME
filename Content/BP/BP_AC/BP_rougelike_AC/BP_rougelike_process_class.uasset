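; Process class for a roguelike mode, holding a run's money, info, character, round and process counters, and battle, normal and boss event pools.
; It constructs and initializes an event object from a selected event struct, stores it as the executing event and updates the roguelike component's flow state.
; Event removal takes the current entry out of the pool matching its type, then clears the current event references.
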(fn Initialize
  (params (money :type Integer) (rougelike_info :type ST%20Rougelike%20Chapters%20Structure) (rougelike_role :type Array%20of%20ST%20Rougelike%20Role%20Structures) (battle_event :type Array%20of%20ST%20Rougelike%20Event%20Assembly%20Structures) (rougelike_normal_event :type Array%20of%20ST%20Rougelike%20Event%20Assembly%20Structures) (boss_battle_event :type Array%20of%20ST%20Rougelike%20Event%20Assembly%20Structures) (rougelike_AC :type BP%20Rougelike%20AC%20Object%20Reference))
  (Variables|player|Setmoney money)
  (Variables|Default|Setrougelike_info rougelike_info)
  (Variables|character|Setcurrent_rougelike_character rougelike_role)
  (Variables|data_Event|Setbattle_event battle_event)
  (Variables|data_Event|Setrougelike_normal_event rougelike_normal_event)
  (Variables|data_Event|Setboss_battle_event boss_battle_event)
  (Variables|player|SetCurrent%20process 1)
  (Variables|player|SetThe%20current%20round 1)
  (Variables|Default|Setrougelike_AC rougelike_AC))

(fn ConstructEventClass
  (params (ST_rougelike_event_assembly :type ST%20Rougelike%20Event%20Assembly%20Structure%20%28by%20ref%29))
  (bind (_rougelike_event_type _consumesmoney _rougelike_event_class _current_level) (Utilities|Struct|BreakST_rougelike_event_assembly ST_rougelike_event_assembly))
  (bind _rougelike_ac (Variables|Default|Getrougelike_AC))
  (bind _returnvalue (Game|ConstructObjectfromClass _rougelike_event_class (Variables|Default|Getrougelike_AC)))
  (Default|InitializetheEvent _returnvalue _rougelike_event_type _consumesmoney _current_level (Variables|Default|Getrougelike_AC))
  (Variables|Default|SetExecuting%20event _returnvalue)
  (Variables|/Game/BP/BP_AC/BP_rougelike_AC/BP_rougelike_AC.BP_rougelike_AC_C|Setrougelike_flow _rougelike_ac "NewEnumerator3")
  (Default|MIND _rougelike_ac "None")
  (Utilities|Array|RemoveItem (Variables|data_Event|Getcurrent_event) ST_rougelike_event_assembly))

(fn RemoveEventByarray
  (Utilities|FlowControl|Sequence
    (:then_0
      (switch Utilities|FlowControl|Switch|SwitchonE_rougelike_event_type (Variables|/Game/BP/BP_AC/BP_rougelike_AC/BP_Rougelike_Event_class.BP_Rougelike_Event_class_C|Getrougelike_event_type (Variables|Default|GetExecuting%20event))
        (:NewEnumerator0
          (Utilities|Array|RemoveItem (Variables|data_Event|Getbattle_event) (Variables|data_Event|Getthis_event)))
        (:NewEnumerator2
          (Utilities|Array|RemoveItem (Variables|data_Event|Getboss_battle_event) (Variables|data_Event|Getthis_event)))
        (:NewEnumerator1
          (Utilities|Array|RemoveItem (Variables|data_Event|Getrougelike_normal_event) (Variables|data_Event|Getthis_event)))))
    (:then_1
      (Utilities|Array|Clear (Variables|data_Event|Getcurrent_event))
      (Variables|Default|SetExecuting%20event 0)
      (Variables|data_Event|Setthis_event ""))))