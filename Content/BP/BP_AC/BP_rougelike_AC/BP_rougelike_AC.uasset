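; BP_rougelike_AC is a component that runs the roguelike mode's event loop through the MIND state switch on RougelikeFlow.
; It builds a BP_rougelike_process_class from a data table to hold money, progress, event pools and roster.
; Events spawn as a boss or a money-weighted battle/normal mix, then get selected, executed and completed, with UI switching.
; Helpers refresh events back into pools, leveling escalatable ones, and derive battle and team bonuses from blessings.
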(event Custom|Bind_rougelike_event
  ;[1 1 1] 这个绑定好像没用，单走都行
  (EventDispatchers|BindEventtoTiggerEventEnd (Variables|/Game/BP/BP_AC/BP_rougelike_AC/BP_rougelike_process_class.BP_rougelike_process_class_C|GetExecuting%20event (Variables|player|Getrougelike_process)) (delegate Custom|Event%20stage)))

(event Custom|Event%20stage
  ;[1 1 1] 这个绑定好像没用，单走都行
)

(fn GainBonusesBasedonBlessings
  (Variables|/Game/BP/BP_AC/BP_rougelike_AC/BP_rougelike_process_class.BP_rougelike_process_class_C|Setteam_bonus (Variables|player|Getrougelike_process) "")
  (for _array_element (Variables|/Game/BP/BP_AC/BP_rougelike_AC/BP_rougelike_process_class.BP_rougelike_process_class_C|Getrougelike_blessing (Variables|player|Getrougelike_process))
    (Variables|/Game/BP/BP_AC/BP_rougelike_AC/BP_rougelike_process_class.BP_rougelike_process_class_C|Setbattle_bonus (Variables|player|Getrougelike_process) (Utilities|Struct|MakeST_battle_data (+ (.InitialActionPoint (Utilities|Struct|BreakST_battle_data (Variables|/Game/BP/BP_AC/BP_rougelike_AC/BP_rougelike_blessing.BP_rougelike_blessing_C|GetBattle%20Bonus _array_element))) (.InitialActionPoint (Utilities|Struct|BreakST_battle_data (Variables|/Game/BP/BP_AC/BP_rougelike_AC/BP_rougelike_process_class.BP_rougelike_process_class_C|Getbattle_bonus (Variables|player|Getrougelike_process))))) (+ (.ActionPointLimit (Utilities|Struct|BreakST_battle_data (Variables|/Game/BP/BP_AC/BP_rougelike_AC/BP_rougelike_blessing.BP_rougelike_blessing_C|GetBattle%20Bonus _array_element))) (.ActionPointLimit (Utilities|Struct|BreakST_battle_data (Variables|/Game/BP/BP_AC/BP_rougelike_AC/BP_rougelike_process_class.BP_rougelike_process_class_C|Getbattle_bonus (Variables|player|Getrougelike_process))))) (+ (.GrowthActionPoints (Utilities|Struct|BreakST_battle_data (Variables|/Game/BP/BP_AC/BP_rougelike_AC/BP_rougelike_blessing.BP_rougelike_blessing_C|GetBattle%20Bonus _array_element))) (.GrowthActionPoints (Utilities|Struct|BreakST_battle_data (Variables|/Game/BP/BP_AC/BP_rougelike_AC/BP_rougelike_process_class.BP_rougelike_process_class_C|Getbattle_bonus (Variables|player|Getrougelike_process))))) (+ (.Consumeactionpoints (Utilities|Struct|BreakST_battle_data (Variables|/Game/BP/BP_AC/BP_rougelike_AC/BP_rougelike_blessing.BP_rougelike_blessing_C|GetBattle%20Bonus _array_element))) (.Consumeactionpoints (Utilities|Struct|BreakST_battle_data (Variables|/Game/BP/BP_AC/BP_rougelike_AC/BP_rougelike_process_class.BP_rougelike_process_class_C|Getbattle_bonus (Variables|player|Getrougelike_process))))) (+ (.Theinitialnumberofmoves (Utilities|Struct|BreakST_battle_data (Variables|/Game/BP/BP_AC/BP_rougelike_AC/BP_rougelike_blessing.BP_rougelike_blessing_C|GetBattle%20Bonus _array_element))) (.Theinitialnumberofmoves (Utilities|Struct|BreakST_battle_data (Variables|/Game/BP/BP_AC/BP_rougelike_AC/BP_rougelike_process_class.BP_rougelike_process_class_C|Getbattle_bonus (Variables|player|Getrougelike_process))))) (+ (.Thenumberofcyclemoves (Utilities|Struct|BreakST_battle_data (Variables|/Game/BP/BP_AC/BP_rougelike_AC/BP_rougelike_blessing.BP_rougelike_blessing_C|GetBattle%20Bonus _array_element))) (.Thenumberofcyclemoves (Utilities|Struct|BreakST_battle_data (Variables|/Game/BP/BP_AC/BP_rougelike_AC/BP_rougelike_process_class.BP_rougelike_process_class_C|Getbattle_bonus (Variables|player|Getrougelike_process))))) (+ (.Additionalmovementcost (Utilities|Struct|BreakST_battle_data (Variables|/Game/BP/BP_AC/BP_rougelike_AC/BP_rougelike_blessing.BP_rougelike_blessing_C|GetBattle%20Bonus _array_element))) (.Additionalmovementcost (Utilities|Struct|BreakST_battle_data (Variables|/Game/BP/BP_AC/BP_rougelike_AC/BP_rougelike_process_class.BP_rougelike_process_class_C|Getbattle_bonus (Variables|player|Getrougelike_process)))))))
    (Variables|/Game/BP/BP_AC/BP_rougelike_AC/BP_rougelike_process_class.BP_rougelike_process_class_C|Setteam_bonus (Variables|player|Getrougelike_process) (Utilities|Struct|Makest_rougelike_unit_bonus (Utilities|Struct|MakeST_pawn_Base_Stat_bonus (+ (.Healthbonus (Utilities|Struct|BreakST_pawn_Base_Stat_bonus (.basestatbonus (Utilities|Struct|Breakst_rougelike_unit_bonus (Variables|/Game/BP/BP_AC/BP_rougelike_AC/BP_rougelike_blessing.BP_rougelike_blessing_C|Getrougelike_attributs _array_element))))) (.Healthbonus (Utilities|Struct|BreakST_pawn_Base_Stat_bonus (.basestatbonus (Utilities|Struct|Breakst_rougelike_unit_bonus (Variables|/Game/BP/BP_AC/BP_rougelike_AC/BP_rougelike_blessing.BP_rougelike_blessing_C|Getrougelike_attributs _array_element)))))) (+ (.Attackdamagebonus (Utilities|Struct|BreakST_pawn_Base_Stat_bonus (.basestatbonus (Utilities|Struct|Breakst_rougelike_unit_bonus (Variables|/Game/BP/BP_AC/BP_rougelike_AC/BP_rougelike_blessing.BP_rougelike_blessing_C|Getrougelike_attributs _array_element))))) (.Attackdamagebonus (Utilities|Struct|BreakST_pawn_Base_Stat_bonus (.basestatbonus (Utilities|Struct|Breakst_rougelike_unit_bonus (Variables|/Game/BP/BP_AC/BP_rougelike_AC/BP_rougelike_blessing.BP_rougelike_blessing_C|Getrougelike_attributs _array_element)))))) (+ (.Defensebonus (Utilities|Struct|BreakST_pawn_Base_Stat_bonus (.basestatbonus (Utilities|Struct|Breakst_rougelike_unit_bonus (Variables|/Game/BP/BP_AC/BP_rougelike_AC/BP_rougelike_blessing.BP_rougelike_blessing_C|Getrougelike_attributs _array_element))))) (.Defensebonus (Utilities|Struct|BreakST_pawn_Base_Stat_bonus (.basestatbonus (Utilities|Struct|Breakst_rougelike_unit_bonus (Variables|/Game/BP/BP_AC/BP_rougelike_AC/BP_rougelike_blessing.BP_rougelike_blessing_C|Getrougelike_attributs _array_element)))))) (+ (.Speedbonus (Utilities|Struct|BreakST_pawn_Base_Stat_bonus (.basestatbonus (Utilities|Struct|Breakst_rougelike_unit_bonus (Variables|/Game/BP/BP_AC/BP_rougelike_AC/BP_rougelike_blessing.BP_rougelike_blessing_C|Getrougelike_attributs _array_element))))) (.Speedbonus (Utilities|Struct|BreakST_pawn_Base_Stat_bonus (.basestatbonus (Utilities|Struct|Breakst_rougelike_unit_bonus (Variables|/Game/BP/BP_AC/BP_rougelike_AC/BP_rougelike_blessing.BP_rougelike_blessing_C|Getrougelike_attributs _array_element)))))) (+ (.Criticalhitbonus (Utilities|Struct|BreakST_pawn_Base_Stat_bonus (.basestatbonus (Utilities|Struct|Breakst_rougelike_unit_bonus (Variables|/Game/BP/BP_AC/BP_rougelike_AC/BP_rougelike_blessing.BP_rougelike_blessing_C|Getrougelike_attributs _array_element))))) (.Criticalhitbonus (Utilities|Struct|BreakST_pawn_Base_Stat_bonus (.basestatbonus (Utilities|Struct|Breakst_rougelike_unit_bonus (Variables|/Game/BP/BP_AC/BP_rougelike_AC/BP_rougelike_blessing.BP_rougelike_blessing_C|Getrougelike_attributs _array_element)))))) (+ (.Criticaldamagebonus (Utilities|Struct|BreakST_pawn_Base_Stat_bonus (.basestatbonus (Utilities|Struct|Breakst_rougelike_unit_bonus (Variables|/Game/BP/BP_AC/BP_rougelike_AC/BP_rougelike_blessing.BP_rougelike_blessing_C|Getrougelike_attributs _array_element))))) (.Criticaldamagebonus (Utilities|Struct|BreakST_pawn_Base_Stat_bonus (.basestatbonus (Utilities|Struct|Breakst_rougelike_unit_bonus (Variables|/Game/BP/BP_AC/BP_rougelike_AC/BP_rougelike_blessing.BP_rougelike_blessing_C|Getrougelike_attributs _array_element))))))) (Utilities|Struct|MakeST_Edge_attributes_A (+ (.Healingbonus (Utilities|Struct|BreakST_Edge_attributes_A (.edgeattrobutes (Utilities|Struct|Breakst_rougelike_unit_bonus (Variables|/Game/BP/BP_AC/BP_rougelike_AC/BP_rougelike_blessing.BP_rougelike_blessing_C|Getrougelike_attributs _array_element))))) (.Healingbonus (Utilities|Struct|BreakST_Edge_attributes_A (.edgeattrobutes (Utilities|Struct|Breakst_rougelike_unit_bonus (Variables|/Game/BP/BP_AC/BP_rougelike_AC/BP_rougelike_blessing.BP_rougelike_blessing_C|Getrougelike_attributs _array_element)))))) (+ (.Healbonus (Utilities|Struct|BreakST_Edge_attributes_A (.edgeattrobutes (Utilities|Struct|Breakst_rougelike_unit_bonus (Variables|/Game/BP/BP_AC/BP_rougelike_AC/BP_rougelike_blessing.BP_rougelike_blessing_C|Getrougelike_attributs _array_element))))) (.Healbonus (Utilities|Struct|BreakST_Edge_attributes_A (.edgeattrobutes (Utilities|Struct|Breakst_rougelike_unit_bonus (Variables|/Game/BP/BP_AC/BP_rougelike_AC/BP_rougelike_blessing.BP_rougelike_blessing_C|Getrougelike_attributs _array_element)))))) (+ (.Shieldedbonus (Utilities|Struct|BreakST_Edge_attributes_A (.edgeattrobutes (Utilities|Struct|Breakst_rougelike_unit_bonus (Variables|/Game/BP/BP_AC/BP_rougelike_AC/BP_rougelike_blessing.BP_rougelike_blessing_C|Getrougelike_attributs _array_element))))) (.Shieldedbonus (Utilities|Struct|BreakST_Edge_attributes_A (.edgeattrobutes (Utilities|Struct|Breakst_rougelike_unit_bonus (Variables|/Game/BP/BP_AC/BP_rougelike_AC/BP_rougelike_blessing.BP_rougelike_blessing_C|Getrougelike_attributs _array_element)))))) (+ (.Shieldbonus (Utilities|Struct|BreakST_Edge_attributes_A (.edgeattrobutes (Utilities|Struct|Breakst_rougelike_unit_bonus (Variables|/Game/BP/BP_AC/BP_rougelike_AC/BP_rougelike_blessing.BP_rougelike_blessing_C|Getrougelike_attributs _array_element))))) (.Shieldbonus (Utilities|Struct|BreakST_Edge_attributes_A (.edgeattrobutes (Utilities|Struct|Breakst_rougelike_unit_bonus (Variables|/Game/BP/BP_AC/BP_rougelike_AC/BP_rougelike_blessing.BP_rougelike_blessing_C|Getrougelike_attributs _array_element)))))) (+ (.aggro_bonus (Utilities|Struct|BreakST_Edge_attributes_A (.edgeattrobutes (Utilities|Struct|Breakst_rougelike_unit_bonus (Variables|/Game/BP/BP_AC/BP_rougelike_AC/BP_rougelike_blessing.BP_rougelike_blessing_C|Getrougelike_attributs _array_element))))) (.aggro_bonus (Utilities|Struct|BreakST_Edge_attributes_A (.edgeattrobutes (Utilities|Struct|Breakst_rougelike_unit_bonus (Variables|/Game/BP/BP_AC/BP_rougelike_AC/BP_rougelike_blessing.BP_rougelike_blessing_C|Getrougelike_attributs _array_element))))))) (Utilities|Struct|MakeST_Fixed_attributes_A (+ (.Speedcap (Utilities|Struct|BreakST_Fixed_attributes_A (.fixedattrobutes (Utilities|Struct|Breakst_rougelike_unit_bonus (Variables|/Game/BP/BP_AC/BP_rougelike_AC/BP_rougelike_blessing.BP_rougelike_blessing_C|Getrougelike_attributs _array_element))))) (.Speedcap (Utilities|Struct|BreakST_Fixed_attributes_A (.fixedattrobutes (Utilities|Struct|Breakst_rougelike_unit_bonus (Variables|/Game/BP/BP_AC/BP_rougelike_AC/BP_rougelike_blessing.BP_rougelike_blessing_C|Getrougelike_attributs _array_element)))))) (+ (.Overloadroundcap (Utilities|Struct|BreakST_Fixed_attributes_A (.fixedattrobutes (Utilities|Struct|Breakst_rougelike_unit_bonus (Variables|/Game/BP/BP_AC/BP_rougelike_AC/BP_rougelike_blessing.BP_rougelike_blessing_C|Getrougelike_attributs _array_element))))) (.Overloadroundcap (Utilities|Struct|BreakST_Fixed_attributes_A (.fixedattrobutes (Utilities|Struct|Breakst_rougelike_unit_bonus (Variables|/Game/BP/BP_AC/BP_rougelike_AC/BP_rougelike_blessing.BP_rougelike_blessing_C|Getrougelike_attributs _array_element)))))) (+ (.Maximumshield (Utilities|Struct|BreakST_Fixed_attributes_A (.fixedattrobutes (Utilities|Struct|Breakst_rougelike_unit_bonus (Variables|/Game/BP/BP_AC/BP_rougelike_AC/BP_rougelike_blessing.BP_rougelike_blessing_C|Getrougelike_attributs _array_element))))) (.Maximumshield (Utilities|Struct|BreakST_Fixed_attributes_A (.fixedattrobutes (Utilities|Struct|Breakst_rougelike_unit_bonus (Variables|/Game/BP/BP_AC/BP_rougelike_AC/BP_rougelike_blessing.BP_rougelike_blessing_C|Getrougelike_attributs _array_element)))))) (+ (.Overloadcap (Utilities|Struct|BreakST_Fixed_attributes_A (.fixedattrobutes (Utilities|Struct|Breakst_rougelike_unit_bonus (Variables|/Game/BP/BP_AC/BP_rougelike_AC/BP_rougelike_blessing.BP_rougelike_blessing_C|Getrougelike_attributs _array_element))))) (.Overloadcap (Utilities|Struct|BreakST_Fixed_attributes_A (.fixedattrobutes (Utilities|Struct|Breakst_rougelike_unit_bonus (Variables|/Game/BP/BP_AC/BP_rougelike_AC/BP_rougelike_blessing.BP_rougelike_blessing_C|Getrougelike_attributs _array_element)))))) (+ (.Energycap (Utilities|Struct|BreakST_Fixed_attributes_A (.fixedattrobutes (Utilities|Struct|Breakst_rougelike_unit_bonus (Variables|/Game/BP/BP_AC/BP_rougelike_AC/BP_rougelike_blessing.BP_rougelike_blessing_C|Getrougelike_attributs _array_element))))) (.Energycap (Utilities|Struct|BreakST_Fixed_attributes_A (.fixedattrobutes (Utilities|Struct|Breakst_rougelike_unit_bonus (Variables|/Game/BP/BP_AC/BP_rougelike_AC/BP_rougelike_blessing.BP_rougelike_blessing_C|Getrougelike_attributs _array_element)))))) (+ (.unit_Actionpointcap (Utilities|Struct|BreakST_Fixed_attributes_A (.fixedattrobutes (Utilities|Struct|Breakst_rougelike_unit_bonus (Variables|/Game/BP/BP_AC/BP_rougelike_AC/BP_rougelike_blessing.BP_rougelike_blessing_C|Getrougelike_attributs _array_element))))) (.unit_Actionpointcap (Utilities|Struct|BreakST_Fixed_attributes_A (.fixedattrobutes (Utilities|Struct|Breakst_rougelike_unit_bonus (Variables|/Game/BP/BP_AC/BP_rougelike_AC/BP_rougelike_blessing.BP_rougelike_blessing_C|Getrougelike_attributs _array_element)))))) (+ (.element_tag_number_MAX (Utilities|Struct|BreakST_Fixed_attributes_A (.fixedattrobutes (Utilities|Struct|Breakst_rougelike_unit_bonus (Variables|/Game/BP/BP_AC/BP_rougelike_AC/BP_rougelike_blessing.BP_rougelike_blessing_C|Getrougelike_attributs _array_element))))) (.element_tag_number_MAX (Utilities|Struct|BreakST_Fixed_attributes_A (.fixedattrobutes (Utilities|Struct|Breakst_rougelike_unit_bonus (Variables|/Game/BP/BP_AC/BP_rougelike_AC/BP_rougelike_blessing.BP_rougelike_blessing_C|Getrougelike_attributs _array_element)))))) (+ (.Initialvelocity (Utilities|Struct|BreakST_Fixed_attributes_A (.fixedattrobutes (Utilities|Struct|Breakst_rougelike_unit_bonus (Variables|/Game/BP/BP_AC/BP_rougelike_AC/BP_rougelike_blessing.BP_rougelike_blessing_C|Getrougelike_attributs _array_element))))) (.Initialvelocity (Utilities|Struct|BreakST_Fixed_attributes_A (.fixedattrobutes (Utilities|Struct|Breakst_rougelike_unit_bonus (Variables|/Game/BP/BP_AC/BP_rougelike_AC/BP_rougelike_blessing.BP_rougelike_blessing_C|Getrougelike_attributs _array_element)))))) (+ (.Initial_unit_actionpoint (Utilities|Struct|BreakST_Fixed_attributes_A (.fixedattrobutes (Utilities|Struct|Breakst_rougelike_unit_bonus (Variables|/Game/BP/BP_AC/BP_rougelike_AC/BP_rougelike_blessing.BP_rougelike_blessing_C|Getrougelike_attributs _array_element))))) (.Initial_unit_actionpoint (Utilities|Struct|BreakST_Fixed_attributes_A (.fixedattrobutes (Utilities|Struct|Breakst_rougelike_unit_bonus (Variables|/Game/BP/BP_AC/BP_rougelike_AC/BP_rougelike_blessing.BP_rougelike_blessing_C|Getrougelike_attributs _array_element))))))) (Utilities|Struct|MakeST_Secondary_attributes_A 0 (+ (.Finaldamagebonus (Utilities|Struct|BreakST_Secondary_attributes_A (.secondaryattrobutes (Utilities|Struct|Breakst_rougelike_unit_bonus (Variables|/Game/BP/BP_AC/BP_rougelike_AC/BP_rougelike_blessing.BP_rougelike_blessing_C|Getrougelike_attributs _array_element))))) (.Finaldamagebonus (Utilities|Struct|BreakST_Secondary_attributes_A (.secondaryattrobutes (Utilities|Struct|Breakst_rougelike_unit_bonus (Variables|/Game/BP/BP_AC/BP_rougelike_AC/BP_rougelike_blessing.BP_rougelike_blessing_C|Getrougelike_attributs _array_element)))))) (+ (.Damagereductionbonus (Utilities|Struct|BreakST_Secondary_attributes_A (.secondaryattrobutes (Utilities|Struct|Breakst_rougelike_unit_bonus (Variables|/Game/BP/BP_AC/BP_rougelike_AC/BP_rougelike_blessing.BP_rougelike_blessing_C|Getrougelike_attributs _array_element))))) (.Damagereductionbonus (Utilities|Struct|BreakST_Secondary_attributes_A (.secondaryattrobutes (Utilities|Struct|Breakst_rougelike_unit_bonus (Variables|/Game/BP/BP_AC/BP_rougelike_AC/BP_rougelike_blessing.BP_rougelike_blessing_C|Getrougelike_attributs _array_element)))))))))))

(fn SelectThisEvent
  (params (player_rougelike :type BP%20Rougelike%20Process%20Class%20Object%20Reference))
  (if (Variables|/Game/BP/BP_AC/BP_rougelike_AC/BP_rougelike_process_class.BP_rougelike_process_class_C|Getchoose player_rougelike)
    (Default|ConstructEventClass player_rougelike (Variables|/Game/BP/BP_AC/BP_rougelike_AC/BP_rougelike_process_class.BP_rougelike_process_class_C|Getthis_event player_rougelike)) ; 实例化事件并执行事件
    (CallFunction|BindRougelikeEvent)))

(fn ConfirmEventNumber
  (params (player_rougelike :type BP%20Rougelike%20Process%20Class%20Object%20Reference) (Condition :type Boolean))
  (if Condition ; 选择
    (bind _output_get (Variables|/Game/BP/BP_AC/BP_rougelike_AC/BP_rougelike_process_class.BP_rougelike_process_class_C|Setevent_number player_rougelike (Variables|/Game/BP/BP_AC/BP_rougelike_AC/BP_rougelike_process_class.BP_rougelike_process_class_C|Getfix_event_number player_rougelike)))
    (return false _output_get)
    (elif (== (Variables|/Game/BP/BP_AC/BP_rougelike_AC/BP_rougelike_process_class.BP_rougelike_process_class_C|Getevent_number player_rougelike) 0)
      (bind _output_get_2 (Variables|/Game/BP/BP_AC/BP_rougelike_AC/BP_rougelike_process_class.BP_rougelike_process_class_C|Setevent_number player_rougelike 1))
      (return true _output_get_2))))

(fn AfterSelectingtheEvent
  (params (event :type BP%20Rougelike%20Event%20Class%20Object%20Reference) (player_process :type BP%20Rougelike%20Process%20Class%20Object%20Reference))
  (bind _event_widget (Variables|/Game/BP/BP_AC/BP_rougelike_AC/BP_rougelike_process_class.BP_rougelike_process_class_C|Getevent_widget player_process))
  (Utilities|FlowControl|Sequence
    (:then_0
      ;[1 1 1] 减少货币
      (Variables|/Game/BP/BP_AC/BP_rougelike_AC/BP_rougelike_process_class.BP_rougelike_process_class_C|Setmoney player_process (- (Variables|/Game/BP/BP_AC/BP_rougelike_AC/BP_rougelike_process_class.BP_rougelike_process_class_C|Getmoney player_process) (Variables|/Game/BP/BP_AC/BP_rougelike_AC/BP_Rougelike_Event_class.BP_Rougelike_Event_class_C|GetConsumes%20money (Variables|/Game/BP/BP_AC/BP_rougelike_AC/BP_rougelike_process_class.BP_rougelike_process_class_C|GetExecuting%20event player_process)))))
    (:then_1
      (Utilities|Array|Add (Variables|/Game/BP/BP_AC/BP_rougelike_AC/BP_rougelike_process_class.BP_rougelike_process_class_C|Getwait_remove_event player_process) event)
      (Utilities|Array|Clear (Variables|/Game/BP/BP_AC/BP_rougelike_AC/BP_rougelike_process_class.BP_rougelike_process_class_C|Getwait_remove_event player_process))
      (bind _aswbp_rougelike_evnt_event_card_widget (Utilities|Casting|CastToWBP_rougelike_evnt_event_card_widget _event_widget))
      (Class|PanelWidget|RemoveChild (Variables|/Game/WBP_common_ui/Small_widget/WBP_rougelike_evnt_event_card_widget.WBP_rougelike_evnt_event_card_widget_C|Get水平框 _aswbp_rougelike_evnt_event_card_widget) _event_widget))
    (:then_2
      ;[1 1 1] 注释
      (if (> (Variables|/Game/BP/BP_AC/BP_rougelike_AC/BP_rougelike_process_class.BP_rougelike_process_class_C|GetCurrent%20process player_process) (Variables|/Game/BP/BP_AC/BP_rougelike_AC/BP_rougelike_process_class.BP_rougelike_process_class_C|GetProcess%20caps player_process))
        (Variables|/Game/BP/BP_AC/BP_rougelike_AC/BP_rougelike_process_class.BP_rougelike_process_class_C|SetCurrent%20process player_process 1)
        (Variables|/Game/BP/BP_AC/BP_rougelike_AC/BP_rougelike_process_class.BP_rougelike_process_class_C|SetThe%20current%20round player_process (+ (Variables|/Game/BP/BP_AC/BP_rougelike_AC/BP_rougelike_process_class.BP_rougelike_process_class_C|GetThe%20current%20round player_process) 1))
        (else
          (bind _result (Math|Integer|IncrementInt (Variables|/Game/BP/BP_AC/BP_rougelike_AC/BP_rougelike_process_class.BP_rougelike_process_class_C|GetCurrent%20process player_process))
            (:%20%20
              (Variables|/Game/BP/BP_AC/BP_rougelike_AC/BP_rougelike_process_class.BP_rougelike_process_class_C|SetCurrent%20process player_process _result))))))))

(fn CheakRoleActorpoint
  (params (player_process :type BP%20Rougelike%20Process%20Class%20Object%20Reference))
  (for _array_element (Variables|/Game/BP/BP_AC/BP_rougelike_AC/BP_rougelike_process_class.BP_rougelike_process_class_C|Getcurrent_rougelike_character player_process)
    (if (>= (.Numberofactions (Utilities|Struct|BreakST_Rougelike_role _array_element)) 0)
      (bind _returnvalue (Utilities|Array|Add (Variables|/Game/BP/BP_AC/BP_rougelike_AC/BP_rougelike_process_class.BP_rougelike_process_class_C|Getdisuse_rougelike_role player_process) _array_element))
      (Utilities|Array|RemoveIndex (Variables|/Game/BP/BP_AC/BP_rougelike_AC/BP_rougelike_process_class.BP_rougelike_process_class_C|Getcurrent_rougelike_character player_process) _returnvalue))))

(fn GenerateEvents
  (params (playerrougelike :type BP%20Rougelike%20Process%20Class%20Object%20Reference) (spawnboss_event :type Boolean) (need%20event_number :type Integer))
  (bind _boss_battle_event (Variables|/Game/BP/BP_AC/BP_rougelike_AC/BP_rougelike_process_class.BP_rougelike_process_class_C|Getboss_battle_event playerrougelike))
  (bind _rougelike_normal_event (Variables|/Game/BP/BP_AC/BP_rougelike_AC/BP_rougelike_process_class.BP_rougelike_process_class_C|Getrougelike_normal_event playerrougelike))
  (bind _battle_event (Variables|/Game/BP/BP_AC/BP_rougelike_AC/BP_rougelike_process_class.BP_rougelike_process_class_C|Getbattle_event playerrougelike))
  (bind _output (Utilities|Array|Get(acopy) _battle_event))
  (bind _output_2 (Utilities|Array|Get(acopy) _rougelike_normal_event))
  (bind _output_3 (Utilities|Array|Get(acopy) _boss_battle_event))
  (if spawnboss_event
    ;[1 1 1] 生成boss事件
    (Utilities|Array|Add (Variables|/Game/BP/BP_AC/BP_rougelike_AC/BP_rougelike_process_class.BP_rougelike_process_class_C|Getcurrent_event playerrougelike) _output_3)
    (Utilities|Array|RemoveItem (Variables|/Game/BP/BP_AC/BP_rougelike_AC/BP_rougelike_process_class.BP_rougelike_process_class_C|Getboss_battle_event playerrougelike) _output_3)
    (else
      (while (< (Utilities|Array|Length (Variables|/Game/BP/BP_AC/BP_rougelike_AC/BP_rougelike_process_class.BP_rougelike_process_class_C|Getcurrent_event playerrougelike)) (Variables|/Game/BP/BP_AC/BP_rougelike_AC/BP_rougelike_process_class.BP_rougelike_process_class_C|Getevent_number playerrougelike))
        (bind _output_get (CallFunction|WeightControl))
        (if (> (Math|Random|RandomInteger 100) _output_get)
          (Utilities|Array|Add (Variables|/Game/BP/BP_AC/BP_rougelike_AC/BP_rougelike_process_class.BP_rougelike_process_class_C|Getcurrent_event playerrougelike) _output_2)
          (Utilities|Array|RemoveItem _rougelike_normal_event _output_2)
          (else
            (Utilities|Array|Add (Variables|/Game/BP/BP_AC/BP_rougelike_AC/BP_rougelike_process_class.BP_rougelike_process_class_C|Getcurrent_event playerrougelike) _output)
            (Utilities|Array|RemoveItem _battle_event _output)))))))

(fn ConstructProcessClass
  (params (RowName :type Name))
  (bind _returnvalue (Utilities|GetDataTableRow "/Game/Struct/rougelike_data/T_rougelike_event_C.T_rougelike_event_C" RowName)
    (:then
      (bind _returnvalue_2 (Game|ConstructObjectfromClass "/Game/BP/BP_AC/BP_rougelike_AC/BP_rougelike_process_class.BP_rougelike_process_class_C"))
      (Default|Initialize _returnvalue_2 160 (.rougelike_info (Utilities|Struct|BreakST_Rougelike_chapter_assembly _returnvalue)) (Utilities|Array|MakeArray (Utilities|Struct|MakeST_Rougelike_role "NewEnumerator0" 2 0)) (.Generalevents (Utilities|Struct|BreakST_Rougelike_chapter_assembly _returnvalue)) (.Combatevents (Utilities|Struct|BreakST_Rougelike_chapter_assembly _returnvalue)) (.boss_event (Utilities|Struct|BreakST_Rougelike_chapter_assembly _returnvalue)) self)
      (bind _output_get (Variables|player|Setrougelike_process _returnvalue_2))
      (Variables|/Game/BP/BP_AC/BP_rougelike_AC/BP_rougelike_process_class.BP_rougelike_process_class_C|SetCurrent%20process _output_get 1)
      (Variables|/Game/BP/BP_AC/BP_rougelike_AC/BP_rougelike_process_class.BP_rougelike_process_class_C|SetThe%20current%20round _output_get 1)
      (Variables|/Game/BP/BP_AC/BP_rougelike_AC/BP_rougelike_process_class.BP_rougelike_process_class_C|SetProcess%20caps _output_get 8)
      (Variables|Default|SetGenerate%20Event%20Phase%20Control true))))

(fn MIND
  (params (RowName :type Name))
  (bind _rougelike_process (Variables|player|Getrougelike_process))
  (bind _rougelike_process_2 (Variables|player|Getrougelike_process))
  (bind _rougelike_process_3 (Variables|player|Getrougelike_process))
  (bind _rougelike_process_4 (Variables|player|Getrougelike_process))
  (bind _executing_event (Variables|/Game/BP/BP_AC/BP_rougelike_AC/BP_rougelike_process_class.BP_rougelike_process_class_C|GetExecuting%20event _rougelike_process_2))
  (switch Utilities|FlowControl|Switch|SwitchonE_rougelike_Stage (Variables|Default|Getrougelike_flow)
    (:NewEnumerator0
      (Variables|Default|SetRow%20Name RowName)
      (Initialize|ConstructProcessClass RowName) ; 生成进程类并初始化
      (bind _asbp_game_instance (Utilities|Casting|CastToBP_GameInstance (Game|GetGameInstance)))
      (bind _output_get (Variables|player|SetAs%20BP%20Game%20Instance _asbp_game_instance))
      (Variables|/Game/gamemode/BP_GameInstance.BP_GameInstance_C|Setcurrent_game_mode _output_get "NewEnumerator1"))
    (:NewEnumerator1
      ;[1 1 1] 生成事件
      (bind (_spawn_event _event_n) (event|ConfirmEventNumber _rougelike_process_4 (Variables|Default|GetGenerate%20Event%20Phase%20Control))) ; 确认事件数量
      (event|GenerateEvents _rougelike_process_4 _spawn_event _event_n) ; 生成事件
      (CallFunction|RougelikeUISwitch))
    (:NewEnumerator2
      ;[1 1 1] 选择事件，在UI中根据数组生成卡牌，选择事件为当前事件
      (if (>= (Variables|/Game/BP/BP_AC/BP_rougelike_AC/BP_rougelike_process_class.BP_rougelike_process_class_C|Getmoney _rougelike_process_3) (Utilities|Struct|BreakST_rougelike_event_assembly (Variables|/Game/BP/BP_AC/BP_rougelike_AC/BP_rougelike_process_class.BP_rougelike_process_class_C|Getthis_event _rougelike_process_3))) ; 检测事件所需货币是否足够
        (if (Variables|/Game/BP/BP_AC/BP_rougelike_AC/BP_rougelike_process_class.BP_rougelike_process_class_C|Getchoose (Variables|player|Getrougelike_process)) ; 二次确认
          (Default|ConstructEventClass _rougelike_process (Variables|/Game/BP/BP_AC/BP_rougelike_AC/BP_rougelike_process_class.BP_rougelike_process_class_C|Getthis_event _rougelike_process)) ; 实例化事件
          (CallFunction|BindRougelikeEvent))))
    (:NewEnumerator3
      (Variables|/Game/BP/BP_AC/BP_rougelike_AC/BP_Rougelike_Event_class.BP_Rougelike_Event_class_C|Setrougelike_event_flow _executing_event "NewEnumerator0")
      (CallFunction|RougelikeUISwitch)
      (Default|EventActivation(R3) _executing_event "NewEnumerator0"))
    (:NewEnumerator4
      (CallFunction|EventCompleted)
      (MIND_F|MIND "None"))))

(fn SettletheGameScorefortheGame
  (params (process :type BP%20Rougelike%20Process%20Class%20Object%20Reference))
  (bind _output_get (LocalVariables|Setpoint (+ (* (Variables|/Game/BP/BP_AC/BP_rougelike_AC/BP_rougelike_process_class.BP_rougelike_process_class_C|GetThe%20current%20round process) 50) (* (Variables|/Game/BP/BP_AC/BP_rougelike_AC/BP_rougelike_process_class.BP_rougelike_process_class_C|GetCurrent%20process process) 10))))
  (return _output_get))

(fn EndtheGame
  (bind _as2dplayer_contrller (Utilities|Casting|CastTo2DplayerContrller (Game|GetPlayerController 0)))
  (Variables|/Game/gamemode/2DplayerContrller.2DplayerContrller_C|SetE_level_flow _as2dplayer_contrller "NewEnumerator5"))

(fn GeteventIsThisEvent
  (params (Dimension%201 :type Integer))
  (bind _rougelike_process (Variables|player|Getrougelike_process))
  (Variables|/Game/BP/BP_AC/BP_rougelike_AC/BP_rougelike_process_class.BP_rougelike_process_class_C|Setthis_event _rougelike_process (Utilities|Array|Get(acopy) (Variables|/Game/BP/BP_AC/BP_rougelike_AC/BP_rougelike_process_class.BP_rougelike_process_class_C|Getcurrent_event _rougelike_process) Dimension%201)))

(fn GainARougelikeCharacter
  (params (NewItem :type ST%20Rougelike%20Role%20Structure%20%28by%20ref%29))
  (Utilities|Array|Add (Variables|/Game/BP/BP_AC/BP_rougelike_AC/BP_rougelike_process_class.BP_rougelike_process_class_C|Getcurrent_rougelike_character (Variables|player|Getrougelike_process)) NewItem))

(fn WeightControl
  (if (< (Variables|/Game/BP/BP_AC/BP_rougelike_AC/BP_rougelike_process_class.BP_rougelike_process_class_C|Getmoney (Variables|player|Getrougelike_process)) 100)
    (bind _output_get (LocalVariables|Setweight 100))
    (return _output_get)
    (else
      (bind _output_get_2 (LocalVariables|Setweight 50))
      (return _output_get_2))))

(fn RefreshEvent
  (bind _rougelike_process (Variables|player|Getrougelike_process))
  (Utilities|FlowControl|Sequence
    (:then_0
      (for _array_element (Variables|/Game/BP/BP_AC/BP_rougelike_AC/BP_rougelike_process_class.BP_rougelike_process_class_C|Getcurrent_event (Variables|player|Getrougelike_process))
        (bind _output_get (LocalVariables|Setevent_current_event _array_element))
        (switch Utilities|FlowControl|Switch|SwitchonE_rougelike_event_type (Utilities|Struct|BreakST_rougelike_event_assembly _output_get)
          (:NewEnumerator0
            (CallFunction|ADDEventArray (Variables|/Game/BP/BP_AC/BP_rougelike_AC/BP_rougelike_process_class.BP_rougelike_process_class_C|Getbattle_event (Variables|player|Getrougelike_process)) (LocalVariables|Getevent_current_event))
            (Utilities|Array|RemoveItem (Variables|/Game/BP/BP_AC/BP_rougelike_AC/BP_rougelike_process_class.BP_rougelike_process_class_C|Getcurrent_event (Variables|player|Getrougelike_process)) (LocalVariables|Getevent_current_event)))
          (:NewEnumerator2
            (CallFunction|ADDEventArray (Variables|/Game/BP/BP_AC/BP_rougelike_AC/BP_rougelike_process_class.BP_rougelike_process_class_C|Getboss_battle_event (Variables|player|Getrougelike_process)) (LocalVariables|Getevent_current_event))
            (Utilities|Array|RemoveItem (Variables|/Game/BP/BP_AC/BP_rougelike_AC/BP_rougelike_process_class.BP_rougelike_process_class_C|Getcurrent_event (Variables|player|Getrougelike_process)) (LocalVariables|Getevent_current_event)))
          (:NewEnumerator1
            (CallFunction|ADDEventArray (Variables|/Game/BP/BP_AC/BP_rougelike_AC/BP_rougelike_process_class.BP_rougelike_process_class_C|Getrougelike_normal_event (Variables|player|Getrougelike_process)) (LocalVariables|Getevent_current_event))
            (Utilities|Array|RemoveItem (Variables|/Game/BP/BP_AC/BP_rougelike_AC/BP_rougelike_process_class.BP_rougelike_process_class_C|Getcurrent_event (Variables|player|Getrougelike_process)) (LocalVariables|Getevent_current_event))))))
    (:then_1
      (bind (_spawn_event _event_n) (event|ConfirmEventNumber _rougelike_process false)) ; 确认事件数量
      (event|GenerateEvents _rougelike_process _spawn_event _event_n) ; 生成事件
    )))

(fn ADDEventArray
  (params (TargetArray :type Array%20of%20ST%20Rougelike%20Event%20Assembly%20Structures) (ST_rougelike_event_assembly :type ST%20Rougelike%20Event%20Assembly%20Structure%20%28by%20ref%29))
  (bind (_rougelike_event_name _rougelike_event_type _consumesmoney _cantheincidentescalate_ _level_cap _rougelike_event_class _current_level) (Utilities|Struct|BreakST_rougelike_event_assembly ST_rougelike_event_assembly))
  (bind (_rougelike_event_name_2 _rougelike_event_type_2 _consumesmoney_2 _cantheincidentescalate__2 _level_cap_2 _rougelike_event_class_2 _current_level_2) (Utilities|Struct|BreakST_rougelike_event_assembly ST_rougelike_event_assembly))
  (if (Utilities|Struct|BreakST_rougelike_event_assembly ST_rougelike_event_assembly)
    (Utilities|Array|Add TargetArray (Utilities|Struct|MakeST_rougelike_event_assembly _rougelike_event_name _rougelike_event_type _consumesmoney _cantheincidentescalate_ _level_cap _rougelike_event_class (+ _current_level 1)))
    (else
      (Utilities|Array|Add TargetArray (Utilities|Struct|MakeST_rougelike_event_assembly _rougelike_event_name_2 _rougelike_event_type_2 _consumesmoney_2 _cantheincidentescalate__2 _level_cap_2 _rougelike_event_class_2 _current_level_2)))))

(fn RougelikeUISwitch
  (bind _rougelike_process (Variables|player|Getrougelike_process))
  (bind _executing_event (Variables|/Game/BP/BP_AC/BP_rougelike_AC/BP_rougelike_process_class.BP_rougelike_process_class_C|GetExecuting%20event _rougelike_process))
  (switch Utilities|FlowControl|Switch|SwitchonE_rougelike_Stage (Variables|Default|Getrougelike_flow)
    (:NewEnumerator1
      (bind _returnvalue (Default|UpdataMainUI (Variables|/Game/gamemode/2DplayerContrller.2DplayerContrller_C|GetAC_UI_ManagerComponent (Variables|Default|GetAs%202Dplayer%20Contrller)) "/Game/WBP_common_ui/Bottom_layer_widget/WBP_rougelike_main.WBP_rougelike_main_C"))
      (Utilities|Casting|CastToWBP_rougelike_main _returnvalue))
    (:NewEnumerator3
      (switch Utilities|FlowControl|Switch|SwitchonE_rougelike_event_stage (Variables|/Game/BP/BP_AC/BP_rougelike_AC/BP_Rougelike_Event_class.BP_Rougelike_Event_class_C|Getrougelike_event_flow _executing_event)
        (:NewEnumerator3
          (switch Utilities|FlowControl|Switch|SwitchonE_rougelike_event_type (Variables|/Game/BP/BP_AC/BP_rougelike_AC/BP_Rougelike_Event_class.BP_Rougelike_Event_class_C|Getrougelike_event_type _executing_event)
            (:NewEnumerator2
              _)
            (:NewEnumerator1
              _))
          (Default|UpdataMainUI (Variables|/Game/gamemode/2DplayerContrller.2DplayerContrller_C|GetAC_UI_ManagerComponent (Variables|Default|GetAs%202Dplayer%20Contrller)) "/Game/WBP_common_ui/Bottom_layer_widget/WBP_rougelike_event.WBP_rougelike_event_C"))))))

(fn EventCompleted
  (bind _rougelike_process (Variables|player|Getrougelike_process))
  (Utilities|Array|RemoveItem (Variables|/Game/BP/BP_AC/BP_rougelike_AC/BP_rougelike_process_class.BP_rougelike_process_class_C|Getcurrent_event (Variables|player|Getrougelike_process)) (Variables|/Game/BP/BP_AC/BP_rougelike_AC/BP_rougelike_process_class.BP_rougelike_process_class_C|Getthis_event _rougelike_process))
  (Variables|/Game/BP/BP_AC/BP_rougelike_AC/BP_rougelike_process_class.BP_rougelike_process_class_C|Setthis_event _rougelike_process "")
  (if (== (Variables|/Game/BP/BP_AC/BP_rougelike_AC/BP_rougelike_process_class.BP_rougelike_process_class_C|Getevent_number (Variables|player|Getrougelike_process)) 0)
    (Variables|Default|Setrougelike_flow "NewEnumerator1")
    (Variables|Default|SetGenerate%20Event%20Phase%20Control (not (Variables|Default|GetGenerate%20Event%20Phase%20Control)))
    (else
      (Variables|Default|Setrougelike_flow "NewEnumerator2"))))