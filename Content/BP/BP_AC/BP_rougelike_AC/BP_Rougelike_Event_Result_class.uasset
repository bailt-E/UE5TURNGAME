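; Roguelike event result class, apparently a base, with empty begin and end activation hooks that receive the Process.
; Two selection functions target random roles from the Process's to-be-selected or disused pool, comparing Persona against SelectRole.
; They add only while looping over existing SelectRole entries, so an empty list stays empty.
; Array helpers append a role or remove it by Persona match; the add helper's duplicate handling is unwired.
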(fn ResultBeginActivation
  (params (process :type BP%20Rougelike%20Process%20Class%20Object%20Reference)))

(fn ResultSelectCharacterfromtobeSelectRole
  (params (process :type BP%20Rougelike%20Process%20Class%20Object%20Reference))
  (bind _to_be_selected_rougelike_role (Variables|/Game/BP/BP_AC/BP_rougelike_AC/BP_rougelike_process_class.BP_rougelike_process_class_C|GetTo%20be%20selected_rougelike_role process))
  (bind _returnvalue (Utilities|Array|Length _to_be_selected_rougelike_role))
  (bind _returnvalue_2 (Math|Random|RandomInteger _returnvalue))
  (bind _output (Utilities|Array|Get(acopy) _to_be_selected_rougelike_role _returnvalue_2))
  (Utilities|FlowControl|Sequence
    (:then_0
      (if (< (Utilities|Array|Length (LocalVariables|Getselect_role)) 2)
        (for _array_element (LocalVariables|Getselect_role)
          (if (not (== (Utilities|Struct|BreakST_Rougelike_role _array_element) (Utilities|Struct|BreakST_Rougelike_role _output)))
            (Utilities|Array|Add (LocalVariables|Getselect_role) _output)))))
    (:then_1
      (return (LocalVariables|Getselect_role)))))

(fn ResultSelectCharacterfromDisuseRole
  (params (process :type BP%20Rougelike%20Process%20Class%20Object%20Reference))
  (bind _disuse_rougelike_role (Variables|/Game/BP/BP_AC/BP_rougelike_AC/BP_rougelike_process_class.BP_rougelike_process_class_C|Getdisuse_rougelike_role process))
  (bind _returnvalue (Utilities|Array|Length _disuse_rougelike_role))
  (bind _returnvalue_2 (Math|Random|RandomInteger _returnvalue))
  (bind _output (Utilities|Array|Get(acopy) _disuse_rougelike_role _returnvalue_2))
  (Utilities|FlowControl|Sequence
    (:then_0
      (if (< (Utilities|Array|Length (LocalVariables|Getselect_role)) 2)
        (for _array_element (LocalVariables|Getselect_role)
          (if (not (== (Utilities|Struct|BreakST_Rougelike_role _array_element) (Utilities|Struct|BreakST_Rougelike_role _output)))
            (Utilities|Array|Add (LocalVariables|Getselect_role) _output)))))
    (:then_1
      (return (LocalVariables|Getselect_role)))))

(fn ResultEndActivation
  (params (process :type BP%20Rougelike%20Process%20Class%20Object%20Reference)))

(fn AddRoleforArray
  (params (role_array :type Array%20of%20ST%20Rougelike%20Role%20Structures) (this_role :type ST%20Rougelike%20Role%20Structure))
  (Utilities|Array|Add role_array this_role) ; 缺少一个角色初始化
  (return role_array))

(fn RemoveRoleforArray
  (params (role_array :type Array%20of%20ST%20Rougelike%20Role%20Structures) (this_role :type ST%20Rougelike%20Role%20Structure))
  (for _array_element role_array
    (if (== (Utilities|Struct|BreakST_Rougelike_role _array_element) (Utilities|Struct|BreakST_Rougelike_role this_role))
      (Utilities|Array|RemoveItem role_array this_role)
      (return role_array))))