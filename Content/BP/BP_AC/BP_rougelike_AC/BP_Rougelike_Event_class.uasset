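; Base class for a roguelike event, which either hands off to battle preparation or plays a text-and-choice event.
; EventActivationR3 steps a flow state machine through intro text, option buttons, outcome text and event end, pushing content into WBP_rougelike_event.
; After the outcome text, it calls SelectEventEffect, an empty stub here, with a random roll for chance-based choices.
; Ending reports back to the roguelike component and resumes the run flow.
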(fn InitializetheEvent
  (params (rougelike_event_type :type E_rougelike_event_type%20Enum :default "NewEnumerator0") (Consumes%20money :type Integer) (event_level :type Integer) (rougelike_C :type BP%20Rougelike%20AC%20Object%20Reference))
  (Variables|Rougelike_event_Info|Setrougelike_event_type rougelike_event_type)
  (Variables|Rougelike_event_Info|SetConsumes%20money Consumes%20money)
  (Variables|Rougelike_event_Info|Setlevel event_level)
  (Variables|Default|Setrougelike_C rougelike_C)
  (return))

(fn PlayEventText0
  (params (text_index :type Integer) (text_array :type Array%20of%20Texts))
  (if (> text_index (Utilities|Array|Length text_array))
    (Variables|player|Setrougelike_event_flow "NewEnumerator1")
    (else
      (CallFunction|SpawnTextWidgetinUI text_array text_index))))

(fn PlayEventText
  (params (text_index :type Integer))
  (if (> text_index (Utilities|Array|Length (Variables|EventData|Getevent_data)))
    (Variables|player|Setrougelike_event_flow "NewEnumerator1")
    (else
      (CallFunction|SpawnTextWidgetinUI (Variables|EventData|Getevent_data) text_index)
      (return))))

(fn EventActivation(R3)
  (params (tirget :type E_rougelike_event_stage%20Enum :default "NewEnumerator0"))
  (bind _rougelike_ac (Variables|fix|Getrougelike_AC))
  (switch Utilities|FlowControl|Switch|SwitchonE_rougelike_event_type (Variables|Rougelike_event_Info|Getrougelike_event_type)
    (:NewEnumerator0
      (Variables|/Game/gamemode/BP_GameInstance.BP_GameInstance_C|Setcurrent_game_mode (Variables|/Game/BP/BP_AC/BP_rougelike_AC/BP_rougelike_AC.BP_rougelike_AC_C|GetAs%20BP%20Game%20Instance (Variables|fix|Getrougelike_AC)) "NewEnumerator1")
      (Default|PrepareforBattle (Variables|/Game/gamemode/2DplayerContrller.2DplayerContrller_C|GetAC_UI_ManagerComponent (Variables|/Game/BP/BP_AC/BP_rougelike_AC/BP_rougelike_AC.BP_rougelike_AC_C|GetAs%202Dplayer%20Contrller (Variables|fix|Getrougelike_AC))) "NewEnumerator1"))
    (:NewEnumerator2
      (if (Utilities|Enum|Equal(Enum) tirget (Variables|player|Getrougelike_event_flow)) :!label _label ; 对任何来源的检查
        (switch Utilities|FlowControl|Switch|SwitchonE_rougelike_event_stage (Variables|player|Getrougelike_event_flow)
          (:NewEnumerator0
            (bind _output_get (Variables|player|Setcurrent_event_data_index (+ (Variables|player|Getcurrent_event_data_index) 1)))
            (if (<= (+ (Variables|player|Getcurrent_event_data_index) 1) (Utilities|Array|Length (Variables|EventData|Getevent_data)))
              (A1|PlayEventText _output_get)
              (else
                (Variables|player|Setrougelike_event_flow "NewEnumerator1")
                (Variables|player|Setcurrent_event_data_index 0))))
          (:NewEnumerator1
            ;[1 1 1] 生成选项
            (for _array_element (Variables|EventData|Getselelct_info)
              (Variables|player|Setrougelike_event_flow "NewEnumerator1")
              (bind _aswbp_main (Utilities|Casting|CastToWBP_Main (Variables|/Game/BP/BP_AC/BP_UIManager/AC_UI_ManagerComponent.AC_UI_ManagerComponent_C|GetMain%20Menu (Variables|/Game/gamemode/2DplayerContrller.2DplayerContrller_C|GetAC_UI_ManagerComponent (Variables|/Game/BP/BP_AC/BP_rougelike_AC/BP_rougelike_AC.BP_rougelike_AC_C|GetAs%202Dplayer%20Contrller (Variables|fix|Getrougelike_AC))))))
              (bind _aswbp_rougelike_event (Utilities|Casting|CastToWBP_rougelike_event (Variables|/Game/WBP_common_ui/Parentcontrol_widget/WBP_Main.WBP_Main_C|GetUnderlying%20stack_widget _aswbp_main)))
              (Default|SpawnSelectButton _aswbp_rougelike_event true (Utilities|Struct|Makest_rougelike_event_select (.event_select_Title (Utilities|Struct|Breakst_rougelike_event_select _array_element)) (.Effectdescription (Utilities|Struct|Breakst_rougelike_event_select _array_element)) (.select_type (Utilities|Struct|Breakst_rougelike_event_select _array_element)) (.Randomevent (Utilities|Struct|Breakst_rougelike_event_select _array_element))))))
          (:NewEnumerator3
            (Development|PrintString 0 "玩家选择，玩家选择之后进入下一阶段"))
          (:NewEnumerator2
            (bind _newparam (A3|SelectEventAfter (Variables|player|GetSelect%20Index)))
            (if _newparam
              (bind _output_get_2 (Variables|player|Setrougelike_event_flow "NewEnumerator4")) ; 由玩家自己操作
              (A2|EventActivation(R3) _output_get_2)
              (else
                (bind _output_get_3 (Variables|player|Setrougelike_event_flow "NewEnumerator2")))))
          (:NewEnumerator4
            (Variables|player|Setrougelike_event_flow "NewEnumerator0")
            (Variables|/Game/BP/BP_AC/BP_rougelike_AC/BP_rougelike_AC.BP_rougelike_AC_C|Setrougelike_flow _rougelike_ac "NewEnumerator4")
            (CallFunction|EndEvent (Variables|Rougelike_event_Info|Getrougelike_event_type))
            (Default|MIND _rougelike_ac (Variables|/Game/BP/BP_AC/BP_rougelike_AC/BP_rougelike_AC.BP_rougelike_AC_C|GetRow%20Name _rougelike_ac))))))
    (:NewEnumerator1
      (goto _label))))

(fn SelectEventAfter
  (params (select_index :type St%20Rougelike%20Event%20Select%20Structure))
  (bind _select_index (Variables|player|GetSelect%20Index))
  (bind _current_event_data_index (Variables|player|Getcurrent_event_data_index))
  (bind (_select_type _randomevent) (Utilities|Struct|Breakst_rougelike_event_select _select_index))
  (bind _returnvalue (+ _current_event_data_index 1))
  (for _array_element (Variables|EventData|Getevent_the_end)
    (if (Utilities|Enum|Equal(Enum) _select_type (.select_index (Utilities|Struct|Breakst_rougelike_event_select_alfte _array_element))) ; 事件枚举查询
      (if (<= _returnvalue (Utilities|Array|Length (.text (Utilities|Struct|Breakst_rougelike_event_select_alfte _array_element)))) ; 检查数组长度和当前数字
        (A1|PlayEventText0 _returnvalue (.text (Utilities|Struct|Breakst_rougelike_event_select_alfte _array_element))) ; 播放文字到控件上
        (return false)
        (elif _randomevent ; 是否是概率性事件
          (CallFunction|SelectEventEffect (.select_index (Utilities|Struct|Breakst_rougelike_event_select_alfte _array_element)) (Math|Integer|InRange(Integer) (Math|Random|RandomInteger 100) 0 100))
          (return true)
          (else
            (CallFunction|SelectEventEffect (.select_index (Utilities|Struct|Breakst_rougelike_event_select_alfte _array_element)) false)
            (return true)))))))

(fn SelectEventEffect
  (params (select :type E_rougelike_event_select%20Enum :default "NewEnumerator0") (Result :type Boolean))
  (return))

(fn SpawnTextWidgetinUI
  (params (Array :type Array%20of%20Texts) (Dimension%20 :type Integer))
  (bind _aswbp_main (Utilities|Casting|CastToWBP_Main (Variables|/Game/BP/BP_AC/BP_UIManager/AC_UI_ManagerComponent.AC_UI_ManagerComponent_C|GetMain%20Menu (Variables|/Game/gamemode/2DplayerContrller.2DplayerContrller_C|GetAC_UI_ManagerComponent (Variables|/Game/BP/BP_AC/BP_rougelike_AC/BP_rougelike_AC.BP_rougelike_AC_C|GetAs%202Dplayer%20Contrller (Variables|fix|Getrougelike_AC))))))
  (bind _aswbp_rougelike_event (Utilities|Casting|CastToWBP_rougelike_event (Variables|/Game/WBP_common_ui/Parentcontrol_widget/WBP_Main.WBP_Main_C|GetUnderlying%20stack_widget _aswbp_main)))
  (Default|ADDTexttoBox _aswbp_rougelike_event (Utilities|Array|Get(acopy) Array Dimension%20)))

(fn EndEvent
  (params (event_Selection :type E_rougelike_event_type%20Enum :default "NewEnumerator0"))
  (bind _rougelike_c (Variables|Default|Getrougelike_C))
  (bind _rougelike_process (Variables|/Game/BP/BP_AC/BP_rougelike_AC/BP_rougelike_AC.BP_rougelike_AC_C|Getrougelike_process _rougelike_c))
  (Default|AfterSelectingtheEvent _rougelike_c (Variables|/Game/BP/BP_AC/BP_rougelike_AC/BP_rougelike_process_class.BP_rougelike_process_class_C|GetExecuting%20event _rougelike_process) _rougelike_process)
  (switch Utilities|FlowControl|Switch|SwitchonE_rougelike_event_type event_Selection
    (:NewEnumerator0
      (bind _array_element (Utilities|Array|ForEachLoopwithBreak (.team_number (Utilities|Struct|Breakst_team_Assembly (Variables|/Game/BP/BP_AC/BP_rougelike_AC/BP_rougelike_process_class.BP_rougelike_process_class_C|Getteam (Variables|/Game/BP/BP_AC/BP_rougelike_AC/BP_rougelike_AC.BP_rougelike_AC_C|Getrougelike_process (Variables|Default|Getrougelike_C))))))
        (:LoopBody
          (if (== (.unit (Utilities|Struct|Breakst_team _array_element)) (Utilities|GetClass (.persona (Utilities|Struct|BreakST_Rougelike_role (stale _array_element)))))
            _))))))