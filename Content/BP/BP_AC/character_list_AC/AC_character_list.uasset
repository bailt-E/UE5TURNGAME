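; Actor component that builds the filtered character list, excluding characters found in the loaded team.
; On BeginPlay it removes LoadTeam members from CharacterssData, then stores the result of RefreshTheListOfRoles in CharacterssList.
; Refresh filters by element, faction and occupation, then branches on level or index and direction.
; The sort compares each pawn with itself, so it never reorders, and it removes entries from the array being looped.
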(event EventBeginPlay
  (CallFunction|LoadAnArrayOfCharacters)
  (bind _array (CallFunction|RefreshtheListOfRoles))
  (Variables|默认|Setcharacterss_list _array))

(event EventTick
  (params (DeltaSeconds :type Float%20%28single-precision%29)))

(fn RefreshtheListOfRoles
  (bind _filter (Variables|player_coll|Getfilter))
  (bind (_element_type _occupation _pawn_faction) (Utilities|Struct|Breakst_character_filter _filter))
  (Utilities|FlowControl|Sequence
    (:then_0
      (for _array_element (Variables|Default|Getcharacterss_data)
        (if (Math|Boolean|ANDBoolean (Utilities|Enum|Equal(Enum) _element_type (Variables|/Game/BP/BP_Battle_Phase/BP_character_class.BP_character_class_C|Getpawn_element _array_element)) (Utilities|Enum|Equal(Enum) _pawn_faction (Variables|/Game/BP/BP_Battle_Phase/BP_character_class.BP_character_class_C|Getpawn%20faction _array_element)) (Utilities|Enum|Equal(Enum) _occupation (Variables|/Game/BP/BP_Battle_Phase/BP_character_class.BP_character_class_C|Getpawn_occupation _array_element)))
          (Utilities|Array|Add (LocalVariables|GetPrimary%20screening) _array_element))))
    (:then_1
      (switch Utilities|FlowControl|Switch|SwitchonE_Sort_by (Variables|player_coll|Getsort%20by)
        (:NewEnumerator0
          (if (Variables|player_coll|GetDescending)
            (for _array_element_2 (LocalVariables|GetPrimary%20screening)
              (bind _output_get (LocalVariables|Setpawn _array_element_2))
              (Math|Integer|CompareInt (Variables|/Game/BP/BP_AC/BP_Player_level_AC/AC_level_exp.AC_level_exp_C|Getcurrent_level (Variables|/Game/BP/BP_Battle_Phase/BP_character_class.BP_character_class_C|GetAC_level _output_get)) (Variables|/Game/BP/BP_AC/BP_Player_level_AC/AC_level_exp.AC_level_exp_C|Getcurrent_level (Variables|/Game/BP/BP_Battle_Phase/BP_character_class.BP_character_class_C|GetAC_level _array_element_2))
                (:>
                  _)
                (:==
                  _))
              (bind _output_get_2 (LocalVariables|Setpawn _output_get))
              (Utilities|Array|Add (LocalVariables|GetFinal%20screening) _output_get_2)
              (Utilities|Array|RemoveItem (LocalVariables|GetPrimary%20screening) _output_get_2))
            (else
              (for _array_element_3 (LocalVariables|GetPrimary%20screening)
                (bind _output_get_3 (LocalVariables|Setpawn _array_element_3))
                (Math|Integer|CompareInt (Variables|/Game/BP/BP_AC/BP_Player_level_AC/AC_level_exp.AC_level_exp_C|Getcurrent_level (Variables|/Game/BP/BP_Battle_Phase/BP_character_class.BP_character_class_C|GetAC_level _output_get_3)) (Variables|/Game/BP/BP_AC/BP_Player_level_AC/AC_level_exp.AC_level_exp_C|Getcurrent_level (Variables|/Game/BP/BP_Battle_Phase/BP_character_class.BP_character_class_C|GetAC_level _array_element_3))
                  (:==
                    _)
                  (:<
                    _))
                (bind _output_get_4 (LocalVariables|Setpawn _output_get_3))
                (Utilities|Array|Add (LocalVariables|GetFinal%20screening) _output_get_4)
                (Utilities|Array|RemoveItem (LocalVariables|GetPrimary%20screening) _output_get_4)))))
        (:NewEnumerator1
          (if (Variables|player_coll|GetDescending)
            (for _array_element_4 (LocalVariables|GetPrimary%20screening)
              (bind _output_get_5 (LocalVariables|Setpawn _array_element_4))
              (Math|Integer|CompareInt (Variables|/Game/BP/BP_Battle_Phase/BP_character_class.BP_character_class_C|Getindex _output_get_5) (Variables|/Game/BP/BP_Battle_Phase/BP_character_class.BP_character_class_C|Getindex _array_element_4)
                (:>
                  _)
                (:==
                  _))
              (bind _output_get_6 (LocalVariables|Setpawn _output_get_5))
              (Utilities|Array|Add (LocalVariables|GetFinal%20screening) _output_get_6)
              (Utilities|Array|RemoveItem (LocalVariables|GetPrimary%20screening) _output_get_6))
            (else
              (for _array_element_5 (LocalVariables|GetPrimary%20screening)
                (bind _output_get_7 (LocalVariables|Setpawn _array_element_5))
                (Math|Integer|CompareInt (Variables|/Game/BP/BP_Battle_Phase/BP_character_class.BP_character_class_C|Getindex _output_get_7) (Variables|/Game/BP/BP_Battle_Phase/BP_character_class.BP_character_class_C|Getindex _array_element_5)
                  (:==
                    _)
                  (:<
                    _))
                (bind _output_get_8 (LocalVariables|Setpawn _output_get_7))
                (Utilities|Array|Add (LocalVariables|GetFinal%20screening) _output_get_8)
                (Utilities|Array|RemoveItem (LocalVariables|GetPrimary%20screening) _output_get_8)))))))
    (:then_2
      (return (LocalVariables|GetFinal%20screening)))))

(fn LoadAnArrayOfCharacters
  (for _array_element (Variables|Default|Getcharacterss_data)
    (for _array_element_2 (Variables|data|Getload_team)
      (if (== _array_element_2 _array_element)
        (Utilities|Array|RemoveItem (Variables|Default|Getcharacterss_data) _array_element_2)))))