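; Actor component that holds a unit's attributes and its current HP and action-point resources, apparently for turn-based play.
; InitializationOfAttributes reads health, attack and defense from either the character-level or unit-level DataTable, chosen by a boolean, and returns them with fixed action-point settings.
; AttributesToResource seeds current resources from UnitAttributes, and Turn adds action-point growth without clamping to the maximum.
; Dealdamage is an empty stub.
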(event EventBeginPlay)

(event EventTick
  (params (DeltaSeconds :type Float%20%28single-precision%29)))

(fn InitializationOfAttributes
  (params (RowName :type Name) (Condition :type Boolean))
  (Utilities|FlowControl|Sequence
    (:then_0
      (if Condition
        (bind _returnvalue (Utilities|GetDataTableRow "/Game/Struct/rank_table/T_character_level_data.T_character_level_data" RowName)
          (:then
            (LocalVariables|Setattributes (Utilities|Struct|Makest_the_unit_attribute (.Health (Utilities|Struct|Breakst_character_bese_level_data _returnvalue)) (.Attack (Utilities|Struct|Breakst_character_bese_level_data _returnvalue)) (.defense (Utilities|Struct|Breakst_character_bese_level_data _returnvalue)) 1 3 1))))
        (else
          (bind _returnvalue_2 (Utilities|GetDataTableRow "/Game/Struct/rank_table/T_unitlevel_data.T_unitlevel_data" RowName)
            (:then
              (LocalVariables|Setattributes (Utilities|Struct|Makest_the_unit_attribute (.hp (Utilities|Struct|Breakst_unit_level_data _returnvalue_2)) (.attack (Utilities|Struct|Breakst_unit_level_data _returnvalue_2)) (.defense (Utilities|Struct|Breakst_unit_level_data _returnvalue_2)) 1 3 1)))))))
    (:then_1
      (return (LocalVariables|Getattributes)))))

(fn AttributestoResource
  (bind _unit_attributes (Variables|Default|Getunit_attributes))
  (bind (_hp_max _initialactionpoint) (Utilities|Struct|Breakst_the_unit_attribute _unit_attributes))
  (Variables|Default|Setunit_resource (Utilities|Struct|Makest_the_unit_resource _hp_max _initialactionpoint)))

(fn Turn
  (Variables|Default|Setunit_resource (Utilities|Struct|Makest_the_unit_resource (.hp (Utilities|Struct|Breakst_the_unit_resource (Variables|Default|Getunit_resource))) (+ (Utilities|Struct|Breakst_the_unit_attribute (Variables|Default|Getunit_attributes)) (.actionpoint (Utilities|Struct|Breakst_the_unit_resource (Variables|Default|Getunit_resource)))))))

(fn Dealdamage
  (params (damage :type Integer) (element_damage_type :type E_element_type%20Enum :default "NewEnumerator0") (damage_type :type e_damage_type%20Enum :default "NewEnumerator1") (element%20damage%20type :type e_element_damage_type%20Enum :default "NewEnumerator1")))