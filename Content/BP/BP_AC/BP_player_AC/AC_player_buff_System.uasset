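; Player component that manages a turn-based action point pool and the player's buffs.
; Action points are typed struct entries that get initialized, restored, eroded, or locked by a cost check and then spent, with temporary points removed.
; Buffs are objects built from data table rows or parameters and queued in a waiting list.
; Current buffs tick cycle and end effects, and fire on matching timings against filtered units; RemoveBuff is an empty stub.
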(event EventBeginPlay)

(event EventTick
  (params (DeltaSeconds :type Float%20%28single-precision%29)))

(fn InitializeActionPoints
  (params (soild- :type Integer) (empty :type Integer))
  (Utilities|FlowControl|Sequence
    (:then_0
      (for _index (range 1 soild-)
        (Utilities|Array|Add (Variables|Default|GetPlayer_actionpoint) (Utilities|Struct|Makest_actionpoint _index "NewEnumerator0" "NewEnumerator1" false))))
    (:then_1
      (for _index_2 (range (+ soild- 1) empty)
        (Utilities|Array|Add (Variables|Default|GetPlayer_actionpoint) (Utilities|Struct|Makest_actionpoint _index_2 "NewEnumerator0" "NewEnumerator0" false))))))

(fn SpendActionPoints
  (for _array_element (Variables|Default|GetPlayer_actionpoint)
    (if (.lock (Utilities|Struct|Breakst_actionpoint _array_element))
      (switch Utilities|FlowControl|Switch|SwitchonE_actionpoint_type (.ACTIONPOINT_TYPE (Utilities|Struct|Breakst_actionpoint _array_element))
        (:NewEnumerator0
          (Utilities|Array|SetArrayElem (Variables|Default|GetPlayer_actionpoint) 0 (Utilities|Struct|Makest_actionpoint (.actionpoint_id (Utilities|Struct|Breakst_actionpoint _array_element)) (.ACTIONPOINT_TYPE (Utilities|Struct|Breakst_actionpoint _array_element)) "NewEnumerator0" false) :!label _label))
        (:NewEnumerator1
          (Utilities|Array|RemoveItem (Variables|Default|GetPlayer_actionpoint) _array_element))
        (:NewEnumerator2
          (goto _label))))))

(fn IncreaseActionPoints
  (params (LastIndex :type Integer) (ACTIONPOINT_TYPE :type E_actionpoint_type%20Enum :default "NewEnumerator0") (actionpoint_status :type e_actionpoint_Status%20Enum :default "NewEnumerator0"))
  (for _index (range 1 LastIndex)
    (Utilities|Array|Add (Variables|Default|GetPlayer_actionpoint) (Utilities|Struct|Makest_actionpoint 0 ACTIONPOINT_TYPE actionpoint_status false))))

(fn ADDBuff
  (params (buff_rowname :type Name))
  (bind _returnvalue (Utilities|GetDataTableRow "/Game/Struct/player_buff/T_player_buff.T_player_buff" buff_rowname)
    (:then
      (for _array_element (Variables|buff|Getcurrent_player_buff)
        (bind (_buff _find) (F1|FindBuffbyIndex (Variables|/Game/BP/BP_AC/BP_player_AC/BP_player_buff_object.BP_player_buff_object_C|Getbuff_info _array_element)))
        (if _find
          (bind _output_get (LocalVariables|Setbuff _buff))
          (switch Utilities|FlowControl|Switch|SwitchonE_BuffTimeUpdataEnum (.buff_updara_mode (Utilities|Struct|Breakst_player_buff_setting (Variables|/Game/BP/BP_AC/BP_player_AC/BP_player_buff_object.BP_player_buff_object_C|GetBUFF_SETTING _output_get)))
            (:NewEnumerator0
              (Variables|/Game/BP/BP_AC/BP_player_AC/BP_player_buff_object.BP_player_buff_object_C|Setresources (LocalVariables|Getbuff) (Utilities|Struct|Makest_PB_Resources (+ (.stack_add (Utilities|Struct|Breakst_player_buff_Numeric_attribute (Variables|/Game/BP/BP_AC/BP_player_AC/BP_player_buff_object.BP_player_buff_object_C|GetNumeric (LocalVariables|Getbuff)))) (.stack (Utilities|Struct|Breakst_PB_Resources (Variables|/Game/BP/BP_AC/BP_player_AC/BP_player_buff_object.BP_player_buff_object_C|Getresources (LocalVariables|Getbuff))))) (.Priority (Utilities|Struct|Breakst_PB_Resources (Variables|/Game/BP/BP_AC/BP_player_AC/BP_player_buff_object.BP_player_buff_object_C|Getresources (LocalVariables|Getbuff)))) (.Threshold (Utilities|Struct|Breakst_PB_Resources (Variables|/Game/BP/BP_AC/BP_player_AC/BP_player_buff_object.BP_player_buff_object_C|Getresources (LocalVariables|Getbuff)))) (+ (.Charge (Utilities|Struct|Breakst_player_buff_Numeric_attribute (Variables|/Game/BP/BP_AC/BP_player_AC/BP_player_buff_object.BP_player_buff_object_C|GetNumeric (LocalVariables|Getbuff)))) (.Energy (Utilities|Struct|Breakst_PB_Resources (Variables|/Game/BP/BP_AC/BP_player_AC/BP_player_buff_object.BP_player_buff_object_C|Getresources (LocalVariables|Getbuff))))) (.current_CycleTurn (Utilities|Struct|Breakst_PB_Resources (Variables|/Game/BP/BP_AC/BP_player_AC/BP_player_buff_object.BP_player_buff_object_C|Getresources (LocalVariables|Getbuff)))) (.PersistentTurn (Utilities|Struct|Breakst_PB_Resources (Variables|/Game/BP/BP_AC/BP_player_AC/BP_player_buff_object.BP_player_buff_object_C|Getresources (LocalVariables|Getbuff))))))))
          (else
            (bind _returnvalue_2 (Game|ConstructObjectfromClass (.buffclass (Utilities|Struct|Breakst_PB_assembly _returnvalue))))
            (Default|InitializeBuff _returnvalue_2 (.base_buff_info (Utilities|Struct|Breakst_PB_assembly _returnvalue)) (.Numeric_attribute (Utilities|Struct|Breakst_PB_assembly _returnvalue)) (.effect_info (Utilities|Struct|Breakst_PB_assembly _returnvalue)) (.targer_data (Utilities|Struct|Breakst_PB_assembly _returnvalue)) (.buffsetting (Utilities|Struct|Breakst_PB_assembly _returnvalue)))
            (Utilities|Array|Add (Variables|buff|Getwait_ADD_player_buff) _returnvalue_2)))))))

(fn RemoveBuff)

(fn BuffTick
  (params (tick :type Integer))
  (for _array_element (Variables|buff|Getcurrent_player_buff)
    (LocalVariables|Setbuff _array_element)
    (Utilities|FlowControl|Sequence
      (:then_0
        (if (>= (- (Utilities|Struct|Breakst_PB_Resources (Variables|/Game/BP/BP_AC/BP_player_AC/BP_player_buff_object.BP_player_buff_object_C|Getresources (LocalVariables|Getbuff))) tick) 0)
          (Default|CycleEffect (LocalVariables|Getbuff))
          (Variables|/Game/BP/BP_AC/BP_player_AC/BP_player_buff_object.BP_player_buff_object_C|Setresources (LocalVariables|Getbuff) (Utilities|Struct|Makest_PB_Resources (.stack (Utilities|Struct|Breakst_PB_Resources (Variables|/Game/BP/BP_AC/BP_player_AC/BP_player_buff_object.BP_player_buff_object_C|Getresources (LocalVariables|Getbuff)))) (.Priority (Utilities|Struct|Breakst_PB_Resources (Variables|/Game/BP/BP_AC/BP_player_AC/BP_player_buff_object.BP_player_buff_object_C|Getresources (LocalVariables|Getbuff)))) (.Threshold (Utilities|Struct|Breakst_PB_Resources (Variables|/Game/BP/BP_AC/BP_player_AC/BP_player_buff_object.BP_player_buff_object_C|Getresources (LocalVariables|Getbuff)))) (.Energy (Utilities|Struct|Breakst_PB_Resources (Variables|/Game/BP/BP_AC/BP_player_AC/BP_player_buff_object.BP_player_buff_object_C|Getresources (LocalVariables|Getbuff)))) (Utilities|Struct|Breakst_player_buff_Numeric_attribute (Variables|/Game/BP/BP_AC/BP_player_AC/BP_player_buff_object.BP_player_buff_object_C|GetNumeric (LocalVariables|Getbuff))) (.PersistentTurn (Utilities|Struct|Breakst_PB_Resources (Variables|/Game/BP/BP_AC/BP_player_AC/BP_player_buff_object.BP_player_buff_object_C|Getresources (LocalVariables|Getbuff))))))
          (else
            (Variables|/Game/BP/BP_AC/BP_player_AC/BP_player_buff_object.BP_player_buff_object_C|Setresources (LocalVariables|Getbuff) (Utilities|Struct|Makest_PB_Resources (.stack (Utilities|Struct|Breakst_PB_Resources (Variables|/Game/BP/BP_AC/BP_player_AC/BP_player_buff_object.BP_player_buff_object_C|Getresources (LocalVariables|Getbuff)))) (.Priority (Utilities|Struct|Breakst_PB_Resources (Variables|/Game/BP/BP_AC/BP_player_AC/BP_player_buff_object.BP_player_buff_object_C|Getresources (LocalVariables|Getbuff)))) (.Threshold (Utilities|Struct|Breakst_PB_Resources (Variables|/Game/BP/BP_AC/BP_player_AC/BP_player_buff_object.BP_player_buff_object_C|Getresources (LocalVariables|Getbuff)))) (.Energy (Utilities|Struct|Breakst_PB_Resources (Variables|/Game/BP/BP_AC/BP_player_AC/BP_player_buff_object.BP_player_buff_object_C|Getresources (LocalVariables|Getbuff)))) (- (Utilities|Struct|Breakst_PB_Resources (Variables|/Game/BP/BP_AC/BP_player_AC/BP_player_buff_object.BP_player_buff_object_C|Getresources (LocalVariables|Getbuff))) tick) (.PersistentTurn (Utilities|Struct|Breakst_PB_Resources (Variables|/Game/BP/BP_AC/BP_player_AC/BP_player_buff_object.BP_player_buff_object_C|Getresources (LocalVariables|Getbuff)))))))))
      (:then_1
        (if (>= (- (Utilities|Struct|Breakst_PB_Resources (Variables|/Game/BP/BP_AC/BP_player_AC/BP_player_buff_object.BP_player_buff_object_C|Getresources (LocalVariables|Getbuff))) 0) 0)
          (Default|EndEffect (LocalVariables|Getbuff))
          (if (not (.Existforever (Utilities|Struct|Breakst_player_buff_setting (Variables|/Game/BP/BP_AC/BP_player_AC/BP_player_buff_object.BP_player_buff_object_C|GetBUFF_SETTING (LocalVariables|Getbuff)))))
            (Utilities|Array|RemoveItem (Variables|buff|Getcurrent_player_buff) (LocalVariables|Getbuff)))
          (else
            (Variables|/Game/BP/BP_AC/BP_player_AC/BP_player_buff_object.BP_player_buff_object_C|Setresources (LocalVariables|Getbuff) (Utilities|Struct|Makest_PB_Resources (.stack (Utilities|Struct|Breakst_PB_Resources (Variables|/Game/BP/BP_AC/BP_player_AC/BP_player_buff_object.BP_player_buff_object_C|Getresources (LocalVariables|Getbuff)))) (.Priority (Utilities|Struct|Breakst_PB_Resources (Variables|/Game/BP/BP_AC/BP_player_AC/BP_player_buff_object.BP_player_buff_object_C|Getresources (LocalVariables|Getbuff)))) (.Threshold (Utilities|Struct|Breakst_PB_Resources (Variables|/Game/BP/BP_AC/BP_player_AC/BP_player_buff_object.BP_player_buff_object_C|Getresources (LocalVariables|Getbuff)))) (.Energy (Utilities|Struct|Breakst_PB_Resources (Variables|/Game/BP/BP_AC/BP_player_AC/BP_player_buff_object.BP_player_buff_object_C|Getresources (LocalVariables|Getbuff)))) (.current_CycleTurn (Utilities|Struct|Breakst_PB_Resources (Variables|/Game/BP/BP_AC/BP_player_AC/BP_player_buff_object.BP_player_buff_object_C|Getresources (LocalVariables|Getbuff)))) (- (Utilities|Struct|Breakst_PB_Resources (Variables|/Game/BP/BP_AC/BP_player_AC/BP_player_buff_object.BP_player_buff_object_C|Getresources (LocalVariables|Getbuff))) 0)))))))))

(fn UseActionPoints（NG）
  (for _array_element (Variables|Default|GetPlayer_actionpoint)
    (if (.lock (Utilities|Struct|Breakst_actionpoint _array_element))
      (switch Utilities|FlowControl|Switch|SwitchonE_actionpoint_type (.ACTIONPOINT_TYPE (Utilities|Struct|Breakst_actionpoint _array_element))
        (:NewEnumerator0
          (Utilities|Array|SetArrayElem (Variables|Default|GetPlayer_actionpoint) 0 (Utilities|Struct|Makest_actionpoint (.actionpoint_id (Utilities|Struct|Breakst_actionpoint _array_element)) (.ACTIONPOINT_TYPE (Utilities|Struct|Breakst_actionpoint _array_element)) "NewEnumerator0" false) :!label _label))
        (:NewEnumerator1
          (Utilities|Array|RemoveItem (Variables|Default|GetPlayer_actionpoint) _array_element))
        (:NewEnumerator2
          (goto _label))))))

(fn ConvertUnusableActionPointsIntoEmptyActionPoints
  (params (LastIndex :type Integer))
  (for _index (range 0 LastIndex)
    (for _array_element (Variables|Default|GetPlayer_actionpoint)
      (if (Utilities|Enum|Equal(Enum) (.actionpoint_status (Utilities|Struct|Breakst_actionpoint _array_element)) "NewEnumerator2")
        (Utilities|Array|SetArrayElem (Variables|Default|GetPlayer_actionpoint) 0 (Utilities|Struct|Makest_actionpoint (.actionpoint_id (Utilities|Struct|Breakst_actionpoint _array_element)) (.ACTIONPOINT_TYPE (Utilities|Struct|Breakst_actionpoint _array_element)) "NewEnumerator0" false))))))

(fn CounttheNumberOfStandardActionPoints
  (params (Array :type Array%20of%20St%20Actionpoint%20Structures))
  (for _array_element Array
    (if (Math|Boolean|ANDBoolean (Utilities|Enum|NotEqual(Enum) (.ACTIONPOINT_TYPE (Utilities|Struct|Breakst_actionpoint _array_element)) "NewEnumerator2") (Utilities|Enum|Equal(Enum) (.actionpoint_status (Utilities|Struct|Breakst_actionpoint _array_element)) "NewEnumerator1") (== (.lock (Utilities|Struct|Breakst_actionpoint _array_element)) false))
      (LocalVariables|SetNewLocalVar (+ (LocalVariables|GetNewLocalVar) 1))))
  (return (LocalVariables|GetNewLocalVar)))

(fn CheckiftheActionItemsAreSufficient
  (params (SP :type Boolean) (need_actionpoint_NO :type Integer))
  (bind _player_actionpoint (Variables|Default|GetPlayer_actionpoint))
  (bind _spap (LocalVariables|GetSPAP))
  (bind _returnvalue (Utilities|Array|Length _spap))
  (bind _returnvalue_2 (- need_actionpoint_NO _returnvalue))
  ;[1 1 1] 重置所有行动点的锁定状态
  (for _array_element (Variables|Default|GetPlayer_actionpoint)
    (Utilities|Array|SetArrayElem (Variables|Default|GetPlayer_actionpoint) 0 (Utilities|Struct|Makest_actionpoint (.actionpoint_id (Utilities|Struct|Breakst_actionpoint _array_element)) (.ACTIONPOINT_TYPE (Utilities|Struct|Breakst_actionpoint _array_element)) (.actionpoint_status (Utilities|Struct|Breakst_actionpoint _array_element)) false))
    (Utilities|FlowControl|Sequence
      (:then_0
        ;[1 1 1] 是否消耗特异行动点
        (if SP ; 是否消耗特异行动点
          (for _array_element_2 (Variables|Default|GetPlayer_actionpoint)
            (if (and (Utilities|Enum|Equal(Enum) (.ACTIONPOINT_TYPE (Utilities|Struct|Breakst_actionpoint _array_element_2)) "NewEnumerator2") (Utilities|Enum|Equal(Enum) (.actionpoint_status (Utilities|Struct|Breakst_actionpoint _array_element_2)) "NewEnumerator1"))
              (if (> need_actionpoint_NO (Utilities|Array|Length (LocalVariables|GetSPAP)))
                (Utilities|Array|SetArrayElem (Variables|Default|GetPlayer_actionpoint) 0 (Utilities|Struct|Makest_actionpoint (.actionpoint_id (Utilities|Struct|Breakst_actionpoint _array_element_2)) (.ACTIONPOINT_TYPE (Utilities|Struct|Breakst_actionpoint _array_element_2)) (.actionpoint_status (Utilities|Struct|Breakst_actionpoint _array_element_2)) true))
                (Utilities|Array|Add (LocalVariables|GetSPAP) _array_element_2)
                (else
                  (return false)))))
          ;[1 1 1] 检查常规行动点是否足够
          (bind _no (U1|CounttheNumberOfStandardActionPoints (Variables|Default|GetPlayer_actionpoint) :!label _label)) ; 检查能使用的常规和临时、无锁的行动点
          (bind _output_get (LocalVariables|Setdo (> _no (LocalVariables|Getneed_actionpoint))))
          (if _output_get
            (while (LocalVariables|Getwhile_loop)
              ;[1 1 1] 查找行动点
              (for _array_element_3 (Variables|Default|GetPlayer_actionpoint) ; 循环每一个行动点
                (if (and (or (Utilities|Enum|Equal(Enum) (.ACTIONPOINT_TYPE (Utilities|Struct|Breakst_actionpoint _array_element_3)) "NewEnumerator1") (Utilities|Enum|Equal(Enum) (.ACTIONPOINT_TYPE (Utilities|Struct|Breakst_actionpoint _array_element_3)) "NewEnumerator0")) (Utilities|Enum|Equal(Enum) (.actionpoint_status (Utilities|Struct|Breakst_actionpoint _array_element_3)) "NewEnumerator1"))
                  (Utilities|Array|SetArrayElem _player_actionpoint (Utilities|Array|FindItem _player_actionpoint _array_element_3) (Utilities|Struct|Makest_actionpoint (.actionpoint_id (Utilities|Struct|Breakst_actionpoint _array_element_3)) (.ACTIONPOINT_TYPE (Utilities|Struct|Breakst_actionpoint _array_element_3)) (.actionpoint_status (Utilities|Struct|Breakst_actionpoint _array_element_3)) true))
                  ;[1 1 1] 检查当前累计的行动点是否小于所需行动点
                  (bind _output_get_2 (LocalVariables|Setcurrent_Cactionpoint (+ (LocalVariables|Getcurrent_Cactionpoint) 1)))
                  (LocalVariables|Setwhile_loop (>= (LocalVariables|Getneed_actionpoint) _output_get_2))
                  (Default|CallWhentheActionPointsChange))))
            (else
              (return false)))))
      (:then_1
        (if (> need_actionpoint_NO _returnvalue)
          (if SP
            (LocalVariables|Setneed_actionpoint (* _returnvalue_2 2))
            (else
              (LocalVariables|Setneed_actionpoint _returnvalue_2)))
          (else
            (return true))))
      (:then_2
        (goto _label))
      (:then_3
        (if (== (LocalVariables|Getwhile_loop) false)
          (return true))))))

(fn EROSIONACTIONPOINT
  (params (LastIndex :type Integer))
  (for _index (range 0 LastIndex)
    (for _array_element (Variables|Default|GetPlayer_actionpoint)
      (if (Utilities|Enum|Equal(Enum) (.ACTIONPOINT_TYPE (Utilities|Struct|Breakst_actionpoint _array_element)) "NewEnumerator1")
        (Utilities|Array|RemoveItem (Variables|Default|GetPlayer_actionpoint) _array_element)
        (elif (and (Utilities|Enum|Equal(Enum) (.ACTIONPOINT_TYPE (Utilities|Struct|Breakst_actionpoint _array_element)) "NewEnumerator0") (Utilities|Enum|NotEqual(Enum) (.actionpoint_status (Utilities|Struct|Breakst_actionpoint _array_element)) "NewEnumerator2"))
          (Utilities|Array|SetArrayElem (Variables|Default|GetPlayer_actionpoint) (Utilities|Array|FindItem (Variables|Default|GetPlayer_actionpoint) _array_element) (Utilities|Struct|Makest_actionpoint (.actionpoint_id (Utilities|Struct|Breakst_actionpoint _array_element)) (.ACTIONPOINT_TYPE (Utilities|Struct|Breakst_actionpoint _array_element)) "NewEnumerator2" false)))))))

(fn RestoreActionPoints
  (params (actionpoint :type Integer))
  (for _index (range 0 actionpoint)
    (for _array_element (Variables|Default|GetPlayer_actionpoint)
      (if (Utilities|Enum|Equal(Enum) (.actionpoint_status (Utilities|Struct|Breakst_actionpoint _array_element)) "NewEnumerator0")
        (Utilities|Array|SetArrayElem (Variables|Default|GetPlayer_actionpoint) (Utilities|Array|FindItem (Variables|Default|GetPlayer_actionpoint) _array_element) (Utilities|Struct|Makest_actionpoint (.actionpoint_id (Utilities|Struct|Breakst_actionpoint _array_element)) (.ACTIONPOINT_TYPE (Utilities|Struct|Breakst_actionpoint _array_element)) "NewEnumerator1" false))))))

(fn CalculatePlayerStActionpoint
  (bind _fixed_actionpoint (Variables|Actionpoint|Getfixed_actionpoint))
  (bind _float_actionpoint (Variables|Actionpoint|Getfloat_actionpoint))
  (bind (_actionpointcap _initializeactionpoints _gainactionpointspercycle _turngainactionpoint_cap _actionpointsconsumed _additionalactionpointsconsumed) (Utilities|Struct|Breakst_player_actionpoint _fixed_actionpoint))
  (bind (_actionpointcap_2 _initializeactionpoints_2 _gainactionpointspercycle_2 _turngainactionpoint_cap_2 _actionpointsconsumed_2 _additionalactionpointsconsumed_2) (Utilities|Struct|Breakst_player_actionpoint _float_actionpoint))
  (Variables|Actionpoint|Setcurrent_actionpoint (Utilities|Struct|Makest_player_actionpoint (+ _actionpointcap _actionpointcap_2) (+ _initializeactionpoints _initializeactionpoints_2) (+ _gainactionpointspercycle _gainactionpointspercycle_2) (+ _turngainactionpoint_cap _turngainactionpoint_cap_2) (+ _actionpointsconsumed _actionpointsconsumed_2) (+ _additionalactionpointsconsumed _additionalactionpointsconsumed_2))))

(fn CalculatetheActionPointsGainedThisTurn
  (params (current_turn :type Integer))
  (bind _current_actionpoint (Variables|Actionpoint|Getcurrent_actionpoint))
  (bind _current_actionpoint_2 (Variables|Actionpoint|Getcurrent_actionpoint))
  (bind _current_actionpoint_3 (Variables|Actionpoint|Getcurrent_actionpoint))
  (bind (_gainactionpointspercycle _turngainactionpoint_cap) (Utilities|Struct|Breakst_player_actionpoint _current_actionpoint_2))
  (bind _actionpointcap (Utilities|Struct|Breakst_player_actionpoint _current_actionpoint))
  (bind (_actionpointcap_2 _initializeactionpoints) (Utilities|Struct|Breakst_player_actionpoint _current_actionpoint_3))
  (bind _returnvalue (+ current_turn 1))
  (bind _returnvalue_2 (* _gainactionpointspercycle _returnvalue))
  (if (== current_turn 0)
    (return _actionpointcap_2 _initializeactionpoints)
    (elif (>= _returnvalue_2 _turngainactionpoint_cap) ; 运算的行动点是否大于行动点上限
      (bind _output_get (LocalVariables|Setactpoint _turngainactionpoint_cap))
      (return _actionpointcap _output_get)
      (else
        (bind _output_get_2 (LocalVariables|Setactpoint _returnvalue_2))
        (return _actionpointcap _output_get_2)))))

(fn CheakActpintEnough
  (params (player_action_point :type Integer) (need_action_point :type Integer))
  (return (>= player_action_point need_action_point)))

(fn FindBuffbyBuff
  (params (Buff :type Object%20Object%20Reference))
  (for _array_element (Variables|buff|Getcurrent_player_buff)
    (if (== _array_element Buff)
      (return (Utilities|Array|FindItem (Variables|buff|Getcurrent_player_buff) _array_element) (== _array_element Buff) _array_element))))

(fn FindBuffbyIndex
  (params (Buff_indexX :type St%20Player%20Buff%20Base%20Info%20Structure))
  (for _array_element (Variables|buff|Getcurrent_player_buff)
    (if (== (.buff_index (Utilities|Struct|Breakst_player_buff_base_info (Variables|/Game/BP/BP_AC/BP_player_AC/BP_player_buff_object.BP_player_buff_object_C|Getbuff_info _array_element))) (.buff_index (Utilities|Struct|Breakst_player_buff_base_info Buff_indexX)))
      (return _array_element (== (.buff_index (Utilities|Struct|Breakst_player_buff_base_info (Variables|/Game/BP/BP_AC/BP_player_AC/BP_player_buff_object.BP_player_buff_object_C|Getbuff_info _array_element))) (.buff_index (Utilities|Struct|Breakst_player_buff_base_info Buff_indexX))) (Utilities|Array|FindItem (Variables|buff|Getcurrent_player_buff) _array_element)))))

(fn GetPlayerBuff
  (params (buff_infoC :type St%20Player%20Buff%20Base%20Info%20Structure) (NumericCC :type St%20Player%20Buff%20Numeric%20Attribute%20Structure) (unit_buff_targerC :type St%20Buff%20Target%20Data%20Structure) (pb_effect_info :type Array%20of%20St%20PB%20Effect%20Info%20Structures) (SETTINGC :type St%20Player%20Buff%20Setting%20Structure) (player_buffC :type BP%20Player%20Buff%20Object%20Class%20Reference))
  (bind _returnvalue (Game|ConstructObjectfromClass player_buffC))
  (Default|InitializeBuff _returnvalue buff_infoC NumericCC pb_effect_info unit_buff_targerC SETTINGC)
  (Utilities|Array|Add (Variables|buff|Getwait_ADD_player_buff) _returnvalue)
  (buff_T|BuffTick))

(fn PlayerBuffActionCheak
  (params (Trigger%20timingX :type E_TriggerTiming%20Enum :default "NewEnumerator0") (action_typeX :type E_TriggerAction_type%20Enum :default "NewEnumerator0") (skill_typeX :type E_SKILL_TYPE%20Enum :default "NewEnumerator3") (Skill_Action_typeX :type E_TriggerAction_skill_mode%20Enum :default "NewEnumerator4") (Action_effect_tyoeX :type E_TriggerActionEffectType%20Enum :default "NewEnumerator0") (actionX :type BP%20BASE%20Pawn%20Object%20Reference) (targetX :type BP%20BASE%20Pawn%20Object%20Reference) (NewParam :type Float%20%28double-precision%29) (unitdata :type Array%20of%20St%20Unit%20Class%20Structures))
  (if (Utilities|Array|IsNotEmpty (Variables|buff|Getcurrent_player_buff))
    (for _array_element (Variables|buff|Getcurrent_player_buff)
      (for _array_element_2 (Variables|/Game/BP/BP_AC/BP_player_AC/BP_player_buff_object.BP_player_buff_object_C|Getpb_effect_info _array_element)
        (if (Utilities|Enum|Equal(Enum) Trigger%20timingX (.P_timing (Utilities|Struct|Breakst_PB_Effect_info _array_element_2)))
          (LocalVariables|Setbuff _array_element)
          (LocalVariables|Setbuff_effect_type (.PB_effect_type (Utilities|Struct|Breakst_PB_Effect_info _array_element_2)))
          (for _array_element_3 unitdata
            (if (Math|Boolean|ANDBoolean (Utilities|Enum|Equal(Enum) (.target_area (Utilities|Struct|BreakST_unit_skill_target_data (.U_select_info (Utilities|Struct|Breakst_PB_Effect_info _array_element_2)))) (.theunitarea (Utilities|Struct|Breakst_unit_class _array_element_3))) (Utilities|Enum|Equal(Enum) (.theunit_Belongs (Utilities|Struct|Breakst_unit_class _array_element_3)) (.target_faction (Utilities|Struct|BreakST_unit_skill_target_data (.U_select_info (Utilities|Struct|Breakst_PB_Effect_info _array_element_2))))) (Utilities|Enum|Equal(Enum) (.gameplay_unit_type (Utilities|Struct|Breakst_unit_class _array_element_3)) (.unit_type (Utilities|Struct|BreakST_unit_skill_target_data (.U_select_info (Utilities|Struct|Breakst_PB_Effect_info _array_element_2))))))
              (LocalVariables|Settarget _array_element_3)
              (switch Utilities|FlowControl|Switch|SwitchonE_skill_target (.target_type (Utilities|Struct|BreakST_unit_skill_target_data (.U_select_info (Utilities|Struct|Breakst_PB_Effect_info _array_element_2))))
                (:NewEnumerator1
                  (bind _asbp_base_pawn (Utilities|Casting|CastToBP_BASE_Pawn (Utilities|Struct|Breakst_unit_class (LocalVariables|Gettarget))))
                  (Default|EffectEvent (LocalVariables|Getbuff) (LocalVariables|Getbuff_effect_type) _asbp_base_pawn))
                (:NewEnumerator0
                  (bind _asbp_base_pawn_2 (Utilities|Casting|CastToBP_BASE_Pawn (Utilities|Struct|Breakst_unit_class (LocalVariables|Gettarget))))
                  (Default|EffectEvent (LocalVariables|Getbuff) (LocalVariables|Getbuff_effect_type) _asbp_base_pawn_2))))))))))