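; Player component that manages action points for turn-based play; its buff add, remove and tick functions are empty stubs.
; An array of action-point structs tracks type, status and lock, with functions to add, restore and erode points.
; Sufficiency checks lock points, optionally special ones first, then spending resets locked routine or special points and removes temporary ones.
; Fixed and floating stats sum into current stats, driving capped per-turn gains.
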(event EventBeginPlay)

(event EventTick
  (params (DeltaSeconds :type Float%20%28single-precision%29)))

(fn InitializeActionPoints
  (params (soild- :type Integer) (empty :type Integer))
  (Utilities|FlowControl|Sequence
    (:then_0
      (for _index (range 1 soild-)
        (Utilities|Array|Add (Variables|Default|GetPlayer_actionpoint) (Utilities|Struct|Makest_actionpoint _index "NewEnumerator0" "NewEnumerator1" false))))
    (:then_1
      (for _index_2 (range (+ soild- 1) empty)
        (Utilities|Array|Add (Variables|Default|GetPlayer_actionpoint) (Utilities|Struct|Makest_actionpoint _index_2 "NewEnumerator0" "NewEnumerator0" false))))))

(fn SpendActionPoints
  (for _array_element (Variables|Default|GetPlayer_actionpoint)
    (if (.lock (Utilities|Struct|Breakst_actionpoint _array_element))
      (switch Utilities|FlowControl|Switch|SwitchonE_actionpoint_type (.ACTIONPOINT_TYPE (Utilities|Struct|Breakst_actionpoint _array_element))
        (:NewEnumerator0
          (Utilities|Array|SetArrayElem (Variables|Default|GetPlayer_actionpoint) 0 (Utilities|Struct|Makest_actionpoint (.actionpoint_id (Utilities|Struct|Breakst_actionpoint _array_element)) (.ACTIONPOINT_TYPE (Utilities|Struct|Breakst_actionpoint _array_element)) "NewEnumerator0" false) :!label _label))
        (:NewEnumerator1
          (Utilities|Array|RemoveItem (Variables|Default|GetPlayer_actionpoint) _array_element))
        (:NewEnumerator2
          (goto _label))))))

(fn IncreaseActionPoints
  (params (LastIndex :type Integer) (ACTIONPOINT_TYPE :type E_actionpoint_type%20Enum :default "NewEnumerator0") (actionpoint_status :type e_actionpoint_Status%20Enum :default "NewEnumerator0"))
  (for _index (range 1 LastIndex)
    (Utilities|Array|Add (Variables|Default|GetPlayer_actionpoint) (Utilities|Struct|Makest_actionpoint 0 ACTIONPOINT_TYPE actionpoint_status false))))

(fn ADDBuff)

(fn RemoveBuff)

(fn BuffTick)

(fn UseActionPoints（NG）
  (for _array_element (Variables|Default|GetPlayer_actionpoint)
    (if (.lock (Utilities|Struct|Breakst_actionpoint _array_element))
      (switch Utilities|FlowControl|Switch|SwitchonE_actionpoint_type (.ACTIONPOINT_TYPE (Utilities|Struct|Breakst_actionpoint _array_element))
        (:NewEnumerator0
          (Utilities|Array|SetArrayElem (Variables|Default|GetPlayer_actionpoint) 0 (Utilities|Struct|Makest_actionpoint (.actionpoint_id (Utilities|Struct|Breakst_actionpoint _array_element)) (.ACTIONPOINT_TYPE (Utilities|Struct|Breakst_actionpoint _array_element)) "NewEnumerator0" false) :!label _label))
        (:NewEnumerator1
          (Utilities|Array|RemoveItem (Variables|Default|GetPlayer_actionpoint) _array_element))
        (:NewEnumerator2
          (goto _label))))))

(fn ConvertUnusableActionPointsIntoEmptyActionPoints
  (params (LastIndex :type Integer))
  (for _index (range 0 LastIndex)
    (for _array_element (Variables|Default|GetPlayer_actionpoint)
      (if (Utilities|Enum|Equal(Enum) (.actionpoint_status (Utilities|Struct|Breakst_actionpoint _array_element)) "NewEnumerator2")
        (Utilities|Array|SetArrayElem (Variables|Default|GetPlayer_actionpoint) 0 (Utilities|Struct|Makest_actionpoint (.actionpoint_id (Utilities|Struct|Breakst_actionpoint _array_element)) (.ACTIONPOINT_TYPE (Utilities|Struct|Breakst_actionpoint _array_element)) "NewEnumerator0" false))))))

(fn CounttheNumberOfStandardActionPoints
  (params (Array :type Array%20of%20St%20Actionpoint%20Structures))
  (for _array_element Array
    (if (Math|Boolean|ANDBoolean (Utilities|Enum|NotEqual(Enum) (.ACTIONPOINT_TYPE (Utilities|Struct|Breakst_actionpoint _array_element)) "NewEnumerator2") (Utilities|Enum|Equal(Enum) (.actionpoint_status (Utilities|Struct|Breakst_actionpoint _array_element)) "NewEnumerator1") (== (.lock (Utilities|Struct|Breakst_actionpoint _array_element)) false))
      (LocalVariables|SetNewLocalVar (+ (LocalVariables|GetNewLocalVar) 1))))
  (return (LocalVariables|GetNewLocalVar)))

(fn CheckiftheActionItemsAreSufficient
  (params (SP :type Boolean) (need_actionpoint_NO :type Integer))
  (bind _player_actionpoint (Variables|Default|GetPlayer_actionpoint))
  (bind _spap (LocalVariables|GetSPAP))
  (bind _returnvalue (Utilities|Array|Length _spap))
  (bind _returnvalue_2 (- need_actionpoint_NO _returnvalue))
  ;[1 1 1] 重置所有行动点的锁定状态
  (for _array_element (Variables|Default|GetPlayer_actionpoint)
    (Utilities|Array|SetArrayElem (Variables|Default|GetPlayer_actionpoint) 0 (Utilities|Struct|Makest_actionpoint (.actionpoint_id (Utilities|Struct|Breakst_actionpoint _array_element)) (.ACTIONPOINT_TYPE (Utilities|Struct|Breakst_actionpoint _array_element)) (.actionpoint_status (Utilities|Struct|Breakst_actionpoint _array_element)) false))
    (Utilities|FlowControl|Sequence
      (:then_0
        ;[1 1 1] 是否消耗特异行动点
        (if SP ; 是否消耗特异行动点
          (for _array_element_2 (Variables|Default|GetPlayer_actionpoint)
            (if (and (Utilities|Enum|Equal(Enum) (.ACTIONPOINT_TYPE (Utilities|Struct|Breakst_actionpoint _array_element_2)) "NewEnumerator2") (Utilities|Enum|Equal(Enum) (.actionpoint_status (Utilities|Struct|Breakst_actionpoint _array_element_2)) "NewEnumerator1"))
              (if (> need_actionpoint_NO (Utilities|Array|Length (LocalVariables|GetSPAP)))
                (Utilities|Array|SetArrayElem (Variables|Default|GetPlayer_actionpoint) 0 (Utilities|Struct|Makest_actionpoint (.actionpoint_id (Utilities|Struct|Breakst_actionpoint _array_element_2)) (.ACTIONPOINT_TYPE (Utilities|Struct|Breakst_actionpoint _array_element_2)) (.actionpoint_status (Utilities|Struct|Breakst_actionpoint _array_element_2)) true))
                (Utilities|Array|Add (LocalVariables|GetSPAP) _array_element_2)
                (else
                  (return false)))))
          ;[1 1 1] 检查常规行动点是否足够
          (bind _no (U1|CounttheNumberOfStandardActionPoints (Variables|Default|GetPlayer_actionpoint) :!label _label)) ; 检查能使用的常规和临时、无锁的行动点
          (bind _output_get (LocalVariables|Setdo (> _no (LocalVariables|Getneed_actionpoint))))
          (if _output_get
            (while (LocalVariables|Getwhile_loop)
              ;[1 1 1] 查找行动点
              (for _array_element_3 (Variables|Default|GetPlayer_actionpoint) ; 循环每一个行动点
                (if (and (or (Utilities|Enum|Equal(Enum) (.ACTIONPOINT_TYPE (Utilities|Struct|Breakst_actionpoint _array_element_3)) "NewEnumerator1") (Utilities|Enum|Equal(Enum) (.ACTIONPOINT_TYPE (Utilities|Struct|Breakst_actionpoint _array_element_3)) "NewEnumerator0")) (Utilities|Enum|Equal(Enum) (.actionpoint_status (Utilities|Struct|Breakst_actionpoint _array_element_3)) "NewEnumerator1"))
                  (Utilities|Array|SetArrayElem _player_actionpoint (Utilities|Array|FindItem _player_actionpoint _array_element_3) (Utilities|Struct|Makest_actionpoint (.actionpoint_id (Utilities|Struct|Breakst_actionpoint _array_element_3)) (.ACTIONPOINT_TYPE (Utilities|Struct|Breakst_actionpoint _array_element_3)) (.actionpoint_status (Utilities|Struct|Breakst_actionpoint _array_element_3)) true))
                  ;[1 1 1] 检查当前累计的行动点是否小于所需行动点
                  (bind _output_get_2 (LocalVariables|Setcurrent_Cactionpoint (+ (LocalVariables|Getcurrent_Cactionpoint) 1)))
                  (LocalVariables|Setwhile_loop (>= (LocalVariables|Getneed_actionpoint) _output_get_2))
                  (Default|CallWhentheActionPointsChange))))
            (else
              (return false)))))
      (:then_1
        (if (> need_actionpoint_NO _returnvalue)
          (if SP
            (LocalVariables|Setneed_actionpoint (* _returnvalue_2 2))
            (else
              (LocalVariables|Setneed_actionpoint _returnvalue_2)))
          (else
            (return true))))
      (:then_2
        (goto _label))
      (:then_3
        (if (== (LocalVariables|Getwhile_loop) false)
          (return true))))))

(fn EROSIONACTIONPOINT
  (params (LastIndex :type Integer))
  (for _index (range 0 LastIndex)
    (for _array_element (Variables|Default|GetPlayer_actionpoint)
      (if (Utilities|Enum|Equal(Enum) (.ACTIONPOINT_TYPE (Utilities|Struct|Breakst_actionpoint _array_element)) "NewEnumerator1")
        (Utilities|Array|RemoveItem (Variables|Default|GetPlayer_actionpoint) _array_element)
        (elif (and (Utilities|Enum|Equal(Enum) (.ACTIONPOINT_TYPE (Utilities|Struct|Breakst_actionpoint _array_element)) "NewEnumerator0") (Utilities|Enum|NotEqual(Enum) (.actionpoint_status (Utilities|Struct|Breakst_actionpoint _array_element)) "NewEnumerator2"))
          (Utilities|Array|SetArrayElem (Variables|Default|GetPlayer_actionpoint) (Utilities|Array|FindItem (Variables|Default|GetPlayer_actionpoint) _array_element) (Utilities|Struct|Makest_actionpoint (.actionpoint_id (Utilities|Struct|Breakst_actionpoint _array_element)) (.ACTIONPOINT_TYPE (Utilities|Struct|Breakst_actionpoint _array_element)) "NewEnumerator2" false)))))))

(fn RestoreActionPoints
  (params (actionpoint :type Integer))
  (for _index (range 0 actionpoint)
    (for _array_element (Variables|Default|GetPlayer_actionpoint)
      (if (Utilities|Enum|Equal(Enum) (.actionpoint_status (Utilities|Struct|Breakst_actionpoint _array_element)) "NewEnumerator0")
        (Utilities|Array|SetArrayElem (Variables|Default|GetPlayer_actionpoint) (Utilities|Array|FindItem (Variables|Default|GetPlayer_actionpoint) _array_element) (Utilities|Struct|Makest_actionpoint (.actionpoint_id (Utilities|Struct|Breakst_actionpoint _array_element)) (.ACTIONPOINT_TYPE (Utilities|Struct|Breakst_actionpoint _array_element)) "NewEnumerator1" false))))))

(fn CalculatePlayerStActionpoint
  (bind _fixed_actionpoint (Variables|Actionpoint|Getfixed_actionpoint))
  (bind _float_actionpoint (Variables|Actionpoint|Getfloat_actionpoint))
  (bind (_actionpointcap _initializeactionpoints _gainactionpointspercycle _turngainactionpoint_cap _actionpointsconsumed _additionalactionpointsconsumed) (Utilities|Struct|Breakst_player_actionpoint _fixed_actionpoint))
  (bind (_actionpointcap_2 _initializeactionpoints_2 _gainactionpointspercycle_2 _turngainactionpoint_cap_2 _actionpointsconsumed_2 _additionalactionpointsconsumed_2) (Utilities|Struct|Breakst_player_actionpoint _float_actionpoint))
  (Variables|Actionpoint|Setcurrent_actionpoint (Utilities|Struct|Makest_player_actionpoint (+ _actionpointcap _actionpointcap_2) (+ _initializeactionpoints _initializeactionpoints_2) (+ _gainactionpointspercycle _gainactionpointspercycle_2) (+ _turngainactionpoint_cap _turngainactionpoint_cap_2) (+ _actionpointsconsumed _actionpointsconsumed_2) (+ _additionalactionpointsconsumed _additionalactionpointsconsumed_2))))

(fn CalculatetheActionPointsGainedThisTurn
  (params (current_turn :type Integer))
  (bind _current_actionpoint (Variables|Actionpoint|Getcurrent_actionpoint))
  (bind _current_actionpoint_2 (Variables|Actionpoint|Getcurrent_actionpoint))
  (bind _current_actionpoint_3 (Variables|Actionpoint|Getcurrent_actionpoint))
  (bind (_gainactionpointspercycle _turngainactionpoint_cap) (Utilities|Struct|Breakst_player_actionpoint _current_actionpoint_2))
  (bind _actionpointcap (Utilities|Struct|Breakst_player_actionpoint _current_actionpoint))
  (bind (_actionpointcap_2 _initializeactionpoints) (Utilities|Struct|Breakst_player_actionpoint _current_actionpoint_3))
  (bind _returnvalue (+ current_turn 1))
  (bind _returnvalue_2 (* _gainactionpointspercycle _returnvalue))
  (if (== current_turn 0)
    (return _actionpointcap_2 _initializeactionpoints)
    (elif (>= _returnvalue_2 _turngainactionpoint_cap) ; 运算的行动点是否大于行动点上限
      (bind _output_get (LocalVariables|Setactpoint _turngainactionpoint_cap))
      (return _actionpointcap _output_get)
      (else
        (bind _output_get_2 (LocalVariables|Setactpoint _returnvalue_2))
        (return _actionpointcap _output_get_2)))))

(fn CheakActpintEnough
  (params (player_action_point :type Integer) (need_action_point :type Integer))
  (return (>= player_action_point need_action_point)))