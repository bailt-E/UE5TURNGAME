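; Base player buff object that stores a buff's info, numeric settings and runtime resources, with empty effect hooks.
; InitializeBuff copies in the config and seeds cycle and persistent turn counters.
; GetResources adjusts stack, energy, threshold and priority, either by supplied amounts or through a percentage mode.
; CommonEffect and EffectEvent dispatch by enum to the begin, cycle, end, trigger and activate stubs.
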(fn GetResources
  (params (Percentage%20mode :type Boolean) (Percentage :type Integer) (new_re :type St%20PB%20Resources%20Structure) (typeC :type E_player_buff_R_type%20Enum :default "NewEnumerator0"))
  (bind _numeric (Variables|A2|GetNumeric))
  (bind (_stack _priority _threshold _energy) (Utilities|Struct|Breakst_PB_Resources new_re))
  (bind (_charge _priority_cap _thresholdbenchmark) (Utilities|Struct|Breakst_player_buff_Numeric_attribute _numeric))
  (if Percentage%20mode
    (switch Utilities|FlowControl|Switch|SwitchonE_player_buff_R_type typeC
      (:NewEnumerator0
        (Variables|A2|Setresources (Utilities|Struct|Makest_PB_Resources (+ (.Energy (Utilities|Struct|Breakst_PB_Resources (Variables|A2|Getresources))) (Math|Integer|%(Integer) (+ Percentage 100) _charge)))))
      (:NewEnumerator1
        (Variables|A2|Setresources (Utilities|Struct|Makest_PB_Resources (+ (.Threshold (Utilities|Struct|Breakst_PB_Resources (Variables|A2|Getresources))) (Math|Integer|%(Integer) (+ Percentage 100) _thresholdbenchmark)))))
      (:NewEnumerator3
        (Variables|A2|Setresources (Utilities|Struct|Makest_PB_Resources (+ (.Priority (Utilities|Struct|Breakst_PB_Resources (Variables|A2|Getresources))) (Math|Integer|%(Integer) (+ Percentage 100) _priority_cap))))))
    (else
      (Variables|A2|Setresources (Utilities|Struct|Makest_PB_Resources (+ (.stack (Utilities|Struct|Breakst_PB_Resources (Variables|A2|Getresources))) _stack) (+ (.Priority (Utilities|Struct|Breakst_PB_Resources (Variables|A2|Getresources))) _priority) (+ (.Threshold (Utilities|Struct|Breakst_PB_Resources (Variables|A2|Getresources))) _threshold) (+ (.Energy (Utilities|Struct|Breakst_PB_Resources (Variables|A2|Getresources))) _energy))))))

(fn InitializeBuff
  (params (buff_infoC :type St%20Player%20Buff%20Base%20Info%20Structure) (NumericC :type St%20Player%20Buff%20Numeric%20Attribute%20Structure) (pb_effect_infoX :type Array%20of%20St%20PB%20Effect%20Info%20Structures) (unit_buff_targer :type St%20Buff%20Target%20Data%20Structure) (BUFF_SETTING :type St%20Player%20Buff%20Setting%20Structure))
  (Variables|A2|Setbuff_info buff_infoC)
  (bind _output_get (Variables|A2|SetNumeric NumericC))
  (Variables|Default|Setpb_effect_info pb_effect_infoX)
  (Variables|A2|Setunit_buff_targer unit_buff_targer)
  (Variables|A2|SetBUFF_SETTING BUFF_SETTING)
  (Variables|A2|Setresources (Utilities|Struct|Makest_PB_Resources 0 0 0 0 (.CycleTurn (Utilities|Struct|Breakst_player_buff_Numeric_attribute _output_get)) (.PersistentTurn (Utilities|Struct|Breakst_player_buff_Numeric_attribute _output_get)))))

(fn EndEffect)

(fn Activate
  (params (base%20pawn :type BP%20BASE%20Pawn%20Object%20Reference)))

(fn CycleEffect)

(fn BeginEffect)

(fn TirggetEffect
  (params (trigger :type E_TriggerTiming%20Enum :default "NewEnumerator0")))

(fn CommonEffect
  (params (buff_Basics :type E_player_buff_Basics_effect_type%20Enum :default "NewEnumerator3") (target :type BP%20BASE%20Pawn%20Object%20Reference) (tirgger_time :type E_TriggerTiming%20Enum :default "NewEnumerator0"))
  (switch Utilities|FlowControl|Switch|SwitchonE_player_buff_Basics_effect_type buff_Basics
    (:NewEnumerator3
      (effect|TirggetEffect tirgger_time))
    (:NewEnumerator0
      (effect|BeginEffect))
    (:NewEnumerator1
      (effect|CycleEffect))
    (:NewEnumerator2
      (effect|EndEffect))))

(fn EffectEvent
  (params (effect_type :type E_player_buff_Basics_effect_type%20Enum :default "NewEnumerator3") (base%20pawnC :type BP%20BASE%20Pawn%20Object%20Reference))
  (switch Utilities|FlowControl|Switch|SwitchonE_player_buff_Basics_effect_type effect_type
    (:NewEnumerator4
      (effect|Activate base%20pawnC))
    (:NewEnumerator5
      (effect|TirggetEffect "NewEnumerator0"))))