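; BP_unit_skill_class is a unit skill class that activates a skill and deals damage to its selected targets.
; Activation constructs a Skilleffect object and, for direct skills, calls its DamageE on each unit in target groups of one selection type.
; Damage values and attack count are hard-coded, with a debug print after each call.
; Ability initialization and skill effect functions are empty stubs, and an alternative target loop is unwired.
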(fn AbilityInitialization)

(fn Activation
  (params (skill%20create :type BP%20BASE%20Pawn%20Object%20Reference) (Selection :type E_SKILL_model%20Enum :default "NewEnumerator0") (be_select_target :type Array%20of%20St%20Select%20Unit%20Target%20Data%20Structures))
  (bind _returnvalue (Game|ConstructObjectfromClass (Variables|Default|Getskilleffect)))
  (LocalVariables|Setskill _returnvalue)
  (switch Utilities|FlowControl|Switch|SwitchonE_SKILL_model Selection
    (:NewEnumerator1
      (for _array_element be_select_target
        (if (Utilities|Enum|Equal(Enum) (.select_target_type (Utilities|Struct|Breakst_select_unit_target_data _array_element)) "NewEnumerator1")
          (for _array_element_2 (.unit (Utilities|Struct|Breakst_select_unit_target_data _array_element))
            (Default|DamageE (LocalVariables|Getskill) _array_element_2 skill%20create (Utilities|Array|MakeArray 100 100 100) 1 "NewEnumerator1" "NewEnumerator0" "NewEnumerator1")
            (Development|PrintString 0 "BP_unit_skill_use-skill" true true "(R=0.000000,G=0.012712,B=1.000000,A=1.000000)" 1e+02)))))))

(fn SkillEffect)