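; Unit skill component that picks an acting unit and a skill target from supplied unit lists.
; SelectUnit returns the first actionable matching unit with more action points than the stored one.
; SelectUnitSkill reads the effect type from T_unit_skill: Treat compares HP ratio, Attack compares aggro on another side, Summon checks skill area.
; Loops return at the first qualifying entry rather than scanning for a true maximum.
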(event EventBeginPlay)

(event EventTick
  (params (DeltaSeconds :type Float%20%28single-precision%29)))

(fn SelectUnit
  (params (unit :type Array%20of%20St%20Unit%20Class%20Structures))
  (for _array_element unit
    (bind _asbp_base_unit (Utilities|Casting|CastToBP_BASE_UNIT (.charter (Utilities|Struct|Breakst_unit_class _array_element))))
    (bind _asbp_unit_class (Utilities|Casting|CastToBP_unit_class _asbp_base_unit))
    (if (Variables|/Game/BP/BP_modelE/BP_BASE_UNIT.BP_BASE_UNIT_C|Getunit_can_action _asbp_unit_class)
      (if (and (Utilities|Enum|Equal(Enum) (.theunit_Belongs (Utilities|Struct|Breakst_unit_class _array_element)) "NewEnumerator0") (Utilities|Enum|Equal(Enum) (Variables|/Game/BP/BP_modelE/BP_BASE_UNIT.BP_BASE_UNIT_C|Getgameplay_unit_type _asbp_base_unit) "NewEnumerator0"))
        (Math|Integer|CompareInt (Utilities|Struct|Breakst_the_unit_resource (Variables|/Game/BP/BP_AC/BP_UNIT_AC/BP_AC_unit_attribute.BP_AC_unit_attribute_C|Getunit_resource (Variables|/Game/BP/BP_modelE/BP_unit_class.BP_unit_class_C|GetBP_AC_unit_attribute _asbp_unit_class))) (Utilities|Struct|Breakst_the_unit_resource (Variables|/Game/BP/BP_AC/BP_UNIT_AC/BP_AC_unit_attribute.BP_AC_unit_attribute_C|Getunit_resource (Variables|/Game/BP/BP_modelE/BP_unit_class.BP_unit_class_C|GetBP_AC_unit_attribute (LocalVariables|Getthebiagetunit))))
          (:>
            (bind _output_get (LocalVariables|Setthebiagetunit _asbp_unit_class))
            (return _output_get)))))))

(fn SelectUnitSkill
  (params (RowName :type Name) (unit :type Array%20of%20St%20Unit%20Class%20Structures) (skill_area :type E_area%20Enum :default "NewEnumerator0"))
  (bind _returnvalue (Utilities|GetDataTableRow "/Game/Struct/ST_UNIT_skill/T_unit_skill.T_unit_skill" RowName)
    (:then
      (switch Utilities|FlowControl|Switch|SwitchonE_unit_skill_effect_type (Utilities|Struct|Breakst_unit_skill_effect (Utilities|Struct|Breakst_unit_skill_Assembly _returnvalue))
        (:NewEnumerator0
          (for _array_element unit
            (if (and (Utilities|Enum|Equal(Enum) (.theunit_Belongs (Utilities|Struct|Breakst_unit_class _array_element)) "NewEnumerator0") (Utilities|Enum|Equal(Enum) (.gameplay_unit_type (Utilities|Struct|Breakst_unit_class _array_element)) "NewEnumerator0"))
              (bind _asbp_base_unit (Utilities|Casting|CastToBP_BASE_UNIT (.charter (Utilities|Struct|Breakst_unit_class _array_element))))
              (bind _asbp_base_pawn_class (Utilities|Casting|CastToBP_base_pawn_class _asbp_base_unit))
              (bind _asbp_base_pawn_class_2 (Utilities|Casting|CastToBP_base_pawn_class (Variables|Default|GetAs%20BP%20BASE%20UNIT)))
              (Math|Integer|CompareInt (/ (Utilities|Struct|Breakst_RoleStatus (Variables|/Game/BP/BP_AC/BP_level_AC/AC_level.AC_level_C|GetCurrent_attribute (Variables|/Game/BP/BP_modelE/BP_base_pawn_class.BP_base_pawn_class_C|GetAC_level _asbp_base_pawn_class))) (Utilities|Struct|BreakST_Full_attributes (Variables|/Game/BP/BP_AC/BP_level_AC/AC_level.AC_level_C|GetFull%20attributes (Variables|/Game/BP/BP_modelE/BP_base_pawn_class.BP_base_pawn_class_C|GetAC_level _asbp_base_pawn_class)))) (/ (Utilities|Struct|Breakst_RoleStatus (Variables|/Game/BP/BP_AC/BP_level_AC/AC_level.AC_level_C|GetCurrent_attribute (Variables|/Game/BP/BP_modelE/BP_base_pawn_class.BP_base_pawn_class_C|GetAC_level _asbp_base_pawn_class_2))) (Utilities|Struct|BreakST_Full_attributes (Variables|/Game/BP/BP_AC/BP_level_AC/AC_level.AC_level_C|GetFull%20attributes (Variables|/Game/BP/BP_modelE/BP_base_pawn_class.BP_base_pawn_class_C|GetAC_level _asbp_base_pawn_class_2))))
                (:>
                  _)
                (:==
                  _))
              (bind _output_get (Variables|Default|SetAs%20BP%20BASE%20UNIT _asbp_base_unit))
              (return _output_get))))
        (:NewEnumerator1
          (for _array_element_2 unit
            (if (Utilities|Enum|Equal(Enum) "NewEnumerator0" skill_area)
              (return (.charter (Utilities|Struct|Breakst_unit_class _array_element_2))))))
        (:NewEnumerator2
          (for _array_element_3 unit
            (if (and (Utilities|Enum|Equal(Enum) (.theunit_Belongs (Utilities|Struct|Breakst_unit_class _array_element_3)) "NewEnumerator1") (Utilities|Enum|Equal(Enum) (.gameplay_unit_type (Utilities|Struct|Breakst_unit_class _array_element_3)) "NewEnumerator0"))
              (bind _asbp_base_unit_2 (Utilities|Casting|CastToBP_BASE_UNIT (.charter (Utilities|Struct|Breakst_unit_class _array_element_3))))
              (Math|Float|CompareFloat (Variables|/Game/BP/BP_modelE/BP_BASE_UNIT.BP_BASE_UNIT_C|GetUnit%20aggro _asbp_base_unit_2) (Variables|/Game/BP/BP_modelE/BP_BASE_UNIT.BP_BASE_UNIT_C|GetUnit%20aggro (Variables|Default|GetAs%20BP%20BASE%20UNIT))
                (:>
                  _)
                (:==
                  _))
              (bind _output_get_2 (Variables|Default|SetAs%20BP%20BASE%20UNIT _asbp_base_unit_2))
              (return _output_get_2))))))))