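; AC_unit_Skill is a skill component that chooses and executes monster unit skills in grid-based, action-point combat.
; It provides functions to pick an able monster by action points and its costliest affordable skill with uses left.
; T_unit_skill rows supply targeting classes for the main objective and coordinate offsets around caster or objective for gathering targets.
; Execution constructs the row's skill class, activates it on those targets, then triggers automatic skills.
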(event EventBeginPlay)

(event EventTick
  (params (DeltaSeconds :type Float%20%28single-precision%29)))

(fn SelectUnitCreater
  (params (unit :type Array%20of%20St%20Unit%20Class%20Structures))
  (for _array_element unit
    (bind _asbp_base_pawn (Utilities|Casting|CastToBP_BASE_Pawn (.charter (Utilities|Struct|Breakst_unit_class _array_element))))
    (bind _asbp_monster_class (Utilities|Casting|CastToBP_Monster_class _asbp_base_pawn))
    (if (Variables|/Game/BP/BP_Battle_Phase/BP_BASE_Pawn.BP_BASE_Pawn_C|Getunit_can_action _asbp_monster_class) ; 检查单位能否行动
      (if (and (Utilities|Enum|Equal(Enum) (.theunit_Belongs (Utilities|Struct|Breakst_unit_class _array_element)) "NewEnumerator0") (Utilities|Enum|Equal(Enum) (Variables|/Game/BP/BP_Battle_Phase/BP_BASE_Pawn.BP_BASE_Pawn_C|Getgameplay_unit_type _asbp_base_pawn) "NewEnumerator0"))
        (Math|Integer|CompareInt (Utilities|Struct|Breakst_the_unit_resource (Variables|/Game/BP/BP_AC/BP_UNIT_AC/BP_AC_unit_attribute.BP_AC_unit_attribute_C|Getunit_resource (Variables|/Game/BP/BP_Battle_Phase/BP_Monster_class.BP_Monster_class_C|GetBP_AC_unit_attribute1 _asbp_monster_class))) (Utilities|Struct|Breakst_the_unit_resource (Variables|/Game/BP/BP_AC/BP_UNIT_AC/BP_AC_unit_attribute.BP_AC_unit_attribute_C|Getunit_resource (Variables|/Game/BP/BP_Battle_Phase/BP_Monster_class.BP_Monster_class_C|GetBP_AC_unit_attribute1 (LocalVariables|Getthebiagetunit)))) ; 选择行动点最大的单位
          (:>
            _)
          (:==
            _))
        (bind _output_get (LocalVariables|Setthebiagetunit _asbp_monster_class))
        (return _output_get)))))

(fn SelectUnitSkill
  (params (unit :type BP%20Monster%20Class%20Object%20Reference))
  (Utilities|FlowControl|Sequence
    (:then_0
      ;[1 1 1] 检查小于当前资源的技能
      (for _array_element (Variables|/Game/BP/BP_Battle_Phase/BP_Monster_class.BP_Monster_class_C|Getunit_skill unit)
        (if (.infinite (Utilities|Struct|Breakst_unitclass_skilldata _array_element)) ; 检查技能能否无限使用
          (if (>= (Utilities|Struct|BreakST_UNIT_Current_resource_AA (Variables|/Game/BP/BP_AC/BP_Generic_attributes_AC/AC_Generic_attributes.AC_Generic_attributes_C|GetCurrent_resource (Variables|/Game/BP/BP_Battle_Phase/BP_BASE_Pawn.BP_BASE_Pawn_C|GetAC_Generic_attributes unit))) (.actionpoint (Utilities|Struct|Breakst_unitclass_skilldata _array_element))) :!label _label
            (Utilities|Array|Add (LocalVariables|Getcan_use_skill_list) _array_element))
          (elif (> (.use_number (Utilities|Struct|Breakst_unitclass_skilldata _array_element)) 0) ; 检查使用次数
            (goto _label)))))
    (:then_1
      ;[1 1 1] 选择可使用技能中行动点最大的技能
      (for _array_element_2 (LocalVariables|Getcan_use_skill_list)
        (Math|Integer|CompareInt (Utilities|Struct|Breakst_unitclass_skilldata _array_element_2) (Utilities|Struct|Breakst_unitclass_skilldata (LocalVariables|Getunitskill))
          (:>
            _)
          (:==
            _))
        (LocalVariables|Setunitskill _array_element_2)))
    (:then_2
      (return (LocalVariables|Getunitskill)))))

(fn FindMainObjective
  (params (RowName :type Name) (skill_create :type BP%20BASE%20Pawn%20Object%20Reference) (skill_mode :type E_SKILL_model%20Enum :default "NewEnumerator0"))
  (LocalVariables|Settempplayer (Variables|/Game/BP/BP_Battle_Phase/BP_BASE_Pawn.BP_BASE_Pawn_C|GetAs%20BP%20GLOBAL%20CHARATER skill_create))
  (bind _returnvalue (Utilities|GetDataTableRow "/Game/Struct/ST_UNIT_skill/T_unit_skill.T_unit_skill" RowName)
    (:then
      (if (Utilities|Enum|Equal(Enum) (.skill_type (Utilities|Struct|Breakst_unit_select_target (Utilities|Struct|Breakst_unit_skill_Assembly _returnvalue))) skill_mode)
        (bind _returnvalue_2 (Game|ConstructObjectfromClass (.select_mind_target (Utilities|Struct|Breakst_unit_select_target (Utilities|Struct|Breakst_unit_skill_Assembly _returnvalue)))))
        (bind _target (Default|SelectTarget _returnvalue_2 (Variables|/Game/BP/BP_Battle_Phase/BP_land_spaner.BP_land_spaner_C|GetUnit%20Class (Variables|/Game/BP/BP_Battle_Phase/BP_GLOBAL_CHARACTER.BP_GLOBAL_CHARACTER_C|Getland (LocalVariables|Gettempplayer)))))
        (return _target (Utilities|IsValid _target))))))

(fn FilterUnit(ng)
  (params (Array :type Array%20of%20Actor%20Object%20References))
  (Utilities|FlowControl|Sequence
    (:then_0
      (for _array_element Array
        (bind _asbp_base_pawn (Utilities|Casting|CastToBP_BASE_Pawn _array_element))
        (bind _asbp_unit_class (Utilities|Casting|CastToBP_Unit_class _asbp_base_pawn))
        (bind _asbp_monster_class (Utilities|Casting|CastToBP_Monster_class _asbp_unit_class)
          (:then
            (Utilities|Array|Add (LocalVariables|Getunit_t) _asbp_monster_class))
          (:CastFailed
            (bind _asbp_character_class (Utilities|Casting|CastToBP_character_class _asbp_unit_class))
            (Utilities|Array|Add (LocalVariables|Getpawn_T) _asbp_character_class)))))
    (:then_1
      (return (LocalVariables|Getpawn_T) (LocalVariables|Getunit_t)))))

(fn UseUnitSkill
  (params (rowname :type Name) (skill_model :type E_SKILL_model%20Enum :default "NewEnumerator0") (create :type BP%20BASE%20Pawn%20Object%20Reference) (targetdata :type Array%20of%20St%20Select%20Unit%20Target%20Data%20Structures))
  (bind _returnvalue (Utilities|GetDataTableRow "/Game/Struct/ST_UNIT_skill/T_unit_skill.T_unit_skill" (LocalVariables|GetRowName))
    (:then
      (bind _returnvalue_2 (Game|ConstructObjectfromClass (.skill_class (Utilities|Struct|Breakst_unit_skill_Assembly _returnvalue))))
      (Default|Activation _returnvalue_2 create skill_model targetdata)
      (Default|CallTriggersAnAutomaticSkill) ; 触发自动技能
      (return (.action_type (Utilities|Struct|Breakst_unit_skill_effect (.skill_effect (Utilities|Struct|Breakst_unit_skill_Assembly _returnvalue)))) (.skill_effect_type (Utilities|Struct|Breakst_unit_skill_effect (.skill_effect (Utilities|Struct|Breakst_unit_skill_Assembly _returnvalue))))))))

(fn FindTargetsBasedonMainObjectives
  (params (create :type BP%20BASE%20Pawn%20Object%20Reference) (main_objectives :type BP%20BASE%20Pawn%20Object%20Reference) (rowname :type Name) (skill_model :type E_SKILL_model%20Enum :default "NewEnumerator0"))
  (bind _asbp_global_character (Utilities|Casting|CastToBP_GLOBAL_CHARACTER (Game|Player|GetPlayerPawn 0)))
  (LocalVariables|Settemp_playter _asbp_global_character)
  (Utilities|FlowControl|Sequence
    (:then_0
      (bind _returnvalue (Game|ConstructObjectfromClass (Variables|Default|Getskill)))
      (LocalVariables|Setskill _returnvalue)
      (bind _returnvalue_2 (Utilities|GetDataTableRow "/Game/Struct/ST_UNIT_skill/T_unit_skill.T_unit_skill" rowname)
        (:then
          (if (Utilities|Enum|Equal(Enum) (.skill_type (Utilities|Struct|Breakst_unit_select_target (Utilities|Struct|Breakst_unit_skill_Assembly _returnvalue_2))) skill_model)
            (for _array_element (.select_unit_type_index (Utilities|Struct|Breakst_unit_select_target (Utilities|Struct|Breakst_unit_skill_Assembly _returnvalue_2)))
              (LocalVariables|Settemp_select_target_type (.select_target_type (Utilities|Struct|Breakst_select_unit_target_index _array_element)))
              (LocalVariables|Settemp_unit_type (.unit_ytpe (Utilities|Struct|Breakst_select_target_index (.select_type (Utilities|Struct|Breakst_select_unit_target_index _array_element)))))
              (bind _output_get (LocalVariables|Settemp_index_target (.IndexTarget (Utilities|Struct|Breakst_select_target_index (.select_type (Utilities|Struct|Breakst_select_unit_target_index _array_element))))))
              (for _array_element_2 (.Coordinates (Utilities|Struct|Breakst_select_target_index (.select_type (Utilities|Struct|Breakst_select_unit_target_index _array_element))))
                (switch Utilities|FlowControl|Switch|SwitchonE_skill_target_base_index _output_get
                  (:NewEnumerator0
                    (if (Utilities|IsValid create)
                      (bind (_actoris_vaild _chear _pawn) (Default|CaculateDirectionYouCanWalkV2(Actor)SKILL (LocalVariables|Gettemp_playter) (Transformation|GetActorLocation create) _array_element_2))
                      (switch Utilities|FlowControl|Switch|SwitchonE_skill_target (LocalVariables|Gettemp_unit_type)
                        (:NewEnumerator1
                          (if (Utilities|IsValid _chear)
                            (Default|AddTarget (LocalVariables|Getskill) (LocalVariables|Gettargetdata) _chear (LocalVariables|Gettemp_select_target_type))))
                        (:NewEnumerator0
                          (if (Utilities|IsValid _pawn)
                            (Default|AddTarget (LocalVariables|Getskill) (LocalVariables|Gettargetdata) _pawn (LocalVariables|Gettemp_select_target_type)))))))
                  (:NewEnumerator1
                    (if (Utilities|IsValid main_objectives)
                      (bind (_actoris_vaild_2 _chear_2 _pawn_2) (Default|CaculateDirectionYouCanWalkV2(Actor)SKILL (LocalVariables|Gettemp_playter) (Transformation|GetActorLocation main_objectives) _array_element_2))
                      (switch Utilities|FlowControl|Switch|SwitchonE_skill_target (LocalVariables|Gettemp_unit_type)
                        (:NewEnumerator1
                          (if (Utilities|IsValid _chear_2)
                            (Default|AddTarget (LocalVariables|Getskill) (LocalVariables|Gettargetdata) _chear_2 (LocalVariables|Gettemp_select_target_type))))
                        (:NewEnumerator0
                          (if (Utilities|IsValid _pawn_2)
                            (Default|AddTarget (LocalVariables|Getskill) (LocalVariables|Gettargetdata) _pawn_2 (LocalVariables|Gettemp_select_target_type))))))))))))))
    (:then_1
      (return (LocalVariables|Gettargetdata)))))