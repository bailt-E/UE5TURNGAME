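; Target-selection component that filters and ranks units for picking a target on what appears to be a tile grid.
; ScreeningUnit filters units by faction, area and type, returning their pawns or "Chear" actors.
; Aggro and health selectors scan monsters but, despite their MAX names, switch to equal or lower values, with no return.
; SelectTarget is an empty stub, and the near-target function only tallies results from an eight-direction walkability check.
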(event EventBeginPlay)

(event EventTick
  (params (DeltaSeconds :type Float%20%28single-precision%29)))

(fn ScreeningUnit
  (params (unit :type Array%20of%20St%20Unit%20Class%20Structures) (area :type E_area%20Enum :default "NewEnumerator0") (unit_type :type E_unit_type%20Enum :default "NewEnumerator0") (unit_faction :type E_unitfaction%20Enum :default "NewEnumerator0") (target_type :type E_skill_target%20Enum :default "NewEnumerator0"))
  (Utilities|FlowControl|Sequence
    (:then_0
      (for _array_element unit
        (bind _asbp_base_pawn (Utilities|Casting|CastToBP_BASE_Pawn (.charter (Utilities|Struct|Breakst_unit_class _array_element))))
        (if (Math|Boolean|ANDBoolean (Utilities|Enum|Equal(Enum) (Variables|/Game/BP/BP_Battle_Phase/BP_BASE_Pawn.BP_BASE_Pawn_C|Getunit_faction _asbp_base_pawn) unit_faction) (Utilities|Enum|Equal(Enum) (.theunitarea (Utilities|Struct|Breakst_unit_class _array_element)) area) (Utilities|Enum|Equal(Enum) (.gameplay_unit_type (Utilities|Struct|Breakst_unit_class _array_element)) unit_type))
          (switch Utilities|FlowControl|Switch|SwitchonE_skill_target target_type
            (:NewEnumerator1
              (Utilities|Array|Add (LocalVariables|Getactor) (.chear (Utilities|Struct|Breakst_unit_class _array_element))))
            (:NewEnumerator0
              (Utilities|Array|Add (LocalVariables|Getactor) (.charter (Utilities|Struct|Breakst_unit_class _array_element))))))))
    (:then_1
      (return (LocalVariables|Getactor)))))

(fn SelectUnitAggroMAX
  (params (NewParam :type Array%20of%20Actor%20Object%20References))
  (for _array_element NewParam
    (bind _asbp_base_pawn (Utilities|Casting|CastToBP_BASE_Pawn _array_element))
    (bind _asbp_monster_class (Utilities|Casting|CastToBP_Monster_class _asbp_base_pawn))
    (Math|Float|CompareFloat (.Current_Unitaggro (Utilities|Struct|BreakST_UNIT_Current_resource_AA (Variables|/Game/BP/BP_AC/BP_Generic_attributes_AC/AC_Generic_attributes.AC_Generic_attributes_C|GetCurrent_resource (Variables|/Game/BP/BP_Battle_Phase/BP_BASE_Pawn.BP_BASE_Pawn_C|GetAC_Generic_attributes (LocalVariables|Getunit))))) (.Current_Unitaggro (Utilities|Struct|BreakST_UNIT_Current_resource_AA (Variables|/Game/BP/BP_AC/BP_Generic_attributes_AC/AC_Generic_attributes.AC_Generic_attributes_C|GetCurrent_resource (Variables|/Game/BP/BP_Battle_Phase/BP_BASE_Pawn.BP_BASE_Pawn_C|GetAC_Generic_attributes _asbp_monster_class))))
      (:>
        _)
      (:==
        _))
    (LocalVariables|Setunit _asbp_monster_class)))

(fn SelectUnitHealthMAX
  (params (NewParam :type Array%20of%20Actor%20Object%20References))
  (for _array_element NewParam
    (bind _asbp_base_pawn (Utilities|Casting|CastToBP_BASE_Pawn _array_element))
    (bind _asbp_monster_class (Utilities|Casting|CastToBP_Monster_class _asbp_base_pawn))
    (Math|Integer|CompareInt (.Currenthealth (Utilities|Struct|BreakST_UNIT_Current_resource_AA (Variables|/Game/BP/BP_AC/BP_Generic_attributes_AC/AC_Generic_attributes.AC_Generic_attributes_C|GetCurrent_resource (Variables|/Game/BP/BP_Battle_Phase/BP_BASE_Pawn.BP_BASE_Pawn_C|GetAC_Generic_attributes (LocalVariables|Getunit))))) (.Currenthealth (Utilities|Struct|BreakST_UNIT_Current_resource_AA (Variables|/Game/BP/BP_AC/BP_Generic_attributes_AC/AC_Generic_attributes.AC_Generic_attributes_C|GetCurrent_resource (Variables|/Game/BP/BP_Battle_Phase/BP_BASE_Pawn.BP_BASE_Pawn_C|GetAC_Generic_attributes _asbp_monster_class))))
      (:>
        _)
      (:==
        _))
    (LocalVariables|Setunit _asbp_monster_class)))

(fn SelectTarget
  (return 0))

(fn SelectUnitNearTargetNumberMax
  (params (chear :type Array%20of%20Actor%20Object%20References))
  (for _array_element chear
    (bind _result (Default|CaculateDirectionYouCanWalkV2(Chear)V2 (LocalVariables|GetNewLocalVar) (Transformation|GetActorLocation _array_element) (Utilities|Array|MakeArray "(X=1.000000,Y=-1.000000)" "(X=1.000000,Y=0.000000)" "(X=-1.000000,Y=0.000000)" "(X=0.000000,Y=1.000000)" "(X=0.000000,Y=-1.000000)" "(X=1.000000,Y=1.000000)" "(X=-1.000000,Y=-1.000000)" "(X=-1.000000,Y=1.000000)")))
    (for _array_element_2 _result
      (LocalVariables|Setnumber (+ (LocalVariables|Getnumber) 1)))))