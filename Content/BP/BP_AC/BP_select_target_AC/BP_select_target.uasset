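; BP_select_target is a target-selection helper that filters and ranks units and their grid cells (Chear).
; ScreeningUnit gathers cell or character actors by area and unit type, ignoring its faction input.
; Selectors aim for highest health, highest aggro, or most walkable eight-way neighbours.
; The aggro selector only ever clears its result, neighbour counts reset every iteration, and SelectTarget is an empty stub.
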(fn SelectUnitHealthMAX
  (params (unit :type Array%20of%20BP%20BASE%20Pawn%20Object%20References))
  (Development|PrintString 0 (Utilities|String|Append "单位数量" (Utilities|String|ToString(Integer) (Utilities|Array|Length unit))) true true "(R=1.000000,G=0.302766,B=0.000000,A=1.000000)" 1e+02)
  (Utilities|FlowControl|Sequence
    (:then_0
      (for _array_element unit
        (if (Utilities|IsValid _array_element)
          (if (Utilities|IsValid (LocalVariables|Gettarget))
            (Math|Integer|CompareInt (Utilities|Struct|BreakST_UNIT_Current_resource_AA (Variables|/Game/BP/BP_AC/BP_Generic_attributes_AC/AC_Generic_attributes.AC_Generic_attributes_C|GetCurrent_resource (Variables|/Game/BP/BP_Battle_Phase/BP_BASE_Pawn.BP_BASE_Pawn_C|GetAC_Generic_attributes _array_element))) (Utilities|Struct|BreakST_UNIT_Current_resource_AA (Variables|/Game/BP/BP_AC/BP_Generic_attributes_AC/AC_Generic_attributes.AC_Generic_attributes_C|GetCurrent_resource (Variables|/Game/BP/BP_Battle_Phase/BP_BASE_Pawn.BP_BASE_Pawn_C|GetAC_Generic_attributes (LocalVariables|Gettarget))))
              (:>
                _)
              (:==
                _))
            (LocalVariables|Settarget _array_element)
            (else
              (LocalVariables|Settarget _array_element))))))
    (:then_1
      (return (LocalVariables|Gettarget)))))

(fn SelectUnitAggroMAX
  (params (NewParam :type Array%20of%20Actor%20Object%20References))
  (Utilities|FlowControl|Sequence
    (:then_0
      (for _array_element NewParam
        (bind _asbp_base_pawn (Utilities|Casting|CastToBP_BASE_Pawn _array_element))
        (Math|Float|CompareFloat (.Current_Unitaggro (Utilities|Struct|BreakST_UNIT_Current_resource_AA (Variables|/Game/BP/BP_AC/BP_Generic_attributes_AC/AC_Generic_attributes.AC_Generic_attributes_C|GetCurrent_resource (Variables|/Game/BP/BP_Battle_Phase/BP_BASE_Pawn.BP_BASE_Pawn_C|GetAC_Generic_attributes (LocalVariables|Getunit))))) (.Current_Unitaggro (Utilities|Struct|BreakST_UNIT_Current_resource_AA (Variables|/Game/BP/BP_AC/BP_Generic_attributes_AC/AC_Generic_attributes.AC_Generic_attributes_C|GetCurrent_resource (Variables|/Game/BP/BP_Battle_Phase/BP_BASE_Pawn.BP_BASE_Pawn_C|GetAC_Generic_attributes _asbp_base_pawn))))
          (:>
            _)
          (:==
            _))
        (LocalVariables|Setunit 0)))
    (:then_1
      (return (LocalVariables|Getunit)))))

(fn ScreeningUnit
  (params (unit :type Array%20of%20St%20Unit%20Class%20Structures) (area :type E_area%20Enum :default "NewEnumerator0") (unit_type :type E_unit_type%20Enum :default "NewEnumerator0") (unit_faction :type E_unitfaction%20Enum :default "NewEnumerator0") (target_type :type E_skill_target%20Enum :default "NewEnumerator0"))
  (Utilities|FlowControl|Sequence
    (:then_0
      (for _array_element unit
        (if (and (Utilities|Enum|Equal(Enum) (.theunitarea (Utilities|Struct|Breakst_unit_class _array_element)) area) (Utilities|Enum|Equal(Enum) (.gameplay_unit_type (Utilities|Struct|Breakst_unit_class _array_element)) unit_type))
          (switch Utilities|FlowControl|Switch|SwitchonE_skill_target target_type
            (:NewEnumerator1
              (if (Utilities|IsValid (.chear (Utilities|Struct|Breakst_unit_class _array_element)))
                (bind _asbp_base_pawn (Utilities|Casting|CastToBP_BASE_Pawn (.chear (Utilities|Struct|Breakst_unit_class _array_element))))
                (Utilities|Array|Add (LocalVariables|Getactor) _asbp_base_pawn)))
            (:NewEnumerator0
              (if (Utilities|IsValid (.charter (Utilities|Struct|Breakst_unit_class _array_element)))
                (bind _asbp_base_pawn_2 (Utilities|Casting|CastToBP_BASE_Pawn (.charter (Utilities|Struct|Breakst_unit_class _array_element))))
                (Utilities|Array|Add (LocalVariables|Getactor) _asbp_base_pawn_2)))))))
    (:then_1
      (return (LocalVariables|Getactor)))))

(fn SelectUnitNearTargetNumberMax
  (params (chear :type Array%20of%20Actor%20Object%20References))
  (Utilities|FlowControl|Sequence
    (:then_0
      (for _array_element chear
        (bind _result (Default|CaculateDirectionYouCanWalkV2(Chear)V2 (LocalVariables|GetNewLocalVar) (Transformation|GetActorLocation _array_element) (Utilities|Array|MakeArray "(X=1.000000,Y=-1.000000)" "(X=1.000000,Y=0.000000)" "(X=-1.000000,Y=0.000000)" "(X=0.000000,Y=1.000000)" "(X=0.000000,Y=-1.000000)" "(X=1.000000,Y=1.000000)" "(X=-1.000000,Y=-1.000000)" "(X=-1.000000,Y=1.000000)")))
        (for _array_element_2 _result
          (bind _output_get (LocalVariables|Setnumber (+ (LocalVariables|Getnumber) 1)))
          (Utilities|Array|Add (LocalVariables|Getactor_number) (Utilities|Struct|Makee_select_chear_number _array_element _output_get))
          (LocalVariables|Setnumber 0))))
    (:then_1
      (for _array_element_3 (LocalVariables|Getactor_number)
        (Math|Integer|CompareInt (Utilities|Struct|Breake_select_chear_number _array_element_3) (Utilities|Struct|Breake_select_chear_number (LocalVariables|Getactor_number_max))
          (:>
            _)
          (:==
            _))
        (LocalVariables|Setactor_number_max _array_element_3)))
    (:then_2
      (return (LocalVariables|Getactor_number_max)))))

(fn SelectTarget
  (params (unit_data :type Array%20of%20St%20Unit%20Class%20Structures))
  (return 0))