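; Target-selection Blueprint that picks the unit with the highest health from the supplied unit data.
; SelectTarget filters the units by area and faction through ScreeningUnit, then passes the result to SelectUnitHealthMAX and returns its pick.
; An unconnected branch holds an inline alternative that loops over the data, filters by owning side and casts to BP_BASE_Pawn before making the same selection.
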(fn SelectTarget
  (params (unit_data :type Array%20of%20St%20Unit%20Class%20Structures))
  (bind _newparam (CallFunction|ScreeningUnit unit_data "NewEnumerator1" "NewEnumerator0" "NewEnumerator1" "NewEnumerator0"))
  (bind _base_unit (CallFunction|SelectUnitHealthMAX _newparam))
  (return _base_unit))