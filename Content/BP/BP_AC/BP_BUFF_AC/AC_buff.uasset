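; Buff manager component that holds turn-based buffs and tags, advanced by the player character's Land turn-switch event.
; Each tick moves queued buffs into the active list, counts them down and removes expired ones.
; Adding builds buff objects from a data table or custom tag parameters, with stack or duration-reset handling.
; Helpers handle dispel, immunity/absorb and priority-searched effects (under attack, treatment, death) that consume buff resources.
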(event Custom|tick
  (general|BuffTick 1))

(event Custom|areabuff%20to%20the%20buff
  (for _array_element (Variables|area|GetQuarantine%20AreaA)
    (Utilities|Array|Add (Variables|A2|Getwait_add_buff) _array_element)))

(event EventBeginPlay
  (bind _asbp_global_character (Utilities|Casting|CastToBP_GLOBAL_CHARACTER (Game|Player|GetPlayerPawn 0)))
  (bind _output_get (Variables|Default|Setland (Variables|/Game/BP/BP_Battle_Phase/BP_GLOBAL_CHARACTER.BP_GLOBAL_CHARACTER_C|Getland _asbp_global_character)))
  (if (Utilities|IsValid _output_get)
    (EventDispatchers|AssignEDTurnSwitch _output_get (delegate Custom|tick))))

(fn ActivateBuffect
  (params (NewParam :type e_buff_effect%20Enum :default "NewEnumerator0"))
  (for _array_element (Variables|A2|Getcurrent_buff)
    (Default|BuffEffect _array_element NewParam 0 0 0 0.0)))

(fn BuffTick
  (params (tick :type Integer))
  (Utilities|FlowControl|Sequence
    (:then_0
      (for _array_element (Variables|A2|Getwait_add_buff)
        (Utilities|Array|Add (Variables|A2|Getcurrent_buff) _array_element)
        (Default|BuffEffect _array_element "NewEnumerator0" 0 (Variables|/Game/BP/BP_AC/BP_BUFF_AC/BP_buff_class.BP_buff_class_C|GetTarget _array_element) (Variables|/Game/BP/BP_AC/BP_BUFF_AC/BP_buff_class.BP_buff_class_C|GetCreate _array_element) 0.0)
        (Utilities|Array|RemoveItem (Variables|A2|Getwait_add_buff) _array_element)))
    (:then_1
      ;[1 1 1] 这个会自动运行
      (for _array_element_2 (Variables|A2|Getcurrent_buff)
        (bind _is_the_end (Default|TurnTick _array_element_2 tick)) ; point
        (if _is_the_end
          (Utilities|Array|Add (Variables|A2|Getwait_remove_buff) _array_element_2)
          (Utilities|Array|RemoveItem (Variables|A2|Getcurrent_buff) _array_element_2))))
    (:then_2
      (for _array_element_3 (Variables|A2|Getwait_remove_buff)
        (Default|BuffEffect _array_element_3 "NewEnumerator1" 0 (Variables|/Game/BP/BP_AC/BP_BUFF_AC/BP_buff_class.BP_buff_class_C|GetTarget _array_element_3) (Variables|/Game/BP/BP_AC/BP_BUFF_AC/BP_buff_class.BP_buff_class_C|GetCreate _array_element_3) 0.0)
        (Utilities|Array|RemoveItem (Variables|A2|Getwait_remove_buff) _array_element_3)))))

(fn CountArrayElementTagNunber
  ;[1 1 1] 统计buff中元素标记数量
  (Variables|Default|Setelement_tag_number 0)
  (for _array_element (Variables|A2|Getcurrent_buff)
    (if (Utilities|Enum|Equal(Enum) (Variables|/Game/BP/BP_AC/BP_BUFF_AC/BP_buff_class.BP_buff_class_C|Getbuff_type _array_element) "NewEnumerator1")
      (Variables|Default|Setelement_tag_number (+ (Variables|Default|Getelement_tag_number) 1)))))

(fn Addbuff0
  (params (buff_rowname :type Name) (target :type Actor%20Object%20Reference) (create :type Actor%20Object%20Reference))
  (Utilities|FlowControl|Sequence
    (:then_0
      (bind _returnvalue (Utilities|GetDataTableRow "/Game/Struct/st_buff/new_buff/T_buff_table.T_buff_table" buff_rowname)
        (:then
          (bind _returnvalue_2 (Game|ConstructObjectfromClass (.buff_class (Utilities|Struct|BreakST_buff_total_structure _returnvalue))))
          (Default|BUFFInitialize _returnvalue_2 create target (.buff_bese_info (Utilities|Struct|BreakST_buff_total_structure _returnvalue)) (Utilities|Struct|Makest_buff_resources (.Initial_stack (Utilities|Struct|Breakbuff_base_attribute (.buff_attribute (Utilities|Struct|BreakST_buff_total_structure _returnvalue)))) (.Initial_Priority (Utilities|Struct|Breakbuff_base_attribute (.buff_attribute (Utilities|Struct|BreakST_buff_total_structure _returnvalue)))) (.Numberofuses (Utilities|Struct|Breakbuff_base_attribute (.buff_attribute (Utilities|Struct|BreakST_buff_total_structure _returnvalue)))) (.initial_ContinuousRound (Utilities|Struct|Breakbuff_base_attribute (.buff_attribute (Utilities|Struct|BreakST_buff_total_structure _returnvalue)))) (.Cycleround (Utilities|Struct|Breakbuff_base_attribute (.buff_attribute (Utilities|Struct|BreakST_buff_total_structure _returnvalue))))) (.buff_type (Utilities|Struct|BreakST_buff_total_structure _returnvalue)) (.buff_Nature_type (Utilities|Struct|BreakST_buff_total_structure _returnvalue)) (.buff_updata (Utilities|Struct|BreakST_buff_total_structure _returnvalue)) (.buff_effect_type (Utilities|Struct|BreakST_buff_total_structure _returnvalue)) (.element (Utilities|Struct|Breakst_buff_element_info (.element_tag_info (Utilities|Struct|BreakST_buff_total_structure _returnvalue)))) (.element_tag_level (Utilities|Struct|Breakst_buff_element_info (.element_tag_info (Utilities|Struct|BreakST_buff_total_structure _returnvalue)))) (.buff_boolset (Utilities|Struct|BreakST_buff_total_structure _returnvalue)) (.buff_type_effect (Utilities|Struct|BreakST_buff_total_structure _returnvalue)) (.buff_immunity_info (Utilities|Struct|BreakST_buff_total_structure _returnvalue))) ; buff
          (if (> (Utilities|Array|Length (Variables|A2|Getcurrent_buff)) 0) ; 检查是否小于0
            (for _array_element (Variables|A2|Getcurrent_buff)
              (if (== _returnvalue_2 _array_element)
                (bind (_id _buff _is_find) (A2|FindBUFFbyID (.buff_index (Utilities|Struct|Breakst_buff_base_info (Variables|/Game/BP/BP_AC/BP_BUFF_AC/BP_buff_class.BP_buff_class_C|Getbuffinfo _returnvalue_2)))))
                (if _is_find
                  (LocalVariables|Setthis_buff _buff)
                  (switch Utilities|FlowControl|Switch|SwitchonE_BuffTimeUpdataEnum (Utilities|Struct|Breakst_buff_boolset (Variables|/Game/BP/BP_AC/BP_BUFF_AC/BP_buff_class.BP_buff_class_C|Getbuff_boolset (LocalVariables|Getthis_buff)))
                    (:NewEnumerator0
                      (if (> (+ (.add_stack (Utilities|Struct|Breakbuff_base_attribute (Variables|/Game/BP/BP_AC/BP_BUFF_AC/BP_buff_class.BP_buff_class_C|Getbuff_base_attribute (LocalVariables|Getthis_buff)))) (Utilities|Struct|Breakst_buff_resources (Variables|/Game/BP/BP_AC/BP_BUFF_AC/BP_buff_class.BP_buff_class_C|Getbuff_resources (LocalVariables|Getthis_buff)))) (.max_stack (Utilities|Struct|Breakbuff_base_attribute (Variables|/Game/BP/BP_AC/BP_BUFF_AC/BP_buff_class.BP_buff_class_C|Getbuff_base_attribute (LocalVariables|Getthis_buff))))) ; 最大层级是否大于合成后的层数
                        (Variables|/Game/BP/BP_AC/BP_BUFF_AC/BP_buff_class.BP_buff_class_C|Setbuff_resources (LocalVariables|Getthis_buff) (Utilities|Struct|Makest_buff_resources (.max_stack (Utilities|Struct|Breakbuff_base_attribute (Variables|/Game/BP/BP_AC/BP_BUFF_AC/BP_buff_class.BP_buff_class_C|Getbuff_base_attribute (LocalVariables|Getthis_buff)))) (.priority (Utilities|Struct|Breakst_buff_resources (Variables|/Game/BP/BP_AC/BP_BUFF_AC/BP_buff_class.BP_buff_class_C|Getbuff_resources (LocalVariables|Getthis_buff)))) (.NumberOfActions (Utilities|Struct|Breakst_buff_resources (Variables|/Game/BP/BP_AC/BP_BUFF_AC/BP_buff_class.BP_buff_class_C|Getbuff_resources (LocalVariables|Getthis_buff)))) (.duration_time (Utilities|Struct|Breakst_buff_resources (Variables|/Game/BP/BP_AC/BP_BUFF_AC/BP_buff_class.BP_buff_class_C|Getbuff_resources (LocalVariables|Getthis_buff)))) (.Cycletime (Utilities|Struct|Breakst_buff_resources (Variables|/Game/BP/BP_AC/BP_BUFF_AC/BP_buff_class.BP_buff_class_C|Getbuff_resources (LocalVariables|Getthis_buff))))))
                        (Utilities|Array|SetArrayElem (Variables|A2|Getcurrent_buff) 0 (LocalVariables|Getthis_buff))
                        (else
                          (Variables|/Game/BP/BP_AC/BP_BUFF_AC/BP_buff_class.BP_buff_class_C|Setbuff_resources (LocalVariables|Getthis_buff) (Utilities|Struct|Makest_buff_resources (+ (.add_stack (Utilities|Struct|Breakbuff_base_attribute (Variables|/Game/BP/BP_AC/BP_BUFF_AC/BP_buff_class.BP_buff_class_C|Getbuff_base_attribute (LocalVariables|Getthis_buff)))) (Utilities|Struct|Breakst_buff_resources (Variables|/Game/BP/BP_AC/BP_BUFF_AC/BP_buff_class.BP_buff_class_C|Getbuff_resources (LocalVariables|Getthis_buff)))) (.priority (Utilities|Struct|Breakst_buff_resources (Variables|/Game/BP/BP_AC/BP_BUFF_AC/BP_buff_class.BP_buff_class_C|Getbuff_resources (LocalVariables|Getthis_buff)))) (.NumberOfActions (Utilities|Struct|Breakst_buff_resources (Variables|/Game/BP/BP_AC/BP_BUFF_AC/BP_buff_class.BP_buff_class_C|Getbuff_resources (LocalVariables|Getthis_buff)))) (.duration_time (Utilities|Struct|Breakst_buff_resources (Variables|/Game/BP/BP_AC/BP_BUFF_AC/BP_buff_class.BP_buff_class_C|Getbuff_resources (LocalVariables|Getthis_buff)))) (.Cycletime (Utilities|Struct|Breakst_buff_resources (Variables|/Game/BP/BP_AC/BP_BUFF_AC/BP_buff_class.BP_buff_class_C|Getbuff_resources (LocalVariables|Getthis_buff))))))
                          (Utilities|Array|SetArrayElem (Variables|A2|Getcurrent_buff) 0 (LocalVariables|Getthis_buff)))))
                    (:NewEnumerator1
                      (Variables|/Game/BP/BP_AC/BP_BUFF_AC/BP_buff_class.BP_buff_class_C|Setbuff_resources (LocalVariables|Getthis_buff) (Utilities|Struct|Makest_buff_resources (.stack (Utilities|Struct|Breakst_buff_resources (Variables|/Game/BP/BP_AC/BP_BUFF_AC/BP_buff_class.BP_buff_class_C|Getbuff_resources (LocalVariables|Getthis_buff)))) (.priority (Utilities|Struct|Breakst_buff_resources (Variables|/Game/BP/BP_AC/BP_BUFF_AC/BP_buff_class.BP_buff_class_C|Getbuff_resources (LocalVariables|Getthis_buff)))) (.NumberOfActions (Utilities|Struct|Breakst_buff_resources (Variables|/Game/BP/BP_AC/BP_BUFF_AC/BP_buff_class.BP_buff_class_C|Getbuff_resources (LocalVariables|Getthis_buff)))) (.initial_ContinuousRound (Utilities|Struct|Breakbuff_base_attribute (Variables|/Game/BP/BP_AC/BP_BUFF_AC/BP_buff_class.BP_buff_class_C|Getbuff_base_attribute (LocalVariables|Getthis_buff)))) (.Cycletime (Utilities|Struct|Breakst_buff_resources (Variables|/Game/BP/BP_AC/BP_BUFF_AC/BP_buff_class.BP_buff_class_C|Getbuff_resources (LocalVariables|Getthis_buff))))))
                      (Utilities|Array|SetArrayElem (Variables|A2|Getcurrent_buff) 0 (LocalVariables|Getthis_buff)))
                    (:NewEnumerator2
                      (Utilities|Array|Add (Variables|A2|Getwait_add_buff) _returnvalue_2))))
                (else
                  (Utilities|Array|Add (Variables|A2|Getwait_add_buff) _returnvalue_2))))
            (else
              (Utilities|Array|Add (Variables|A2|Getwait_add_buff) _returnvalue_2))))))
    (:then_1
      (if (Utilities|IsValid (LocalVariables|Getthis_buff))
        (return (LocalVariables|Getthis_buff))))))

(fn Addbuff
  (params (buff_rowname :type Name) (target :type Actor%20Object%20Reference) (create :type Actor%20Object%20Reference) (buff_in_table :type Boolean) (Custom_buff_index :type Integer) (Custom_buff_type :type E_BUFF_type%20Enum :default "NewEnumerator0") (Custom_buff_Updata :type E_BuffTimeUpdataEnum%20Enum :default "NewEnumerator0") (Custom_element_type :type E_element_type%20Enum :default "NewEnumerator0") (Custom_element_type_level :type E_element_advance%20Enum :default "NewEnumerator0"))
  (if buff_in_table
    (bind _returnvalue (Utilities|GetDataTableRow "/Game/Struct/st_buff/new_buff/T_buff_table.T_buff_table" buff_rowname)
      (:then
        (bind _returnvalue_2 (Game|ConstructObjectfromClass (.buff_class (Utilities|Struct|BreakST_buff_total_structure _returnvalue))))
        (for _array_element (Variables|A2|Getcurrent_buff) ; 检查buff数组中是否存在buff
          (if (== _returnvalue_2 _array_element)
            (switch Utilities|FlowControl|Switch|SwitchonE_BuffTimeUpdataEnum (Utilities|Struct|Breakst_buff_boolset (Variables|/Game/BP/BP_AC/BP_BUFF_AC/BP_buff_class.BP_buff_class_C|Getbuff_boolset _array_element))
              (:NewEnumerator0
                (bind (_id _buff) (A2|FindBUFFbyID (.buff_index (Utilities|Struct|Breakst_buff_base_info (Variables|/Game/BP/BP_AC/BP_BUFF_AC/BP_buff_class.BP_buff_class_C|Getbuffinfo _array_element)))))
                (Variables|/Game/BP/BP_AC/BP_BUFF_AC/BP_buff_class.BP_buff_class_C|Setbuff_resources _buff (Utilities|Struct|Makest_buff_resources (+ (.add_stack (Utilities|Struct|Breakbuff_base_attribute (.buff_attribute (Utilities|Struct|BreakST_buff_total_structure _returnvalue)))) (.stack (Utilities|Struct|Breakst_buff_resources (Variables|/Game/BP/BP_AC/BP_BUFF_AC/BP_buff_class.BP_buff_class_C|Getbuff_resources _buff)))) (.priority (Utilities|Struct|Breakst_buff_resources (Variables|/Game/BP/BP_AC/BP_BUFF_AC/BP_buff_class.BP_buff_class_C|Getbuff_resources _buff))) (.NumberOfActions (Utilities|Struct|Breakst_buff_resources (Variables|/Game/BP/BP_AC/BP_BUFF_AC/BP_buff_class.BP_buff_class_C|Getbuff_resources _buff))) (.duration_time (Utilities|Struct|Breakst_buff_resources (Variables|/Game/BP/BP_AC/BP_BUFF_AC/BP_buff_class.BP_buff_class_C|Getbuff_resources _buff))) (.Cycletime (Utilities|Struct|Breakst_buff_resources (Variables|/Game/BP/BP_AC/BP_BUFF_AC/BP_buff_class.BP_buff_class_C|Getbuff_resources _buff)))))
                (Utilities|Array|SetArrayElem (Variables|A2|Getcurrent_buff) _id _buff))
              (:NewEnumerator1
                (bind (_id_2 _buff_2) (A2|FindBUFFbyID (.buff_index (Utilities|Struct|Breakst_buff_base_info (Variables|/Game/BP/BP_AC/BP_BUFF_AC/BP_buff_class.BP_buff_class_C|Getbuffinfo _array_element)))))
                (Variables|/Game/BP/BP_AC/BP_BUFF_AC/BP_buff_class.BP_buff_class_C|Setbuff_resources _buff_2 (Utilities|Struct|Makest_buff_resources (.stack (Utilities|Struct|Breakst_buff_resources (Variables|/Game/BP/BP_AC/BP_BUFF_AC/BP_buff_class.BP_buff_class_C|Getbuff_resources _buff_2))) (.priority (Utilities|Struct|Breakst_buff_resources (Variables|/Game/BP/BP_AC/BP_BUFF_AC/BP_buff_class.BP_buff_class_C|Getbuff_resources _buff_2))) (.NumberOfActions (Utilities|Struct|Breakst_buff_resources (Variables|/Game/BP/BP_AC/BP_BUFF_AC/BP_buff_class.BP_buff_class_C|Getbuff_resources _buff_2))) (.initial_ContinuousRound (Utilities|Struct|Breakbuff_base_attribute (.buff_attribute (Utilities|Struct|BreakST_buff_total_structure _returnvalue)))) (.Cycletime (Utilities|Struct|Breakst_buff_resources (Variables|/Game/BP/BP_AC/BP_BUFF_AC/BP_buff_class.BP_buff_class_C|Getbuff_resources _buff_2)))))
                (Utilities|Array|SetArrayElem (Variables|A2|Getcurrent_buff) _id_2 _buff_2))
              (:NewEnumerator2
                (Default|BUFFInitialize _returnvalue_2 create target (.buff_bese_info (Utilities|Struct|BreakST_buff_total_structure _returnvalue)) (Utilities|Struct|Makest_buff_resources (.Initial_stack (Utilities|Struct|Breakbuff_base_attribute (.buff_attribute (Utilities|Struct|BreakST_buff_total_structure _returnvalue)))) (.Initial_Priority (Utilities|Struct|Breakbuff_base_attribute (.buff_attribute (Utilities|Struct|BreakST_buff_total_structure _returnvalue)))) (.Numberofuses (Utilities|Struct|Breakbuff_base_attribute (.buff_attribute (Utilities|Struct|BreakST_buff_total_structure _returnvalue)))) (.initial_ContinuousRound (Utilities|Struct|Breakbuff_base_attribute (.buff_attribute (Utilities|Struct|BreakST_buff_total_structure _returnvalue)))) (.Cycleround (Utilities|Struct|Breakbuff_base_attribute (.buff_attribute (Utilities|Struct|BreakST_buff_total_structure _returnvalue))))) (.buff_type (Utilities|Struct|BreakST_buff_total_structure _returnvalue)) (.buff_Nature_type (Utilities|Struct|BreakST_buff_total_structure _returnvalue)) "NewEnumerator2" (.buff_effect_type (Utilities|Struct|BreakST_buff_total_structure _returnvalue)) "NewEnumerator0" "NewEnumerator0" (.buff_boolset (Utilities|Struct|BreakST_buff_total_structure _returnvalue)) (.buff_type_effect (Utilities|Struct|BreakST_buff_total_structure _returnvalue)) (.buff_immunity_info (Utilities|Struct|BreakST_buff_total_structure _returnvalue)) :!label _label) ; buff
                (Utilities|Array|Add (Variables|A2|Getwait_add_buff) _returnvalue_2)))
            (else
              (goto _label))))))
    (else
      (bind _returnvalue_3 (Game|ConstructObjectfromClass "/Game/BP/BP_AC/BP_BUFF_AC/BP_buff_class.BP_buff_class_C"))
      (switch Utilities|FlowControl|Switch|SwitchonE_BUFF_type Custom_buff_type
        (:NewEnumerator1
          ;[1 1 1] 检查元素标记数量数量上限和当前元素标记
          (bind _asbp_base_pawn (Utilities|Casting|CastToBP_BASE_Pawn target))
          (if (> (.element_tag_number_MAX (Utilities|Struct|BreakST_Fixed_attributes_A (.Fixed_attributes (Utilities|Struct|BreakST_Attribute_collection_AA (Variables|/Game/BP/BP_AC/BP_Generic_attributes_AC/AC_Generic_attributes.AC_Generic_attributes_C|GetUNIT_Current%20properties (Variables|/Game/BP/BP_Battle_Phase/BP_BASE_Pawn.BP_BASE_Pawn_C|GetAC_Generic_attributes _asbp_base_pawn)))))) (Variables|Default|Getelement_tag_number))
            (bind _buff_3 (A2|FindBUFFbyID))
            (A2|RemoveBuffinArray (Variables|A2|Getcurrent_buff) _buff_3)
            (Default|BUFFInitialize :self _returnvalue_3 :buff_nature_typeE "NewEnumerator2")
            (Utilities|Array|Add (Variables|A2|Getwait_add_buff) _returnvalue_3)
            (else
              (Default|BUFFInitialize :self _returnvalue_3 :createC create :targetC target :buff_nature_typeE "NewEnumerator2") ; 元素标记
              (Utilities|Array|Add (Variables|A2|Getwait_add_buff) _returnvalue_3))))
        (:NewEnumerator2
          (for _array_element_2 (Variables|A2|Getcurrent_buff)
            (if (Utilities|Enum|Equal(Enum) (Variables|/Game/BP/BP_AC/BP_BUFF_AC/BP_buff_class.BP_buff_class_C|Getbuff_type _array_element_2) "NewEnumerator2") ; 检查是否存在个人标记
              (for _array_element_3 (Variables|A2|Getcurrent_buff)
                (if (and (Utilities|Enum|Equal(Enum) Custom_buff_type (Variables|/Game/BP/BP_AC/BP_BUFF_AC/BP_buff_class.BP_buff_class_C|Getbuff_type _array_element_3)) (== (.buff_index (Utilities|Struct|Breakst_buff_base_info (Variables|/Game/BP/BP_AC/BP_BUFF_AC/BP_buff_class.BP_buff_class_C|Getbuffinfo _array_element_3))) Custom_buff_index)) ; buff_index和标记类型是否一致
                  (switch Utilities|FlowControl|Switch|SwitchonE_BuffTimeUpdataEnum (Variables|/Game/BP/BP_AC/BP_BUFF_AC/BP_buff_class.BP_buff_class_C|Getbuff_Updata _array_element_3)
                    (:NewEnumerator0
                      (Variables|/Game/BP/BP_AC/BP_BUFF_AC/BP_buff_class.BP_buff_class_C|Setbuff_resources _array_element_3 (Utilities|Struct|Makest_buff_resources (+ (.stack (Utilities|Struct|Breakst_buff_resources (Variables|/Game/BP/BP_AC/BP_BUFF_AC/BP_buff_class.BP_buff_class_C|Getbuff_resources _array_element_3))) 1) (.priority (Utilities|Struct|Breakst_buff_resources (Variables|/Game/BP/BP_AC/BP_BUFF_AC/BP_buff_class.BP_buff_class_C|Getbuff_resources _array_element_3))) (.NumberOfActions (Utilities|Struct|Breakst_buff_resources (Variables|/Game/BP/BP_AC/BP_BUFF_AC/BP_buff_class.BP_buff_class_C|Getbuff_resources _array_element_3))) (.duration_time (Utilities|Struct|Breakst_buff_resources (Variables|/Game/BP/BP_AC/BP_BUFF_AC/BP_buff_class.BP_buff_class_C|Getbuff_resources _array_element_3))) (.Cycletime (Utilities|Struct|Breakst_buff_resources (Variables|/Game/BP/BP_AC/BP_BUFF_AC/BP_buff_class.BP_buff_class_C|Getbuff_resources _array_element_3)))))
                      (Utilities|Array|SetArrayElem (Variables|A2|Getcurrent_buff) 0 _array_element_3))
                    (:NewEnumerator1
                      (Variables|/Game/BP/BP_AC/BP_BUFF_AC/BP_buff_class.BP_buff_class_C|Setbuff_resources _array_element_3 (Utilities|Struct|Makest_buff_resources (.stack (Utilities|Struct|Breakst_buff_resources (Variables|/Game/BP/BP_AC/BP_BUFF_AC/BP_buff_class.BP_buff_class_C|Getbuff_resources _array_element_3))) (.priority (Utilities|Struct|Breakst_buff_resources (Variables|/Game/BP/BP_AC/BP_BUFF_AC/BP_buff_class.BP_buff_class_C|Getbuff_resources _array_element_3))) (.NumberOfActions (Utilities|Struct|Breakst_buff_resources (Variables|/Game/BP/BP_AC/BP_BUFF_AC/BP_buff_class.BP_buff_class_C|Getbuff_resources _array_element_3))) (.duration_time (Utilities|Struct|Breakst_buff_resources (Variables|/Game/BP/BP_AC/BP_BUFF_AC/BP_buff_class.BP_buff_class_C|Getbuff_resources _array_element_3))) (.Cycletime (Utilities|Struct|Breakst_buff_resources (Variables|/Game/BP/BP_AC/BP_BUFF_AC/BP_buff_class.BP_buff_class_C|Getbuff_resources _array_element_3)))))
                      (Utilities|Array|SetArrayElem (Variables|A2|Getcurrent_buff) 0 _array_element_3)))))
              (else
                (Default|BUFFInitialize :self _returnvalue_3 :createC create :targetC target :buff_typeI Custom_buff_type :buff_nature_typeE "NewEnumerator1" :buff_UpdataC Custom_buff_Updata :element_typeI Custom_element_type :element_type_level_I Custom_element_type_level)
                (Utilities|Array|Add (Variables|A2|Getwait_add_buff) _returnvalue_3)))))))))

(fn RemoveBuffinArray
  (params (current_buff%20array :type Array%20of%20BP%20Buff%20Class%20Object%20References) (buff :type BP%20Buff%20Class%20Object%20Reference))
  (for _array_element current_buff%20array
    (if (== _array_element buff)
      (Utilities|Array|RemoveItem current_buff%20array _array_element))))

(fn FindBUFFbyID
  (params (buffID :type Integer))
  (bind _current_buff (Variables|A2|Getcurrent_buff))
  (for _array_element _current_buff
    (if (== (.buff_index (Utilities|Struct|Breakst_buff_base_info (Variables|/Game/BP/BP_AC/BP_BUFF_AC/BP_buff_class.BP_buff_class_C|Getbuffinfo _array_element))) buffID)
      (return (Utilities|Array|FindItem _current_buff _array_element) _array_element (== (.buff_index (Utilities|Struct|Breakst_buff_base_info (Variables|/Game/BP/BP_AC/BP_BUFF_AC/BP_buff_class.BP_buff_class_C|Getbuffinfo _array_element))) buffID)))))

(fn RemoveBuff
  (params (buff :type Object%20Object%20Reference))
  (bind _current_buff (Variables|A2|Getcurrent_buff))
  (for _array_element _current_buff
    (if (== _array_element buff)
      (Utilities|Array|RemoveItem _current_buff _array_element))))

(fn FindBUFFbySelect
  (params (buffID :type Integer))
  (bind _current_buff (Variables|A2|Getcurrent_buff))
  (for _array_element _current_buff
    (if (== (.buff_index (Utilities|Struct|Breakst_buff_base_info (Variables|/Game/BP/BP_AC/BP_BUFF_AC/BP_buff_class.BP_buff_class_C|Getbuffinfo _array_element))) buffID)
      (return (Utilities|Array|FindItem _current_buff _array_element) _array_element (== (.buff_index (Utilities|Struct|Breakst_buff_base_info (Variables|/Game/BP/BP_AC/BP_BUFF_AC/BP_buff_class.BP_buff_class_C|Getbuffinfo _array_element))) buffID)))))

(fn DispelBuff
  (params (ItemToFind :type BP%20Buff%20Class%20Object%20Reference%20%28by%20ref%29))
  (for _array_element (Variables|A2|Getcurrent_buff)
    (if (== _array_element ItemToFind)
      (if (Utilities|Struct|Breakst_buff_boolset (Variables|/Game/BP/BP_AC/BP_BUFF_AC/BP_buff_class.BP_buff_class_C|Getbuff_boolset _array_element))
        (A2|RemoveBuff _array_element)
        (else
          (Development|PrintString "buff"))))))

(fn ConsumeResources
  (params (resources :type St%20Buff%20Effect%20Structure) (buff :type BP%20Buff%20Class%20Object%20Reference))
  (bind (_stack _priority _numberofactions) (Utilities|Struct|Breakst_buff_effect resources))
  (if (Utilities|Struct|Breakst_buff_effect resources)
    (Utilities|Array|RemoveItem (Variables|A2|Getcurrent_buff) buff)
    (else
      (Variables|/Game/BP/BP_AC/BP_BUFF_AC/BP_buff_class.BP_buff_class_C|Setbuff_resources buff (Utilities|Struct|Makest_buff_resources (- (.stack (Utilities|Struct|Breakst_buff_resources (Variables|/Game/BP/BP_AC/BP_BUFF_AC/BP_buff_class.BP_buff_class_C|Getbuff_resources buff))) _stack) (- (.priority (Utilities|Struct|Breakst_buff_resources (Variables|/Game/BP/BP_AC/BP_BUFF_AC/BP_buff_class.BP_buff_class_C|Getbuff_resources buff))) _priority) (- (.NumberOfActions (Utilities|Struct|Breakst_buff_resources (Variables|/Game/BP/BP_AC/BP_BUFF_AC/BP_buff_class.BP_buff_class_C|Getbuff_resources buff))) _numberofactions))))))

(fn FindBuffsThatHaveActiveEffects
  (params (BUFF_EFFECT_TYPE :type e_buff_effect%20Enum :default "NewEnumerator0") (buff_prioity :type Integer))
  (Utilities|FlowControl|Sequence
    (:then_0
      (for _array_element (Variables|A2|Getcurrent_buff)
        (for _array_element_2 (Variables|/Game/BP/BP_AC/BP_BUFF_AC/BP_buff_class.BP_buff_class_C|Getbuff_effect_info _array_element)
          (if (and (Utilities|Enum|Equal(Enum) (.buff_type (Utilities|Struct|Breakst_buff_type_effect _array_element_2)) BUFF_EFFECT_TYPE) (== (.buff_priority (Utilities|Struct|Breakst_buff_type_effect _array_element_2)) buff_prioity))
            (if (Math|Boolean|ANDBoolean (>= (.stack (Utilities|Struct|Breakst_buff_resources (Variables|/Game/BP/BP_AC/BP_BUFF_AC/BP_buff_class.BP_buff_class_C|Getbuff_resources _array_element))) (.stack (Utilities|Struct|Breakst_buff_effect (.buff_effectConsumption (Utilities|Struct|Breakst_buff_type_effect _array_element_2))))) (>= (.priority (Utilities|Struct|Breakst_buff_resources (Variables|/Game/BP/BP_AC/BP_BUFF_AC/BP_buff_class.BP_buff_class_C|Getbuff_resources _array_element))) (.Priority (Utilities|Struct|Breakst_buff_effect (.buff_effectConsumption (Utilities|Struct|Breakst_buff_type_effect _array_element_2))))) (>= (.NumberOfActions (Utilities|Struct|Breakst_buff_resources (Variables|/Game/BP/BP_AC/BP_BUFF_AC/BP_buff_class.BP_buff_class_C|Getbuff_resources _array_element))) (.NumberOfActions (Utilities|Struct|Breakst_buff_effect (.buff_effectConsumption (Utilities|Struct|Breakst_buff_type_effect _array_element_2))))))
              (Utilities|Array|Add (LocalVariables|Getbuff) _array_element)
              (else
                (LocalVariables|Setisf false)))))))
    (:then_1
      (return (LocalVariables|Getbuff) (LocalVariables|Getisf)))))

(fn ExecuteBuffEffect
  (params (Buff_effect_type :type e_buff_effect%20Enum :default "NewEnumerator0") (priority :type Integer) (buff :type BP%20Buff%20Class%20Object%20Reference) (indamage :type Float%20%28double-precision%29))
  (for _array_element (Variables|/Game/BP/BP_AC/BP_BUFF_AC/BP_buff_class.BP_buff_class_C|Getbuff_effect_info buff)
    (if (and (Utilities|Enum|Equal(Enum) (.buff_type (Utilities|Struct|Breakst_buff_type_effect _array_element)) Buff_effect_type) (== (.buff_priority (Utilities|Struct|Breakst_buff_type_effect _array_element)) priority))
      (LocalVariables|Setbuffeffect_consumption (.buff_effectConsumption (Utilities|Struct|Breakst_buff_type_effect _array_element)))
      (switch Utilities|FlowControl|Switch|Switchone_buff_effect Buff_effect_type
        (:NewEnumerator3
          (bind _ouput_damage (Default|UnderAttackEffect buff indamage))
          (A1|ConsumeResources (LocalVariables|Getbuffeffect_consumption) buff)
          (return true _ouput_damage false))
        (:NewEnumerator4
          (Default|TreatmentEffect buff)
          (A1|ConsumeResources (LocalVariables|Getbuffeffect_consumption) buff)
          (return true 0.0 false))
        (:NewEnumerator5
          (Default|DeadEffect buff)
          (A1|ConsumeResources (LocalVariables|Getbuffeffect_consumption) buff)
          (return true 0.0 false))
        (:NewEnumerator6
          (Default|AbsorbEffect buff)
          (A1|ConsumeResources (LocalVariables|Getbuffeffect_consumption) buff)
          (return true 0.0 false))
        (:NewEnumerator7
          (Default|ImmunityEffect buff)
          (A1|ConsumeResources (LocalVariables|Getbuffeffect_consumption) buff)
          (return true 0.0 false))))))

(fn 新函数
  (params (buff_prioity1 :type Integer) (effect_type1 :type e_buff_effect%20Enum :default "NewEnumerator0") (prioity_max1 :type Integer))
  ;[1 1 1] 初始化
  (LocalVariables|Setbuff_prioity buff_prioity1)
  (LocalVariables|Seteffect_type effect_type1)
  (LocalVariables|Setprioity_max prioity_max1)
  (LocalVariables|Setinterrupt false)
  (LocalVariables|Setfind false)
  (while (Math|Boolean|NORBoolean (LocalVariables|Getinterrupt) false) ; 检查是否中断
    (bind (_array_element _find) (B2|FindBuffsThatHaveActiveEffects (LocalVariables|Geteffect_type) (LocalVariables|Getbuff_prioity))) ; 查找buff
    (if _find ; 有没有找到
      (for _array_element_2 _array_element
        (bind _interrupt (B2|ExecuteBuffEffect (LocalVariables|Geteffect_type) (LocalVariables|Getbuff_prioity) _array_element_2 0.0)) ; 执行buff效果
        (LocalVariables|Setinterrupt _interrupt))
      (elif (< (LocalVariables|Getbuff_prioity) (LocalVariables|Getprioity_max))
        (LocalVariables|Setbuff_prioity (+ (LocalVariables|Getbuff_prioity) 1))
        (LocalVariables|Setinterrupt true)))))

(fn Immunity
  (params (this_buff :type BP%20Buff%20Class%20Object%20Reference))
  (for _array_element (Variables|A2|Getcurrent_buff)
    (for _array_element_2 (Variables|/Game/BP/BP_AC/BP_BUFF_AC/BP_buff_class.BP_buff_class_C|Getimmunity_info _array_element)
      (switch Utilities|FlowControl|Switch|SwitchonE_BUFF_type (Variables|/Game/BP/BP_AC/BP_BUFF_AC/BP_buff_class.BP_buff_class_C|Getbuff_type this_buff)
        (:NewEnumerator0
          (if (Utilities|Enum|Equal(Enum) (Variables|/Game/BP/BP_AC/BP_BUFF_AC/BP_buff_class.BP_buff_class_C|GetBuff%20Nature%20Type this_buff) (.buff_nature_type (Utilities|Struct|Breakst_buff_search_criteria (.buff_search_info (Utilities|Struct|Breakst_buff_immunity _array_element_2)))))
            _
            (else
              (return))))
        (:NewEnumerator1
          (if (and (Utilities|Enum|Equal(Enum) (Variables|/Game/BP/BP_AC/BP_BUFF_AC/BP_buff_class.BP_buff_class_C|Getelement_type this_buff) (.element_type (Utilities|Struct|Breakst_buff_search_criteria (.buff_search_info (Utilities|Struct|Breakst_buff_immunity _array_element_2))))) (Utilities|Enum|Equal(Enum) (Variables|/Game/BP/BP_AC/BP_BUFF_AC/BP_buff_class.BP_buff_class_C|Getelement_type_level this_buff) (.element_level (Utilities|Struct|Breakst_buff_search_criteria (.buff_search_info (Utilities|Struct|Breakst_buff_immunity _array_element_2))))))
            _
            (else
              (return)))))
      (switch Utilities|FlowControl|Switch|Switchone_buff_Immunity (.immunity_type (Utilities|Struct|Breakst_buff_immunity _array_element_2))
        (:NewEnumerator1
          (Default|AbsorbEffect _array_element))
        (:NewEnumerator0
          (Default|ImmunityEffect _array_element))))))