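; Base buff class for turn-based combat, holding creator, target, type, resources and effect rules.
; Initialization stores these and, for one buff type, pulls an element-and-level icon from a data table.
; TurnTick counts down cycle and duration, firing Cycle effects.
; BuffEffect matches type and priority, compares resources, calls mostly stub hooks, consumes resources for all but Obtain/Remove, then triggers the target pawn's health check.
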(fn BuffSimpleInitialization
  (params (CreateX :type Actor%20Object%20Reference) (TargetX :type Actor%20Object%20Reference) (buff_typeX :type E_BUFF_type%20Enum :default "NewEnumerator0") (buff_UpdataX :type E_BuffTimeUpdataEnum%20Enum :default "NewEnumerator0") (buffEffectPolarityX :type E_buff_Nature_type%20Enum :default "NewEnumerator0") (Buff%20Nature%20TypeX :type E_buff_Nature_type%20Enum :default "NewEnumerator0"))
  (Variables|Besedata|SetCreate CreateX)
  (Variables|besedata|SetTarget TargetX)
  (Variables|besedata|Setbuffinfo (Variables|besedata|Getbuffinfo))
  (Variables|other|Setbuff_type buff_typeX)
  (Variables|other|Setbuff_Updata buff_UpdataX)
  (Variables|other|SetbuffEffectPolarity buffEffectPolarityX)
  (Variables|element|SetBuff%20Nature%20Type Buff%20Nature%20TypeX))

(fn BUFFInitialize
  (params (createC :type Actor%20Object%20Reference) (targetC :type Actor%20Object%20Reference) (buffinfoC :type St%20Buff%20Base%20Info%20Structure) (resourcesC :type St%20Buff%20Resources%20Structure) (buff_typeI :type E_BUFF_type%20Enum :default "NewEnumerator0") (buff_nature_typeE :type E_buff_Nature_type%20Enum :default "NewEnumerator0") (buff_UpdataC :type E_BuffTimeUpdataEnum%20Enum :default "NewEnumerator0") (buffEffectPolarityC :type E_buff_Nature_type%20Enum :default "NewEnumerator0") (element_typeI :type E_element_type%20Enum :default "NewEnumerator0") (element_type_level_I :type E_element_advance%20Enum :default "NewEnumerator0") (boolsetX :type St%20Buff%20Boolset%20Structure) (buff_type_effectN :type Array%20of%20St%20Buff%20Type%20Effect%20Structures) (immunity_infoe :type Array%20of%20St%20Buff%20Immunity%20Structures))
  (Utilities|FlowControl|Sequence
    (:then_0
      (Variables|Besedata|SetCreate createC)
      (Variables|besedata|SetTarget targetC)
      (Variables|besedata|Setbuffinfo buffinfoC)
      (Variables|other|Setbuff_type buff_typeI)
      (Variables|bese|Setbuff_resources resourcesC)
      (Variables|bese|Setbuff_boolset boolsetX)
      (Variables|other|Setbuff_Updata buff_UpdataC)
      (Variables|other|SetbuffEffectPolarity buffEffectPolarityC)
      (Variables|element|SetBuff%20Nature%20Type buff_nature_typeE)
      (Variables|Bese|Setbuff_effect_info buff_type_effectN)
      (Variables|Bese|Setimmunity_info immunity_infoe))
    (:then_1
      (if (Utilities|Enum|Equal(Enum) buff_typeI "NewEnumerator1")
        (Variables|element|Setelement_type element_typeI)
        (Variables|element|Setelement_type_level element_type_level_I)
        (bind _returnvalue (Utilities|GetDataTableRow "/Game/Struct/st_buff/buff_elemetn_data/T_element_type_icon.T_element_type_icon" (Utilities|Name|EnumtoName element_typeI))
          (:then
            (bind _output_get (Variables|Default|Setelement_icon _returnvalue))
            (if (Utilities|Enum|Equal(Enum) (.element_type (Utilities|Struct|Breakst_element_type_icon _output_get)) (Variables|element|Getelement_type))
              (for _array_element (.element_level_icon (Utilities|Struct|Breakst_element_type_icon _output_get))
                (if (Utilities|Enum|Equal(Enum) (.element_type_level (Utilities|Struct|Breakst_element_icon _array_element)) (Variables|element|Getelement_type_level))
                  (Variables|besedata|Setbuffinfo (Utilities|Struct|Makest_buff_base_info (.buff_icon (Utilities|Struct|Breakst_element_icon _array_element)) (.buffname (Utilities|Struct|Breakst_buff_base_info (Variables|besedata|Getbuffinfo))) (.buff_index (Utilities|Struct|Breakst_buff_base_info (Variables|besedata|Getbuffinfo))))))))))
        (else
          (Variables|element|Setelement_type "NewEnumerator0")
          (Variables|element|Setelement_type_level "NewEnumerator2"))))))

(fn TurnTick
  (params (B :type Integer))
  (LocalVariables|Setturn B)
  (Utilities|FlowControl|Sequence
    (:then_0
      (if (>= 0 (- (Utilities|Struct|Breakst_buff_resources (Variables|bese|Getbuff_resources)) (LocalVariables|Getturn))) ; 周期效果时间检查
        (A3|BuffEffect "NewEnumerator2" 0 (Variables|besedata|GetTarget) (Variables|Besedata|GetCreate) 0.0)
        (else
          (Variables|bese|Setbuff_resources (Utilities|Struct|Makest_buff_resources (.stack (Utilities|Struct|Breakst_buff_resources (Variables|bese|Getbuff_resources))) (.priority (Utilities|Struct|Breakst_buff_resources (Variables|bese|Getbuff_resources))) (.NumberOfActions (Utilities|Struct|Breakst_buff_resources (Variables|bese|Getbuff_resources))) (.duration_time (Utilities|Struct|Breakst_buff_resources (Variables|bese|Getbuff_resources))) (- (Utilities|Struct|Breakst_buff_resources (Variables|bese|Getbuff_resources)) (LocalVariables|Getturn)))))))
    (:then_1
      (if (> (- (Utilities|Struct|Breakst_buff_resources (Variables|bese|Getbuff_resources)) (LocalVariables|Getturn)) 0) ; 检查buff的当前持续时间
        (Variables|bese|Setbuff_resources (Utilities|Struct|Makest_buff_resources (.stack (Utilities|Struct|Breakst_buff_resources (Variables|bese|Getbuff_resources))) (.priority (Utilities|Struct|Breakst_buff_resources (Variables|bese|Getbuff_resources))) (.NumberOfActions (Utilities|Struct|Breakst_buff_resources (Variables|bese|Getbuff_resources))) (- (Utilities|Struct|Breakst_buff_resources (Variables|bese|Getbuff_resources)) (LocalVariables|Getturn)) (.Cycletime (Utilities|Struct|Breakst_buff_resources (Variables|bese|Getbuff_resources)))))
        (return false)
        (elif (>= (Utilities|Struct|Breakst_buff_resources (Variables|bese|Getbuff_resources)) 1) ; 检查当前使用次数
          (return true)
          (else
            (Variables|bese|Setbuff_resources (Utilities|Struct|Makest_buff_resources (- (Utilities|Struct|Breakst_buff_resources (Variables|bese|Getbuff_resources)) 1) (.initial_ContinuousRound (Utilities|Struct|Breakbuff_base_attribute (Variables|bese|Getbuff_base_attribute)))))
            (if (not (Utilities|Struct|Breakst_buff_boolset (Variables|bese|Getbuff_boolset)))
              (return false))))))))

(fn ElementTagEffect)

(fn DeadEffect)

(fn UnderAttackEffect
  (params (input_damage :type Float%20%28double-precision%29))
  (return input_damage))

(fn EndEffect)

(fn CreateEffect
  (Development|PrintString 0 "skill_create_over"))

(fn TreatmentEffect)

(fn ImmunityEffect)

(fn AbsorbEffect)

(fn CycleEffect)

(fn BuffEffect
  (params (effect_type :type e_buff_effect%20Enum :default "NewEnumerator0") (priority :type Integer) (target :type Actor%20Object%20Reference) (create :type Actor%20Object%20Reference) (damage :type Float%20%28double-precision%29))
  (bind _buff_resources (Variables|bese|Getbuff_resources))
  (bind (_stack _priority _numberofactions) (Utilities|Struct|Breakst_buff_resources _buff_resources))
  ;[1 1 1] 判断是否存在
  (for _array_element (Variables|Bese|Getbuff_effect_info)
    (if (and (Utilities|Enum|Equal(Enum) effect_type (.buff_type (Utilities|Struct|Breakst_buff_type_effect _array_element))) (== priority (.buff_priority (Utilities|Struct|Breakst_buff_type_effect _array_element))))
      (LocalVariables|Setconsumption (.buff_effectConsumption (Utilities|Struct|Breakst_buff_type_effect _array_element)))
      (if (Math|Boolean|ANDBoolean (>= (.stack (Utilities|Struct|Breakst_buff_effect (LocalVariables|Getconsumption))) _stack) (>= (.Priority (Utilities|Struct|Breakst_buff_effect (LocalVariables|Getconsumption))) _priority) (>= (.NumberOfActions (Utilities|Struct|Breakst_buff_effect (LocalVariables|Getconsumption))) _numberofactions))
        (switch Utilities|FlowControl|Switch|Switchone_buff_effect effect_type
          (:NewEnumerator0
            (A1|CreateEffect)
            (T1|PRINT "NewEnumerator0")
            (bind _asbp_base_pawn (Utilities|Casting|CastToBP_BASE_Pawn target))
            (Default|CheakHealth（NG） _asbp_base_pawn)
            (return true 0.0))
          (:NewEnumerator1
            (A1|EndEffect)
            (T1|PRINT "NewEnumerator1")
            (bind _asbp_base_pawn_2 (Utilities|Casting|CastToBP_BASE_Pawn target))
            (Default|CheakHealth（NG） _asbp_base_pawn_2)
            (return true 0.0))
          (:NewEnumerator2
            (A1|CycleEffect)
            (T1|PRINT "NewEnumerator2")
            (CallFunction|ConsumeResources (LocalVariables|Getconsumption))
            (bind _asbp_base_pawn_3 (Utilities|Casting|CastToBP_BASE_Pawn target))
            (Default|CheakHealth（NG） _asbp_base_pawn_3)
            (return true 0.0))
          (:NewEnumerator3
            (T1|PRINT "NewEnumerator3")
            (bind _ouput_damage (A1|UnderAttackEffect damage))
            (CallFunction|ConsumeResources (LocalVariables|Getconsumption))
            (bind _asbp_base_pawn_4 (Utilities|Casting|CastToBP_BASE_Pawn target))
            (Default|CheakHealth（NG） _asbp_base_pawn_4)
            (return true _ouput_damage))
          (:NewEnumerator4
            (T1|PRINT "NewEnumerator4")
            (A1|TreatmentEffect)
            (CallFunction|ConsumeResources (LocalVariables|Getconsumption))
            (bind _asbp_base_pawn_5 (Utilities|Casting|CastToBP_BASE_Pawn target))
            (Default|CheakHealth（NG） _asbp_base_pawn_5)
            (return true 0.0))
          (:NewEnumerator5
            (A1|DeadEffect)
            (T1|PRINT "NewEnumerator5")
            (CallFunction|ConsumeResources (LocalVariables|Getconsumption))
            (bind _asbp_base_pawn_6 (Utilities|Casting|CastToBP_BASE_Pawn target))
            (Default|CheakHealth（NG） _asbp_base_pawn_6)
            (return true 0.0))
          (:NewEnumerator6
            (T1|PRINT "NewEnumerator6")
            (A1|AbsorbEffect)
            (CallFunction|ConsumeResources (LocalVariables|Getconsumption))
            (bind _asbp_base_pawn_7 (Utilities|Casting|CastToBP_BASE_Pawn target))
            (Default|CheakHealth（NG） _asbp_base_pawn_7)
            (return true 0.0))
          (:NewEnumerator7
            (T1|PRINT "NewEnumerator7")
            (A1|ImmunityEffect)
            (CallFunction|ConsumeResources (LocalVariables|Getconsumption))
            (bind _asbp_base_pawn_8 (Utilities|Casting|CastToBP_BASE_Pawn target))
            (Default|CheakHealth（NG） _asbp_base_pawn_8)
            (return true 0.0)))
        (else
          (return false 0.0))))))

(fn ConsumeResources
  (params (st_buff_effect :type St%20Buff%20Effect%20Structure%20%28by%20ref%29))
  (bind (_stack _priority _numberofactions) (Utilities|Struct|Breakst_buff_effect st_buff_effect))
  (Variables|bese|Setbuff_resources (Utilities|Struct|Makest_buff_resources (- (.stack (Utilities|Struct|Breakst_buff_resources (Variables|bese|Getbuff_resources))) _stack) (- (.priority (Utilities|Struct|Breakst_buff_resources (Variables|bese|Getbuff_resources))) _priority) (- (.NumberOfActions (Utilities|Struct|Breakst_buff_resources (Variables|bese|Getbuff_resources))) _numberofactions))))

(fn PRINT
  (params (NewParam :type e_buff_effect%20Enum :default "NewEnumerator0"))
  (Development|PrintString 0 (Utilities|String|Append "buff效果类型" (Utilities|String|EnumtoString NewParam)) true true "(R=1.000000,G=0.012242,B=0.000000,A=1.000000)"))