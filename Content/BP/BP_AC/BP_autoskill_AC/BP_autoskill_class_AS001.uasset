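; Autoskill class AS001 Blueprint that handles activation of the Synergism autoskill against the supplied target unit data.
; Activation constructs a Skill object and scans the target entries, routing Adjacent Targets and Core Target types into one shared damage path.
; That path calls the Skill object's DamageE for a fixed single-attack hit and returns true inside the loop, so only the first matching unit is damaged.
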(fn Activation
  (params (autoskill :type E_autoskill_emun%20Enum :default "NewEnumerator0") (targetunitdata :type Array%20of%20St%20Select%20Unit%20Target%20Data%20Structures))
  (bind _returnvalue (Game|ConstructObjectfromClass (Variables|Default|Getskill)))
  (switch Utilities|FlowControl|Switch|SwitchonE_autoskill_emun autoskill
    (:NewEnumerator1
      (for _array_element targetunitdata
        (switch Utilities|FlowControl|Switch|SwitchonE_unit_skill_select_target_type (.select_target_type (Utilities|Struct|Breakst_select_unit_target_data _array_element))
          (:NewEnumerator2
            _)
          (:NewEnumerator4
            _))
        (for _array_element_2 (.unit (Utilities|Struct|Breakst_select_unit_target_data _array_element))
          (Default|DamageE _returnvalue _array_element_2 0 (Utilities|Array|MakeArray 400) 1 "NewEnumerator1" "NewEnumerator0" "NewEnumerator1")
          (return true))))))