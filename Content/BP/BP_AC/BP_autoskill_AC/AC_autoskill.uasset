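; Actor component that manages automatic skills for units in grid-based combat, triggered by events such as counterattacks, round starts and deaths.
; BuildAutomaticSkills creates skill objects from T_autoskill_V2 rows, with Reset or Add handling for recurring skills.
; AutoSkillUse gathers candidate units by trigger, resolves targets from each unit's skill coordinate offsets, then activates the skill.
; After activation it prunes non-permanent skills and calls the land's AfterTheAction.
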(fn BuildAutomaticSkills
  (params (RowName :type Name) (skilldataNC :type St%20Skill%20Level%20Info%20Structure) (targetAA :type Actor%20Object%20Reference) (createAA :type Actor%20Object%20Reference))
  (bind _returnvalue (Utilities|GetDataTableRow "/Game/Struct/st_autoskill/T_autoskill_V2.T_autoskill_V2" RowName)
    (:then
      (for _array_element (Variables|Default|Getautoskill)
        (if (== (Utilities|Struct|BreakST_auto_skill_info (Utilities|Struct|Breakst_autoskill_Assembly (Variables|/Game/BP/BP_AC/BP_autoskill_AC/BP_autoskill_class.BP_autoskill_class_C|GetNEW_auto (LocalVariables|GetTEMPautoskillcclass)))) (Utilities|Struct|BreakST_auto_skill_info (.info (Utilities|Struct|Breakst_autoskill_Assembly _returnvalue)))) ; 检查是否存在这个自动技能
          (bind _output_get (LocalVariables|SetTEMPautoskillcclass _array_element))
          (switch Utilities|FlowControl|Switch|Switchone_auto_skill_recurring (Utilities|Struct|Breakst_autoskill_group (Utilities|Struct|Breakst_autoskill_Assembly (Variables|/Game/BP/BP_AC/BP_autoskill_AC/BP_autoskill_class.BP_autoskill_class_C|GetNEW_auto _output_get)))
            (:NewEnumerator1
              (Variables|/Game/BP/BP_AC/BP_autoskill_AC/BP_autoskill_class.BP_autoskill_class_C|SetNumber%20of%20uses (LocalVariables|GetTEMPautoskillcclass) (Utilities|Struct|Breakst_auto_skill_resource (.autoskill_Resources (Utilities|Struct|Breakst_autoskill_Assembly _returnvalue))))
              (Utilities|Array|SetArrayElem (Variables|Default|Getautoskill) 0 (LocalVariables|GetTEMPautoskillcclass)))
            (:NewEnumerator2
              (Variables|/Game/BP/BP_AC/BP_autoskill_AC/BP_autoskill_class.BP_autoskill_class_C|Setpoint (LocalVariables|GetTEMPautoskillcclass) (+ (Variables|/Game/BP/BP_AC/BP_autoskill_AC/BP_autoskill_class.BP_autoskill_class_C|Getpoint (LocalVariables|GetTEMPautoskillcclass)) (Utilities|Struct|Breakst_auto_skill_resource (Utilities|Struct|Breakst_autoskill_Assembly (Variables|/Game/BP/BP_AC/BP_autoskill_AC/BP_autoskill_class.BP_autoskill_class_C|GetNEW_auto (LocalVariables|GetTEMPautoskillcclass))))))
              (Utilities|Array|SetArrayElem (Variables|Default|Getautoskill) 0 (LocalVariables|GetTEMPautoskillcclass))))
          (else
            (bind _returnvalue_2 (Game|ConstructObjectfromClass (.auto_skill_class (Utilities|Struct|Breakst_autoskill_Assembly _returnvalue))))
            (Default|AutoSkillInitialize _returnvalue_2 _returnvalue skilldataNC targetAA createAA)
            (Utilities|Array|Add (Variables|Default|Getautoskill) _returnvalue_2)))))))

(fn AutoskillSelectUnit
  (params (unit :type Array%20of%20St%20Unit%20Class%20Structures) (action :type St%20Action%20Structure) (auto_skill :type E_autoskill_emun%20Enum :default "NewEnumerator0"))
  (bind _defenders (Utilities|Struct|Breakst_action action))
  (bind _attacker (Utilities|Struct|Breakst_action action))
  (bind _attacker_2 (Utilities|Struct|Breakst_action action))
  (bind _defenders_2 (Utilities|Struct|Breakst_action action))
  (bind _defenders_3 (Utilities|Struct|Breakst_action action))
  (bind _asbp_global_character (Utilities|Casting|CastToBP_GLOBAL_CHARACTER (Game|Player|GetPlayerPawn 0)))
  (LocalVariables|Setplayer _asbp_global_character)
  (Utilities|FlowControl|Sequence
    (:then_0
      (switch Utilities|FlowControl|Switch|SwitchonE_autoskill_emun auto_skill ; 根据技能枚举选择单位
        (:NewEnumerator0
          (for _array_element unit
            (if (Utilities|IsValid (.charter (Utilities|Struct|Breakst_unit_class _array_element)))
              (if (and (Utilities|Enum|Equal(Enum) (Variables|/Game/BP/BP_Battle_Phase/BP_BASE_Pawn.BP_BASE_Pawn_C|Getunit_faction (Utilities|Struct|Breakst_action action)) (.theunit_Belongs (Utilities|Struct|Breakst_unit_class _array_element))) (Utilities|Enum|Equal(Enum) (.gameplay_unit_type (Utilities|Struct|Breakst_unit_class _array_element)) "NewEnumerator0"))
                (Utilities|Array|Add (LocalVariables|Getskillcreate) (.charter (Utilities|Struct|Breakst_unit_class _array_element)))))))
        (:NewEnumerator1
          (for _array_element_2 unit
            (if (Utilities|IsValid _attacker)
              (if (and (Utilities|Enum|Equal(Enum) (Variables|/Game/BP/BP_Battle_Phase/BP_BASE_Pawn.BP_BASE_Pawn_C|Getunit_faction _attacker) (.theunit_Belongs (Utilities|Struct|Breakst_unit_class _array_element_2))) (Utilities|Enum|Equal(Enum) (.gameplay_unit_type (Utilities|Struct|Breakst_unit_class _array_element_2)) "NewEnumerator0"))
                (Utilities|Array|Add (LocalVariables|Getskillcreate) (.charter (Utilities|Struct|Breakst_unit_class _array_element_2)))))))
        (:NewEnumerator2
          (for _array_element_3 unit
            (if (Utilities|IsValid (.charter (Utilities|Struct|Breakst_unit_class _array_element_3)))
              (if (Utilities|Enum|Equal(Enum) (.gameplay_unit_type (Utilities|Struct|Breakst_unit_class _array_element_3)) "NewEnumerator0")
                (Utilities|Array|Add (LocalVariables|Getskillcreate) (.charter (Utilities|Struct|Breakst_unit_class _array_element_3)))))))
        (:NewEnumerator3
          (for _array_element_4 unit
            (if (Utilities|IsValid _defenders)
              (if (Utilities|Enum|Equal(Enum) (Variables|/Game/BP/BP_Battle_Phase/BP_BASE_Pawn.BP_BASE_Pawn_C|Getunit_faction _defenders) (.theunit_Belongs (Utilities|Struct|Breakst_unit_class _array_element_4)))
                (Utilities|Array|Add (LocalVariables|Getskillcreate) (.charter (Utilities|Struct|Breakst_unit_class _array_element_4)))))))
        (:NewEnumerator4
          (if (Utilities|IsValid _attacker_2)
            (Utilities|Array|Add (LocalVariables|Getskillcreate) _attacker_2)))
        (:NewEnumerator5
          (for _array_element_5 unit
            (Utilities|Array|Add (LocalVariables|Getskillcreate) (.charter (Utilities|Struct|Breakst_unit_class _array_element_5)))))
        (:NewEnumerator6
          (for _array_element_6 unit
            (Utilities|Array|Add (LocalVariables|Getskillcreate) (.charter (Utilities|Struct|Breakst_unit_class _array_element_6)))))
        (:NewEnumerator7
          (if (Utilities|IsValid _defenders_2)
            (Utilities|Array|Add (LocalVariables|Getskillcreate) _defenders_2)))
        (:NewEnumerator8
          (for _array_element_7 (Variables|/Game/BP/BP_Battle_Phase/BP_land_spaner.BP_land_spaner_C|GetUnit%20Class (Variables|/Game/BP/BP_Battle_Phase/BP_GLOBAL_CHARACTER.BP_GLOBAL_CHARACTER_C|Getland (LocalVariables|Getplayer)))
            (bind _asbp_base_pawn (Utilities|Casting|CastToBP_BASE_Pawn (.charter (Utilities|Struct|Breakst_unit_class _array_element_7))))
            (if (Utilities|IsValid _defenders_3)
              (if (Utilities|Enum|Equal(Enum) (Variables|/Game/BP/BP_Battle_Phase/BP_BASE_Pawn.BP_BASE_Pawn_C|Getunit_faction _asbp_base_pawn) (Variables|/Game/BP/BP_Battle_Phase/BP_BASE_Pawn.BP_BASE_Pawn_C|Getunit_faction _defenders_3))
                (Utilities|Array|Add (LocalVariables|Getskillcreate) _asbp_base_pawn)))))))
    (:then_2
      (return (LocalVariables|Getskillcreate) (LocalVariables|Gettarget)))))

(fn SelectAutoSkillTarget
  (params (create :type BP%20BASE%20Pawn%20Object%20Reference) (action :type St%20Action%20Structure) (autoskill_enum :type E_autoskill_emun%20Enum :default "NewEnumerator0") (autoskill_priority :type Integer))
  (bind _autoskill (LocalVariables|Getautoskill))
  (Utilities|FlowControl|Sequence
    (:then_0
      (for _array_element (Variables|AC_autoskill_C|Getautoskill (Variables|/Game/BP/BP_Battle_Phase/BP_BASE_Pawn.BP_BASE_Pawn_C|GetAC_autoskill create))
        (for _array_element_2 (Utilities|Struct|Breakst_autoskill_Assembly (Variables|/Game/BP/BP_AC/BP_autoskill_AC/BP_autoskill_class.BP_autoskill_class_C|GetNEW_auto _array_element))
          (if (and (Utilities|Enum|Equal(Enum) autoskill_enum (.autoskill_enum (Utilities|Struct|Breakst_autoskill_activation_mechanism _array_element_2))) (Utilities|Enum|Equal(Enum) (Utilities|Struct|Breakst_action action) (.action_type (Utilities|Struct|Breakst_autoskill_activation_mechanism _array_element_2))))
            (for _array_element_3 (.select_target_index (Utilities|Struct|Breakst_autoskill_activation_mechanism _array_element_2))
              (switch Utilities|FlowControl|Switch|SwitchonE_skill_target (.unit_ytpe (Utilities|Struct|Breakst_select_target_index (.select_type (Utilities|Struct|Breakst_select_unit_target_index _array_element_3))))
                (:NewEnumerator1
                  (for _array_element_4 (.Coordinates (Utilities|Struct|Breakst_select_target_index (.select_type (Utilities|Struct|Breakst_select_unit_target_index _array_element_3))))
                    (bind _chear (Default|CaculateDirectionYouCanWalkV2(Actor) (Variables|Default|GetGAME) (Transformation|GetActorLocation create) _array_element_4 (Variables|/Game/BP/BP_Battle_Phase/BP_BASE_Pawn.BP_BASE_Pawn_C|Getunit_area (LocalVariables|Gettarget_unit))))
                    (bind _asbp_base_pawn (Utilities|Casting|CastToBP_BASE_Pawn _chear))
                    (for _array_element_5 (LocalVariables|Getunit)
                      (if (Utilities|Enum|Equal(Enum) (.select_target_type (Utilities|Struct|Breakst_select_unit_target_index _array_element_3)) (.select_target_type (Utilities|Struct|Breakst_select_unit_target_data _array_element_5)))
                        (Utilities|Array|Add (.unit (Utilities|Struct|Breakst_select_unit_target_data _array_element_5)) _asbp_base_pawn)))))
                (:NewEnumerator0
                  (for _array_element_6 (.Coordinates (Utilities|Struct|Breakst_select_target_index (.select_type (Utilities|Struct|Breakst_select_unit_target_index _array_element_3))))
                    (bind _pawn (Default|CaculateDirectionYouCanWalkV2(Actor) (Variables|Default|GetGAME) (Transformation|GetActorLocation create) _array_element_6 (Variables|/Game/BP/BP_Battle_Phase/BP_BASE_Pawn.BP_BASE_Pawn_C|Getunit_area (LocalVariables|Gettarget_unit))))
                    (bind _asbp_base_pawn_2 (Utilities|Casting|CastToBP_BASE_Pawn _pawn))
                    (for _array_element_7 (LocalVariables|Getunit)
                      (if (Utilities|Enum|Equal(Enum) (.select_target_type (Utilities|Struct|Breakst_select_unit_target_index _array_element_3)) (.select_target_type (Utilities|Struct|Breakst_select_unit_target_data _array_element_7)))
                        (Utilities|Array|Add (.unit (Utilities|Struct|Breakst_select_unit_target_data _array_element_7)) _asbp_base_pawn_2)))))))))))
    (:then_1
      (return (Utilities|IsValid _autoskill) _autoskill (LocalVariables|Getenum) (LocalVariables|Getunit)))))

(fn AutoSkillUse
  (params (unit :type Array%20of%20St%20Unit%20Class%20Structures) (action :type St%20Action%20Structure) (auto_skill :type E_autoskill_emun%20Enum :default "NewEnumerator0") (autoskill_priority :type Integer))
  (bind _create (CallFunction|AutoskillSelectUnit unit action auto_skill)) ; 基于枚举选择单位
  (for _array_element _create
    (if (Utilities|IsValid _array_element)
      (bind _asbp_base_pawn (Utilities|Casting|CastToBP_BASE_Pawn _array_element))
      (if (Variables|/Game/BP/BP_Battle_Phase/BP_BASE_Pawn.BP_BASE_Pawn_C|Getunit_can_action _asbp_base_pawn)
        (bind (_returnvalue _autoskill_class _autoskillenum _newparam) (CallFunction|SelectAutoSkillTarget (Variables|/Game/BP/BP_Battle_Phase/BP_BASE_Pawn.BP_BASE_Pawn_C|GetAC_autoskill _asbp_base_pawn) _asbp_base_pawn action auto_skill autoskill_priority)) ; 基于自动技能选择目标
        (if _returnvalue
          (bind _effect_done (Default|AutoSkillActivation _autoskill_class _autoskillenum _newparam))
          (CallFunction|CheckAutomaticSkills)
          (Default|AftertheAction (Variables|/Game/BP/BP_Battle_Phase/BP_GLOBAL_CHARACTER.BP_GLOBAL_CHARACTER_C|Getland (Variables|Default|GetGAME)))
          (return _effect_done)
          (else
            (return false)))
        (else
          (Development|PrintText "no autoskill")
          (return false))))))

(fn CheckAutomaticSkills
  (for _array_element (Variables|Default|Getautoskill)
    (if (> (Variables|/Game/BP/BP_AC/BP_autoskill_AC/BP_autoskill_class.BP_autoskill_class_C|GetNumber%20of%20uses _array_element) 0)
      (if (not (Utilities|Struct|Breakst_autoskill_group (Utilities|Struct|Breakst_autoskill_Assembly (Variables|/Game/BP/BP_AC/BP_autoskill_AC/BP_autoskill_class.BP_autoskill_class_C|GetNEW_auto _array_element))))
        (Utilities|Array|RemoveItem (Variables|Default|Getautoskill) _array_element)))))