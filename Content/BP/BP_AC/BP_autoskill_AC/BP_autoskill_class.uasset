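; Base auto-skill class that gates automatic skill activation on a point resource and tracks remaining uses.
; Initialization stores the skill config, data, target and creator; activation either accrues gain points or, once the threshold is reachable, calls Activation.
; On success, ConsumeResources matches the trigger type and deducts points or uses according to its flags, clamping at zero.
; Activation always returns true and SelfselectionTarget is empty, both apparent override stubs.
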(fn AutoSkillInitialize
  (params (NEW_auto :type St%20Autoskill%20Assembly%20Structure) (skilldataN :type St%20Skill%20Level%20Info%20Structure) (target :type Actor%20Object%20Reference) (create :type Actor%20Object%20Reference))
  (bind _output_get (Variables|Default|SetNEW_auto NEW_auto))
  (Variables|ressource|SetNumber%20of%20uses (.Numberofuses (Utilities|Struct|Breakst_auto_skill_resource (Utilities|Struct|Breakst_autoskill_Assembly _output_get))))
  (Variables|Default|SettargetZ target)
  (Variables|Default|SetcreateZ create)
  (Variables|Default|Setskilldata skilldataN))

(fn AutoSkillActivation
  (params (auto_skill_type :type E_autoskill_emun%20Enum :default "NewEnumerator0") (target_unit_array :type Array%20of%20St%20Select%20Unit%20Target%20Data%20Structures))
  (bind _new_auto (Variables|Default|GetNEW_auto))
  (bind _autoskill_resources (Utilities|Struct|Breakst_autoskill_Assembly _new_auto))
  (bind (_consumepoints _gainpoints) (Utilities|Struct|Breakst_auto_skill_resource _autoskill_resources))
  (Utilities|FlowControl|Sequence
    (:then_0
      (if (<= _consumepoints (+ _gainpoints (Variables|ressource|Getpoint)))
        (bind _done (CallFunction|Activation auto_skill_type target_unit_array))
        (if _done
          (CallFunction|ConsumeResources auto_skill_type))
        (else
          (Variables|ressource|Setpoint (+ _gainpoints (Variables|ressource|Getpoint))))))
    (:then_1
      (return (LocalVariables|Getdone)))))

(fn Activation
  (params (autoskill :type E_autoskill_emun%20Enum :default "NewEnumerator0") (targetunitdata :type Array%20of%20St%20Select%20Unit%20Target%20Data%20Structures))
  (return true))

(fn Self-selectionTarget
  (params (unit :type Array%20of%20St%20Unit%20Class%20Structures))
  (return 0))

(fn ConsumeResources
  (params (auto_skill_type :type E_autoskill_emun%20Enum :default "NewEnumerator0"))
  (bind _new_auto (Variables|Default|GetNEW_auto))
  (bind (_autoskill_resources _automaticskillactivationmechanism) (Utilities|Struct|Breakst_autoskill_Assembly _new_auto))
  (for _array_element _automaticskillactivationmechanism
    (if (Utilities|Enum|Equal(Enum) auto_skill_type (.autoskill_enum (Utilities|Struct|Breakst_autoskill_activation_mechanism _array_element)))
      (Utilities|FlowControl|Sequence
        (:then_0
          (if (.Consumepoints (Utilities|Struct|Breakst_autoskill_activation_mechanism _array_element))
            (if (< (- (Variables|ressource|Getpoint) (Utilities|Struct|Breakst_auto_skill_resource _autoskill_resources)) 0)
              (Variables|ressource|Setpoint 0)
              (else
                (Variables|ressource|Setpoint (- (Variables|ressource|Getpoint) (Utilities|Struct|Breakst_auto_skill_resource _autoskill_resources)))))))
        (:then_1
          (if (not (.Numberofuses (Utilities|Struct|Breakst_autoskill_activation_mechanism _array_element)))
            (if (< (- (Variables|ressource|GetNumber%20of%20uses) 1) 0)
              (Variables|ressource|SetNumber%20of%20uses 0)
              (else
                (Variables|ressource|SetNumber%20of%20uses (- (Variables|ressource|GetNumber%20of%20uses) 1))))))))))