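; Skill component for an element skill that deals multi-hit elemental damage and consumes element buffs on its targets.
; On a direct-skill activation, it damages every unit in the first target group of the required type, then dispels the buffs returned by the simple element assertion check.
; The assertion's bonus-damage effect and a complex element markup variant exist, but only disconnected nodes use them.
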(fn Activation
  (params (skill_model :type E_SKILL_model%20Enum :default "NewEnumerator0") (create :type BP%20BASE%20Pawn%20Object%20Reference) (skill%20target :type Array%20of%20St%20Select%20Unit%20Target%20Data%20Structures))
  (switch Utilities|FlowControl|Switch|SwitchonE_SKILL_model skill_model
    (:NewEnumerator1
      (for _array_element skill%20target
        (if (Utilities|Enum|Equal(Enum) (.select_target_type (Utilities|Struct|Breakst_select_unit_target_data _array_element)) "NewEnumerator1")
          (for _array_element_2 (.unit (Utilities|Struct|Breakst_select_unit_target_data _array_element))
            (CallFunction|DamageE _array_element_2 create (Utilities|Array|MakeArray 400 10 100) 3 "NewEnumerator1" "NewEnumerator0" "NewEnumerator0"))
          (bind _targett1 (CallFunction|SimpleElementAssertionAssembly skill%20target create "NewEnumerator1" "NewEnumerator1" "NewEnumerator0" "NewEnumerator0" 1))
          (for _array_element_3 _targett1
            (Default|DispelBuff (Variables|/Game/BP/BP_Battle_Phase/BP_BASE_Pawn.BP_BASE_Pawn_C|GetAC_buff (.pawn (Utilities|Struct|Breakst_basepawn_buff _array_element_3))) (.buff (Utilities|Struct|Breakst_basepawn_buff _array_element_3))))
          (return true))))))

(fn SimpleElementAssertion(effect)
  (params (assertion_target :type BP%20BASE%20Pawn%20Object%20Reference) (assertion_create :type BP%20BASE%20Pawn%20Object%20Reference))
  (CallFunction|DamageE assertion_target assertion_create (Utilities|Array|MakeArray 100 400) 1 "NewEnumerator1" "NewEnumerator0" "NewEnumerator1"))