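; Attack skill class Blueprint that applies a damaging hit and a buff when a direct skill activates.
; Activation scans the skill target groups for one selection type, deals fixed single-hit damage to a unit, then applies the table-defined EH1 buff to it.
; It returns inside the inner loop, so only the first matching unit is affected.
; The usability check is an empty stub.
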(fn Activation
  (params (skill_model :type E_SKILL_model%20Enum :default "NewEnumerator0") (create :type BP%20BASE%20Pawn%20Object%20Reference) (skill%20target :type Array%20of%20St%20Select%20Unit%20Target%20Data%20Structures))
  (switch Utilities|FlowControl|Switch|SwitchonE_SKILL_model skill_model
    (:NewEnumerator1
      (for _array_element skill%20target
        (if (Utilities|Enum|Equal(Enum) (.select_target_type (Utilities|Struct|Breakst_select_unit_target_data _array_element)) "NewEnumerator1")
          (for _array_element_2 (.unit (Utilities|Struct|Breakst_select_unit_target_data _array_element))
            (CallFunction|DamageE _array_element_2 create (Utilities|Array|MakeArray 100 100 100) 1 "NewEnumerator1" "NewEnumerator0" "NewEnumerator0")
            (CallFunction|BuildBuffE _array_element_2 "EH1" true create)
            (return true)))))))

(fn SkillCanUse)