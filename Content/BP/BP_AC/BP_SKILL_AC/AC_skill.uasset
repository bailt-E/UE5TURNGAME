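; Skill component for turn-based units, driven by rows of the T_skill_V2 data table.
; Check functions pick a skill stage (preparatory, padding, direct, advanced, end), verify action points, speed or power, and find targets and range.
; Use functions construct skill and effect objects, storing prepared skills and their resources in SkillArray.
; Auto-skills gain points from matching actions and refresh uses on Tick; post-use consumption branches are empty stubs.
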(event EventBeginPlay)

(event EventTick
  (params (DeltaSeconds :type Float%20%28single-precision%29))
  (for _array_element (Variables|Default|Getskill_array)
    (Default|CheckAutoSkillNumberOfUses _array_element)))

(fn 检查使用什么技能
  (params (RowName :type Name) (Controller :type BP%20GLOBAL%20CHARATER%20Object%20Reference))
  (Utilities|FlowControl|Sequence
    (:then_0
      (bind _returnvalue (Utilities|GetDataTableRow "/Game/Struct/ST_NEW_skill/T_skill_V2.T_skill_V2" RowName)
        (:then
          (bind _returnvalue_2 (Game|ConstructObjectfromClass (.skill_class (Utilities|Struct|BreakST_skill_Group_Assembly _returnvalue))))
          (LocalVariables|Set当前技能 _returnvalue_2)
          (if (.能否直接使用 (Utilities|Struct|Breakst_skill_Group_boolset (.技能设置 (Utilities|Struct|BreakST_skill_Group_Assembly _returnvalue)))) ; 能否直接使用技能
            (if (.Compositeconditions (Utilities|Struct|Breakst_skill_Group_boolset (.技能设置 (Utilities|Struct|BreakST_skill_Group_Assembly _returnvalue)))) ; 双重累计道具物检查
              (if (>= (.Accumulateitems (Utilities|Struct|Breakst_Skills_Resources (Variables|/Game/BP/BP_AC/BP_SKILL_AC/BP_skill_class.BP_skill_class_C|Getskill_resources (stale _skill)))) (.Accumulateditems_required (Utilities|Struct|Breakst_skill_Group_resource (.技能资源 (Utilities|Struct|BreakST_skill_Group_Assembly _returnvalue))))) ; 检查道具物是否足够
                (return "NewEnumerator6" "NewEnumerator1")
                (elif (>= (.Obtain_accumulatedpriority (Utilities|Struct|Breakst_skill_Group_resource (.技能资源 (Utilities|Struct|BreakST_skill_Group_Assembly _returnvalue)))) (.currentaccumulatedpriority (Utilities|Struct|Breakst_Skills_Resources (Variables|/Game/BP/BP_AC/BP_SKILL_AC/BP_skill_class.BP_skill_class_C|Getskill_resources (stale _skill)))))
                  (return "NewEnumerator1" "NewEnumerator1")))
              (else
                (bind _output_get (Variables|Default|Setskill_model "NewEnumerator1"))
                (return _output_get "NewEnumerator1")))
            (elif (.是否需要前置技能 (Utilities|Struct|Breakst_skill_Group_boolset (.技能设置 (Utilities|Struct|BreakST_skill_Group_Assembly _returnvalue))))
              (bind (_find _skill) (newsskill|在技能数组查找技能 (Variables|Default|Getskill_array_CD) (Variables|/Game/BP/BP_AC/BP_SKILL_AC/BP_skill_class.BP_skill_class_C|GetID (LocalVariables|Get当前技能))))
              (if _find ; 检查技能数组是否存在技能
                (if (.技能是否消耗技能 (Utilities|Struct|Breakst_skill_Group_boolset (.技能设置 (Utilities|Struct|BreakST_skill_Group_Assembly _returnvalue)))) ; 是否消耗技能变量
                  (bind _output_get_2 (Variables|Default|Setskill_model "NewEnumerator4"))
                  (return _output_get_2 "NewEnumerator1")
                  (else
                    ;[1 1 1] 注释
                    (if (.技能是否消耗道具物 (Utilities|Struct|Breakst_skill_Group_boolset (.技能设置 (Utilities|Struct|BreakST_skill_Group_Assembly _returnvalue)))) ; 是否消耗道具物
                      (if (>= (.所需道具物 (Utilities|Struct|Breakst_skill_Group_resource (.技能资源 (Utilities|Struct|BreakST_skill_Group_Assembly _returnvalue)))) (.SkillNumberOfActions (Utilities|Struct|Breakst_Skills_Resources (Variables|/Game/BP/BP_AC/BP_SKILL_AC/BP_skill_class.BP_skill_class_C|Getskill_resources (LocalVariables|Get当前技能))))) ; 检查道具物是否足够
                        (bind _output_get_3 (Variables|Default|Setskill_model "NewEnumerator1"))
                        (return _output_get_3 "NewEnumerator1")
                        (else
                          (bind _output_get_4 (Variables|Default|Setskill_model "NewEnumerator5"))
                          (return _output_get_4 "NewEnumerator1")))
                      (elif (>= (.消耗层数 (Utilities|Struct|Breakst_skill_Group_resource (.技能资源 (Utilities|Struct|BreakST_skill_Group_Assembly _returnvalue)))) (.stack (Utilities|Struct|Breakst_Skills_Resources (Variables|/Game/BP/BP_AC/BP_SKILL_AC/BP_skill_class.BP_skill_class_C|Getskill_resources (LocalVariables|Get当前技能))))) ; 检查层数是否足够
                        (bind _output_get_5 (Variables|Default|Setskill_model "NewEnumerator1"))
                        (return _output_get_5 "NewEnumerator1")
                        (else
                          (bind _output_get_6 (Variables|Default|Setskill_model "NewEnumerator5"))
                          (return _output_get_6 "NewEnumerator1"))))))
                (else
                  (bind _output_get_7 (Variables|Default|Setskill_model "NewEnumerator0"))
                  (return _output_get_7 "NewEnumerator1"))))))))
    (:then_1
      ;[1 1 1] 查找技能技能效果类型
      (bind _returnvalue_3 (Utilities|GetDataTableRow "/Game/Struct/ST_NEW_skill/T_skill_V2.T_skill_V2" RowName)
        (:then
          (for _array_element (Utilities|Struct|BreakST_skill_Group_Assembly _returnvalue_3)
            (if (Utilities|Enum|Equal(Enum) (Variables|Default|Getskill_model) (.技能枚举 (Utilities|Struct|Breakst_skilleffect_Assembly _array_element)))
              (switch Utilities|FlowControl|Switch|SwitchonE_skill_effect_type (.skill_effect_type (Utilities|Struct|Breakst_skilleffect_Assembly _array_element))
                (:NewEnumerator1
                  (bind _output_get_8 (Variables|Default|SetSkill%20Effect%20Type (.skill_effect_type (Utilities|Struct|Breakst_skilleffect_Assembly _array_element))))
                  (return (Variables|Default|Getskill_model) _output_get_8))
                (:NewEnumerator0
                  (bind (_skill_model _skilleffect) (newsskill|SecondaryInspection(summon) Controller false))
                  (return _skill_model _skilleffect))))))))
    (:then_2
      (Utilities|FlowControl|Sequence
        (:then_0
          (switch Utilities|FlowControl|Switch|SwitchonE_skill_effect_type (Variables|Default|GetSkill%20Effect%20Type)
            (:NewEnumerator1
              (Development|PrintText "通用技能"))
            (:NewEnumerator0
              (Development|PrintText "召唤技能"))))
        (:then_1
          (switch Utilities|FlowControl|Switch|SwitchonE_SKILL_model (Variables|Default|Getskill_model)
            (:NewEnumerator0
              (Development|PrintText "预备技能"))
            (:NewEnumerator5
              (Development|PrintText "填充技能"))
            (:NewEnumerator1
              (Development|PrintText "直接技能"))
            (:NewEnumerator6
              (Development|PrintText "第二直接技能"))
            (:NewEnumerator2
              (Development|PrintText "周期技能"))
            (:NewEnumerator3
              (Development|PrintText "协同技能"))
            (:NewEnumerator7
              (Development|PrintText "反击技能"))
            (:NewEnumerator4
              (Development|PrintText "终结技能"))))))))

(fn SecondaryInspection(summon)
  (params (Controller :type BP%20GLOBAL%20CHARATER%20Object%20Reference) (have%20secondary_skill? :type Boolean))
  (bind _land (Variables|/Game/BP/BP_modelE/BP_GLOBAL_CHARATER.BP_GLOBAL_CHARATER_C|Getland Controller))
  (if (<= (Variables|/Game/BP/BP_modelE/BP_land_spaner.BP_land_spaner_C|GetLocalized%20summons _land) (Variables|/Game/BP/BP_modelE/BP_land_spaner.BP_land_spaner_C|GetsummonsMAX _land)) ; 检查能否使用召唤系技能
    (return "NewEnumerator1" "NewEnumerator0")
    (elif have%20secondary_skill? ; 在召唤物满了之后能否使用其他技能
      (return "NewEnumerator6" "NewEnumerator1"))))

(fn 检查技能能否使用
  (params (role_name :type Name) (skill_model :type E_SKILL_model%20Enum :default "NewEnumerator0") (skill_effect_type :type E_skill_effect_type%20Enum :default "NewEnumerator0") (Caster :type BP%20Base%20Pawn%20Class%20Object%20Reference) (Controller :type BP%20GLOBAL%20CHARATER%20Object%20Reference))
  ;[1 1 1] 第一阶段
  (bind _returnvalue (Utilities|GetDataTableRow "/Game/Struct/ST_NEW_skill/T_skill_V2.T_skill_V2" role_name)
    (:then
      (switch Utilities|FlowControl|Switch|SwitchonE_SKILL_TYPE (Utilities|Struct|Breakst_skill_Group_base_info (.技能组基本信息 (Utilities|Struct|BreakST_skill_Group_Assembly _returnvalue)))
        (:NewEnumerator2
          (for _array_element (.技能效果结构体 (Utilities|Struct|BreakST_skill_Group_Assembly _returnvalue)) :!label _label
            (if (Utilities|Enum|Equal(Enum) (.技能枚举 (Utilities|Struct|Breakst_skilleffect_Assembly _array_element)) (Variables|Default|Getskill_model)) ; 检查技能枚举是否等于技能枚举
              (if (and (>= (Variables|/Game/BP/BP_modelE/BP_GLOBAL_CHARATER.BP_GLOBAL_CHARATER_C|GetActionPoint Controller) (.阵营行动点 (Utilities|Struct|Breakst_skill_effect_resource (.技能所需资源 (Utilities|Struct|Breakst_skilleffect_Assembly _array_element))))) (>= (Math|Conversions|ToFloat(Integer) (Utilities|Struct|Breakst_RoleStatus (Variables|/Game/BP/BP_AC/BP_level_AC/AC_level.AC_level_C|GetCurrent_attribute (Variables|/Game/BP/BP_modelE/BP_base_pawn_class.BP_base_pawn_class_C|GetAC_level Caster)))) (.角色速度 (Utilities|Struct|Breakst_skill_effect_resource (.技能所需资源 (Utilities|Struct|Breakst_skilleffect_Assembly _array_element)))))) ; 检查资源是否足够
                (switch Utilities|FlowControl|Switch|SwitchonE_skill_effect_type skill_effect_type ; 技能类型
                  (:NewEnumerator1
                    (return true))
                  (:NewEnumerator0
                    (return true)))))))
        (:NewEnumerator0
          (goto _label))
        (:NewEnumerator1
          (if (>= (Utilities|Struct|Breakst_RoleStatus (Variables|/Game/BP/BP_AC/BP_level_AC/AC_level.AC_level_C|GetCurrent_attribute (Variables|/Game/BP/BP_modelE/BP_base_pawn_class.BP_base_pawn_class_C|GetAC_level Caster))) 50)
            (switch Utilities|FlowControl|Switch|SwitchonE_skill_effect_type skill_effect_type ; 技能类型
              (:NewEnumerator1
                (return true))
              (:NewEnumerator0
                (return true)))))))))

(fn DisplaystheRangeOfSkills
  (params (RowName :type Name))
  (bind _returnvalue (Utilities|GetDataTableRow "/Game/Struct/ST_NEW_skill/T_skill_V2.T_skill_V2" RowName)
    (:then
      (for _array_element (.技能效果结构体 (Utilities|Struct|BreakST_skill_Group_Assembly _returnvalue))
        (if (Utilities|Enum|Equal(Enum) (.技能枚举 (Utilities|Struct|Breakst_skilleffect_Assembly _array_element)) (Variables|Default|Getskill_model))
          (bind _outactors (Actor|GetAllActorsOfClass (.技能所需目标 (Utilities|Struct|Breakst_skilleffect_Assembly _array_element))))
          (bind _output_get (LocalVariables|Setskill_range _outactors))
          (for _array_element_2 _output_get
            (Utilities|Array|Add (LocalVariables|GetEligible%20actors) _array_element_2))
          (return (LocalVariables|GetEligible%20actors)))))))

(fn 在技能数组查找技能
  (params (skill_Array :type Array%20of%20BP%20Skill%20Class%20Object%20References) (ID :type Integer))
  (for _array_element skill_Array
    (if (== (Variables|/Game/BP/BP_AC/BP_SKILL_AC/BP_skill_class.BP_skill_class_C|GetID _array_element) ID)
      (return false _array_element ID))))

(fn 显示命中范围以及结果V2
  (params (skill_model :type E_SKILL_model%20Enum :default "NewEnumerator0") (RowName :type Name) (base_unit%28getactorlocation%29 :type BP%20BASE%20UNIT%20Object%20Reference))
  (bind _returnvalue (Utilities|GetDataTableRow "/Game/Struct/ST_NEW_skill/T_skill_V2.T_skill_V2" RowName)
    (:then
      (for _array_element (Utilities|Struct|BreakST_skill_Group_Assembly _returnvalue)
        (if (Utilities|Enum|Equal(Enum) skill_model (.技能枚举 (Utilities|Struct|Breakst_skilleffect_Assembly _array_element))) ; 检查技能枚举和技能类型
          (bind _asbp_global_charater (Utilities|Casting|CastToBP_GLOBAL_CHARATER (Game|Player|GetPlayerPawn 0)))
          (bind _final_data (Default|CaculateDirectionYouCanWalkV2(Skill) _asbp_global_charater (Transformation|GetActorLocation base_unit%28getactorlocation%29) (.技能作用目标 (Utilities|Struct|Breakst_skilleffect_Assembly _array_element)))) ; 获得技能的数组，并基于数组
          (return _final_data))))))

(fn UseSkill
  (params (create :type Actor%20Object%20Reference) (skill_type :type E_SKILL_model%20Enum :default "NewEnumerator0") (skill_name :type Name) (skill_target :type Array%20of%20BP%20BASE%20UNIT%20Object%20References))
  (Useskill(R1)|使用技能A create 0 skill_name (Variables|Default|Getskill_model))
  (Useskill(R1)|使用技能B (Variables|Default|Getskill_model) skill_name skill_target)
  (bind _asbp_base_unit (Utilities|Casting|CastToBP_BASE_UNIT create))
  (bind _asbp_base_pawn_class (Utilities|Casting|CastToBP_base_pawn_class _asbp_base_unit))
  (Useskill(R1)|AfterUsingtheSkill skill_name (Variables|Default|Getskill_model) _asbp_base_pawn_class))

(fn 使用技能A
  (params (create :type Actor%20Object%20Reference) (skilltarger :type Actor%20Object%20Reference) (RowName :type Name) (skill_type :type E_SKILL_model%20Enum :default "NewEnumerator0"))
  (bind _returnvalue (Utilities|GetDataTableRow "/Game/Struct/ST_NEW_skill/T_skill_V2.T_skill_V2" RowName)
    (:then
      (LocalVariables|Setskill_data _returnvalue)
      (Development|PrintString (Utilities|String|EnumtoString skill_type))
      (Utilities|FlowControl|Sequence
        (:then_0
          ;[1 1 1] 公共事件
          (switch Utilities|FlowControl|Switch|SwitchonE_SKILL_model skill_type
            (:NewEnumerator0
              (bind _returnvalue_2 (Game|ConstructObjectfromClass (Utilities|Struct|BreakST_skill_Group_Assembly (LocalVariables|Getskill_data))))
              (Default|SkillInitialize _returnvalue_2 (.skill_index (Utilities|Struct|Breakst_skill_Group_base_info (.技能组基本信息 (Utilities|Struct|BreakST_skill_Group_Assembly (LocalVariables|Getskill_data))))) (.skill_name (Utilities|Struct|Breakst_skill_Group_base_info (.技能组基本信息 (Utilities|Struct|BreakST_skill_Group_Assembly (LocalVariables|Getskill_data))))) (Utilities|Struct|Makest_Skills_Resources (.初始道具物 (Utilities|Struct|Breakst_skill_Group_resource (.技能资源 (Utilities|Struct|BreakST_skill_Group_Assembly (LocalVariables|Getskill_data))))) (.初始层数 (Utilities|Struct|Breakst_skill_Group_resource (.技能资源 (Utilities|Struct|BreakST_skill_Group_Assembly (LocalVariables|Getskill_data))))) (.初始点数 (Utilities|Struct|Breakst_skill_Group_resource (.技能资源 (Utilities|Struct|BreakST_skill_Group_Assembly (LocalVariables|Getskill_data))))) 3 3) RowName)
              (Default|SkillAutoInitialize _returnvalue_2 (.auto_skill (Utilities|Struct|BreakST_skill_Group_Assembly (LocalVariables|Getskill_data))))
              (Utilities|Array|Add (Variables|Default|Getskill_array) _returnvalue_2))
            (:NewEnumerator5
              (bind (_find _skill _index) (newsskill|在技能数组查找技能 (Variables|Default|Getskill_array) (.skill_index (Utilities|Struct|Breakst_skill_Group_base_info (Utilities|Struct|BreakST_skill_Group_Assembly (LocalVariables|Getskill_data))))))
              (Default|SkillInitialize _skill _index (.skill_name (Utilities|Struct|Breakst_skill_Group_base_info (Utilities|Struct|BreakST_skill_Group_Assembly (LocalVariables|Getskill_data)))) (Utilities|Struct|Makest_Skills_Resources (+ (.SkillNumberOfActions (Utilities|Struct|Breakst_Skills_Resources (Variables|/Game/BP/BP_AC/BP_SKILL_AC/BP_skill_class.BP_skill_class_C|Getskill_resources _skill))) (.获得道具物 (Utilities|Struct|Breakst_skill_Group_resource (.技能资源 (Utilities|Struct|BreakST_skill_Group_Assembly (LocalVariables|Getskill_data)))))) (+ (.stack (Utilities|Struct|Breakst_Skills_Resources (Variables|/Game/BP/BP_AC/BP_SKILL_AC/BP_skill_class.BP_skill_class_C|Getskill_resources _skill))) (.增加层数 (Utilities|Struct|Breakst_skill_Group_resource (.技能资源 (Utilities|Struct|BreakST_skill_Group_Assembly (LocalVariables|Getskill_data)))))) (+ (.priority (Utilities|Struct|Breakst_Skills_Resources (Variables|/Game/BP/BP_AC/BP_SKILL_AC/BP_skill_class.BP_skill_class_C|Getskill_resources _skill))) (.增加点数 (Utilities|Struct|Breakst_skill_Group_resource (.技能资源 (Utilities|Struct|BreakST_skill_Group_Assembly (LocalVariables|Getskill_data)))))) 5) RowName)
              (auto_skill|AutosskillRepeat RowName _skill))))
        (:then_1
          (for _array_element (.技能效果结构体 (Utilities|Struct|BreakST_skill_Group_Assembly (LocalVariables|Getskill_data)))
            (if (Utilities|Enum|Equal(Enum) skill_type (.技能枚举 (Utilities|Struct|Breakst_skilleffect_Assembly _array_element)))
              (Development|PrintString "这里是技能组，已经使用级技能")
              (bind _returnvalue_3 (Game|ConstructObjectfromClass (.skill_class (Utilities|Struct|BreakST_skill_Group_Assembly (LocalVariables|Getskill_data)))))
              (Default|Activation _returnvalue_3 create skilltarger) ; 实际上无论是什么技能都有激活效果
            )))))))

(fn 使用技能B
  (params (e_skill_model :type E_SKILL_model%20Enum :default "NewEnumerator0") (RowName :type Name) (skill_target :type Array%20of%20BP%20BASE%20UNIT%20Object%20References))
  (bind _returnvalue (Utilities|GetDataTableRow "/Game/Struct/ST_NEW_skill/T_skill_V2.T_skill_V2" RowName)
    (:then
      (for _array_element (Utilities|Struct|BreakST_skill_Group_Assembly _returnvalue)
        (if (Utilities|Enum|Equal(Enum) e_skill_model (.技能枚举 (Utilities|Struct|Breakst_skilleffect_Assembly _array_element)))
          (for _array_element_2 (.skill_effect_target (Utilities|Struct|Breakst_skilleffect_Assembly _array_element))
            (for _array_element_3 skill_target
              (if (== (Utilities|GetClass _array_element_3) (.skill_target (Utilities|Struct|BreakST_skilleffect_target _array_element_2))) ; 判断技能目标是否等于目标
                (bind _returnvalue_2 (Game|ConstructObjectfromClass (.BP_skilleffect_class (Utilities|Struct|BreakST_skilleffect_target _array_element_2))))
                (Default|Activation _returnvalue_2 _array_element_3)
                (return (.action_type (Utilities|Struct|Breakst_skilleffect_Assembly _array_element)))))))))))

(fn AfterUsingtheSkill
  (params (skillname :type Name) (skill :type E_SKILL_model%20Enum :default "NewEnumerator0") (create :type BP%20Base%20Pawn%20Class%20Object%20Reference))
  (bind _returnvalue (Utilities|GetDataTableRow "/Game/Struct/ST_NEW_skill/T_skill_V2.T_skill_V2" skillname)
    (:then
      (for _array_element (.技能效果结构体 (Utilities|Struct|BreakST_skill_Group_Assembly _returnvalue))
        (if (Utilities|Enum|Equal(Enum) (.技能枚举 (Utilities|Struct|Breakst_skilleffect_Assembly _array_element)) skill)
          (Utilities|FlowControl|Sequence
            (:then_0
              (if (.技能是否消耗技能 (Utilities|Struct|Breakst_skill_effect_boolset (.skill_effect_boolset (Utilities|Struct|Breakst_skilleffect_Assembly _array_element))))
                _))
            (:then_1
              (if (.技能是否消耗道具物 (Utilities|Struct|Breakst_skill_effect_boolset (.skill_effect_boolset (Utilities|Struct|Breakst_skilleffect_Assembly _array_element))))
                _))
            (:then_2
              (if (.是否销毁技能变量 (Utilities|Struct|Breakst_skill_effect_boolset (.skill_effect_boolset (Utilities|Struct|Breakst_skilleffect_Assembly _array_element))))
                _))))))))

(fn AutosskillRepeat
  (params (skill_name :type Name) (skill :type Object%20Object%20Reference))
  (bind _returnvalue (Utilities|GetDataTableRow "/Game/Struct/ST_NEW_skill/T_skill_V2.T_skill_V2" skill_name)
    (:then
      (for _array_element (Utilities|Struct|BreakST_skill_Group_Assembly _returnvalue)
        (for _array_element_2 (Variables|Default|Getskill_array)
          (if (== _array_element_2 skill)
            (switch Utilities|FlowControl|Switch|Switchone_auto_skill_recurring (.auto_skill_repeat_E (Utilities|Struct|Breakst_auto_skill _array_element))
              (:NewEnumerator1
                (Utilities|Array|Clear (Variables|/Game/BP/BP_AC/BP_SKILL_AC/BP_skill_class.BP_skill_class_C|Getauto_skill_resource _array_element_2))
                (Utilities|Array|Clear (Variables|/Game/BP/BP_AC/BP_SKILL_AC/BP_skill_class.BP_skill_class_C|Getauto_skill _array_element_2))
                (Default|SkillAutoInitialize _array_element_2 (Utilities|Struct|BreakST_skill_Group_Assembly _returnvalue))))))))))

(fn AutoskillCanUse?
  (params (action_type :type E_action_type%20Enum :default "NewEnumerator0") (pawn :type BP%20Base%20Pawn%20Class%20Object%20Reference) (target :type BP%20BASE%20UNIT%20Object%20Reference) (have_target? :type Boolean))
  (for _array_element (Variables|AC_skill_C|Getskill_array (Variables|/Game/BP/BP_modelE/BP_base_pawn_class.BP_base_pawn_class_C|GetAC_skill pawn))
    (for _array_element_2 (Variables|/Game/BP/BP_AC/BP_SKILL_AC/BP_skill_class.BP_skill_class_C|Getauto_skill _array_element)
      (for _array_element_3 (.action-actior_type (Utilities|Struct|Breakst_auto_skill _array_element_2))
        (if (Utilities|Enum|Equal(Enum) _array_element_3 action_type) ; 检查行动是否一致
          (if have_target?
            (if (== (.autoskill_target (Utilities|Struct|Breakst_auto_skill _array_element_2)) target) ; 检查目标是否一致
              (for _array_element_4 (Variables|/Game/BP/BP_AC/BP_SKILL_AC/BP_skill_class.BP_skill_class_C|Getauto_skill_resource _array_element) :!label _label
                (if (Utilities|Enum|Equal(Enum) (.auto_skill_type (Utilities|Struct|Breakst_auto_skill _array_element_2)) (Utilities|Struct|Breakst_auto_skill_resource _array_element_4))
                  (Utilities|Array|SetArrayElem (Variables|/Game/BP/BP_AC/BP_SKILL_AC/BP_skill_class.BP_skill_class_C|Getauto_skill_resource _array_element) (Utilities|Array|FindItem (Variables|/Game/BP/BP_AC/BP_SKILL_AC/BP_skill_class.BP_skill_class_C|Getauto_skill_resource _array_element) _array_element_4) (Utilities|Struct|Makest_auto_skill_resource (.skill_model (Utilities|Struct|Breakst_auto_skill_resource _array_element_4)) (.Numberofuses (Utilities|Struct|Breakst_auto_skill_resource _array_element_4)) (+ (.point (Utilities|Struct|Breakst_auto_skill_resource _array_element_4)) (.Gainpoints (Utilities|Struct|Breakst_auto_skill _array_element_2)))))
                  (return))))
            (else
              (goto _label))))))))

(fn AutoskillCanUse
  (params (actiontype :type E_action_type%20Enum :default "NewEnumerator0") (pawn :type BP%20Base%20Pawn%20Class%20Object%20Reference) (target :type BP%20BASE%20UNIT%20Object%20Reference))
  (for _array_element (Variables|AC_skill_C|Getskill_array (Variables|/Game/BP/BP_modelE/BP_base_pawn_class.BP_base_pawn_class_C|GetAC_skill pawn))
    (for _array_element_2 (Variables|/Game/BP/BP_AC/BP_SKILL_AC/BP_skill_class.BP_skill_class_C|Getauto_skill _array_element)
      (if (and (Utilities|Enum|Equal(Enum) (.auto_skill_type (Utilities|Struct|Breakst_auto_skill _array_element_2)) (.skill_model (Utilities|Struct|Breakst_auto_skill_resource (stale _array_element)))) (Utilities|Enum|Equal(Enum) (.action_move_type (Utilities|Struct|Breakst_auto_skill _array_element_2)) actiontype)) ; 检查技能枚举和行动模式是否正确
        (if (and (>= (.point (Utilities|Struct|Breakst_auto_skill_resource (stale _array_element))) (.Consumepoints (Utilities|Struct|Breakst_auto_skill _array_element_2))) (>= (.Numberofuses (Utilities|Struct|Breakst_auto_skill_resource (stale _array_element))) 1)) ; 检查资源是否足够
          (if (== (Utilities|GetClass target) (.autoskill_target (Utilities|Struct|Breakst_auto_skill _array_element_2)))
            (return (.auto_skill_type (Utilities|Struct|Breakst_auto_skill _array_element_2)) (.skill_row_name (Utilities|Struct|Breakst_auto_skill _array_element_2)))))))))

(fn Useskillintegration
  (params (skill_model :type E_SKILL_model%20Enum :default "NewEnumerator0") (RowName :type Name) (skill_target :type Array%20of%20BP%20BASE%20UNIT%20Object%20References) (create :type BP%20Base%20Pawn%20Class%20Object%20Reference))
  (bind _skilldata (Useskill(R2)|UseSkillPublic skill_model RowName))
  (bind _returnvalue (Game|ConstructObjectfromClass (Utilities|Struct|BreakST_skill_Group_Assembly _skilldata)))
  (Default|SkillEffect _returnvalue skill_model skill_target create _skilldata)
  (Useskill(R1)|AfterUsingtheSkill RowName (Variables|Default|Getskill_model) create))

(fn UseSkillPublic
  (params (Selection :type E_SKILL_model%20Enum :default "NewEnumerator0") (RowName :type Name))
  (bind _returnvalue (Utilities|GetDataTableRow "/Game/Struct/ST_NEW_skill/T_skill_V2.T_skill_V2" RowName)
    (:then
      (Utilities|FlowControl|Sequence
        (:then_0
          (return _returnvalue))
        (:then_1
          (switch Utilities|FlowControl|Switch|SwitchonE_SKILL_model Selection
            (:NewEnumerator0
              (bind _returnvalue_2 (Game|ConstructObjectfromClass (Utilities|Struct|BreakST_skill_Group_Assembly _returnvalue)))
              (Default|SkillInitialize _returnvalue_2 (.skill_index (Utilities|Struct|Breakst_skill_Group_base_info (.技能组基本信息 (Utilities|Struct|BreakST_skill_Group_Assembly _returnvalue)))) (.skill_name (Utilities|Struct|Breakst_skill_Group_base_info (.技能组基本信息 (Utilities|Struct|BreakST_skill_Group_Assembly _returnvalue)))) (Utilities|Struct|Makest_Skills_Resources (.初始道具物 (Utilities|Struct|Breakst_skill_Group_resource (.技能资源 (Utilities|Struct|BreakST_skill_Group_Assembly _returnvalue)))) (.初始层数 (Utilities|Struct|Breakst_skill_Group_resource (.技能资源 (Utilities|Struct|BreakST_skill_Group_Assembly _returnvalue)))) (.初始点数 (Utilities|Struct|Breakst_skill_Group_resource (.技能资源 (Utilities|Struct|BreakST_skill_Group_Assembly _returnvalue)))) 3 3) RowName)
              (Default|SkillAutoInitialize _returnvalue_2 (.auto_skill (Utilities|Struct|BreakST_skill_Group_Assembly _returnvalue)))
              (Utilities|Array|Add (Variables|Default|Getskill_array) _returnvalue_2))
            (:NewEnumerator5
              (bind (_find _skill _index) (newsskill|在技能数组查找技能 (Variables|Default|Getskill_array) (.skill_index (Utilities|Struct|Breakst_skill_Group_base_info (Utilities|Struct|BreakST_skill_Group_Assembly _returnvalue)))))
              (Default|SkillInitialize _skill _index (.skill_name (Utilities|Struct|Breakst_skill_Group_base_info (Utilities|Struct|BreakST_skill_Group_Assembly _returnvalue))) (Utilities|Struct|Makest_Skills_Resources (+ (.SkillNumberOfActions (Utilities|Struct|Breakst_Skills_Resources (Variables|/Game/BP/BP_AC/BP_SKILL_AC/BP_skill_class.BP_skill_class_C|Getskill_resources _skill))) (.获得道具物 (Utilities|Struct|Breakst_skill_Group_resource (.技能资源 (Utilities|Struct|BreakST_skill_Group_Assembly _returnvalue))))) (+ (.stack (Utilities|Struct|Breakst_Skills_Resources (Variables|/Game/BP/BP_AC/BP_SKILL_AC/BP_skill_class.BP_skill_class_C|Getskill_resources _skill))) (.增加层数 (Utilities|Struct|Breakst_skill_Group_resource (.技能资源 (Utilities|Struct|BreakST_skill_Group_Assembly _returnvalue))))) (+ (.priority (Utilities|Struct|Breakst_Skills_Resources (Variables|/Game/BP/BP_AC/BP_SKILL_AC/BP_skill_class.BP_skill_class_C|Getskill_resources _skill))) (.增加点数 (Utilities|Struct|Breakst_skill_Group_resource (.技能资源 (Utilities|Struct|BreakST_skill_Group_Assembly _returnvalue))))) 5) RowName)
              (auto_skill|AutosskillRepeat RowName _skill))))))))