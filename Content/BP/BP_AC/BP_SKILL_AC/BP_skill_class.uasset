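; BP_skill_class is a skill class with initializers for identity, resources, auto-skill and countdown.
; Activation only prints debug messages, while CdTick and Cycle are empty stubs.
; TurnTick looks up T_skill_V2 by row name, calling Cycle and restoring CycleTime when CycleTime is at least Turntime.
; It then returns false only if Turntime is below DurationTurn and the skill is permanent, otherwise true.
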(fn Activation
  (params (create :type Actor%20Object%20Reference) (skilltager :type Actor%20Object%20Reference))
  (Development|PrintString create (Utilities|String|Append "角色" (Utilities|GetDisplayName create) "单位" (Utilities|GetDisplayName skilltager)) true true "(R=0.000000,G=0.660000,B=1.000000,A=1.000000)" 1e+02)
  (Development|PrintText 0 "这里是技能类、技能已经执行"))

(fn SkillInitialize
  (params (ID :type Integer) (skillname :type Name) (skill_resources :type St%20Skills%20Resources%20Structure) (auto_skill :type Array%20of%20St%20Auto%20Skill%20Structures) (rowname :type Name))
  (Variables|Default|SetID ID)
  (Variables|Default|SetSkillname skillname)
  (Variables|Resource|Setskill_resources skill_resources)
  (Variables|array|Setauto_skill auto_skill)
  (Variables|Default|Setrowname rowname))

(fn SkillInitializeCountDown
  (params (Skill%20Countdown :type Integer))
  (Variables|Default|SetSkill%20Countdown Skill%20Countdown))

(fn TurnTick
  (params (turntime :type Integer))
  (bind _returnvalue (Utilities|GetDataTableRow "/Game/Struct/ST_NEW_skill/T_skill_V2.T_skill_V2" (Variables|Default|Getrowname))
    (:then
      (Utilities|FlowControl|Sequence
        (:then_0
          (if (>= (- (.Cycletime (Utilities|Struct|Breakst_Skills_Resources (Variables|Resource|Getskill_resources))) turntime) 0)
            (CallFunction|Cycle)
            (Variables|Resource|Setskill_resources (Utilities|Struct|Makest_Skills_Resources (.SkillNumberOfActions (Utilities|Struct|Breakst_Skills_Resources (Variables|Resource|Getskill_resources))) (.stack (Utilities|Struct|Breakst_Skills_Resources (Variables|Resource|Getskill_resources))) (.priority (Utilities|Struct|Breakst_Skills_Resources (Variables|Resource|Getskill_resources))) (.duration_turn (Utilities|Struct|Breakst_Skills_Resources (Variables|Resource|Getskill_resources))) (Utilities|Struct|Breakst_skill_Group_resource (.技能资源 (Utilities|Struct|BreakST_skill_Group_Assembly _returnvalue)))))))
        (:then_1
          (if (>= (- turntime (.duration_turn (Utilities|Struct|Breakst_Skills_Resources (Variables|Resource|Getskill_resources)))) 0)
            (return true)
            (elif (Utilities|Struct|Breakst_skill_Group_boolset (.技能设置 (Utilities|Struct|BreakST_skill_Group_Assembly _returnvalue)))
              (return false)
              (else
                (return true)))))))))

(fn CdTick)

(fn Cycle)