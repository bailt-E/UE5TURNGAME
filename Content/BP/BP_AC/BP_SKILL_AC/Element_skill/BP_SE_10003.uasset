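; BP_SE_10003 is an element skill that deals multi-hit damage and spreads an element effect across grid units.
; Activation deals three-hit damage to units of one target type, running a simple element assertion on the whole target set for each unit hit.
; The assertion effect deals a single extra hit, gathers pawns from the target's cell and six surrounding offsets, then runs the element assertion on them as a different target type.
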(fn Activation
  (params (skill_model :type E_SKILL_model%20Enum :default "NewEnumerator0") (create :type BP%20BASE%20Pawn%20Object%20Reference) (skill%20target :type Array%20of%20St%20Select%20Unit%20Target%20Data%20Structures))
  (for _array_element skill%20target
    (if (Utilities|Enum|Equal(Enum) (.select_target_type (Utilities|Struct|Breakst_select_unit_target_data _array_element)) "NewEnumerator1")
      (for _array_element_2 (.unit (Utilities|Struct|Breakst_select_unit_target_data _array_element))
        (CallFunction|DamageE _array_element_2 create (Utilities|Array|MakeArray 60 80 120) 3 "NewEnumerator1" "NewEnumerator0" "NewEnumerator1")
        (CallFunction|SimpleElementAssertionAssembly skill%20target create "NewEnumerator1" "NewEnumerator1" "NewEnumerator0" "NewEnumerator0"))))
  (return true))

(fn SimpleElementAssertion(effect)
  (params (assertion_target :type BP%20BASE%20Pawn%20Object%20Reference) (assertion_create :type BP%20BASE%20Pawn%20Object%20Reference))
  (CallFunction|DamageE assertion_target assertion_create (Utilities|Array|MakeArray 100) 1 "NewEnumerator1" "NewEnumerator0" "NewEnumerator1")
  (bind _final_data (Default|CaculateDirectionYouCanWalkV2(actortoChear) (Variables|/Game/BP/BP_Battle_Phase/BP_BASE_Pawn.BP_BASE_Pawn_C|GetAs%20BP%20GLOBAL%20CHARATER assertion_target) (Transformation|GetActorLocation assertion_target) (Utilities|Array|MakeArray "(X=-0.000000,Y=-1.000000)" "(X=0.000000,Y=1.000000)" "(X=1.000000,Y=0.000000)" "(X=-1.000000,Y=0.000000)" "" "(X=-1.000000,Y=-1.000000)" "(X=1.000000,Y=1.000000)")))
  (for _array_element _final_data
    (bind _asbp_base_pawn (Utilities|Casting|CastToBP_BASE_Pawn _array_element))
    (Utilities|Array|Add (LocalVariables|Gettarget) _asbp_base_pawn))
  (if (not (Utilities|Array|IsEmpty (LocalVariables|Gettarget)))
    (Development|PrintString 0 "100")
    (CallFunction|SimpleElementAssertionAssembly (Utilities|Array|MakeArray (Utilities|Struct|Makest_select_unit_target_data "NewEnumerator3" (LocalVariables|Gettarget))) assertion_create "NewEnumerator3" "NewEnumerator1" "NewEnumerator0" "NewEnumerator0")))