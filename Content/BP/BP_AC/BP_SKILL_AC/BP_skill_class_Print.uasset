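; BP_skill_class_Print is a skill Blueprint that appears to be a debug or test skill, printing messages when activated.
; Activation casts the caster through BP_BASE_UNIT to BP_base_pawn_class and prints its Sdsd value with a caster-number label.
; If the skill target is valid, it prints "Hello" and destroys that actor.
; SkillCanUse is empty, and an unconnected DealDamageMessage call never runs.
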(fn Activation
  (params (create :type Actor%20Object%20Reference) (skilltager :type Actor%20Object%20Reference) (skill_effect :type BP%20Skilleffect%20Class%20Class%20Reference))
  (Utilities|FlowControl|Sequence
    (:then_0
      (bind _asbp_base_unit (Utilities|Casting|CastToBP_BASE_UNIT create))
      (bind _asbp_base_pawn_class (Utilities|Casting|CastToBP_base_pawn_class _asbp_base_unit))
      (Development|PrintString 0 (Utilities|String|Append "施法者数字" (Utilities|String|ToString(Integer) (Variables|/Game/BP/BP_modelE/BP_base_pawn_class.BP_base_pawn_class_C|Getsdsd _asbp_base_pawn_class)))))
    (:then_1
      (if (Utilities|IsValid skilltager)
        (Development|PrintText 0 "Hello")
        (Actor|DestroyActor skilltager)))))

(fn SkillCanUse)