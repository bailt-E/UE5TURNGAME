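; General level component that manages player chapter and level progression per difficulty.
; Initialization loads system chapters for the current chapter and game mode from T_System_Chapter, while save and load functions target the GameInstance's player array.
; Two battle-over variants mark difficulties passed and unlock the next; BattleOver1 then re-evaluates chapter completion and preface-chapter states.
; A separate check unlocks levels whose prerequisites are passed on Simple.
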(fn Initialization
  (bind _asbp_game_instance (Utilities|Casting|CastToBP_GameInstance (Game|GetGameInstance)))
  (Variables|Default|SetAs%20BP%20Game%20Instance _asbp_game_instance)
  (Variables|Default|Setsouce (Variables|/Game/gamemode/BP_GameInstance.BP_GameInstance_C|Getchapter_souce_array%28GI%29 (Variables|Default|GetAs%20BP%20Game%20Instance)))
  (for _array_element (Variables|Default|Getsouce)
    (if (and (== (.chapter_index (Utilities|Struct|Breakst_charpter_info (.chapter_index (Utilities|Struct|Breakst_chapter_souce _array_element)))) (Variables|A1|GetCurrent%20Chapter)) (Utilities|Enum|Equal(Enum) (.level_type (Utilities|Struct|Breakst_charpter_info (.chapter_index (Utilities|Struct|Breakst_chapter_souce _array_element)))) (Variables|A1|Getgame_mode)))
      (bind _returnvalue (Utilities|GetDataTableRow "/Game/Struct/st_new_level/T_System_Chapter.T_System_Chapter" (.chapter_rowname (Utilities|Struct|Breakst_chapter_souce _array_element)))
        (:then
          (Utilities|Array|Add (Variables|A1|GetSystem_chapter_level_data) _returnvalue))))))

(fn SAVELEVEL
  (for _array_element (Variables|/Game/gamemode/BP_GameInstance.BP_GameInstance_C|Getplayer_level_data%28GI%29 (Variables|Default|GetAs%20BP%20Game%20Instance))
    (if (and (== (.chapter_index (Utilities|Struct|Breakst_charpter_info (Utilities|Struct|Breakst_player_Chapter_N2_info _array_element))) (Variables|A1|GetCurrent%20Chapter)) (Utilities|Enum|Equal(Enum) (.level_type (Utilities|Struct|Breakst_charpter_info (Utilities|Struct|Breakst_player_Chapter_N2_info _array_element))) (Variables|A1|Getgame_mode)))
      (Utilities|Array|SetArrayElem :TargetArray (Variables|/Game/gamemode/BP_GameInstance.BP_GameInstance_C|Getplayer_level_data%28GI%29 (Variables|Default|GetAs%20BP%20Game%20Instance))))))

(fn LOADLEVEL
  (bind _as_bp_game_instance (Variables|Default|GetAs%20BP%20Game%20Instance))
  (bind _player_level_data_gi_ (Variables|/Game/gamemode/BP_GameInstance.BP_GameInstance_C|Getplayer_level_data%28GI%29 _as_bp_game_instance))
  (for _array_element _player_level_data_gi_
    (if (and (== (Variables|A1|GetCurrent%20Chapter) (.chapter_index (Utilities|Struct|Breakst_charpter_info (Utilities|Struct|Breakst_player_Chapter_N2_info _array_element)))) (Utilities|Enum|Equal(Enum) (.level_type (Utilities|Struct|Breakst_charpter_info (Utilities|Struct|Breakst_player_Chapter_N2_info _array_element))) (Variables|A1|Getgame_mode)))
      (Variables|Default|Setplayer_level_data _player_level_data_gi_))))

(fn BattleOver
  (params (charpter_levelX :type St%20System%20Level%20Info%20N2%20Structure) (battle_rusule :type E_battle_state_enum%20Enum :default "NewEnumerator0") (current_diff :type E_battle_Difficulty%20Enum :default "NewEnumerator0"))
  (bind _level_info (Utilities|Struct|Breakst_system_level_info_N2 charpter_levelX))
  (bind _level_info_2 (Utilities|Struct|Breakst_system_level_info_N2 charpter_levelX))
  (bind _returnvalue (Math|Conversions|ToInteger(Byte) current_diff))
  (bind (_level_index _branch) (Utilities|Struct|Breakst_level_base_info_N2 _level_info))
  (bind (_level_index_2 _branch_2) (Utilities|Struct|Breakst_level_base_info_N2 _level_info_2))
  (bind _returnvalue_2 (+ _returnvalue 1))
  (bind _returnvalue_3 (Math|Conversions|ToByte(Integer) _returnvalue_2))
  (bind _returnvalue_4 (Utilities|Enum|ByteToEnumE_battle_Difficulty _returnvalue_3))
  (Utilities|FlowControl|Sequence
    (:then_0
      (for _array_element (Variables|Default|Getplayer_level_data)
        (for _array_element_2 (Utilities|Struct|Breakst_player_Chapter_N2_info _array_element)
          (if (and (== (.level_index (Utilities|Struct|Breakst_level_base_info_N2 (.level_info (Utilities|Struct|Breakst_player_level _array_element_2)))) _level_index) (== (.Branch (Utilities|Struct|Breakst_level_base_info_N2 (.level_info (Utilities|Struct|Breakst_player_level _array_element_2)))) _branch))
            (for _array_element_3 (.level_state (Utilities|Struct|Breakst_player_level _array_element_2))
              (if (Utilities|Enum|Equal(Enum) (Utilities|Struct|Breakst_player_level_state _array_element_3) current_diff)
                (Utilities|Array|SetArrayElem (.level_state (Utilities|Struct|Breakst_player_level _array_element_2)) 0 (Utilities|Struct|Makest_player_level_state current_diff "NewEnumerator2"))))))))
    (:then_1
      (for _array_element_4 (Variables|A1|GetSystem_chapter_level_data)
        (for _array_element_5 (Utilities|Struct|BreakST_System_Chapter _array_element_4)
          (if (and (== _level_index_2 (.level_index (Utilities|Struct|Breakst_level_base_info_N2 (.level_info (Utilities|Struct|Breakst_system_level_info_N2 _array_element_5))))) (== _branch_2 (.Branch (Utilities|Struct|Breakst_level_base_info_N2 (.level_info (Utilities|Struct|Breakst_system_level_info_N2 _array_element_5)))))) ; 基于当前战斗的关卡和系统关卡进行匹配
            (for _array_element_6 (.level_battle_info (Utilities|Struct|Breakst_system_level_info_N2 _array_element_5))
              (if (Utilities|Enum|Equal(Enum) (.Difficulty (Utilities|Struct|Breakst_level_battle_info _array_element_6)) _returnvalue_4) ; 检查在当前的系统关卡是否存在下一难度
                (for _array_element_7 (Variables|Default|Getplayer_level_data)
                  (for _array_element_8 (Utilities|Struct|Breakst_player_Chapter_N2_info _array_element_7)
                    (if (and (== (.level_index (Utilities|Struct|Breakst_level_base_info_N2 (.level_info (Utilities|Struct|Breakst_player_level _array_element_8)))) (.level_index (Utilities|Struct|Breakst_level_base_info_N2 (.level_info (Utilities|Struct|Breakst_system_level_info_N2 _array_element_5))))) (== (.Branch (Utilities|Struct|Breakst_level_base_info_N2 (.level_info (Utilities|Struct|Breakst_player_level _array_element_8)))) (.Branch (Utilities|Struct|Breakst_level_base_info_N2 (.level_info (Utilities|Struct|Breakst_system_level_info_N2 _array_element_5))))))
                      (Utilities|Array|Add (.level_state (Utilities|Struct|Breakst_player_level _array_element_8)) (Utilities|Struct|Makest_player_level_state _returnvalue_4 "NewEnumerator1")))))))))))
    (:then_2
      (for _array_element_9 (Variables|A1|GetSystem_chapter_level_data)
        (for _array_element_10 (Utilities|Struct|BreakST_System_Chapter _array_element_9)
          (for _array_element_11 (.Preliminarylevel (Utilities|Struct|Breakst_system_level_info_N2 _array_element_10)) ; 循环所有关卡的前置关卡
            ;[1 1 1] 检查是所有系统关卡的前置关卡在角色关卡是否存在
            (for _array_element_12 (Variables|Default|Getplayer_level_data)
              (for _array_element_13 (Utilities|Struct|Breakst_player_Chapter_N2_info _array_element_12)
                (if (not (and (== (.level_index (Utilities|Struct|Breakst_level_base_info_N2 (.level_info (Utilities|Struct|Breakst_player_level _array_element_13)))) (.level_index (Utilities|Struct|Breakst_level_base_info_N2 _array_element_11))) (== (.Branch (Utilities|Struct|Breakst_level_base_info_N2 (.level_info (Utilities|Struct|Breakst_player_level _array_element_13)))) (.Branch (Utilities|Struct|Breakst_level_base_info_N2 _array_element_11)))))
                  (for _array_element_14 (.level_state (Utilities|Struct|Breakst_player_level _array_element_13))
                    (if (Utilities|Enum|Equal(Enum) (.level_diffculty (Utilities|Struct|Breakst_player_level_state _array_element_14)) "NewEnumerator0")
                      (for _array_element_15 (Variables|Default|Getplayer_level_data)
                        (Utilities|Array|Add (Utilities|Struct|Breakst_player_Chapter_N2_info _array_element_15) (Utilities|Struct|Makest_player_level (.level_info (Utilities|Struct|Breakst_system_level_info_N2 _array_element_10)) (Utilities|Array|MakeArray (Utilities|Struct|Makest_player_level_state (.level_diffculty (Utilities|Struct|Breakst_player_level_state _array_element_14)) "NewEnumerator1"))))))))))))))))

(fn SetPlayerFirstStageOpen)

(fn InitAllChapterStage
  (for _array_element (Variables|A1|GetSystem_chapter_level_data)
    (if (.InitialChapter (Utilities|Struct|BreakST_System_Chapter _array_element))
      (for _array_element_2 (.level_data (Utilities|Struct|BreakST_System_Chapter _array_element))
        (for _array_element_3 (.level_battle_info (Utilities|Struct|Breakst_system_level_info_N2 _array_element_2))
          (Utilities|Array|Add (Variables|Default|Getplayer_level_data) (Utilities|Struct|Makest_player_Chapter_N2_info (.charpter_info (Utilities|Struct|BreakST_System_Chapter _array_element)) "NewEnumerator0" (Utilities|Array|MakeArray (Utilities|Struct|Makest_player_level (.level_info (Utilities|Struct|Breakst_system_level_info_N2 _array_element_2)) (Utilities|Array|MakeArray (Utilities|Struct|Makest_player_level_state (.Difficulty (Utilities|Struct|Breakst_level_battle_info _array_element_3)) (.Initialstate (Utilities|Struct|Breakst_level_battle_info _array_element_3)))))))))))))

(fn BattleOver1
  (params (battle_rusule :type E_battle_state_enum%20Enum :default "NewEnumerator0") (st_player_level_info :type St%20Player%20Chapter%20Level%20Structure))
  (bind _charpter_index (Utilities|Struct|Breakst_player_chapter_level st_player_level_info))
  (bind _level_data (Utilities|Struct|Breakst_player_chapter_level st_player_level_info))
  (bind _level_diff (Utilities|Struct|Breakst_player_chapter_level st_player_level_info))
  (bind (_chapter_index _level_type) (Utilities|Struct|Breakst_charpter_info _charpter_index))
  (bind (_level_index _branch) (Utilities|Struct|Breakst_level_base_info_N2 _level_data))
  (bind _level_diffculty (Utilities|Struct|Breakst_player_level_state _level_diff))
  (bind _returnvalue (Math|Conversions|ToInteger(Byte) _level_diffculty))
  (bind _returnvalue_2 (+ _returnvalue 1))
  (bind _returnvalue_3 (Math|Conversions|ToByte(Integer) _returnvalue_2))
  (bind _returnvalue_4 (Utilities|Enum|ByteToEnumE_battle_Difficulty _returnvalue_3))
  (if (Utilities|Enum|Equal(Enum) battle_rusule "NewEnumerator0")
    (for _array_element (Variables|Default|Getplayer_level_data)
      (if (and (== _chapter_index (.chapter_index (Utilities|Struct|Breakst_charpter_info (.charpte_info (Utilities|Struct|Breakst_player_Chapter_N2_info _array_element))))) (Utilities|Enum|Equal(Enum) _level_type (.level_type (Utilities|Struct|Breakst_charpter_info (.charpte_info (Utilities|Struct|Breakst_player_Chapter_N2_info _array_element))))))
        (LocalVariables|Setplayer_info _array_element)
        (for _array_element_2 (.level (Utilities|Struct|Breakst_player_Chapter_N2_info _array_element))
          (if (and (== _level_index (.level_index (Utilities|Struct|Breakst_level_base_info_N2 (.level_info (Utilities|Struct|Breakst_player_level _array_element_2))))) (== _branch (.Branch (Utilities|Struct|Breakst_level_base_info_N2 (.level_info (Utilities|Struct|Breakst_player_level _array_element_2))))))
            (for _array_element_3 (.level_state (Utilities|Struct|Breakst_player_level _array_element_2))
              (if (Utilities|Enum|Equal(Enum) (Utilities|Struct|Breakst_player_level_state _array_element_3) _level_diffculty) ; 查找难度
                (Utilities|Array|Add (LocalVariables|Getdiff) (Utilities|Struct|Makest_player_level_state (Utilities|Struct|Breakst_player_level_state _array_element_3) "NewEnumerator2"))
                (elif (Utilities|Enum|Equal(Enum) (Utilities|Struct|Breakst_player_level_state _array_element_3) _returnvalue_4)
                  (Utilities|Array|Add (LocalVariables|Getdiff) (Utilities|Struct|Makest_player_level_state _returnvalue_4 "NewEnumerator1"))
                  (else
                    (Utilities|Array|Add (LocalVariables|Getdiff) _array_element_3)))))
            (Utilities|Array|SetArrayElem (.level (Utilities|Struct|Breakst_player_Chapter_N2_info _array_element)) 0 (Utilities|Struct|Makest_player_level (Utilities|Struct|Makest_level_base_info_N2 (.level_index (Utilities|Struct|Breakst_level_base_info_N2 (.level_info (Utilities|Struct|Breakst_player_level _array_element_2)))) (.Branch (Utilities|Struct|Breakst_level_base_info_N2 (.level_info (Utilities|Struct|Breakst_player_level _array_element_2)))) (.level_name (Utilities|Struct|Breakst_level_base_info_N2 (.level_info (Utilities|Struct|Breakst_player_level _array_element_2)))) "NewEnumerator2" (.level_type (Utilities|Struct|Breakst_level_base_info_N2 (.level_info (Utilities|Struct|Breakst_player_level _array_element_2))))) (LocalVariables|Getdiff)))
            (C1|ChearChapterLevelState (LocalVariables|Getplayer_info))
            (C1|ChearPlayerChapter)))))))

(fn FindLevel
  (params (index_system_level :type St%20System%20Level%20Info%20N2%20Structure%20%28by%20ref%29) (player_level_array :type Array%20of%20St%20Player%20Level%20Structures))
  (bind _level_info (Utilities|Struct|Breakst_system_level_info_N2 index_system_level))
  (bind (_level_index _branch) (Utilities|Struct|Breakst_level_base_info_N2 _level_info))
  (for _array_element player_level_array
    (if (and (== _level_index (.level_index (Utilities|Struct|Breakst_level_base_info_N2 (.level_info (Utilities|Struct|Breakst_player_level _array_element))))) (== _branch (.Branch (Utilities|Struct|Breakst_level_base_info_N2 (.level_info (Utilities|Struct|Breakst_player_level _array_element))))))
      (for _array_element_2 (.level_state (Utilities|Struct|Breakst_player_level _array_element))
        (if (Utilities|Enum|Equal(Enum) (.level_diffculty (Utilities|Struct|Breakst_player_level_state _array_element_2)) "NewEnumerator0")
          (return (.level_state (Utilities|Struct|Breakst_player_level _array_element)) (Utilities|Array|FindItem player_level_array _array_element) _array_element))))))

(fn CheckthePlayer'sLevelStatusAccordingtotheSystemLevel
  (params (NEEDlevel :type Array%20of%20St%20Level%20Base%20Info%20N2%20Structures) (chapter_info :type St%20Charpter%20Info%20Structure))
  (bind (_chapter_index _level_type) (Utilities|Struct|Breakst_charpter_info chapter_info))
  (for _array_element (Variables|Default|Getplayer_level_data)
    (if (and (== _chapter_index (.chapter_index (Utilities|Struct|Breakst_charpter_info (.charpte_info (Utilities|Struct|Breakst_player_Chapter_N2_info _array_element))))) (Utilities|Enum|Equal(Enum) _level_type (.level_type (Utilities|Struct|Breakst_charpter_info (.charpte_info (Utilities|Struct|Breakst_player_Chapter_N2_info _array_element))))))
      (for _array_element_2 (.level (Utilities|Struct|Breakst_player_Chapter_N2_info _array_element))
        (for _array_element_3 NEEDlevel
          (if (and (== (.level_index (Utilities|Struct|Breakst_level_base_info_N2 _array_element_3)) (.level_index (Utilities|Struct|Breakst_level_base_info_N2 (.level_info (Utilities|Struct|Breakst_player_level _array_element_2))))) (== (.Branch (Utilities|Struct|Breakst_level_base_info_N2 _array_element_3)) (.Branch (Utilities|Struct|Breakst_level_base_info_N2 (.level_info (Utilities|Struct|Breakst_player_level _array_element_2))))))
            (for _array_element_4 (.level_state (Utilities|Struct|Breakst_player_level _array_element_2))
              (if (and (Utilities|Enum|Equal(Enum) (.level_diffculty (Utilities|Struct|Breakst_player_level_state _array_element_4)) "NewEnumerator0") (Utilities|Enum|Equal(Enum) (.level_state (Utilities|Struct|Breakst_player_level_state _array_element_4)) "NewEnumerator2"))
                (LocalVariables|Setint (+ (LocalVariables|Getint) 1)))))))))
  (return (LocalVariables|Getint)))

(fn ChearPlayerLevel
  (for _array_element (Variables|A1|GetSystem_chapter_level_data)
    (for _array_element_2 (.level_data (Utilities|Struct|BreakST_System_Chapter _array_element))
      (bind _int1 (E1|CheckthePlayer'sLevelStatusAccordingtotheSystemLevel (Utilities|Struct|Breakst_system_level_info_N2 _array_element_2) (.charpter_info (Utilities|Struct|BreakST_System_Chapter _array_element))))
      (if (== _int1 (Utilities|Array|Length (Utilities|Struct|Breakst_system_level_info_N2 _array_element_2))) ; 前置关卡数量是否符合
        (for _array_element_3 (Variables|Default|Getplayer_level_data)
          (if (and (== (.chapter_index (Utilities|Struct|Breakst_charpter_info (.charpter_info (Utilities|Struct|BreakST_System_Chapter _array_element)))) (.chapter_index (Utilities|Struct|Breakst_charpter_info (.charpte_info (Utilities|Struct|Breakst_player_Chapter_N2_info _array_element_3))))) (Utilities|Enum|Equal(Enum) (.level_type (Utilities|Struct|Breakst_charpter_info (.charpter_info (Utilities|Struct|BreakST_System_Chapter _array_element)))) (.level_type (Utilities|Struct|Breakst_charpter_info (.charpte_info (Utilities|Struct|Breakst_player_Chapter_N2_info _array_element_3))))))
            (for (_array_element_4 _array_index) (.level (Utilities|Struct|Breakst_player_Chapter_N2_info _array_element_3))
              (if (and (== (.level_index (Utilities|Struct|Breakst_level_base_info_N2 (Utilities|Struct|Breakst_player_level _array_element_4))) (.level_index (Utilities|Struct|Breakst_level_base_info_N2 (Utilities|Struct|Breakst_system_level_info_N2 _array_element_2)))) (== (.Branch (Utilities|Struct|Breakst_level_base_info_N2 (Utilities|Struct|Breakst_player_level _array_element_4))) (.Branch (Utilities|Struct|Breakst_level_base_info_N2 (Utilities|Struct|Breakst_system_level_info_N2 _array_element_2)))))
                (LocalVariables|Setlevel_info (Utilities|Struct|Makest_level_base_info_N2 (.level_index (Utilities|Struct|Breakst_level_base_info_N2 (.level_info (Utilities|Struct|Breakst_player_level _array_element_4)))) (.Branch (Utilities|Struct|Breakst_level_base_info_N2 (.level_info (Utilities|Struct|Breakst_player_level _array_element_4)))) (.level_name (Utilities|Struct|Breakst_level_base_info_N2 (.level_info (Utilities|Struct|Breakst_player_level _array_element_4)))) "NewEnumerator1" (.level_type (Utilities|Struct|Breakst_level_base_info_N2 (.level_info (Utilities|Struct|Breakst_player_level _array_element_4))))))
                (for _array_element_5 (.level_state (Utilities|Struct|Breakst_player_level _array_element_4))
                  (if (Utilities|Enum|Equal(Enum) (.level_diffculty (Utilities|Struct|Breakst_player_level_state _array_element_5)) "NewEnumerator0")
                    (Utilities|Array|Add (LocalVariables|Getlevel_state) (Utilities|Struct|Makest_player_level_state "NewEnumerator0" "NewEnumerator1"))
                    (else
                      (Utilities|Array|Add (LocalVariables|Getlevel_state) _array_element_5))))))
            (Utilities|Array|SetArrayElem (.level (Utilities|Struct|Breakst_player_Chapter_N2_info _array_element_3)) _array_index (Utilities|Struct|Makest_player_level (LocalVariables|Getlevel_info) (LocalVariables|Getlevel_state)))
            (LocalVariables|Setlevel_info "")
            (Utilities|Array|Clear (LocalVariables|Getlevel_state))))))))

(fn ChearChapterLevelState
  (params (player_chapter_info :type St%20Player%20Chapter%20N2%20Info%20Structure))
  (bind _charpte_info (Utilities|Struct|Breakst_player_Chapter_N2_info player_chapter_info))
  (bind (_chapter_index _level_type) (Utilities|Struct|Breakst_charpter_info _charpte_info))
  (for (_array_element _array_index) (Variables|Default|Getplayer_level_data)
    (if (and (== _chapter_index (.chapter_index (Utilities|Struct|Breakst_charpter_info (.charpte_info (Utilities|Struct|Breakst_player_Chapter_N2_info _array_element))))) (Utilities|Enum|Equal(Enum) _level_type (.level_type (Utilities|Struct|Breakst_charpter_info (.charpte_info (Utilities|Struct|Breakst_player_Chapter_N2_info _array_element))))))
      (for _array_element_2 (.level (Utilities|Struct|Breakst_player_Chapter_N2_info _array_element))
        (if (Utilities|Enum|Equal(Enum) (Utilities|Struct|Breakst_level_base_info_N2 (.level_info (Utilities|Struct|Breakst_player_level _array_element_2))) "NewEnumerator2")
          (LocalVariables|Setlevel_pass_cont (+ (LocalVariables|Getlevel_pass_cont) 1))))
      (if (== (LocalVariables|Getlevel_pass_cont) (Utilities|Array|Length (.level (Utilities|Struct|Breakst_player_Chapter_N2_info _array_element))))
        (Utilities|Array|SetArrayElem (Variables|Default|Getplayer_level_data) _array_index (Utilities|Struct|Makest_player_Chapter_N2_info (.charpte_info (Utilities|Struct|Breakst_player_Chapter_N2_info _array_element)) "NewEnumerator1" (.level (Utilities|Struct|Breakst_player_Chapter_N2_info _array_element))))))))

(fn ChearPlayerChapter
  (for _array_element (Variables|A1|GetSystem_chapter_level_data)
    (for (_array_element_2 _array_index) (Variables|Default|Getplayer_level_data)
      (if (and (== (.chapter_index (Utilities|Struct|Breakst_charpter_info (.charpte_info (Utilities|Struct|Breakst_player_Chapter_N2_info _array_element_2)))) (.chapter_index (Utilities|Struct|Breakst_charpter_info (Utilities|Struct|BreakST_System_Chapter _array_element)))) (Utilities|Enum|Equal(Enum) (.level_type (Utilities|Struct|Breakst_charpter_info (.charpte_info (Utilities|Struct|Breakst_player_Chapter_N2_info _array_element_2)))) (.level_type (Utilities|Struct|Breakst_charpter_info (Utilities|Struct|BreakST_System_Chapter _array_element)))))
        (if (Utilities|Enum|Equal(Enum) (.charpte_state (Utilities|Struct|Breakst_player_Chapter_N2_info _array_element_2)) "NewEnumerator1")
          (Utilities|Array|SetArrayElem (Variables|Default|Getplayer_level_data) _array_index (Utilities|Struct|Makest_player_Chapter_N2_info (.charpte_info (Utilities|Struct|Breakst_player_Chapter_N2_info _array_element_2)) "NewEnumerator0" (.level (Utilities|Struct|Breakst_player_Chapter_N2_info _array_element_2)))))))))