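; Player character data object that holds one character's record: info, modules, normal and finisher skills, level and favorability.
; Two initializers build that record with starting skill, module and favorability defaults: R0 takes a data struct and looks up the level in T_character_level_data, while R2 reads a data asset and starts at level 1.
; save_character_data overwrites the stored data, voice, skills, 3D mesh and level.
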(fn CharacterInitializationR0
  (params (character_data%28NG%29 :type ST%20Character%20Library%20Structure) (levelX :type Name) (role_rowname%28NG%29 :type Name))
  (bind (_character_module _character_rand_item_demand _skill_data _finsher_skill_) (Utilities|Struct|BreakST_Character_library character_data%28NG%29))
  (bind _character_index (Utilities|Struct|BreakST_Character_library character_data%28NG%29))
  (bind (_rowname _character_index_2 _character_name _character_rarity _occupation _elementtype _characterfaction _character_standingillustration _characteravatar) (Utilities|Struct|Breakst_character_info _character_index))
  (Variables|NDATA|Setlevel levelX)
  (LocalVariables|SetTEMP_charaacter_index (Utilities|Struct|Makest_character_info (Utilities|Struct|Breakst_character_info (Utilities|Struct|BreakST_Character_library character_data%28NG%29)) _character_index_2 _character_name _character_rarity _occupation _elementtype _characterfaction _character_standingillustration _characteravatar))
  (for _array_element _character_module
    (Utilities|Array|Add (LocalVariables|Getmodule) (Utilities|Struct|Makest_pawn_module (.Module_Index (Utilities|Struct|Breakst_character_Module _array_element)) (.Module_name (Utilities|Struct|Breakst_character_Module _array_element)))))
  (for _array_element_2 _skill_data
    (Utilities|Array|Add (LocalVariables|Getskill_N) (Utilities|Struct|Makest_character_skill (LocalVariables|Getskill_index) (.skill_type (Utilities|Struct|Breakst_role_skill _array_element_2)) (.skill_id (Utilities|Struct|Breakst_role_skill _array_element_2)) 1 true))
    (LocalVariables|Setskill_index (+ (LocalVariables|Getskill_index) 1)))
  (for _array_element_3 _finsher_skill_
    (Utilities|Array|Add (LocalVariables|GetSKILL_F) (Utilities|Struct|Makest_character_skill (.finsher_skill_index (Utilities|Struct|Breakst_Finisher _array_element_3)) "NewEnumerator1" (.rowname (Utilities|Struct|Breakst_Finisher _array_element_3)) 1 (.Unlockedstatus (Utilities|Struct|Breakst_Finisher _array_element_3)))))
  (bind _returnvalue (Utilities|GetDataTableRow "/Game/Struct/rank_table/T_character_level_data.T_character_level_data" levelX) ; 基于真实等级确定等级和阶段
    (:then
      (Variables|FIX_data|Setcharacter_data (Utilities|Struct|Makest_player_character_data (LocalVariables|GetTEMP_charaacter_index) (LocalVariables|Getmodule) (Utilities|Struct|Makest_character_level_data (.rank (Utilities|Struct|Breakst_character_bese_level_data _returnvalue)) (.level (Utilities|Struct|Breakst_character_bese_level_data _returnvalue)) (.need_xp (Utilities|Struct|Breakst_character_bese_level_data _returnvalue))) 1 (Utilities|Struct|Makest_character_skill_Assembly 1 (LocalVariables|Getskill_N) (LocalVariables|GetSKILL_F)) (Utilities|Struct|Makest_character_Favorability "NewEnumerator0" 20 false)))
      (return))))

(fn SaveCharacterData
  (params (character_data :type St%20Player%20Character%20Data%20Structure) (voice :type Array%20of%20St%20Character%20Voice%20Data%20Structures) (skill_data :type Array%20of%20St%20Role%20Skill%20Structures) (finish_skill :type Array%20of%20St%20Finisher%20Structures) (3D :type Skeletal%20Mesh%20Object%20Reference) (level :type Name))
  (Variables|FIX_data|Setcharacter_data character_data)
  (Variables|NDATA|Setvoice voice)
  (Variables|FIX_data|SetSkill%20Data skill_data)
  (Variables|FIX_data|SetFinish%20Skill finish_skill)
  (Variables|NDATA|Set3Dmesh 3D)
  (Variables|NDATA|Setlevel level))

(fn CharacterInitializationR2
  (params (Data_Asset :type DA%20Character%20Object%20Reference))
  (bind _output_get (Variables|Default|SetCharacter_Data_Asset Data_Asset))
  (LocalVariables|SetTEMP_charaacter_index (Utilities|Struct|Makest_character_info (Utilities|Struct|Breakst_character_info (Variables|/Game/Data_Asset/character_data_Asset/DA_character.DA_character_C|Getcharacter_base_info (Variables|Default|GetCharacter_Data_Asset))) (.character_index (Utilities|Struct|Breakst_character_info (Variables|/Game/Data_Asset/character_data_Asset/DA_character.DA_character_C|Getcharacter_base_info _output_get))) (.character_name (Utilities|Struct|Breakst_character_info (Variables|/Game/Data_Asset/character_data_Asset/DA_character.DA_character_C|Getcharacter_base_info _output_get))) (.character_Rarity (Utilities|Struct|Breakst_character_info (Variables|/Game/Data_Asset/character_data_Asset/DA_character.DA_character_C|Getcharacter_base_info _output_get))) (.occupation (Utilities|Struct|Breakst_character_info (Variables|/Game/Data_Asset/character_data_Asset/DA_character.DA_character_C|Getcharacter_base_info _output_get))) (.elementtype (Utilities|Struct|Breakst_character_info (Variables|/Game/Data_Asset/character_data_Asset/DA_character.DA_character_C|Getcharacter_base_info _output_get))) (.characterfaction (Utilities|Struct|Breakst_character_info (Variables|/Game/Data_Asset/character_data_Asset/DA_character.DA_character_C|Getcharacter_base_info _output_get))) (.character_Standingillustration (Utilities|Struct|Breakst_character_info (Variables|/Game/Data_Asset/character_data_Asset/DA_character.DA_character_C|Getcharacter_base_info _output_get))) (.CharacterAvatar (Utilities|Struct|Breakst_character_info (Variables|/Game/Data_Asset/character_data_Asset/DA_character.DA_character_C|Getcharacter_base_info _output_get)))))
  (for _array_element (Variables|/Game/Data_Asset/character_data_Asset/DA_character.DA_character_C|Getmodule (Variables|Default|GetCharacter_Data_Asset))
    (Utilities|Array|Add (LocalVariables|Getmodule) (Utilities|Struct|Makest_pawn_module (.Module_Index (Utilities|Struct|Breakst_character_Module _array_element)) (.Module_name (Utilities|Struct|Breakst_character_Module _array_element)))))
  (for _array_element_2 (Variables|/Game/Data_Asset/character_data_Asset/DA_character.DA_character_C|Getskill_data (Variables|Default|GetCharacter_Data_Asset))
    (Utilities|Array|Add (LocalVariables|Getskill_N) (Utilities|Struct|Makest_character_skill (LocalVariables|Getskill_index) (.skill_type (Utilities|Struct|Breakst_role_skill _array_element_2)) (.skill_id (Utilities|Struct|Breakst_role_skill _array_element_2)) 1 true))
    (LocalVariables|Setskill_index (+ (LocalVariables|Getskill_index) 1)))
  (for _array_element_3 (Variables|/Game/Data_Asset/character_data_Asset/DA_character.DA_character_C|Getfinish_skill (Variables|Default|GetCharacter_Data_Asset))
    (Utilities|Array|Add (LocalVariables|GetSKILL_F) (Utilities|Struct|Makest_character_skill (.finsher_skill_index (Utilities|Struct|Breakst_Finisher _array_element_3)) "NewEnumerator1" (.rowname (Utilities|Struct|Breakst_Finisher _array_element_3)) 1 (.Unlockedstatus (Utilities|Struct|Breakst_Finisher _array_element_3)))))
  (Variables|FIX_data|Setcharacter_data (Utilities|Struct|Makest_player_character_data (LocalVariables|GetTEMP_charaacter_index) (LocalVariables|Getmodule) (Utilities|Struct|Makest_character_level_data 1 1) 1 (Utilities|Struct|Makest_character_skill_Assembly 1 (LocalVariables|Getskill_N) (LocalVariables|GetSKILL_F)) (Utilities|Struct|Makest_character_Favorability "NewEnumerator0" 20 false)))
  (return))