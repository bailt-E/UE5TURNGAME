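; Player-controller component that manages the player's character roster and progression: acquiring characters, leveling, rank promotion checks, skill and module upgrades, and upgrade item accounting.
; Data tables drive requirements and EXP costs, with each rank mapping to a row range in the level table.
; Most helpers return modified struct copies; auto level-up loops while EXP suffices, then saves into the BP_character_object roster by row name.
; The finisher-skill upgrade check is a stub returning false.
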(event EventBeginPlay)

(event EventTick
  (params (DeltaSeconds :type Float%20%28single-precision%29)))

(fn GetItem
  (params (player_item :type Array%20of%20St%20Inventory%20Number%20Structures) (item_number :type Integer) (ITEM_rowname :type Name))
  (LocalVariables|Setthe_player_item player_item)
  (bind _returnvalue (Utilities|GetDataTableRow "/Game/Struct/Inventory_system/T_inventory_table.T_inventory_table" ITEM_rowname)
    (:then
      (for _array_element (LocalVariables|Getthe_player_item)
        (if (Math|Boolean|ANDBoolean (== (.Inventory_name (Utilities|Struct|BreakST_Inventory_base_info _returnvalue)) (.Inventory_name (Utilities|Struct|BreakST_Inventory_lite_info (.inventory_info (Utilities|Struct|Breakst_inventory_number _array_element))))) (== (.Inventory_index (Utilities|Struct|BreakST_Inventory_base_info _returnvalue)) (.Inventory_index (Utilities|Struct|BreakST_Inventory_lite_info (.inventory_info (Utilities|Struct|Breakst_inventory_number _array_element))))) (Utilities|Enum|Equal(Enum) (.Inventory_type (Utilities|Struct|BreakST_Inventory_base_info _returnvalue)) (.Inventory_type (Utilities|Struct|BreakST_Inventory_lite_info (.inventory_info (Utilities|Struct|Breakst_inventory_number _array_element)))))) ; 在角色中是否存在
          (if (<= (.maximum (Utilities|Struct|BreakST_Inventory_base_info _returnvalue)) (+ (.number (Utilities|Struct|Breakst_inventory_number _array_element)) item_number)) ; 获得数量是否大于最大值
            (Utilities|Array|SetArrayElem (LocalVariables|Getthe_player_item) 0 (Utilities|Struct|Makest_inventory_number (Utilities|Struct|MakeST_Inventory_lite_info (.Inventory_name (Utilities|Struct|BreakST_Inventory_base_info _returnvalue)) ITEM_rowname (.Inventory_index (Utilities|Struct|BreakST_Inventory_base_info _returnvalue)) (.Inventory_type (Utilities|Struct|BreakST_Inventory_base_info _returnvalue))) item_number))
            (else
              (Utilities|Array|Add (LocalVariables|Getthe_player_item) (Utilities|Struct|Makest_inventory_number (Utilities|Struct|MakeST_Inventory_lite_info (.Inventory_name (Utilities|Struct|BreakST_Inventory_lite_info (.inventory_info (Utilities|Struct|Breakst_inventory_number _array_element)))) (.rowname (Utilities|Struct|BreakST_Inventory_lite_info (.inventory_info (Utilities|Struct|Breakst_inventory_number _array_element)))) (.Inventory_index (Utilities|Struct|BreakST_Inventory_lite_info (.inventory_info (Utilities|Struct|Breakst_inventory_number _array_element)))) (.Inventory_type (Utilities|Struct|BreakST_Inventory_lite_info (.inventory_info (Utilities|Struct|Breakst_inventory_number _array_element))))) 1) :!label _label)))
          (else
            (goto _label))))
      (return (LocalVariables|Getthe_player_item)))))

(fn FilterCharacterMaterials
  (params (inventory_type :type E_Inventory_TYPE%20Enum :default "NewEnumerator0") (player_item :type Array%20of%20St%20Inventory%20Number%20Structures))
  (for _array_element player_item
    (if (Utilities|Enum|Equal(Enum) (Utilities|Struct|BreakST_Inventory_lite_info (Utilities|Struct|Breakst_inventory_number _array_element)) inventory_type)
      (Utilities|Array|Add (LocalVariables|GetFilter_item) _array_element)))
  (return (LocalVariables|GetFilter_item)))

(fn ChearItemIsEnought
  (params (need_item :type Array%20of%20St%20Inventory%20Number%20Structures) (player_array :type Array%20of%20St%20Inventory%20Number%20Structures))
  (for _array_element need_item
    (for _array_element_2 player_array
      (if (Math|Boolean|ANDBoolean (== (.Inventory_name (Utilities|Struct|BreakST_Inventory_lite_info (.inventory_info (Utilities|Struct|Breakst_inventory_number _array_element_2)))) (.Inventory_name (Utilities|Struct|BreakST_Inventory_lite_info (.inventory_info (Utilities|Struct|Breakst_inventory_number _array_element))))) (== (.Inventory_index (Utilities|Struct|BreakST_Inventory_lite_info (.inventory_info (Utilities|Struct|Breakst_inventory_number _array_element_2)))) (.Inventory_index (Utilities|Struct|BreakST_Inventory_lite_info (.inventory_info (Utilities|Struct|Breakst_inventory_number _array_element))))) (Utilities|Enum|Equal(Enum) (.Inventory_type (Utilities|Struct|BreakST_Inventory_lite_info (.inventory_info (Utilities|Struct|Breakst_inventory_number _array_element_2)))) (.Inventory_type (Utilities|Struct|BreakST_Inventory_lite_info (.inventory_info (Utilities|Struct|Breakst_inventory_number _array_element))))))
        (Utilities|Array|Add (LocalVariables|Getcount_item) (Utilities|Struct|Makest_inventory_number (.inventory_info (Utilities|Struct|Breakst_inventory_number _array_element_2)) (.number (Utilities|Struct|Breakst_inventory_number _array_element_2)) (.need_number (Utilities|Struct|Breakst_inventory_number _array_element))))
        (else
          (Utilities|Array|Add (LocalVariables|Getcount_item) (Utilities|Struct|Makest_inventory_number (.inventory_info (Utilities|Struct|Breakst_inventory_number _array_element_2)) 0 (.need_number (Utilities|Struct|Breakst_inventory_number _array_element))))))))
  (for _array_element_3 (LocalVariables|Getcount_item)
    (if (not (>= (.number (Utilities|Struct|Breakst_inventory_number _array_element_3)) (.need_number (Utilities|Struct|Breakst_inventory_number _array_element_3))))
      (LocalVariables|Setitem_enought false)))
  (return (LocalVariables|Getcount_item) (LocalVariables|Getitem_enought)))

(fn ReduceItem
  (params (item_listx :type Array%20of%20St%20Inventory%20Number%20Structures) (player_itemx :type Array%20of%20St%20Inventory%20Number%20Structures))
  (for _array_element item_listx
    (for _array_element_2 player_itemx
      (if (Math|Boolean|ANDBoolean (== (.Inventory_name (Utilities|Struct|BreakST_Inventory_lite_info (.inventory_info (Utilities|Struct|Breakst_inventory_number _array_element)))) (.Inventory_name (Utilities|Struct|BreakST_Inventory_lite_info (.inventory_info (Utilities|Struct|Breakst_inventory_number _array_element_2))))) (== (.Inventory_index (Utilities|Struct|BreakST_Inventory_lite_info (.inventory_info (Utilities|Struct|Breakst_inventory_number _array_element)))) (.Inventory_index (Utilities|Struct|BreakST_Inventory_lite_info (.inventory_info (Utilities|Struct|Breakst_inventory_number _array_element_2))))) (Utilities|Enum|Equal(Enum) (.Inventory_type (Utilities|Struct|BreakST_Inventory_lite_info (.inventory_info (Utilities|Struct|Breakst_inventory_number _array_element)))) (.Inventory_type (Utilities|Struct|BreakST_Inventory_lite_info (.inventory_info (Utilities|Struct|Breakst_inventory_number _array_element_2))))))
        (Utilities|Array|SetArrayElem player_itemx 0 (Utilities|Struct|Makest_inventory_number (.inventory_info (Utilities|Struct|Breakst_inventory_number _array_element_2)) (- (.number (Utilities|Struct|Breakst_inventory_number _array_element_2)) (.number (Utilities|Struct|Breakst_inventory_number _array_element))))))))
  (return player_itemx))

(fn SetPlayerItem
  (params (item_list :type Array%20of%20St%20Inventory%20Number%20Structures) (GI :type BP%20Game%20Instance%20Object%20Reference))
  (for _array_element item_list
    (for _array_element_2 (Variables|/Game/gamemode/BP_GameInstance.BP_GameInstance_C|Getplayer_item GI)
      (if (Math|Boolean|ANDBoolean (== (.Inventory_name (Utilities|Struct|BreakST_Inventory_lite_info (.inventory_info (Utilities|Struct|Breakst_inventory_number _array_element)))) (.Inventory_name (Utilities|Struct|BreakST_Inventory_lite_info (.inventory_info (Utilities|Struct|Breakst_inventory_number _array_element_2))))) (== (.Inventory_index (Utilities|Struct|BreakST_Inventory_lite_info (.inventory_info (Utilities|Struct|Breakst_inventory_number _array_element)))) (.Inventory_index (Utilities|Struct|BreakST_Inventory_lite_info (.inventory_info (Utilities|Struct|Breakst_inventory_number _array_element_2))))) (Utilities|Enum|Equal(Enum) (.Inventory_type (Utilities|Struct|BreakST_Inventory_lite_info (.inventory_info (Utilities|Struct|Breakst_inventory_number _array_element)))) (.Inventory_type (Utilities|Struct|BreakST_Inventory_lite_info (.inventory_info (Utilities|Struct|Breakst_inventory_number _array_element_2))))))
        (Utilities|Array|SetArrayElem (Variables|/Game/gamemode/BP_GameInstance.BP_GameInstance_C|Getplayer_item GI) 0 (Utilities|Struct|Makest_inventory_number (.inventory_info (Utilities|Struct|Breakst_inventory_number _array_element)) (.number (Utilities|Struct|Breakst_inventory_number _array_element)) (.need_number (Utilities|Struct|Breakst_inventory_number _array_element))))))))

(fn CoverRole
  (params (player_character :type Array%20of%20St%20Player%20Character%20Data%20Structures) (select_character :type St%20Player%20Character%20Data%20Structure))
  (bind (_character_info _module_info _level _default_finishing _character_skill_data _favorability) (Utilities|Struct|Breakst_player_character_data select_character))
  (bind _character_info_2 (Utilities|Struct|Breakst_player_character_data select_character))
  (bind (_rowname _character_index _character_name) (Utilities|Struct|Breakst_character_info _character_info_2))
  (bind _output_get (LocalVariables|Setcharacteter player_character))
  (for _array_element _output_get
    (if (Math|Boolean|ANDBoolean (== (.rowname (Utilities|Struct|Breakst_character_info (Utilities|Struct|Breakst_player_character_data _array_element))) _rowname) (== (.character_index (Utilities|Struct|Breakst_character_info (Utilities|Struct|Breakst_player_character_data _array_element))) _character_index) (== (.character_name (Utilities|Struct|Breakst_character_info (Utilities|Struct|Breakst_player_character_data _array_element))) _character_name))
      (Utilities|Array|SetArrayElem (LocalVariables|Getcharacteter) 0 (Utilities|Struct|Makest_player_character_data _character_info _module_info _level _default_finishing _character_skill_data _favorability))))
  (return (LocalVariables|Getcharacteter)))

(fn UpdataCharacterLevel
  (params (rand :type Integer) (level :type Integer) (curent_level_exp :type Integer))
  (bind _输出行 (level_GE|GetTureLevel rand level))
  (bind _output_get (LocalVariables|Setcharacter_level (Utilities|Struct|Makest_character_level_data rand (+ level 1) curent_level_exp (Utilities|Struct|Breakst_character_bese_level_data _输出行))))
  (return _output_get))

(fn GetStateLocat
  (params (Selection :type Integer))
  (switch int Selection
    (:0
      (bind _returnvalue (Utilities|GetDataTableRow "/Game/Struct/common_Character_data/T_characer_rank_level_max.T_characer_rank_level_max" "rand0")
        (:then
          (return _returnvalue))))
    (:1
      (bind _returnvalue_2 (Utilities|GetDataTableRow "/Game/Struct/common_Character_data/T_characer_rank_level_max.T_characer_rank_level_max" "rand1")
        (:then
          (return _returnvalue_2))))
    (:2
      (bind _returnvalue_3 (Utilities|GetDataTableRow "/Game/Struct/common_Character_data/T_characer_rank_level_max.T_characer_rank_level_max" "rand2")
        (:then
          (return _returnvalue_3))))
    (:3
      (bind _returnvalue_4 (Utilities|GetDataTableRow "/Game/Struct/common_Character_data/T_characer_rank_level_max.T_characer_rank_level_max" "rand3")
        (:then
          (return _returnvalue_4))))))

(fn GetTureLevel
  (params (rand :type Integer) (level :type Integer))
  (bind _out_data (level_GE|GetStateLocat rand))
  (for _index (range (+ level (.Initial (Utilities|Struct|Breakst_character_rank_info _out_data))) (.End (Utilities|Struct|Breakst_character_rank_info _out_data)))
    (bind _returnvalue (Utilities|GetDataTableRow "/Game/Struct/rank_table/T_character_level_data.T_character_level_data" (Utilities|String|StringToName (Utilities|String|ToString(Integer) _index)))
      (:then
        (return _returnvalue (Utilities|String|StringToName (Utilities|String|ToString(Integer) _index)))))))

(fn ComputationalEmpiricalObject
  (params (item :type Array%20of%20St%20Inventory%20Number%20Structures))
  (for _array_element item
    (bind _returnvalue (Utilities|GetDataTableRow "/Game/Struct/Inventory_system/T_inventory_table.T_inventory_table" (Utilities|Struct|BreakST_Inventory_lite_info (.inventory_info (Utilities|Struct|Breakst_inventory_number _array_element))))
      (:then
        (LocalVariables|Setexp (+ (* (Utilities|Struct|BreakST_Inventory_base_info _returnvalue) (.number (Utilities|Struct|Breakst_inventory_number _array_element))) (LocalVariables|Getexp))))))
  (return (LocalVariables|Getexp)))

(fn CharacterLevelUp
  (params (data :type St%20Player%20Character%20Data%20Structure%20%28by%20ref%29))
  (LocalVariables|Setcharacter_data data)
  (bind _输出行 (level_GE|GetTureLevel (.level_rand (Utilities|Struct|Breakst_character_level_data (Utilities|Struct|Breakst_player_character_data (LocalVariables|Getcharacter_data)))) (+ (.level (Utilities|Struct|Breakst_character_level_data (Utilities|Struct|Breakst_player_character_data (LocalVariables|Getcharacter_data)))) 1)))
  (bind _output_get (LocalVariables|Setcharacter_data (Utilities|Struct|Makest_player_character_data (.character_info (Utilities|Struct|Breakst_player_character_data (LocalVariables|Getcharacter_data))) (.module_info (Utilities|Struct|Breakst_player_character_data (LocalVariables|Getcharacter_data))) (Utilities|Struct|Makest_character_level_data (.level_rand (Utilities|Struct|Breakst_character_level_data (.level (Utilities|Struct|Breakst_player_character_data (LocalVariables|Getcharacter_data))))) (+ (.level (Utilities|Struct|Breakst_character_level_data (.level (Utilities|Struct|Breakst_player_character_data (LocalVariables|Getcharacter_data))))) 1) (- (.curent_level_exp (Utilities|Struct|Breakst_character_level_data (.level (Utilities|Struct|Breakst_player_character_data (LocalVariables|Getcharacter_data))))) (.need_exp (Utilities|Struct|Breakst_character_level_data (.level (Utilities|Struct|Breakst_player_character_data (LocalVariables|Getcharacter_data)))))) (Utilities|Struct|Breakst_character_bese_level_data _输出行)) (.default_Finishing (Utilities|Struct|Breakst_player_character_data (LocalVariables|Getcharacter_data))) (.character_skill_data (Utilities|Struct|Breakst_player_character_data (LocalVariables|Getcharacter_data))) (.Favorability (Utilities|Struct|Breakst_player_character_data (LocalVariables|Getcharacter_data))))))
  (return _output_get))

(fn ClearExpandAutoLevelUp
  (params (character_data :type St%20Player%20Character%20Data%20Structure))
  (LocalVariables|Setlocal_characterdata (LocalVariables|Getlocal_characterdata))
  (while (LocalVariables|GetCAN_upgrade)
    (bind _returnvalue (level_upgrade|CharacterLevelExpChear (LocalVariables|Getlocal_characterdata)))
    (bind _output_get (LocalVariables|SetCAN_upgrade _returnvalue))
    (if _output_get
      (bind _newparam (level_upgrade|CharacterLevelUp (LocalVariables|Getlocal_characterdata)))
      (bind _output_get_2 (LocalVariables|Setlocal_characterdata _newparam))
      (bind _returnvalue_2 (level_upgrade|CharacterLevelExpChear _output_get_2))
      (LocalVariables|SetCAN_upgrade _returnvalue_2)))
  (bind _as2dplayer_contrller (Utilities|Casting|CastTo2DplayerContrller (Game|GetPlayerController 0)))
  (bind _turn_level (level_GE|GetTureLevel (.level_rand (Utilities|Struct|Breakst_character_level_data (Utilities|Struct|Breakst_player_character_data (LocalVariables|Getlocal_characterdata)))) (.level (Utilities|Struct|Breakst_character_level_data (Utilities|Struct|Breakst_player_character_data (LocalVariables|Getlocal_characterdata))))))
  (N5|SaveCharacterData (Variables|/Game/gamemode/2DplayerContrller.2DplayerContrller_C|GetAC_RoleUpgradeManager _as2dplayer_contrller) (LocalVariables|Getlocal_characterdata) _turn_level)
  (return (LocalVariables|Getlocal_characterdata)))

(fn GetCharacterCurrentRandNeedExp
  (params (NewParam :type St%20Character%20Level%20Data%20Structure))
  (bind _output_get (LocalVariables|Setcharacter_level NewParam))
  (bind _returnvalue (CallFunction|GetcharacterRand (.level_rand (Utilities|Struct|Breakst_character_level_data _output_get))))
  (for _index (range (+ (.Initial (Utilities|Struct|Breakst_character_rank_info _returnvalue)) (.level (Utilities|Struct|Breakst_character_level_data _output_get))) (.End (Utilities|Struct|Breakst_character_rank_info _returnvalue)))
    (bind _returnvalue_2 (Utilities|GetDataTableRow "/Game/Struct/rank_table/T_character_level_data.T_character_level_data" (Utilities|String|StringToName (Utilities|String|ToString(Integer) _index)))
      (:then
        (LocalVariables|Setrand_exp (+ (Utilities|Struct|Breakst_character_bese_level_data _returnvalue_2) (LocalVariables|Getrand_exp))))))
  (LocalVariables|Setrand_exp (- (LocalVariables|Getrand_exp) (.curent_level_exp (Utilities|Struct|Breakst_character_level_data (LocalVariables|Getcharacter_level)))))
  (bind _output_get_2 (LocalVariables|Setcharacter_level (Utilities|Struct|Makest_character_level_data (.level_rand (Utilities|Struct|Breakst_character_level_data (LocalVariables|Getcharacter_level))) (.level (Utilities|Struct|Breakst_character_level_data (LocalVariables|Getcharacter_level))) (.curent_level_exp (Utilities|Struct|Breakst_character_level_data (LocalVariables|Getcharacter_level))) (.need_exp (Utilities|Struct|Breakst_character_level_data (LocalVariables|Getcharacter_level))) (LocalVariables|Getrand_exp))))
  (return _output_get_2))

(fn CharacterLevelExpChear
  (params (st_player_character_data :type St%20Player%20Character%20Data%20Structure%20%28by%20ref%29))
  (bind _level (Utilities|Struct|Breakst_player_character_data st_player_character_data))
  (bind (_level_rand _level_2 _curent_level_exp) (Utilities|Struct|Breakst_character_level_data _level))
  (bind _输出行 (level_GE|GetTureLevel _level_rand _level_2))
  (bind _returnvalue (CallFunction|GetcharacterRand _level_rand))
  (return (and (>= (Utilities|Struct|Breakst_character_rank_info _returnvalue) _level_2) (>= _curent_level_exp (Utilities|Struct|Breakst_character_bese_level_data _输出行)))))

(fn CharacterFinishSkillCanUpgrade
  (params (skill_level :type Integer))
  (return false))

(fn CharacterSkillCanUpgrade
  (params (skill_level :type Integer) (character :type St%20Player%20Character%20Data%20Structure))
  (bind _level (Utilities|Struct|Breakst_player_character_data character))
  (bind (_level_rand _level_2) (Utilities|Struct|Breakst_character_level_data _level))
  (bind _returnvalue (Utilities|GetDataTableRow "/Game/Struct/common_Character_data/T_character_skill_level_Requirements.T_character_skill_level_Requirements" (Utilities|String|StringToName (Utilities|String|ToString(Integer) skill_level)))
    (:then
      (return (and (>= (.characrer_level (Utilities|Struct|BreakST_Public_Skill_Level_Requirements _returnvalue)) _level_2) (>= _level_rand (.rand_state (Utilities|Struct|BreakST_Public_Skill_Level_Requirements _returnvalue))))))))

(fn CharacterCanPromotion
  (params (current_level :type Integer) (rand :type Integer))
  (bind _out_data (level_GE|GetStateLocat rand))
  (return (>= (Utilities|Struct|Breakst_character_rank_info _out_data) current_level)))

(fn ModuleCanUpgrade
  (params (character :type St%20Player%20Character%20Data%20Structure) (module_index :type Integer))
  (bind (_module_info _level) (Utilities|Struct|Breakst_player_character_data character))
  (bind (_level_rand _level_2) (Utilities|Struct|Breakst_character_level_data _level))
  (bind _output (Utilities|Array|Get(acopy) _module_info module_index))
  (bind _module_level (Utilities|Struct|Breakst_pawn_module _output))
  (if (>= _module_level 3)
    (LocalVariables|Setcan_upgrade false)
    (else
      (bind _returnvalue (Utilities|GetDataTableRow "/Game/Struct/common_Character_data/T_character_module_level_Requirements.T_character_module_level_Requirements" (Utilities|String|StringToName (Utilities|String|ToString(Integer) _module_level)))
        (:then
          (LocalVariables|Setcan_upgrade (and (>= _level_rand (.rand_state (Utilities|Struct|BreakST_Public_Skill_Level_Requirements _returnvalue))) (>= _level_2 (.characrer_level (Utilities|Struct|BreakST_Public_Skill_Level_Requirements _returnvalue)))))))))
  (return (LocalVariables|Getcan_upgrade)))

(fn CharacterSkillLock
  (params (skill_lock_state :type Boolean) (character :type St%20Player%20Character%20Data%20Structure) (skill_index :type Integer))
  (LocalVariables|Setloca_character character)
  (if skill_lock_state
    (Utilities|Array|SetArrayElem (.GeneralSkillList (Utilities|Struct|Breakst_character_skill_Assembly (Utilities|Struct|Breakst_player_character_data (LocalVariables|Getloca_character)))) 0 (Utilities|Struct|Makest_character_skill (.character_skill_index (Utilities|Struct|Breakst_character_skill (Utilities|Array|Get(acopy) (.GeneralSkillList (Utilities|Struct|Breakst_character_skill_Assembly (Utilities|Struct|Breakst_player_character_data (LocalVariables|Getloca_character)))) skill_index))) (.skill_type (Utilities|Struct|Breakst_character_skill (Utilities|Array|Get(acopy) (.GeneralSkillList (Utilities|Struct|Breakst_character_skill_Assembly (Utilities|Struct|Breakst_player_character_data (LocalVariables|Getloca_character)))) skill_index))) (.skill_rowname (Utilities|Struct|Breakst_character_skill (Utilities|Array|Get(acopy) (.GeneralSkillList (Utilities|Struct|Breakst_character_skill_Assembly (Utilities|Struct|Breakst_player_character_data (LocalVariables|Getloca_character)))) skill_index))) (.current_skill_level (Utilities|Struct|Breakst_character_skill (Utilities|Array|Get(acopy) (.GeneralSkillList (Utilities|Struct|Breakst_character_skill_Assembly (Utilities|Struct|Breakst_player_character_data (LocalVariables|Getloca_character)))) skill_index))) true))
    (else
      (Utilities|Array|SetArrayElem (.ListofFinishers (Utilities|Struct|Breakst_character_skill_Assembly (Utilities|Struct|Breakst_player_character_data (LocalVariables|Getloca_character)))) 0 (Utilities|Struct|Makest_character_skill (.character_skill_index (Utilities|Struct|Breakst_character_skill (Utilities|Array|Get(acopy) (.ListofFinishers (Utilities|Struct|Breakst_character_skill_Assembly (Utilities|Struct|Breakst_player_character_data (LocalVariables|Getloca_character)))) skill_index))) (.skill_type (Utilities|Struct|Breakst_character_skill (Utilities|Array|Get(acopy) (.ListofFinishers (Utilities|Struct|Breakst_character_skill_Assembly (Utilities|Struct|Breakst_player_character_data (LocalVariables|Getloca_character)))) skill_index))) (.skill_rowname (Utilities|Struct|Breakst_character_skill (Utilities|Array|Get(acopy) (.ListofFinishers (Utilities|Struct|Breakst_character_skill_Assembly (Utilities|Struct|Breakst_player_character_data (LocalVariables|Getloca_character)))) skill_index))) (.current_skill_level (Utilities|Struct|Breakst_character_skill (Utilities|Array|Get(acopy) (.ListofFinishers (Utilities|Struct|Breakst_character_skill_Assembly (Utilities|Struct|Breakst_player_character_data (LocalVariables|Getloca_character)))) skill_index))) true))))
  (return (LocalVariables|Getloca_character)))

(fn SkillUpgrad
  (params (character :type St%20Player%20Character%20Data%20Structure) (array_skill_index :type Integer) (skill_switch :type Boolean))
  (LocalVariables|Setloca_character character)
  (if skill_switch
    (Utilities|Array|SetArrayElem (.GeneralSkillList (Utilities|Struct|Breakst_character_skill_Assembly (Utilities|Struct|Breakst_player_character_data (LocalVariables|Getloca_character)))) 0 (Utilities|Struct|Makest_character_skill (.character_skill_index (Utilities|Struct|Breakst_character_skill (Utilities|Array|Get(acopy) (.GeneralSkillList (Utilities|Struct|Breakst_character_skill_Assembly (Utilities|Struct|Breakst_player_character_data (LocalVariables|Getloca_character)))) array_skill_index))) (.skill_type (Utilities|Struct|Breakst_character_skill (Utilities|Array|Get(acopy) (.GeneralSkillList (Utilities|Struct|Breakst_character_skill_Assembly (Utilities|Struct|Breakst_player_character_data (LocalVariables|Getloca_character)))) array_skill_index))) (.skill_rowname (Utilities|Struct|Breakst_character_skill (Utilities|Array|Get(acopy) (.GeneralSkillList (Utilities|Struct|Breakst_character_skill_Assembly (Utilities|Struct|Breakst_player_character_data (LocalVariables|Getloca_character)))) array_skill_index))) (+ (.current_skill_level (Utilities|Struct|Breakst_character_skill (Utilities|Array|Get(acopy) (.GeneralSkillList (Utilities|Struct|Breakst_character_skill_Assembly (Utilities|Struct|Breakst_player_character_data (LocalVariables|Getloca_character)))) array_skill_index))) 1) (.skill_unclok_state (Utilities|Struct|Breakst_character_skill (Utilities|Array|Get(acopy) (.GeneralSkillList (Utilities|Struct|Breakst_character_skill_Assembly (Utilities|Struct|Breakst_player_character_data (LocalVariables|Getloca_character)))) array_skill_index)))))
    (else
      (Utilities|Array|SetArrayElem (.ListofFinishers (Utilities|Struct|Breakst_character_skill_Assembly (Utilities|Struct|Breakst_player_character_data (LocalVariables|Getloca_character)))) 0 (Utilities|Struct|Makest_character_skill (.character_skill_index (Utilities|Struct|Breakst_character_skill (Utilities|Array|Get(acopy) (.ListofFinishers (Utilities|Struct|Breakst_character_skill_Assembly (Utilities|Struct|Breakst_player_character_data (LocalVariables|Getloca_character)))) array_skill_index))) (.skill_type (Utilities|Struct|Breakst_character_skill (Utilities|Array|Get(acopy) (.ListofFinishers (Utilities|Struct|Breakst_character_skill_Assembly (Utilities|Struct|Breakst_player_character_data (LocalVariables|Getloca_character)))) array_skill_index))) (.skill_rowname (Utilities|Struct|Breakst_character_skill (Utilities|Array|Get(acopy) (.ListofFinishers (Utilities|Struct|Breakst_character_skill_Assembly (Utilities|Struct|Breakst_player_character_data (LocalVariables|Getloca_character)))) array_skill_index))) (+ (.current_skill_level (Utilities|Struct|Breakst_character_skill (Utilities|Array|Get(acopy) (.ListofFinishers (Utilities|Struct|Breakst_character_skill_Assembly (Utilities|Struct|Breakst_player_character_data (LocalVariables|Getloca_character)))) array_skill_index))) 1) (.skill_unclok_state (Utilities|Struct|Breakst_character_skill (Utilities|Array|Get(acopy) (.ListofFinishers (Utilities|Struct|Breakst_character_skill_Assembly (Utilities|Struct|Breakst_player_character_data (LocalVariables|Getloca_character)))) array_skill_index)))))))
  (return (LocalVariables|Getloca_character)))

(fn ModuleLevelUpgrade
  (params (character :type St%20Player%20Character%20Data%20Structure) (module_index :type Integer))
  (LocalVariables|Setloca_character character)
  (Utilities|Array|SetArrayElem (Utilities|Struct|Breakst_player_character_data (LocalVariables|Getloca_character)) 0 (Utilities|Struct|Makest_pawn_module (.module_index (Utilities|Struct|Breakst_pawn_module (Utilities|Array|Get(acopy) (Utilities|Struct|Breakst_player_character_data (LocalVariables|Getloca_character)) module_index))) (.module_name (Utilities|Struct|Breakst_pawn_module (Utilities|Array|Get(acopy) (Utilities|Struct|Breakst_player_character_data (LocalVariables|Getloca_character)) module_index))) (+ (.module_level (Utilities|Struct|Breakst_pawn_module (Utilities|Array|Get(acopy) (Utilities|Struct|Breakst_player_character_data (LocalVariables|Getloca_character)) module_index))) 1)))
  (return (LocalVariables|Getloca_character)))

(fn GetNewCharacter
  (params (character_name :type Name))
  (bind _outassetdata (Class|AssetRegistry|GetAssetsbyClass (Class|AssetRegistryHelpers|GetAssetRegistry) (Utilities|MakeTopLevelAssetPath "/Game/Data_Asset/character_data_Asset/DA_character.DA_character" "") false))
  (for _array_element _outassetdata
    (if (== (.AssetName (Utilities|Struct|BreakAssetData _array_element)) character_name)
      (bind _returnvalue (Utilities|LoadAssetBlocking (Class|KismetSystemLibrary|ToSoftObjRef(SoftObjPath) (Utilities|MakeSoftObjectPath (Class|KismetSystemLibrary|BreakTopLevelAssetPath (.AssetClassPath (Utilities|Struct|BreakAssetData _array_element)))))))
      (bind _asda_character (Utilities|Casting|CastToDA_character _returnvalue))
      (bind _returnvalue_2 (Game|ConstructObjectfromClass "/Game/BP/BP_AC/BP_Player_level_AC/BP_character_object.BP_character_object_C"))
      (Default|CharacterInitializationR2 _returnvalue_2 _asda_character)
      (bind _output_get (level_upgrade|GetCharacterCurrentRandNeedExp (Utilities|Struct|Breakst_player_character_data (Variables|/Game/BP/BP_AC/BP_Player_level_AC/BP_character_object.BP_character_object_C|Getcharacter_data (LocalVariables|Getcharacter_object)))))
      (Variables|/Game/BP/BP_AC/BP_Player_level_AC/BP_character_object.BP_character_object_C|Setcharacter_data (LocalVariables|Getcharacter_object) (Utilities|Struct|Makest_player_character_data (.character_info (Utilities|Struct|Breakst_player_character_data (Variables|/Game/BP/BP_AC/BP_Player_level_AC/BP_character_object.BP_character_object_C|Getcharacter_data (LocalVariables|Getcharacter_object)))) (.module_info (Utilities|Struct|Breakst_player_character_data (Variables|/Game/BP/BP_AC/BP_Player_level_AC/BP_character_object.BP_character_object_C|Getcharacter_data (LocalVariables|Getcharacter_object)))) _output_get (.default_Finishing (Utilities|Struct|Breakst_player_character_data (Variables|/Game/BP/BP_AC/BP_Player_level_AC/BP_character_object.BP_character_object_C|Getcharacter_data (LocalVariables|Getcharacter_object)))) (.character_skill_data (Utilities|Struct|Breakst_player_character_data (Variables|/Game/BP/BP_AC/BP_Player_level_AC/BP_character_object.BP_character_object_C|Getcharacter_data (LocalVariables|Getcharacter_object)))) (.Favorability (Utilities|Struct|Breakst_player_character_data (Variables|/Game/BP/BP_AC/BP_Player_level_AC/BP_character_object.BP_character_object_C|Getcharacter_data (LocalVariables|Getcharacter_object))))))
      (Utilities|Array|Add (Variables|Default|GetPLAYER_character_object) (LocalVariables|Getcharacter_object))))
  (return))

(fn GetNewCharacter(NG)
  (params (character_rowname :type Name))
  (bind _returnvalue (Utilities|GetDataTableRow "/Game/Struct/character/T_character_library.T_character_library" character_rowname)
    (:then
      (if (Utilities|Array|IsEmpty (Variables|Default|GetPLAYER_character_object))
        (bind _returnvalue_2 (Game|ConstructObjectfromClass "/Game/BP/BP_AC/BP_Player_level_AC/BP_character_object.BP_character_object_C" :!label _label))
        (bind _output_get (LocalVariables|Setcharacter_object _returnvalue_2))
        (Default|CharacterInitializationR0 _output_get _returnvalue "1" character_rowname)
        (bind _output_get_2 (level_upgrade|GetCharacterCurrentRandNeedExp (Utilities|Struct|Breakst_player_character_data (Variables|/Game/BP/BP_AC/BP_Player_level_AC/BP_character_object.BP_character_object_C|Getcharacter_data (LocalVariables|Getcharacter_object)))))
        (Variables|/Game/BP/BP_AC/BP_Player_level_AC/BP_character_object.BP_character_object_C|Setcharacter_data (LocalVariables|Getcharacter_object) (Utilities|Struct|Makest_player_character_data (.character_info (Utilities|Struct|Breakst_player_character_data (Variables|/Game/BP/BP_AC/BP_Player_level_AC/BP_character_object.BP_character_object_C|Getcharacter_data (LocalVariables|Getcharacter_object)))) (.module_info (Utilities|Struct|Breakst_player_character_data (Variables|/Game/BP/BP_AC/BP_Player_level_AC/BP_character_object.BP_character_object_C|Getcharacter_data (LocalVariables|Getcharacter_object)))) _output_get_2 (.default_Finishing (Utilities|Struct|Breakst_player_character_data (Variables|/Game/BP/BP_AC/BP_Player_level_AC/BP_character_object.BP_character_object_C|Getcharacter_data (LocalVariables|Getcharacter_object)))) (.character_skill_data (Utilities|Struct|Breakst_player_character_data (Variables|/Game/BP/BP_AC/BP_Player_level_AC/BP_character_object.BP_character_object_C|Getcharacter_data (LocalVariables|Getcharacter_object)))) (.Favorability (Utilities|Struct|Breakst_player_character_data (Variables|/Game/BP/BP_AC/BP_Player_level_AC/BP_character_object.BP_character_object_C|Getcharacter_data (LocalVariables|Getcharacter_object))))))
        (Utilities|Array|Add (Variables|Default|GetPLAYER_character_object) (LocalVariables|Getcharacter_object))
        (else
          ;[0.15 0.15 0.15 0.5] 检查是否重复
          (for _array_element (Variables|Default|GetPLAYER_character_object)
            (if (not (== (.rowname (Utilities|Struct|Breakst_character_info (Utilities|Struct|Breakst_player_character_data (Variables|/Game/BP/BP_AC/BP_Player_level_AC/BP_character_object.BP_character_object_C|Getcharacter_data _array_element)))) (.rowname (Utilities|Struct|Breakst_character_info (Utilities|Struct|BreakST_Character_library _returnvalue)))))
              (goto _label)))
          (return))))))

(fn SaveCharacterData
  (params (new_character_data :type St%20Player%20Character%20Data%20Structure) (level :type Name))
  (bind _character_object (N5|FindCharacter new_character_data))
  (Variables|/Game/BP/BP_AC/BP_Player_level_AC/BP_character_object.BP_character_object_C|Setlevel _character_object level)
  (Variables|/Game/BP/BP_AC/BP_Player_level_AC/BP_character_object.BP_character_object_C|Setcharacter_data _character_object new_character_data)
  (Utilities|Array|SetArrayElem (Variables|Default|GetPLAYER_character_object) 0 _character_object))

(fn FindCharacterbyRowname
  (params (rowname :type Name))
  (for _array_element (Variables|Default|GetPLAYER_character_object)
    (if (== rowname (Utilities|Struct|Breakst_character_info (Utilities|Struct|Breakst_player_character_data (Variables|/Game/BP/BP_AC/BP_Player_level_AC/BP_character_object.BP_character_object_C|Getcharacter_data _array_element))))
      (LocalVariables|Setcharacter_core _array_element)))
  (if (Utilities|IsValid (LocalVariables|Getcharacter_core))
    (return (LocalVariables|Getcharacter_core))
    (else
      (Development|PrintString "角色组件_查找单位_没有找到单位"))))

(fn FindCharacter
  (params (character_data :type St%20Player%20Character%20Data%20Structure))
  (for _array_element (Variables|Default|GetPLAYER_character_object)
    (if (== (Utilities|Struct|Breakst_character_info (.character_info (Utilities|Struct|Breakst_player_character_data (Variables|/Game/BP/BP_AC/BP_Player_level_AC/BP_character_object.BP_character_object_C|Getcharacter_data _array_element)))) (Utilities|Struct|Breakst_character_info (Utilities|Struct|Breakst_player_character_data character_data)))
      (LocalVariables|Setchracter_object _array_element)))
  (return (LocalVariables|Getchracter_object)))