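; Actor component for player character levelling: experience, stage promotion and module upgrades, with several parts unfinished.
; It imports character data and an experience pool, and builds attributes and stage experience needs from the T_character_level_data table.
; Experience items are preselected by tier into a preload array; the tally and upgrade functions are empty stubs.
; Gain, promotion and module functions rebuild the character struct, which export writes back to the matching PlayerState entry.
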(fn InitializetheLevel
  (params (RowName :type Name))
  (bind _returnvalue (Utilities|GetDataTableRow "/Game/Struct/rank_table/T_character_level_data.T_character_level_data" RowName)
    (:then
      (bind _output_get (Variables|first_Attributes|Setstandard_attribute (Utilities|Struct|Makest_Standard_attribute (.Health (Utilities|Struct|Breakst_character_bese_level_data _returnvalue)) (.Attack (Utilities|Struct|Breakst_character_bese_level_data _returnvalue)) (.defense (Utilities|Struct|Breakst_character_bese_level_data _returnvalue)))))
      (bind _output_get_2 (Variables|first_Attributes|SetFull%20attributes (Utilities|Struct|MakeST_Full_attributes (.Health (Utilities|Struct|Breakst_Standard_attribute _output_get)) (.Attack (Utilities|Struct|Breakst_Standard_attribute _output_get)) (.defense (Utilities|Struct|Breakst_Standard_attribute _output_get)) 50)))
      (Variables|first_Attributes|SetCurrent_attribute (Utilities|Struct|Makest_RoleResource (.HP (Utilities|Struct|BreakST_Full_attributes _output_get_2)) (.speed (Utilities|Struct|BreakST_Full_attributes _output_get_2)) 0 0 50)))))

(fn GainAlltheExperienceOftheCurrentStage
  (params (NewParam :type Name))
  (for _index (range (+ (Variables|level|Getcurrent_level) 1) (- (Variables|level|Getlevel_max) 1))
    (bind _returnvalue (Utilities|GetDataTableRow "/Game/Struct/rank_table/T_character_level_data.T_character_level_data" (Utilities|String|StringToName (Utilities|String|ToString(Integer) _index)))
      (:then
        (bind _returnvalue_2 (Utilities|GetDataTableRow "/Game/Struct/rank_table/T_character_level_data.T_character_level_data" NewParam)
          (:then
            (Variables|level|Setrand_exp (+ (Utilities|Struct|Breakst_character_bese_level_data _returnvalue) (- (Utilities|Struct|Breakst_character_bese_level_data _returnvalue_2) (Variables|level|Getcurrent_exp))))))))))

(fn AutoSelectAnExperienceF
  (bind _exp (auto_selecet_experience|CheakExpIsEnough))
  (auto_selecet_experience|SelectAnExperience _exp)
  (auto_selecet_experience|StatisticalExperience))

(fn StatisticalExperience)

(fn CheakExpIsEnough
  (bind _rand_exp (Variables|level|Getrand_exp))
  (bind _preloaded_exp (Variables|exp|GetPreloaded_exp))
  (if (>= _rand_exp _preloaded_exp)
    (bind _output_get (Variables|exp|Setremainder_exp (- _rand_exp _preloaded_exp)))
    (return _output_get)))

(fn SelectAnExperience
  (params (exp :type Integer) (NEED_exp :type Integer))
  (for _array_element (Variables|Exp_array|Getbad_empiricalmatter)
    (if (== (Variables|exp|Getexp_lv) (.matter_level (Utilities|Struct|BreakST_Empirical_matter _array_element))) ; 基于经验物级别查找经验物
      (if (>= (.quantity (Utilities|Struct|BreakST_Empirical_matter _array_element)) 1) ; 经验物是否有数量
        (if (>= (.quantity (Utilities|Struct|BreakST_Empirical_matter _array_element)) 1) ; 检查经验物是否足够
          ;[1 1 1] 检查是否存在
          (for _array_element_2 (Variables|Exp_array|GetPreloaded_empiricalmatter)
            (if (== (Variables|exp|Getexp_lv) (.matter_level (Utilities|Struct|BreakST_Empirical_matter _array_element_2)))
              (for _array_element_3 (Variables|Exp_array|GetPreloaded_empiricalmatter)
                (if (== (Variables|exp|Getexp_lv) (.matter_level (Utilities|Struct|BreakST_Empirical_matter _array_element_3))) ; 查找对应的经验
                  (if (> (.quantity (Utilities|Struct|BreakST_Empirical_matter _array_element)) (.quantity (Utilities|Struct|BreakST_Empirical_matter _array_element_3))) ; 同级别经验物对比
                    (if (> (+ (LocalVariables|GetCURRENT_EXP_X) (.Offerexperience (Utilities|Struct|BreakST_Empirical_matter _array_element))) NEED_exp) ; 当前经验是否大于所需经验
                      (if (not (>= (- (Variables|exp|Getexp_lv) 1) 0)) ; 当前经验物是否为最小的经验物
                        (Utilities|Array|SetArrayElem (Variables|Exp_array|GetPreloaded_empiricalmatter) 0 (Utilities|Struct|MakeST_Empirical_matter (.matter_level (Utilities|Struct|BreakST_Empirical_matter _array_element_3)) (.Offerexperience (Utilities|Struct|BreakST_Empirical_matter _array_element_3)) (+ (.quantity (Utilities|Struct|BreakST_Empirical_matter _array_element_3)) 1))))))))
              (else
                (Utilities|Array|Add (Variables|Exp_array|GetPreloaded_empiricalmatter) (Utilities|Struct|MakeST_Empirical_matter (Variables|exp|Getexp_lv) 0 1))))))))))

(fn GainExperience
  (params (exp :type Integer))
  (Variables|NewCharacter|Setcharacter_data (Utilities|Struct|Makest_player_character_data (.character_info (Utilities|Struct|Breakst_player_character_data (Variables|NewCharacter|Getcharacter_data))) (.module_info (Utilities|Struct|Breakst_player_character_data (Variables|NewCharacter|Getcharacter_data))) (Utilities|Struct|Makest_character_level_data (.level_rand (Utilities|Struct|Breakst_character_level_data (.level (Utilities|Struct|Breakst_player_character_data (Variables|NewCharacter|Getcharacter_data))))) (.level (Utilities|Struct|Breakst_character_level_data (.level (Utilities|Struct|Breakst_player_character_data (Variables|NewCharacter|Getcharacter_data))))) (+ exp (.curent_level_exp (Utilities|Struct|Breakst_character_level_data (.level (Utilities|Struct|Breakst_player_character_data (Variables|NewCharacter|Getcharacter_data)))))) (.need_exp (Utilities|Struct|Breakst_character_level_data (.level (Utilities|Struct|Breakst_player_character_data (Variables|NewCharacter|Getcharacter_data))))) (.rand_level_need_exp (Utilities|Struct|Breakst_character_level_data (.level (Utilities|Struct|Breakst_player_character_data (Variables|NewCharacter|Getcharacter_data)))))) (.default_Finishing (Utilities|Struct|Breakst_player_character_data (Variables|NewCharacter|Getcharacter_data)))))
  (Variables|Default|Setexperience (- (Variables|Default|Getexperience) exp)))

(fn Upgrade)

(fn UnlockorUpgradeMods
  (params (module_index :type Integer))
  (for _array_element (.module_info (Utilities|Struct|Breakst_player_character_data (Variables|NewCharacter|Getcharacter_data)))
    (if (== (.module_index (Utilities|Struct|Breakst_pawn_module _array_element)) module_index)
      (Utilities|Array|SetArrayElem (.module_info (Utilities|Struct|Breakst_player_character_data (Variables|NewCharacter|Getcharacter_data))) 0 (Utilities|Struct|Makest_pawn_module (.module_index (Utilities|Struct|Breakst_pawn_module _array_element)) "None" (+ (.module_level (Utilities|Struct|Breakst_pawn_module _array_element)) 1)))
      (Variables|NewCharacter|Setcharacter_data (Utilities|Struct|Makest_player_character_data (.character_info (Utilities|Struct|Breakst_player_character_data (Variables|NewCharacter|Getcharacter_data))) (.level (Utilities|Struct|Breakst_player_character_data (Variables|NewCharacter|Getcharacter_data))) (.default_Finishing (Utilities|Struct|Breakst_player_character_data (Variables|NewCharacter|Getcharacter_data))))))))

(fn PromotionLevelStage
  (Variables|NewCharacter|Setcharacter_data (Utilities|Struct|Makest_player_character_data (.character_info (Utilities|Struct|Breakst_player_character_data (Variables|NewCharacter|Getcharacter_data))) (.module_info (Utilities|Struct|Breakst_player_character_data (Variables|NewCharacter|Getcharacter_data))) (Utilities|Struct|Makest_character_level_data (+ (.level_rand (Utilities|Struct|Breakst_character_level_data (.level (Utilities|Struct|Breakst_player_character_data (Variables|NewCharacter|Getcharacter_data))))) 1) (+ (.level (Utilities|Struct|Breakst_character_level_data (.level (Utilities|Struct|Breakst_player_character_data (Variables|NewCharacter|Getcharacter_data))))) 1) (- (.curent_level_exp (Utilities|Struct|Breakst_character_level_data (.level (Utilities|Struct|Breakst_player_character_data (Variables|NewCharacter|Getcharacter_data))))) (.need_exp (Utilities|Struct|Breakst_character_level_data (.level (Utilities|Struct|Breakst_player_character_data (Variables|NewCharacter|Getcharacter_data)))))) (.need_exp (Utilities|Struct|Breakst_character_level_data (.level (Utilities|Struct|Breakst_player_character_data (Variables|NewCharacter|Getcharacter_data))))) (.rand_level_need_exp (Utilities|Struct|Breakst_character_level_data (.level (Utilities|Struct|Breakst_player_character_data (Variables|NewCharacter|Getcharacter_data)))))) (.default_Finishing (Utilities|Struct|Breakst_player_character_data (Variables|NewCharacter|Getcharacter_data))))))

(fn C-ImportRoleData
  (params (this%20character :type St%20Player%20Character%20Data%20Structure) (experience%20l :type Integer))
  (bind _level (Utilities|Struct|Breakst_player_character_data this%20character))
  (bind (_level_rand _level_2 _curent_level_exp _need_exp _rand_level_need_exp) (Utilities|Struct|Breakst_character_level_data _level))
  (Utilities|FlowControl|Sequence
    (:then_0
      (Variables|NewCharacter|Setcharacter_data this%20character)
      (Variables|Default|Setexperience experience%20l))
    (:then_1
      (Variables|level|Setcurrent_rank _level_rand))
    (:then_2
      (Variables|level|Setcurrent_level _level_2))
    (:then_3
      (Variables|level|Setcurrent_exp _curent_level_exp))
    (:then_4
      (Variables|level|Setrand_exp _rand_level_need_exp))))

(fn C-ExportCharacterData
  (bind _character_data (Variables|NewCharacter|Getcharacter_data))
  (bind (_character_info _module_info _level _default_finishing) (Utilities|Struct|Breakst_player_character_data _character_data))
  (bind (_rowname _character_index _character_name) (Utilities|Struct|Breakst_character_info _character_info))
  (bind _as2dgame_player_state (Utilities|Casting|CastTo2Dgame_PlayerState (Game|GetPlayerState 0)))
  (for _array_element (Variables|/Game/gamemode/2Dgame_PlayerState.2Dgame_PlayerState_C|Getplayerdata _as2dgame_player_state)
    (if (and (== (.character_index (Utilities|Struct|Breakst_character_info (.character_info (Utilities|Struct|Breakst_player_character_data _array_element)))) _character_index) (== (.character_name (Utilities|Struct|Breakst_character_info (.character_info (Utilities|Struct|Breakst_player_character_data _array_element)))) _character_name))
      (Utilities|Array|SetArrayElem (Variables|/Game/gamemode/2Dgame_PlayerState.2Dgame_PlayerState_C|Getplayerdata _as2dgame_player_state) 0 (Utilities|Struct|Makest_player_character_data _character_info _module_info _level _default_finishing)))))

(fn AutoSelectExperience
  (while (LocalVariables|Getcanselect_exp)
    (auto_selecet_experience|SelectAnExperience (LocalVariables|GetThe%20amount%20of%20experience%20in%20the%20selection)))
  (auto_selecet_experience|StatisticalExperience))

(fn SelectCharacter
  (params (Dimension%201 :type Integer))
  (Variables|NewCharacter|Setcharacter_data (Utilities|Array|Get(acopy) (Variables|NewCharacter|Getcharacter_data_array) Dimension%201)))