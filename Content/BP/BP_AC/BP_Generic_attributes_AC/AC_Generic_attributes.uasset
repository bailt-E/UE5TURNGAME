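; Generic attribute component that holds a battle unit's stats, current resources and status flags for turn-based combat.
; TickAttributes sums fixed and floating attributes, plus battle bonuses for edge and fixed stats, into current properties.
; Reset functions update health, action points and speed with overload per turn, while other functions apply damage, healing and movement costs.
; Level stats come from data tables, and buff status is merged with unit status.
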(event EventBeginPlay)

(event EventTick
  (params (DeltaSeconds :type Float%20%28single-precision%29)))

(fn NaturalElapsedTime
  (Variables|actionpoint|Setcurrent_action_point (- (Variables|actionpoint|Getcurrent_action_point) 3)))

(fn WhenActionPointsChange
  (params (NewParam :type Float%20%28double-precision%29))
  (Variables|actionpoint|Setcurrent_action_point (Math|Float|Truncate (* (Variables|actionpoint|Getcurrent_action_point) (/ (+ NewParam 1e+02) 1e+02))))
  (return))

(fn TickAttributes
  (params (unit_bouns_battle :type St%20Rougelike%20Unit%20Bonus%20Structure) (level :type ST%20Attribute%20Collection%20AA%20Structure))
  (bind _unit_floating_attributes (Variables|properties|GetUNIT_Floating%20attributes))
  (bind _unit_floating_attributes_2 (Variables|properties|GetUNIT_Floating%20attributes))
  (bind _unit_floating_attributes_3 (Variables|properties|GetUNIT_Floating%20attributes))
  (bind _secondary_attributes (Utilities|Struct|BreakST_Attribute_collection_AA _unit_floating_attributes))
  (bind _edgeattrobutes (Utilities|Struct|Breakst_rougelike_unit_bonus unit_bouns_battle))
  (bind _fixed_attributes (Utilities|Struct|BreakST_Attribute_collection_AA _unit_floating_attributes_3))
  (bind _fixedattrobutes (Utilities|Struct|Breakst_rougelike_unit_bonus (Variables|Default|Getunit_bouns_battle)))
  (bind (_base_attributes _edge_attributes) (Utilities|Struct|BreakST_Attribute_collection_AA _unit_floating_attributes_2))
  (bind (_element_bonus _finaldamagebonus _damagereductionbonus) (Utilities|Struct|BreakST_Secondary_attributes_A _secondary_attributes))
  (bind (_healingbonus _healbonus _shieldedbonus _shieldbonus _aggro_bonus) (Utilities|Struct|BreakST_Edge_attributes_A _edgeattrobutes))
  (bind (_speedcap _overloadroundcap _maximumshield _overloadcap _energycap _unit_actionpointcap _element_tag_number_max _initialvelocity) (Utilities|Struct|BreakST_Fixed_attributes_A _fixedattrobutes))
  (bind (_healthy _attack _defense _velocity _criticalhits _criticaldamage _unit_actionpoints) (Utilities|Struct|BreakST_Base_attributes_A _base_attributes))
  (bind (_healingbonus_2 _healbonus_2 _shieldedbonus_2 _shieldbonus_2 _aggro_bonus_2) (Utilities|Struct|BreakST_Edge_attributes_A _edge_attributes))
  (bind (_speedcap_2 _overloadroundcap_2 _maximumshield_2 _overloadcap_2 _energycap_2 _unit_actionpointcap_2 _element_tag_number_max_2 _initialvelocity_2) (Utilities|Struct|BreakST_Fixed_attributes_A _fixed_attributes))
  (Variables|properties|SetUNIT_Fixed%20attributes level)
  (bind _output_get (Variables|properties|SetUNIT_Current%20properties (Utilities|Struct|MakeST_Attribute_collection_AA (Utilities|Struct|MakeST_Base_attributes_A (+ _healthy (.healthy (Utilities|Struct|BreakST_Base_attributes_A (.base_attributes (Utilities|Struct|BreakST_Attribute_collection_AA (Variables|properties|GetUNIT_Fixed%20attributes)))))) (+ _attack (.attack (Utilities|Struct|BreakST_Base_attributes_A (.base_attributes (Utilities|Struct|BreakST_Attribute_collection_AA (Variables|properties|GetUNIT_Fixed%20attributes)))))) (+ _defense (.defense (Utilities|Struct|BreakST_Base_attributes_A (.base_attributes (Utilities|Struct|BreakST_Attribute_collection_AA (Variables|properties|GetUNIT_Fixed%20attributes)))))) (+ _velocity (.velocity (Utilities|Struct|BreakST_Base_attributes_A (.base_attributes (Utilities|Struct|BreakST_Attribute_collection_AA (Variables|properties|GetUNIT_Fixed%20attributes)))))) (+ _criticalhits (.Criticalhits (Utilities|Struct|BreakST_Base_attributes_A (.base_attributes (Utilities|Struct|BreakST_Attribute_collection_AA (Variables|properties|GetUNIT_Fixed%20attributes)))))) (+ _criticaldamage (.Criticaldamage (Utilities|Struct|BreakST_Base_attributes_A (.base_attributes (Utilities|Struct|BreakST_Attribute_collection_AA (Variables|properties|GetUNIT_Fixed%20attributes)))))) (+ _unit_actionpoints (.Unit_Actionpoints (Utilities|Struct|BreakST_Base_attributes_A (.base_attributes (Utilities|Struct|BreakST_Attribute_collection_AA (Variables|properties|GetUNIT_Fixed%20attributes))))))) (Utilities|Struct|MakeST_Edge_attributes_A (+ _healingbonus (+ _healingbonus_2 (.Healingbonus (Utilities|Struct|BreakST_Edge_attributes_A (.edge_attributes (Utilities|Struct|BreakST_Attribute_collection_AA (Variables|properties|GetUNIT_Fixed%20attributes))))))) (+ _healbonus (+ _healbonus_2 (.Healbonus (Utilities|Struct|BreakST_Edge_attributes_A (.edge_attributes (Utilities|Struct|BreakST_Attribute_collection_AA (Variables|properties|GetUNIT_Fixed%20attributes))))))) (+ _shieldedbonus (+ _shieldedbonus_2 (.Shieldedbonus (Utilities|Struct|BreakST_Edge_attributes_A (.edge_attributes (Utilities|Struct|BreakST_Attribute_collection_AA (Variables|properties|GetUNIT_Fixed%20attributes))))))) (+ (+ _shieldbonus_2 (.Shieldbonus (Utilities|Struct|BreakST_Edge_attributes_A (.edge_attributes (Utilities|Struct|BreakST_Attribute_collection_AA (Variables|properties|GetUNIT_Fixed%20attributes)))))) _shieldbonus) (+ _aggro_bonus (+ _aggro_bonus_2 (.aggro_bonus (Utilities|Struct|BreakST_Edge_attributes_A (.edge_attributes (Utilities|Struct|BreakST_Attribute_collection_AA (Variables|properties|GetUNIT_Fixed%20attributes)))))))) (Utilities|Struct|MakeST_Fixed_attributes_A (+ (+ _speedcap_2 (.Speedcap (Utilities|Struct|BreakST_Fixed_attributes_A (.Fixed_attributes (Utilities|Struct|BreakST_Attribute_collection_AA (Variables|properties|GetUNIT_Fixed%20attributes)))))) _speedcap) (+ (+ _overloadroundcap_2 (.Overloadroundcap (Utilities|Struct|BreakST_Fixed_attributes_A (.Fixed_attributes (Utilities|Struct|BreakST_Attribute_collection_AA (Variables|properties|GetUNIT_Fixed%20attributes)))))) _overloadroundcap) (+ (+ _maximumshield_2 (.Maximumshield (Utilities|Struct|BreakST_Fixed_attributes_A (.Fixed_attributes (Utilities|Struct|BreakST_Attribute_collection_AA (Variables|properties|GetUNIT_Fixed%20attributes)))))) _maximumshield) (+ (+ _overloadcap_2 (.Overloadcap (Utilities|Struct|BreakST_Fixed_attributes_A (.Fixed_attributes (Utilities|Struct|BreakST_Attribute_collection_AA (Variables|properties|GetUNIT_Fixed%20attributes)))))) _overloadcap) (+ (+ _energycap_2 (.Energycap (Utilities|Struct|BreakST_Fixed_attributes_A (.Fixed_attributes (Utilities|Struct|BreakST_Attribute_collection_AA (Variables|properties|GetUNIT_Fixed%20attributes)))))) _energycap) (+ (+ _unit_actionpointcap_2 (.unit_Actionpointcap (Utilities|Struct|BreakST_Fixed_attributes_A (.Fixed_attributes (Utilities|Struct|BreakST_Attribute_collection_AA (Variables|properties|GetUNIT_Fixed%20attributes)))))) _unit_actionpointcap) (+ (+ _element_tag_number_max_2 (.element_tag_number_MAX (Utilities|Struct|BreakST_Fixed_attributes_A (.Fixed_attributes (Utilities|Struct|BreakST_Attribute_collection_AA (Variables|properties|GetUNIT_Fixed%20attributes)))))) _element_tag_number_max) (+ (+ _initialvelocity_2 (.Initialvelocity (Utilities|Struct|BreakST_Fixed_attributes_A (.Fixed_attributes (Utilities|Struct|BreakST_Attribute_collection_AA (Variables|properties|GetUNIT_Fixed%20attributes)))))) _initialvelocity)) (Utilities|Struct|MakeST_Secondary_attributes_A 0 (+ _finaldamagebonus (.Finaldamagebonus (Utilities|Struct|BreakST_Secondary_attributes_A (Utilities|Struct|BreakST_Attribute_collection_AA (Variables|properties|GetUNIT_Fixed%20attributes))))) (+ _damagereductionbonus (.Damagereductionbonus (Utilities|Struct|BreakST_Secondary_attributes_A (Utilities|Struct|BreakST_Attribute_collection_AA (Variables|properties|GetUNIT_Fixed%20attributes)))))))))
  (return _output_get))

(fn TurnPawnReset
  (params (land :type BP%20Land%20Spaner%20Object%20Reference))
  (Utilities|FlowControl|Sequence
    (:then_0
      (if (>= (.Thecurrentspeedisoverloaded (Utilities|Struct|BreakST_UNIT_Current_resource_AA (Variables|Default|GetCurrent_resource))) (Utilities|Struct|BreakST_Fixed_attributes_A (.Fixed_attributes (Utilities|Struct|BreakST_Attribute_collection_AA (Variables|properties|GetUNIT_Current%20properties))))) ; 检查当前过载是否大于单回合的过载量
        (LocalVariables|Setoverloaded (.Overloadcap (Utilities|Struct|BreakST_Fixed_attributes_A (.Fixed_attributes (Utilities|Struct|BreakST_Attribute_collection_AA (Variables|properties|GetUNIT_Current%20properties))))))
        (else
          (LocalVariables|Setoverloaded (.Thecurrentspeedisoverloaded (Utilities|Struct|BreakST_UNIT_Current_resource_AA (Variables|Default|GetCurrent_resource)))))))
    (:then_1
      (if (>= (LocalVariables|Getoverloaded) (Utilities|Struct|BreakST_Base_attributes_A (.base_attributes (Utilities|Struct|BreakST_Attribute_collection_AA (Variables|properties|GetUNIT_Current%20properties))))) ; 检查超载是否大于新增速度
        (LocalVariables|Setoverloaded (Utilities|Struct|BreakST_Base_attributes_A (.base_attributes (Utilities|Struct|BreakST_Attribute_collection_AA (Variables|properties|GetUNIT_Current%20properties)))))
        (else
          (LocalVariables|Setoverloaded (LocalVariables|Getoverloaded)))))
    (:then_2
      (if (== (Variables|/Game/BP/BP_Battle_Phase/BP_land_spaner.BP_land_spaner_C|Getcurrent_turn_no land) 1) ; 检查回合
        (Variables|Default|SetCurrent_resource (Utilities|Struct|MakeST_UNIT_Current_resource_AA (Utilities|Struct|BreakST_Base_attributes_A (.base_attributes (Utilities|Struct|BreakST_Attribute_collection_AA (Variables|properties|GetUNIT_Current%20properties)))) (Utilities|Struct|BreakST_Fixed_attributes_A (.Fixed_attributes (Utilities|Struct|BreakST_Attribute_collection_AA (Variables|properties|GetUNIT_Current%20properties)))))) ; 初始化速度
        (elif (>= (+ (.Currentspeed (Utilities|Struct|BreakST_UNIT_Current_resource_AA (Variables|Default|GetCurrent_resource))) (- (Utilities|Struct|BreakST_Base_attributes_A (.base_attributes (Utilities|Struct|BreakST_Attribute_collection_AA (Variables|properties|GetUNIT_Current%20properties)))) (LocalVariables|Getoverloaded))) (.Speedcap (Utilities|Struct|BreakST_Fixed_attributes_A (.Fixed_attributes (Utilities|Struct|BreakST_Attribute_collection_AA (Variables|properties|GetUNIT_Current%20properties))))))
          (Variables|Default|SetCurrent_resource (Utilities|Struct|MakeST_UNIT_Current_resource_AA (.Currenthealth (Utilities|Struct|BreakST_UNIT_Current_resource_AA (Variables|Default|GetCurrent_resource))) (.Currenthealtherosion (Utilities|Struct|BreakST_UNIT_Current_resource_AA (Variables|Default|GetCurrent_resource))) (.Currentlifedebt (Utilities|Struct|BreakST_UNIT_Current_resource_AA (Variables|Default|GetCurrent_resource))) (Utilities|Struct|BreakST_Fixed_attributes_A (Utilities|Struct|BreakST_Attribute_collection_AA (Variables|properties|GetUNIT_Current%20properties))) (.Currentenergy (Utilities|Struct|BreakST_UNIT_Current_resource_AA (Variables|Default|GetCurrent_resource))) (- (.Thecurrentspeedisoverloaded (Utilities|Struct|BreakST_UNIT_Current_resource_AA (Variables|Default|GetCurrent_resource))) (LocalVariables|Getoverloaded)) (.Current_shield (Utilities|Struct|BreakST_UNIT_Current_resource_AA (Variables|Default|GetCurrent_resource))) (.Current_Unitaggro (Utilities|Struct|BreakST_UNIT_Current_resource_AA (Variables|Default|GetCurrent_resource))) (.CurrentActionPoint (Utilities|Struct|BreakST_UNIT_Current_resource_AA (Variables|Default|GetCurrent_resource)))))
          (else
            (Variables|Default|SetCurrent_resource (Utilities|Struct|MakeST_UNIT_Current_resource_AA (.Currenthealth (Utilities|Struct|BreakST_UNIT_Current_resource_AA (Variables|Default|GetCurrent_resource))) (.Currenthealtherosion (Utilities|Struct|BreakST_UNIT_Current_resource_AA (Variables|Default|GetCurrent_resource))) (.Currentlifedebt (Utilities|Struct|BreakST_UNIT_Current_resource_AA (Variables|Default|GetCurrent_resource))) (+ (.Currentspeed (Utilities|Struct|BreakST_UNIT_Current_resource_AA (Variables|Default|GetCurrent_resource))) (- (Utilities|Struct|BreakST_Base_attributes_A (.base_attributes (Utilities|Struct|BreakST_Attribute_collection_AA (Variables|properties|GetUNIT_Current%20properties)))) (LocalVariables|Getoverloaded))) (.Currentenergy (Utilities|Struct|BreakST_UNIT_Current_resource_AA (Variables|Default|GetCurrent_resource))) (- (LocalVariables|Getoverloaded) (.Thecurrentspeedisoverloaded (Utilities|Struct|BreakST_UNIT_Current_resource_AA (Variables|Default|GetCurrent_resource)))) (.Current_shield (Utilities|Struct|BreakST_UNIT_Current_resource_AA (Variables|Default|GetCurrent_resource))) (.Current_Unitaggro (Utilities|Struct|BreakST_UNIT_Current_resource_AA (Variables|Default|GetCurrent_resource))) (.CurrentActionPoint (Utilities|Struct|BreakST_UNIT_Current_resource_AA (Variables|Default|GetCurrent_resource)))))))))))

(fn InitializetheProperty
  (params (current_properties :type ST%20Attribute%20Collection%20AA%20Structure))
  (Variables|Default|SetCurrent_resource (Utilities|Struct|MakeST_UNIT_Current_resource_AA (Utilities|Struct|BreakST_Base_attributes_A (.base_attributes (Utilities|Struct|BreakST_Attribute_collection_AA (Variables|properties|GetUNIT_Current%20properties)))) 3))
  (StateCheak|MoveStateCheak))

(fn InAttack
  (params (damage :type Float%20%28double-precision%29) (Critical%20hit :type Boolean) (Critical%20hit%20volume :type Float%20%28double-precision%29) (element_type :type E_element_type%20Enum :default "NewEnumerator5") (damage_type :type e_damage_type%20Enum :default "NewEnumerator1") (element_damage_type :type e_element_damage_type%20Enum :default "NewEnumerator1") (Damage%20final%20bonus :type Float%20%28double-precision%29))
  (Variables|Default|SetCurrent_resource (Utilities|Struct|MakeST_UNIT_Current_resource_AA (Math|Float|Truncate (- (Utilities|Struct|BreakST_UNIT_Current_resource_AA (Variables|Default|GetCurrent_resource)) damage)))))

(fn InTreaed
  (params (NewParam :type Float%20%28double-precision%29))
  (Variables|Default|SetCurrent_resource (Utilities|Struct|MakeST_UNIT_Current_resource_AA (Math|Float|Truncate (+ NewParam (.Currenthealth (Utilities|Struct|BreakST_UNIT_Current_resource_AA (Variables|Default|GetCurrent_resource))))) (.Currenthealtherosion (Utilities|Struct|BreakST_UNIT_Current_resource_AA (Variables|Default|GetCurrent_resource))) (.Currentlifedebt (Utilities|Struct|BreakST_UNIT_Current_resource_AA (Variables|Default|GetCurrent_resource))) (.Currentspeed (Utilities|Struct|BreakST_UNIT_Current_resource_AA (Variables|Default|GetCurrent_resource))) (.Currentenergy (Utilities|Struct|BreakST_UNIT_Current_resource_AA (Variables|Default|GetCurrent_resource))) (.Thecurrentspeedisoverloaded (Utilities|Struct|BreakST_UNIT_Current_resource_AA (Variables|Default|GetCurrent_resource))) (.Current_shield (Utilities|Struct|BreakST_UNIT_Current_resource_AA (Variables|Default|GetCurrent_resource))) (.Current_Unitaggro (Utilities|Struct|BreakST_UNIT_Current_resource_AA (Variables|Default|GetCurrent_resource))) (.CurrentActionPoint (Utilities|Struct|BreakST_UNIT_Current_resource_AA (Variables|Default|GetCurrent_resource))))))

(fn Attack(ng)
  (params (damage :type Float%20%28double-precision%29)))

(fn TurnUnitReset
  (params (battleC :type BP%20Land%20Spaner%20Object%20Reference))
  (if (== (Variables|/Game/BP/BP_Battle_Phase/BP_land_spaner.BP_land_spaner_C|Getcurrent_turn_no battleC) 1)
    (Variables|Default|SetCurrent_resource (Utilities|Struct|MakeST_UNIT_Current_resource_AA (Utilities|Struct|BreakST_Base_attributes_A (.base_attributes (Utilities|Struct|BreakST_Attribute_collection_AA (Variables|properties|GetUNIT_Current%20properties)))) (.Currenthealtherosion (Utilities|Struct|BreakST_UNIT_Current_resource_AA (Variables|Default|GetCurrent_resource))) (.Currentlifedebt (Utilities|Struct|BreakST_UNIT_Current_resource_AA (Variables|Default|GetCurrent_resource))) (.Currentspeed (Utilities|Struct|BreakST_UNIT_Current_resource_AA (Variables|Default|GetCurrent_resource))) (.Currentenergy (Utilities|Struct|BreakST_UNIT_Current_resource_AA (Variables|Default|GetCurrent_resource))) (.Thecurrentspeedisoverloaded (Utilities|Struct|BreakST_UNIT_Current_resource_AA (Variables|Default|GetCurrent_resource))) (.Current_shield (Utilities|Struct|BreakST_UNIT_Current_resource_AA (Variables|Default|GetCurrent_resource))) (.Current_Unitaggro (Utilities|Struct|BreakST_UNIT_Current_resource_AA (Variables|Default|GetCurrent_resource))) (Utilities|Struct|BreakST_Fixed_attributes_A (.Fixed_attributes (Utilities|Struct|BreakST_Attribute_collection_AA (Variables|properties|GetUNIT_Current%20properties))))))
    (else
      (Variables|Default|SetCurrent_resource (Utilities|Struct|MakeST_UNIT_Current_resource_AA (.Currenthealth (Utilities|Struct|BreakST_UNIT_Current_resource_AA (Variables|Default|GetCurrent_resource))) (.Currenthealtherosion (Utilities|Struct|BreakST_UNIT_Current_resource_AA (Variables|Default|GetCurrent_resource))) (.Currentlifedebt (Utilities|Struct|BreakST_UNIT_Current_resource_AA (Variables|Default|GetCurrent_resource))) (.Currentspeed (Utilities|Struct|BreakST_UNIT_Current_resource_AA (Variables|Default|GetCurrent_resource))) (.Currentenergy (Utilities|Struct|BreakST_UNIT_Current_resource_AA (Variables|Default|GetCurrent_resource))) (.Thecurrentspeedisoverloaded (Utilities|Struct|BreakST_UNIT_Current_resource_AA (Variables|Default|GetCurrent_resource))) (.Current_shield (Utilities|Struct|BreakST_UNIT_Current_resource_AA (Variables|Default|GetCurrent_resource))) (.Current_Unitaggro (Utilities|Struct|BreakST_UNIT_Current_resource_AA (Variables|Default|GetCurrent_resource))) (+ (.CurrentActionPoint (Utilities|Struct|BreakST_UNIT_Current_resource_AA (Variables|Default|GetCurrent_resource))) (Utilities|Struct|BreakST_Base_attributes_A (Utilities|Struct|BreakST_Attribute_collection_AA (Variables|properties|GetUNIT_Fixed%20attributes))) 1))))))

(fn CheckLifeAttributes
  (if (<= (Utilities|Struct|BreakST_UNIT_Current_resource_AA (Variables|Default|GetCurrent_resource)) 0)
    (return true)
    (else
      (return false))))

(fn AttributeDetermination
  (params (table_switch :type Boolean) (level :type Name) (fix :type Boolean) (fix_attributs :type St%20the%20Unit%20Attribute%20Structure))
  (LocalVariables|Setunittable table_switch)
  (LocalVariables|SetfixDATA fix)
  (Utilities|FlowControl|Sequence
    (:then_0
      (if (LocalVariables|GetfixDATA)
        (if (LocalVariables|Getunittable)
          (bind _returnvalue (Utilities|GetDataTableRow "/Game/Struct/rank_table/T_character_level_data.T_character_level_data" level)
            (:then
              (LocalVariables|SetattributsM (Utilities|Struct|Makest_the_unit_attribute (.Health (Utilities|Struct|Breakst_character_bese_level_data _returnvalue)) (.Attack (Utilities|Struct|Breakst_character_bese_level_data _returnvalue)) (.defense (Utilities|Struct|Breakst_character_bese_level_data _returnvalue)) 1 3 1))))
          (else
            (bind _returnvalue_2 (Utilities|GetDataTableRow "/Game/Struct/rank_table/T_unitlevel_data.T_unitlevel_data" level)
              (:then
                (LocalVariables|SetattributsM (Utilities|Struct|Makest_the_unit_attribute (.hp (Utilities|Struct|Breakst_unit_level_data _returnvalue_2)) (.attack (Utilities|Struct|Breakst_unit_level_data _returnvalue_2)) (.defense (Utilities|Struct|Breakst_unit_level_data _returnvalue_2)) 1 3 1))))))
        (else
          (LocalVariables|SetattributsM fix_attributs))))
    (:then_1
      (return (LocalVariables|GetattributsM)))))

(fn UnitCanMove?
  (if (>= (Utilities|Struct|BreakST_UNIT_Current_resource_AA (Variables|Default|GetCurrent_resource)) (Utilities|Struct|BreakST_Fixed_attributes_A (Utilities|Struct|BreakST_Attribute_collection_AA (Variables|properties|GetUNIT_Current%20properties))))
    (return true)
    (else
      (return false))))

(fn ConsumeMovementPoints
  (if (< (- (.pawn_move_munber (Utilities|Struct|BreakST_UNIT_Current_resource_AA (Variables|Default|GetCurrent_resource))) (Utilities|Struct|BreakST_Fixed_attributes_A (Utilities|Struct|BreakST_Attribute_collection_AA (Variables|properties|GetUNIT_Current%20properties)))) 0)
    (Variables|Default|SetCurrent_resource (Utilities|Struct|MakeST_UNIT_Current_resource_AA (.Currenthealth (Utilities|Struct|BreakST_UNIT_Current_resource_AA (Variables|Default|GetCurrent_resource))) (.Currenthealtherosion (Utilities|Struct|BreakST_UNIT_Current_resource_AA (Variables|Default|GetCurrent_resource))) (.Currentlifedebt (Utilities|Struct|BreakST_UNIT_Current_resource_AA (Variables|Default|GetCurrent_resource))) (.Currentspeed (Utilities|Struct|BreakST_UNIT_Current_resource_AA (Variables|Default|GetCurrent_resource))) (.Currentenergy (Utilities|Struct|BreakST_UNIT_Current_resource_AA (Variables|Default|GetCurrent_resource))) (.Thecurrentspeedisoverloaded (Utilities|Struct|BreakST_UNIT_Current_resource_AA (Variables|Default|GetCurrent_resource))) (.Current_shield (Utilities|Struct|BreakST_UNIT_Current_resource_AA (Variables|Default|GetCurrent_resource))) (.Current_Unitaggro (Utilities|Struct|BreakST_UNIT_Current_resource_AA (Variables|Default|GetCurrent_resource))) (.CurrentActionPoint (Utilities|Struct|BreakST_UNIT_Current_resource_AA (Variables|Default|GetCurrent_resource))) 0))
    (else
      (Variables|Default|SetCurrent_resource (Utilities|Struct|MakeST_UNIT_Current_resource_AA (.Currenthealth (Utilities|Struct|BreakST_UNIT_Current_resource_AA (Variables|Default|GetCurrent_resource))) (.Currenthealtherosion (Utilities|Struct|BreakST_UNIT_Current_resource_AA (Variables|Default|GetCurrent_resource))) (.Currentlifedebt (Utilities|Struct|BreakST_UNIT_Current_resource_AA (Variables|Default|GetCurrent_resource))) (.Currentspeed (Utilities|Struct|BreakST_UNIT_Current_resource_AA (Variables|Default|GetCurrent_resource))) (.Currentenergy (Utilities|Struct|BreakST_UNIT_Current_resource_AA (Variables|Default|GetCurrent_resource))) (.Thecurrentspeedisoverloaded (Utilities|Struct|BreakST_UNIT_Current_resource_AA (Variables|Default|GetCurrent_resource))) (.Current_shield (Utilities|Struct|BreakST_UNIT_Current_resource_AA (Variables|Default|GetCurrent_resource))) (.Current_Unitaggro (Utilities|Struct|BreakST_UNIT_Current_resource_AA (Variables|Default|GetCurrent_resource))) (.CurrentActionPoint (Utilities|Struct|BreakST_UNIT_Current_resource_AA (Variables|Default|GetCurrent_resource))) (- (.pawn_move_munber (Utilities|Struct|BreakST_UNIT_Current_resource_AA (Variables|Default|GetCurrent_resource))) (Utilities|Struct|BreakST_Fixed_attributes_A (Utilities|Struct|BreakST_Attribute_collection_AA (Variables|properties|GetUNIT_Current%20properties))))))
      (Development|PrintString (Utilities|String|ToString(Integer) (- (.pawn_move_munber (Utilities|Struct|BreakST_UNIT_Current_resource_AA (Variables|Default|GetCurrent_resource))) (Utilities|Struct|BreakST_Fixed_attributes_A (Utilities|Struct|BreakST_Attribute_collection_AA (Variables|properties|GetUNIT_Current%20properties)))))))))

(fn GetInitialActionPoints
  (bind _output_get (Variables|actionpoint|SetInitial%20Action%20Value (/ 10000 (Utilities|Struct|BreakST_Base_attributes_A (.base_attributes (Utilities|Struct|BreakST_Attribute_collection_AA (Variables|properties|GetUNIT_Current%20properties)))))))
  (bind _output_get_2 (Variables|actionpoint|Setcurrent_action_point _output_get))
  (return _output_get_2))

(fn MoveStateCheak
  (bind _canmove (CallFunction|UnitCanMove?))
  (Variables|Default|Setunit_status (Utilities|Struct|Makest_unit_status _canmove (.unit_can_action (Utilities|Struct|Breakst_unit_status (Variables|Default|Getunit_status))) (.falldown (Utilities|Struct|Breakst_unit_status (Variables|Default|Getunit_status))) (.Tauntstatus (Utilities|Struct|Breakst_unit_status (Variables|Default|Getunit_status))) (.Unstoppable (Utilities|Struct|Breakst_unit_status (Variables|Default|Getunit_status))) (.Immunetocontagion (Utilities|Struct|Breakst_unit_status (Variables|Default|Getunit_status))) (.Unfettered (Utilities|Struct|Breakst_unit_status (Variables|Default|Getunit_status))))))

(fn UpdataUnitFinalState
  (params (buff_status :type St%20Unit%20Status%20Structure))
  (bind (_can_move _unit_can_action _falldown _tauntstatus _unstoppable _immunetocontagion _unfettered) (Utilities|Struct|Breakst_unit_status buff_status))
  (bind (_can_move_2 _unit_can_action_2 _falldown_2 _tauntstatus_2 _unstoppable_2 _immunetocontagion_2 _unfettered_2) (Utilities|Struct|Breakst_unit_status buff_status))
  (Utilities|FlowControl|Sequence
    (:then_0
      (if _can_move_2
        (Variables|Default|Setthe_final_status (Utilities|Struct|Makest_unit_status _can_move))
        (else
          (Variables|Default|Setthe_final_status (Utilities|Struct|Makest_unit_status (Utilities|Struct|Breakst_unit_status (Variables|Default|Getunit_status)))))))
    (:then_1
      (if _unit_can_action_2
        (Variables|Default|Setthe_final_status (Utilities|Struct|Makest_unit_status _unit_can_action))
        (else
          (Variables|Default|Setthe_final_status (Utilities|Struct|Makest_unit_status (Utilities|Struct|Breakst_unit_status (Variables|Default|Getunit_status)))))))
    (:then_2
      (if _falldown_2
        (Variables|Default|Setthe_final_status (Utilities|Struct|Makest_unit_status _falldown))
        (else
          (Variables|Default|Setthe_final_status (Utilities|Struct|Makest_unit_status (Utilities|Struct|Breakst_unit_status (Variables|Default|Getunit_status)))))))
    (:then_3
      (if _tauntstatus_2
        (Variables|Default|Setthe_final_status (Utilities|Struct|Makest_unit_status _tauntstatus))
        (else
          (Variables|Default|Setthe_final_status (Utilities|Struct|Makest_unit_status (.Tauntstatus (Utilities|Struct|Breakst_unit_status (Variables|Default|Getunit_status))) false)))))
    (:then_4
      (if _unstoppable_2
        (Variables|Default|Setthe_final_status (Utilities|Struct|Makest_unit_status _unstoppable))
        (else
          (Variables|Default|Setthe_final_status (Utilities|Struct|Makest_unit_status (.Unstoppable (Utilities|Struct|Breakst_unit_status (Variables|Default|Getunit_status))) false)))))
    (:then_5
      (if _immunetocontagion_2
        (Variables|Default|Setthe_final_status (Utilities|Struct|Makest_unit_status _immunetocontagion))
        (else
          (Variables|Default|Setthe_final_status (Utilities|Struct|Makest_unit_status (.Immunetocontagion (Utilities|Struct|Breakst_unit_status (Variables|Default|Getunit_status))) false)))))
    (:then_6
      (if _unfettered_2
        (Variables|Default|Setthe_final_status (Utilities|Struct|Makest_unit_status _unfettered))
        (else
          (Variables|Default|Setthe_final_status (Utilities|Struct|Makest_unit_status (Utilities|Struct|Breakst_unit_status (Variables|Default|Getunit_status)))))))))

(fn UpdataUnitStatus
  (if (> (Utilities|Struct|BreakST_UNIT_Current_resource_AA (Variables|Default|GetCurrent_resource)) 0)
    (Variables|Default|Setunit_status (Utilities|Struct|Makest_unit_status true (.unit_can_action (Utilities|Struct|Breakst_unit_status (Variables|Default|Getunit_status))) (.falldown (Utilities|Struct|Breakst_unit_status (Variables|Default|Getunit_status))) (.Tauntstatus (Utilities|Struct|Breakst_unit_status (Variables|Default|Getunit_status))) (.Unstoppable (Utilities|Struct|Breakst_unit_status (Variables|Default|Getunit_status))) (.Immunetocontagion (Utilities|Struct|Breakst_unit_status (Variables|Default|Getunit_status))) (.Unfettered (Utilities|Struct|Breakst_unit_status (Variables|Default|Getunit_status)))))
    (return)
    (else
      (Variables|Default|Setunit_status (Utilities|Struct|Makest_unit_status false (.unit_can_action (Utilities|Struct|Breakst_unit_status (Variables|Default|Getunit_status))) (.falldown (Utilities|Struct|Breakst_unit_status (Variables|Default|Getunit_status))) (.Tauntstatus (Utilities|Struct|Breakst_unit_status (Variables|Default|Getunit_status))) (.Unstoppable (Utilities|Struct|Breakst_unit_status (Variables|Default|Getunit_status))) (.Immunetocontagion (Utilities|Struct|Breakst_unit_status (Variables|Default|Getunit_status))) (.Unfettered (Utilities|Struct|Breakst_unit_status (Variables|Default|Getunit_status)))))
      (return))))

(fn UpdataMoveStatus
  (params (buff_unit_status :type St%20Unit%20Status%20Structure))
  (bind _can_move (Utilities|Struct|Breakst_unit_status buff_unit_status))
  (if _can_move
    (Variables|Default|Setthe_final_status (Utilities|Struct|Makest_unit_status _can_move))
    (else
      (Variables|Default|Setthe_final_status (Utilities|Struct|Makest_unit_status (Utilities|Struct|Breakst_unit_status (Variables|Default|Getunit_status)))))))