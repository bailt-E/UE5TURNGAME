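; UI manager component that creates the root CommonUI screen and routes activatable widgets into it.
; CreateUI adds the root to the viewport as MainMenu; other functions cast it to WBP_Main to push or deactivate widgets.
; Main and middle layers have push functions; only the middle update removes before pushing, as the main removal is unwired.
; PrepareForBattle pushes the battle-ready screen and hands it the game mode.
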(event EventBeginPlay)

(event EventTick
  (params (DeltaSeconds :type Float%20%28single-precision%29)))

(fn CreateUI
  (params (Class :type User%20Widget%20Class%20Reference))
  (bind _returnvalue (UserInterface|CreateWidget Class))
  (bind _as通用可激活控件 (Utilities|Casting|CastToCommonActivatableWidget _returnvalue))
  (bind _output_get (Variables|Default|SetMain%20Menu _as通用可激活控件))
  (UserInterface|Viewport|AddtoViewport _output_get 0)
  (bind _aswbp_main (Utilities|Casting|CastToWBP_Main _output_get))
  (return _aswbp_main))

(fn UpdataMainUI
  (params (ActivatableWidgetClass :type Common%20Activatable%20Widget%20Class%20Reference))
  (bind _aswbp_main (Utilities|Casting|CastToWBP_Main (Variables|Default|GetMain%20Menu)))
  (bind _returnvalue (Default|PlshUIWidget(main) _aswbp_main ActivatableWidgetClass))
  (return _returnvalue))

(fn PrepareforBattle
  (params (gamemodeC :type E_level_game_mode%20Enum :default "NewEnumerator3"))
  (bind _returnvalue (MainStackEvent|UpdataMainUI "/Game/WBP_common_ui/Bottom_layer_widget/Wbp_battle_Ready.Wbp_battle_Ready_C"))
  (bind _aswbp_battle_ready (Utilities|Casting|CastToWbp_battle_Ready _returnvalue))
  (Variables|/Game/WBP_common_ui/Bottom_layer_widget/Wbp_battle_Ready.Wbp_battle_Ready_C|Setgamemode _aswbp_battle_ready gamemodeC))

(fn DisableandRemoveSlot
  (params (ttarget :type Common%20Activatable%20Widget%20Object%20Reference))
  (bind _aswbp_main (Utilities|Casting|CastToWBP_Main (Variables|Default|GetMain%20Menu)))
  (Default|Deactivate _aswbp_main ttarget))

(fn AddWidgettoViewport
  (params (ActivatableWidgetClass :type Common%20Activatable%20Widget%20Class%20Reference))
  (bind _aswbp_main (Utilities|Casting|CastToWBP_Main (Variables|Default|GetMain%20Menu)))
  (bind _returnvalue (Default|PlshUIWidget(main) _aswbp_main ActivatableWidgetClass))
  (return _returnvalue))

(fn UpdataMiddleWidget
  (params (ActivatableWidgetClass :type Common%20Activatable%20Widget%20Class%20Reference))
  (bind _aswbp_main (Utilities|Casting|CastToWBP_Main (Variables|Default|GetMain%20Menu)))
  (Default|RemoveUIWidget(Middle) _aswbp_main)
  (bind _returnvalue (Default|PlshUIWidget(Middle) _aswbp_main ActivatableWidgetClass))
  (return _returnvalue))

(fn AddWidgettoViewport(middle)
  (params (ActivatableWidgetClass :type Common%20Activatable%20Widget%20Class%20Reference))
  (bind _aswbp_main (Utilities|Casting|CastToWBP_Main (Variables|Default|GetMain%20Menu)))
  (bind _returnvalue (Default|PlshUIWidget(Middle) _aswbp_main ActivatableWidgetClass))
  (return _returnvalue))