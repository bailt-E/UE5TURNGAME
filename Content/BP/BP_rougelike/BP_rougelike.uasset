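; Roguelike run manager that tracks coins, the current events and the blessings that buff units.
; Blessing attributes are summed field by field into one unit bonus struct covering base, edge, fixed and secondary stats.
; Event generation fills free slots from the front of normal or battle pools, favouring battles when coins are low.
; Initialization constructs event objects for the normal pool only; nothing here fills the battle pool.
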(fn GainBonusesBasedonBlessings
  (Variables|Globalinformation|Setrougelike_unit_attributs "")
  (for _array_element (Variables|blessing|Getrougelike_blessing_array)
    (Variables|Globalinformation|Setrougelike_unit_attributs (Utilities|Struct|Makest_rougelike_unit_bonus (Utilities|Struct|MakeST_pawn_Base_Stat_bonus (+ (.Attackdamagebonus (Utilities|Struct|BreakST_pawn_Base_Stat_bonus (.basestatbonus (Utilities|Struct|Breakst_rougelike_unit_bonus (Variables|/Game/BP/BP_rougelike/BP_rougelike_blessing.BP_rougelike_blessing_C|Getrougelike_attributs _array_element))))) (.Attackdamagebonus (Utilities|Struct|BreakST_pawn_Base_Stat_bonus (.basestatbonus (Utilities|Struct|Breakst_rougelike_unit_bonus (Variables|Globalinformation|Getrougelike_unit_attributs)))))) (+ (.Speedbonus (Utilities|Struct|BreakST_pawn_Base_Stat_bonus (.basestatbonus (Utilities|Struct|Breakst_rougelike_unit_bonus (Variables|/Game/BP/BP_rougelike/BP_rougelike_blessing.BP_rougelike_blessing_C|Getrougelike_attributs _array_element))))) (.Speedbonus (Utilities|Struct|BreakST_pawn_Base_Stat_bonus (.basestatbonus (Utilities|Struct|Breakst_rougelike_unit_bonus (Variables|Globalinformation|Getrougelike_unit_attributs)))))) (+ (.Healthbonus (Utilities|Struct|BreakST_pawn_Base_Stat_bonus (.basestatbonus (Utilities|Struct|Breakst_rougelike_unit_bonus (Variables|/Game/BP/BP_rougelike/BP_rougelike_blessing.BP_rougelike_blessing_C|Getrougelike_attributs _array_element))))) (.Healthbonus (Utilities|Struct|BreakST_pawn_Base_Stat_bonus (.basestatbonus (Utilities|Struct|Breakst_rougelike_unit_bonus (Variables|Globalinformation|Getrougelike_unit_attributs)))))) (+ (.Defensebonus (Utilities|Struct|BreakST_pawn_Base_Stat_bonus (.basestatbonus (Utilities|Struct|Breakst_rougelike_unit_bonus (Variables|/Game/BP/BP_rougelike/BP_rougelike_blessing.BP_rougelike_blessing_C|Getrougelike_attributs _array_element))))) (.Defensebonus (Utilities|Struct|BreakST_pawn_Base_Stat_bonus (.basestatbonus (Utilities|Struct|Breakst_rougelike_unit_bonus (Variables|Globalinformation|Getrougelike_unit_attributs)))))) (+ (.Criticalhitbonus (Utilities|Struct|BreakST_pawn_Base_Stat_bonus (.basestatbonus (Utilities|Struct|Breakst_rougelike_unit_bonus (Variables|/Game/BP/BP_rougelike/BP_rougelike_blessing.BP_rougelike_blessing_C|Getrougelike_attributs _array_element))))) (.Criticalhitbonus (Utilities|Struct|BreakST_pawn_Base_Stat_bonus (.basestatbonus (Utilities|Struct|Breakst_rougelike_unit_bonus (Variables|Globalinformation|Getrougelike_unit_attributs)))))) (+ (.Criticaldamagebonus (Utilities|Struct|BreakST_pawn_Base_Stat_bonus (.basestatbonus (Utilities|Struct|Breakst_rougelike_unit_bonus (Variables|/Game/BP/BP_rougelike/BP_rougelike_blessing.BP_rougelike_blessing_C|Getrougelike_attributs _array_element))))) (.Criticaldamagebonus (Utilities|Struct|BreakST_pawn_Base_Stat_bonus (.basestatbonus (Utilities|Struct|Breakst_rougelike_unit_bonus (Variables|Globalinformation|Getrougelike_unit_attributs))))))) (Utilities|Struct|MakeST_Edge_attributes_A (+ (.Healingbonus (Utilities|Struct|BreakST_Edge_attributes_A (.edgeattrobutes (Utilities|Struct|Breakst_rougelike_unit_bonus (Variables|/Game/BP/BP_rougelike/BP_rougelike_blessing.BP_rougelike_blessing_C|Getrougelike_attributs _array_element))))) (.Healingbonus (Utilities|Struct|BreakST_Edge_attributes_A (.edgeattrobutes (Utilities|Struct|Breakst_rougelike_unit_bonus (Variables|Globalinformation|Getrougelike_unit_attributs)))))) (+ (.Healbonus (Utilities|Struct|BreakST_Edge_attributes_A (.edgeattrobutes (Utilities|Struct|Breakst_rougelike_unit_bonus (Variables|/Game/BP/BP_rougelike/BP_rougelike_blessing.BP_rougelike_blessing_C|Getrougelike_attributs _array_element))))) (.Healbonus (Utilities|Struct|BreakST_Edge_attributes_A (.edgeattrobutes (Utilities|Struct|Breakst_rougelike_unit_bonus (Variables|Globalinformation|Getrougelike_unit_attributs)))))) (+ (.Shieldedbonus (Utilities|Struct|BreakST_Edge_attributes_A (.edgeattrobutes (Utilities|Struct|Breakst_rougelike_unit_bonus (Variables|/Game/BP/BP_rougelike/BP_rougelike_blessing.BP_rougelike_blessing_C|Getrougelike_attributs _array_element))))) (.Shieldedbonus (Utilities|Struct|BreakST_Edge_attributes_A (.edgeattrobutes (Utilities|Struct|Breakst_rougelike_unit_bonus (Variables|Globalinformation|Getrougelike_unit_attributs)))))) (+ (.Shieldbonus (Utilities|Struct|BreakST_Edge_attributes_A (.edgeattrobutes (Utilities|Struct|Breakst_rougelike_unit_bonus (Variables|/Game/BP/BP_rougelike/BP_rougelike_blessing.BP_rougelike_blessing_C|Getrougelike_attributs _array_element))))) (.Shieldbonus (Utilities|Struct|BreakST_Edge_attributes_A (.edgeattrobutes (Utilities|Struct|Breakst_rougelike_unit_bonus (Variables|Globalinformation|Getrougelike_unit_attributs)))))) (+ (.aggro_bonus (Utilities|Struct|BreakST_Edge_attributes_A (.edgeattrobutes (Utilities|Struct|Breakst_rougelike_unit_bonus (Variables|/Game/BP/BP_rougelike/BP_rougelike_blessing.BP_rougelike_blessing_C|Getrougelike_attributs _array_element))))) (.aggro_bonus (Utilities|Struct|BreakST_Edge_attributes_A (.edgeattrobutes (Utilities|Struct|Breakst_rougelike_unit_bonus (Variables|Globalinformation|Getrougelike_unit_attributs))))))) (Utilities|Struct|MakeST_Fixed_attributes_A (+ (.Speedcap (Utilities|Struct|BreakST_Fixed_attributes_A (.fixedattrobutes (Utilities|Struct|Breakst_rougelike_unit_bonus (Variables|/Game/BP/BP_rougelike/BP_rougelike_blessing.BP_rougelike_blessing_C|Getrougelike_attributs _array_element))))) (.Speedcap (Utilities|Struct|BreakST_Fixed_attributes_A (.fixedattrobutes (Utilities|Struct|Breakst_rougelike_unit_bonus (Variables|Globalinformation|Getrougelike_unit_attributs)))))) (+ (.Overloadroundcap (Utilities|Struct|BreakST_Fixed_attributes_A (.fixedattrobutes (Utilities|Struct|Breakst_rougelike_unit_bonus (Variables|/Game/BP/BP_rougelike/BP_rougelike_blessing.BP_rougelike_blessing_C|Getrougelike_attributs _array_element))))) (.Overloadroundcap (Utilities|Struct|BreakST_Fixed_attributes_A (.fixedattrobutes (Utilities|Struct|Breakst_rougelike_unit_bonus (Variables|Globalinformation|Getrougelike_unit_attributs)))))) (+ (.Maximumshield (Utilities|Struct|BreakST_Fixed_attributes_A (.fixedattrobutes (Utilities|Struct|Breakst_rougelike_unit_bonus (Variables|/Game/BP/BP_rougelike/BP_rougelike_blessing.BP_rougelike_blessing_C|Getrougelike_attributs _array_element))))) (.Maximumshield (Utilities|Struct|BreakST_Fixed_attributes_A (.fixedattrobutes (Utilities|Struct|Breakst_rougelike_unit_bonus (Variables|Globalinformation|Getrougelike_unit_attributs)))))) (+ (.Overloadcap (Utilities|Struct|BreakST_Fixed_attributes_A (.fixedattrobutes (Utilities|Struct|Breakst_rougelike_unit_bonus (Variables|/Game/BP/BP_rougelike/BP_rougelike_blessing.BP_rougelike_blessing_C|Getrougelike_attributs _array_element))))) (.Overloadcap (Utilities|Struct|BreakST_Fixed_attributes_A (.fixedattrobutes (Utilities|Struct|Breakst_rougelike_unit_bonus (Variables|Globalinformation|Getrougelike_unit_attributs)))))) (+ (.Energycap (Utilities|Struct|BreakST_Fixed_attributes_A (.fixedattrobutes (Utilities|Struct|Breakst_rougelike_unit_bonus (Variables|/Game/BP/BP_rougelike/BP_rougelike_blessing.BP_rougelike_blessing_C|Getrougelike_attributs _array_element))))) (.Energycap (Utilities|Struct|BreakST_Fixed_attributes_A (.fixedattrobutes (Utilities|Struct|Breakst_rougelike_unit_bonus (Variables|Globalinformation|Getrougelike_unit_attributs)))))) (+ (.unit_Actionpointcap (Utilities|Struct|BreakST_Fixed_attributes_A (.fixedattrobutes (Utilities|Struct|Breakst_rougelike_unit_bonus (Variables|/Game/BP/BP_rougelike/BP_rougelike_blessing.BP_rougelike_blessing_C|Getrougelike_attributs _array_element))))) (.unit_Actionpointcap (Utilities|Struct|BreakST_Fixed_attributes_A (.fixedattrobutes (Utilities|Struct|Breakst_rougelike_unit_bonus (Variables|Globalinformation|Getrougelike_unit_attributs)))))) (+ (.element_tag_number_MAX (Utilities|Struct|BreakST_Fixed_attributes_A (.fixedattrobutes (Utilities|Struct|Breakst_rougelike_unit_bonus (Variables|/Game/BP/BP_rougelike/BP_rougelike_blessing.BP_rougelike_blessing_C|Getrougelike_attributs _array_element))))) (.element_tag_number_MAX (Utilities|Struct|BreakST_Fixed_attributes_A (.fixedattrobutes (Utilities|Struct|Breakst_rougelike_unit_bonus (Variables|Globalinformation|Getrougelike_unit_attributs)))))) (+ (.Initialvelocity (Utilities|Struct|BreakST_Fixed_attributes_A (.fixedattrobutes (Utilities|Struct|Breakst_rougelike_unit_bonus (Variables|/Game/BP/BP_rougelike/BP_rougelike_blessing.BP_rougelike_blessing_C|Getrougelike_attributs _array_element))))) (.Initialvelocity (Utilities|Struct|BreakST_Fixed_attributes_A (.fixedattrobutes (Utilities|Struct|Breakst_rougelike_unit_bonus (Variables|Globalinformation|Getrougelike_unit_attributs)))))) (+ (.Initial_unit_actionpoint (Utilities|Struct|BreakST_Fixed_attributes_A (.fixedattrobutes (Utilities|Struct|Breakst_rougelike_unit_bonus (Variables|/Game/BP/BP_rougelike/BP_rougelike_blessing.BP_rougelike_blessing_C|Getrougelike_attributs _array_element))))) (.Initial_unit_actionpoint (Utilities|Struct|BreakST_Fixed_attributes_A (.fixedattrobutes (Utilities|Struct|Breakst_rougelike_unit_bonus (Variables|Globalinformation|Getrougelike_unit_attributs))))))) (Utilities|Struct|MakeST_Secondary_attributes_A 0 (+ (.Finaldamagebonus (Utilities|Struct|BreakST_Secondary_attributes_A (.secondaryattrobutes (Utilities|Struct|Breakst_rougelike_unit_bonus (Variables|/Game/BP/BP_rougelike/BP_rougelike_blessing.BP_rougelike_blessing_C|Getrougelike_attributs _array_element))))) (.Finaldamagebonus (Utilities|Struct|BreakST_Secondary_attributes_A (.secondaryattrobutes (Utilities|Struct|Breakst_rougelike_unit_bonus (Variables|Globalinformation|Getrougelike_unit_attributs)))))) (+ (.Damagereductionbonus (Utilities|Struct|BreakST_Secondary_attributes_A (.secondaryattrobutes (Utilities|Struct|Breakst_rougelike_unit_bonus (Variables|/Game/BP/BP_rougelike/BP_rougelike_blessing.BP_rougelike_blessing_C|Getrougelike_attributs _array_element))))) (.Damagereductionbonus (Utilities|Struct|BreakST_Secondary_attributes_A (.secondaryattrobutes (Utilities|Struct|Breakst_rougelike_unit_bonus (Variables|Globalinformation|Getrougelike_unit_attributs)))))))))))

(fn InitializetheCurrency
  (params (current_coins :type Integer))
  (Variables|Globalinformation|Setcurrent_coins current_coins)
  (Utilities|Array|Resize (Variables|event|GetCurrent%20events) 3))

(fn RemoveEvent
  (params (Item :type BP%20Rougelike%20Event%20Class%20Object%20Reference%20%28by%20ref%29))
  (Utilities|Array|RemoveItem (Variables|event|GetCurrent%20events) Item))

(fn GenerateEvents
  (bind _rougelike_battle_event (Variables|event|Getrougelike_battle_event))
  (bind _rougelike_normal_event (Variables|event|Getrougelike_normal_event))
  (bind _output (Utilities|Array|Get(acopy) _rougelike_battle_event))
  (bind _output_2 (Utilities|Array|Get(acopy) _rougelike_normal_event))
  (Utilities|FlowControl|Sequence
    (:then_0
      (if (< (Variables|Globalinformation|Getcurrent_coins) 100)
        (LocalVariables|Setweight 75)
        (else
          (LocalVariables|Setweight 50))))
    (:then_1
      (LocalVariables|SetNumber%20of%20events (Utilities|Array|Length (Variables|event|GetCurrent%20events))))
    (:then_2
      (if (< (LocalVariables|GetNumber%20of%20events) (Variables|Default|GetCurrent%20event%20cap))
        (if (> (Math|Random|RandomInteger 100) (LocalVariables|Getweight))
          (Utilities|Array|Add (Variables|event|GetCurrent%20events) _output_2)
          (Utilities|Array|RemoveItem (Variables|event|Getrougelike_normal_event) _output_2)
          (else
            (Utilities|Array|Add (Variables|event|GetCurrent%20events) _output)
            (Utilities|Array|RemoveItem (Variables|event|Getrougelike_battle_event) _output)))))))

(fn InitializeEventandRole
  (Utilities|FlowControl|Sequence
    (:then_0
      (bind _returnvalue (Game|ConstructObjectfromClass (Variables|Default|Getevent_class)))
      (Default|InitializetheEvent _returnvalue "NewEnumerator0")
      (Utilities|Array|Add (Variables|event|Getrougelike_normal_event) _returnvalue))
    (:then_1
      (bind _returnvalue_2 (Game|ConstructObjectfromClass (Variables|Default|Getevent_class)))
      (Default|InitializetheEvent _returnvalue_2 "NewEnumerator0")
      (Utilities|Array|Add (Variables|event|Getrougelike_normal_event) _returnvalue_2))))