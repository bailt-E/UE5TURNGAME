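; Blueprint class for battle-phase units, handling each unit's info widget, buff display and selection decal.
; On BeginPlay it creates a unit display widget bound to itself, then runs parent BeginPlay.
; Buff functions tell that widget to resync, while a custom event clears area buffs, compares buff data and updates buffs.
; The decal uses a dynamic material, tinted by enemy, pawn or neutral faction, with a Standby parameter reflecting selection.
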(event Custom|自定义事件
  (CallFunction|ChearAreabuffDockingPawnBuff)
  (bind _newparam (CallFunction|BuffDataComparison))
  (bind _output_get (Variables|Default|SetRotate _newparam))
  (CallFunction|UpdateBuff _output_get))

(event EventBeginPlay
  (Utilities|FlowControl|Sequence
    (:then_0
      (CallFunction|SetWidget))
    (:then_1
      (|CallParentFunction))))

(fn ConstructionScript
  (|CallParentFunction))

(fn SetWidget
  (bind _self self)
  (if (Utilities|IsValid _self)
    (bind _returnvalue (UserInterface|CreateWidget "/Game/WBP/wbp_unit/WBP_unit_display_widget.WBP_unit_display_widget_C" 0 _self))
    (UserInterface|SetWidget (Variables|Default|Getunit_datainfoWidget) _returnvalue)))

(fn AfterReceivingtheBuff
  (params (buff :type BP%20Buff%20Class%20Object%20Reference))
  (bind _aswbp_unit_display_widget (Utilities|Casting|CastToWBP_unit_display_widget (UserInterface|GetWidget (Variables|Default|Getunit_datainfoWidget))))
  (Default|SynchronizeBuffInformationtotheUnitControl _aswbp_unit_display_widget))

(fn UpdataUnitElementBuff
  (bind _aswbp_unit_display_widget (Utilities|Casting|CastToWBP_unit_display_widget (UserInterface|GetWidget (Variables|Default|Getunit_datainfoWidget))))
  (Default|SynchronizeBuffInformationtotheUnitControl _aswbp_unit_display_widget))

(fn UpdataDecal
  (params (unit_f :type E_unitfaction%20Enum :default "NewEnumerator0") (select_state :type Boolean))
  (bind _returnvalue (Rendering|Material|CreateDynamicMaterialInstance "/Game/M_MAT/M_character/M_character_Decal.M_character_Decal" "None" "None" :!class /Script/Engine.KismetMaterialLibrary))
  (LocalVariables|SetNewLocalVar _returnvalue)
  (Utilities|FlowControl|Sequence
    (:then_0
      (Utilities|FlowControl|Sequence
        (:then_0
          (if select_state
            (Rendering|Material|SetScalarParameterValue (LocalVariables|GetNewLocalVar) "Standby" 1.0 :!class /Script/Engine.MaterialInstanceDynamic)
            (else
              (Rendering|Material|SetScalarParameterValue (LocalVariables|GetNewLocalVar) "Standby" 1e+01 :!class /Script/Engine.MaterialInstanceDynamic))))
        (:then_1
          (switch Utilities|FlowControl|Switch|SwitchonE_unitfaction unit_f
            (:NewEnumerator0
              (Rendering|Material|SetVectorParameterValue (LocalVariables|GetNewLocalVar) "Friendly" "(R=1.000000,G=0.000000,B=0.018130,A=1.000000)" :!class /Script/Engine.MaterialInstanceDynamic))
            (:NewEnumerator1
              (Rendering|Material|SetVectorParameterValue (LocalVariables|GetNewLocalVar) "Friendly" "(R=0.000000,G=0.535382,B=1.000000,A=1.000000)" :!class /Script/Engine.MaterialInstanceDynamic))
            (:NewEnumerator2
              (Rendering|Material|SetVectorParameterValue (LocalVariables|GetNewLocalVar) "Friendly" "(R=0.007949,G=1.000000,B=0.311587,A=1.000000)" :!class /Script/Engine.MaterialInstanceDynamic))))))
    (:then_1
      (Rendering|Components|Decal|SetDecalMaterial (Variables|Default|GetDecal) (LocalVariables|GetNewLocalVar)))))