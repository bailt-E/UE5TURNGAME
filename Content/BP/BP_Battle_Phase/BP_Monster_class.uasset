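; Monster unit class for the battle phase, providing attribute setup and selection as a skill target.
; BeginPlay runs parent logic, sets the widget, then feeds HP, attack and defense with unit bonuses into the generic attribute component.
; Beselect registers the monster as the player character's TargetActor and triggers skill-target follow-up; NewMacro duplicates this logic.
; DataDocking rebuilds base attributes from the unit attribute component, ignoring its RowName input.
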(event EventBeselect
  (Utilities|FlowControl|Sequence
    (:then_0
      (bind _asbp_global_character (Utilities|Casting|CastToBP_GLOBAL_CHARACTER (Game|Player|GetPlayerPawn 0)))
      (Variables|/Game/BP/BP_Battle_Phase/BP_GLOBAL_CHARACTER.BP_GLOBAL_CHARACTER_C|Settarget_actor _asbp_global_character self))
    (:then_1
      (CallFunction|IsClickedEvent)
      (Default|SelectUnitSkillTargetAfter (Variables|Default|GetAs%20BP%20GLOBAL%20CHARATER))
      (CallFunction|CallPlayer))))

(event EventBeginPlay
  (bind _initialize_unit_information (Variables|Default|GetInitialize%20unit%20information))
  (bind _unit_attribute (Utilities|Struct|Breakst_level_unit_Initialize_DATA _initialize_unit_information))
  (bind (_hp_max _attack _defense) (Utilities|Struct|Breakst_the_unit_attribute _unit_attribute))
  (Utilities|FlowControl|Sequence
    (:then_0
      (|CallParentFunction))
    (:then_1
      (CallFunction|SetWidget)
      (bind _output_get (Variables|/Game/BP/BP_AC/BP_Generic_attributes_AC/AC_Generic_attributes.AC_Generic_attributes_C|SetUNIT_Fixed%20attributes (Variables|Default|GetAC_Generic_attributes) (Utilities|Struct|MakeST_Attribute_collection_AA (Utilities|Struct|MakeST_Base_attributes_A _hp_max _attack _defense) "(element_bonus_3_7E47476240021223A27EB1B15F25B237=((),(element_type_2_A382164746729B1F7E90C0B960DFA649=NewEnumerator1),(element_type_2_A382164746729B1F7E90C0B960DFA649=NewEnumerator2),(element_type_2_A382164746729B1F7E90C0B960DFA649=NewEnumerator4),(element_type_2_A382164746729B1F7E90C0B960DFA649=NewEnumerator3)),Finaldamagebonus_7_C0F6EFE54D0D41C34BEE3BA503A9A25C=0.000000,Damagereductionbonus_9_9010B5E8408BD39C6EABC9BBEBF850BC=0.000000)")))
      (bind _output_get_2 (Default|TickAttributes (Variables|Default|GetAC_Generic_attributes) (Variables|Default|Getunit_bonus) _output_get))
      (Default|InitializetheProperty (Variables|Default|GetAC_Generic_attributes) _output_get_2))))

(event MouseInput|EventActorOnClicked
  (params (ButtonPressed :type Key%20Structure)))

(fn ConstructionScript)

(fn DataDocking
  (params (RowName :type Name :default "None"))
  (bind _bp_ac_unit_attribute1 (Variables|Default|GetBP_AC_unit_attribute1))
  (bind _unit_attributes (Variables|/Game/BP/BP_AC/BP_UNIT_AC/BP_AC_unit_attribute.BP_AC_unit_attribute_C|Getunit_attributes _bp_ac_unit_attribute1))
  (bind (_hp_max _attack _defense) (Utilities|Struct|Breakst_the_unit_attribute _unit_attributes))
  (bind _output_get (Variables|/Game/BP/BP_AC/BP_Generic_attributes_AC/AC_Generic_attributes.AC_Generic_attributes_C|SetUNIT_Fixed%20attributes (Variables|Default|GetAC_Generic_attributes) (Utilities|Struct|MakeST_Attribute_collection_AA (Utilities|Struct|MakeST_Base_attributes_A _hp_max _attack _defense) "(element_bonus_3_7E47476240021223A27EB1B15F25B237=((),(element_type_2_A382164746729B1F7E90C0B960DFA649=NewEnumerator1),(element_type_2_A382164746729B1F7E90C0B960DFA649=NewEnumerator2),(element_type_2_A382164746729B1F7E90C0B960DFA649=NewEnumerator4),(element_type_2_A382164746729B1F7E90C0B960DFA649=NewEnumerator3)),Finaldamagebonus_7_C0F6EFE54D0D41C34BEE3BA503A9A25C=0.000000,Damagereductionbonus_9_9010B5E8408BD39C6EABC9BBEBF850BC=0.000000)")))
  (return _output_get))