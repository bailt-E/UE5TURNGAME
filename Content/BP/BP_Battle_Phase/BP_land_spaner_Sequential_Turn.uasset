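; Battle controller that runs sequential, action-point-ordered turn combat between player and enemy units.
; BattleProcess switches on battle phase: Prepare loads level data and spawns boards, characters and the first wave, then sequence init seeds action points and selects the unit with the fewest.
; In the round loop, turn start ticks that unit's buffs and fires auto skills.
; Action selection builds enemy actions through Enemyteam or signals the player's turn start.
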(event EventBeginPlay
  (|CallParentFunction) ; 此节点被禁用，将不会被调用。\n从引脚连出引线来编译功能。
)

(event Collision|EventActorBeginOverlap
  (params (OtherActor :type Actor%20Object%20Reference)))

(event EventTick
  (params (DeltaSeconds :type Float%20%28single-precision%29)))

(fn ConstructionScript
  (|CallParentFunction))

(fn BattleProcess
  (switch Utilities|FlowControl|Switch|SwitchonE_Sequence_Battle_Phase (Variables|Default|Getbattle_phase)
    (:NewEnumerator0
      (CallFunction|DataInitialize)
      (CallFunction|GetlevelData (Variables|Default|Getlevel_rowname))
      (CallFunction|SpawnEnemyBoards)
      (CallFunction|GenerateYourBoardandCharacters (Variables|Default|Getteam_data))
      (CallFunction|SpawnNewRoundsOfUnitontheBattlefield 0 (Variables|Default|Getlevel_rowname)))
    (:NewEnumerator1
      (CallFunction|ActionpointInitial)
      (bind _base_pawn (CallFunction|UnitwiththeFewestActionPoints))
      (Variables|Default|SetBase%20Pawn _base_pawn)
      (Variables|Default|Setbattle_phase "NewEnumerator2"))
    (:NewEnumerator2
      (switch Utilities|FlowControl|Switch|SwitchonE_Sequence_Round_Phase (Variables|Default|Getbattle_round_phase)
        (:NewEnumerator0
          (Default|Tick (Variables|/Game/BP/BP_Battle_Phase/BP_BASE_Pawn.BP_BASE_Pawn_C|GetAC_buff (Variables|Default|GetBase%20Pawn)))
          (Default|AutoSkillUse (Variables|Default|GetAC_autoskill) (Variables|Default|GetUnit%20Class) (Variables|Default|Getaction_info) "NewEnumerator2") ; 使用自动技能
        )
        (:NewEnumerator1
          (for _array_element (Variables|Default|GetUnit%20Class)
            (bind _asbp_base_pawn (Utilities|Casting|CastToBP_BASE_Pawn (.charter (Utilities|Struct|Breakst_unit_class _array_element))))
            (if (== (Variables|Default|GetBase%20Pawn) _asbp_base_pawn)
              (switch Utilities|FlowControl|Switch|SwitchonE_unitfaction (.theunit_Belongs (Utilities|Struct|Breakst_unit_class _array_element))
                (:NewEnumerator0
                  (bind (_canact _create _target _action_type) (Default|UseUnitSkill (Variables|Default|Getenemyteam) (Variables|Default|GetBase%20Pawn)))
                  (Variables|Default|Setaction_info (Utilities|Struct|Makest_action _create _target _action_type)))
                (:NewEnumerator1
                  (Default|AttheBeginningOfOurUnit'sTurn (Variables|Default|GetAs%20BP%20GLOBAL%20CHARATER) (Variables|Default|GetBase%20Pawn)))))))))))

(fn ActionpointInitial
  (for _array_element (Variables|Default|GetUnit%20Class)
    (bind _asbp_base_pawn (Utilities|Casting|CastToBP_BASE_Pawn (.charter (Utilities|Struct|Breakst_unit_class _array_element))))
    (Default|GetInitialActionPoints (Variables|/Game/BP/BP_Battle_Phase/BP_BASE_Pawn.BP_BASE_Pawn_C|GetAC_Generic_attributes _asbp_base_pawn))))

(fn UnitwiththeFewestActionPoints
  (for _array_element (Variables|Default|GetUnit%20Class)
    (bind _asbp_base_pawn (Utilities|Casting|CastToBP_BASE_Pawn (.charter (Utilities|Struct|Breakst_unit_class _array_element))))
    (if (Utilities|IsValid (LocalVariables|Getpawn))
      (if (< (Variables|/Game/BP/BP_AC/BP_Generic_attributes_AC/AC_Generic_attributes.AC_Generic_attributes_C|Getcurrent_action_point (Variables|/Game/BP/BP_Battle_Phase/BP_BASE_Pawn.BP_BASE_Pawn_C|GetAC_Generic_attributes _asbp_base_pawn)) (Variables|/Game/BP/BP_AC/BP_Generic_attributes_AC/AC_Generic_attributes.AC_Generic_attributes_C|Getcurrent_action_point (Variables|/Game/BP/BP_Battle_Phase/BP_BASE_Pawn.BP_BASE_Pawn_C|GetAC_Generic_attributes (LocalVariables|Getpawn)))) ; 当前单位的行动值是否小于
        (LocalVariables|Setpawn _asbp_base_pawn))
      (else
        (LocalVariables|Setpawn _asbp_base_pawn))))
  (return (LocalVariables|Getpawn)))