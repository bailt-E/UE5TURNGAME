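; Sequential-turn battle character Blueprint that turns player key presses into turn actions in the battle phase.
; Q and E set the same player action with different skill types and call GetTheSkillNumber, while F sets a second action with no skill lookup.
; All three keys set the turn game state, then run SequentialTurn.
; An unconnected branch that would set the land spawner's battle round phase never runs.
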(event EventBeginPlay)

(event Collision|EventActorBeginOverlap
  (params (OtherActor :type Actor%20Object%20Reference)))

(event EventTick
  (params (DeltaSeconds :type Float%20%28single-precision%29)))

(event Input|KeyboardEvents|F
  (params (Key :type Key%20Structure))
  (:Pressed
    (Variables|Default|Setplayer_action "NewEnumerator1")
    (Variables|Default|SetTurn_GAME_state "NewEnumerator2")
    (CallFunction|SequentialTurn)))

(event Input|KeyboardEvents|SpaceBar
  (params (Key :type Key%20Structure)))

(event Input|KeyboardEvents|E
  (params (Key :type Key%20Structure))
  (:Pressed
    (Variables|Default|Setplayer_action "NewEnumerator0")
    (Variables|Default|SetTurn_GAME_state "NewEnumerator2")
    (bind _output_get (Variables|Default|Setskill_type "NewEnumerator0"))
    (CallFunction|GettheSkillNumber _output_get)
    (CallFunction|SequentialTurn)))

(event Input|KeyboardEvents|3
  (params (Key :type Key%20Structure)))

(event Input|KeyboardEvents|1
  (params (Key :type Key%20Structure)))

(event Input|KeyboardEvents|2
  (params (Key :type Key%20Structure)))

(event Input|KeyboardEvents|4
  (params (Key :type Key%20Structure)))

(event Input|KeyboardEvents|Q
  (params (Key :type Key%20Structure))
  (:Pressed
    (Variables|Default|Setplayer_action "NewEnumerator0")
    (Variables|Default|SetTurn_GAME_state "NewEnumerator2")
    (bind _output_get (Variables|Default|Setskill_type "NewEnumerator2"))
    (CallFunction|GettheSkillNumber _output_get)
    (CallFunction|SequentialTurn)))

(fn ConstructionScript
  (|CallParentFunction))