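; Enemy team controller for the battle phase, which picks and executes monster skill actions against a team action point budget.
; It resets monster turn attributes through the battle Land, then filters actionable units by skill cost and picks the one with the most action points.
; That unit's skill component chooses a skill, finds main and derived targets and uses it.
; The team then loses a point and Land's player buff component responds.
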(fn InitializationEvenUnitActionpoint
  (params (unit :type Array%20of%20St%20Unit%20Class%20Structures) (landx :type BP%20Land%20Spaner%20Object%20Reference))
  (for _array_element unit
    (bind _asbp_base_pawn (Utilities|Casting|CastToBP_BASE_Pawn (.charter (Utilities|Struct|Breakst_unit_class _array_element))))
    (if (Utilities|IsValid _asbp_base_pawn)
      (if (and (Utilities|Enum|Equal(Enum) (Variables|/Game/BP/BP_Battle_Phase/BP_BASE_Pawn.BP_BASE_Pawn_C|Getgameplay_unit_type _asbp_base_pawn) "NewEnumerator0") (Utilities|Enum|Equal(Enum) (Variables|/Game/BP/BP_Battle_Phase/BP_BASE_Pawn.BP_BASE_Pawn_C|Getunit_faction _asbp_base_pawn) "NewEnumerator0"))
        (bind _asbp_monster_class (Utilities|Casting|CastToBP_Monster_class _asbp_base_pawn))
        (Default|TurnUnitReset (Variables|/Game/BP/BP_Battle_Phase/BP_BASE_Pawn.BP_BASE_Pawn_C|GetAC_Generic_attributes _asbp_monster_class) landx)
        (Variables|Default|Setland landx)))))

(fn TheNumberOfInitializationActions
  (Variables|Default|SetCurrent%20Action%20Point (Variables|Default|Getactionpoint_max)))

(fn CheckifYouCanAct
  (params (unit_class :type Array%20of%20St%20Unit%20Class%20Structures))
  (bind _filter_unit (CallFunction|FilterUnitsThatCanTakeAction unit_class)) ; 筛选单位
  (bind (_continue _asbp_unit_class) (action|SelectActionPintMaxUNIT _filter_unit))
  (if _continue
    (if (Utilities|IsValid _asbp_unit_class)
      (bind _output_get (LocalVariables|Setskillcreate _asbp_unit_class))
      (if (Utilities|IsValid _output_get)
        (bind _unit_skill (Default|SelectUnitSkill (Variables|/Game/BP/BP_Battle_Phase/BP_Monster_class.BP_Monster_class_C|GetAC_unit_Skill (LocalVariables|Getskillcreate)) (LocalVariables|Getskillcreate))) ; 选择单位的技能
        (bind _output_get_2 (LocalVariables|Setskillname (Utilities|Struct|Breakst_unitclass_skilldata _unit_skill)))
        (bind (_skill_mind_target _returnvalue) (Default|FindMainObjective (Variables|/Game/BP/BP_Battle_Phase/BP_Monster_class.BP_Monster_class_C|GetAC_unit_Skill (LocalVariables|Getskillcreate)) _output_get_2 (LocalVariables|Getskillcreate) "NewEnumerator1"))
        (if _returnvalue
          (LocalVariables|Setmind_target _skill_mind_target)
          (bind _targetdata1 (Default|FindTargetsBasedonMainObjectives (Variables|/Game/BP/BP_Battle_Phase/BP_Monster_class.BP_Monster_class_C|GetAC_unit_Skill (LocalVariables|Getskillcreate)) (LocalVariables|Getskillcreate) (LocalVariables|Getmind_target) (LocalVariables|Getskillname) "NewEnumerator1")) ; 问题
          (bind _action_type (Default|UseUnitSkill (Variables|/Game/BP/BP_Battle_Phase/BP_Monster_class.BP_Monster_class_C|GetAC_unit_Skill (LocalVariables|Getskillcreate)) (LocalVariables|Getskillname) "NewEnumerator1" (LocalVariables|Getskillcreate) _targetdata1))
          (LocalVariables|Setlocal_action_type _action_type)
          (action|ReduceActionPoints)
          (Default|ActionUnitResponse (Variables|/Game/BP/BP_Battle_Phase/BP_land_spaner.BP_land_spaner_C|GetAC_player_buff_C (Variables|Default|Getland)) "NewEnumerator8" "NewEnumerator1" "NewEnumerator2" "NewEnumerator0" (LocalVariables|Getlocal_action_type) "NewEnumerator0" (LocalVariables|Getskillcreate) (LocalVariables|Getmind_target) 0.0)
          (return true (LocalVariables|Getskillcreate) (LocalVariables|Getmind_target) (LocalVariables|Getlocal_action_type))
          (else
            (Development|PrintString 0 "主要单位失效" true true "(R=1.000000,G=0.832202,B=0.000000,A=1.000000)" 1e+02)
            (return false 0 0 "NewEnumerator0"))))
      (else
        (Development|PrintString 0 "单位不存在" true true "(R=1.000000,G=0.900080,B=0.000000,A=1.000000)" 1e+02)
        (return false 0 0 "NewEnumerator0")))
    (else
      (return _continue 0 0 "NewEnumerator0"))))

(fn SelectActionPintMaxUNIT
  (params (Array :type Array%20of%20St%20Unit%20Class%20Structures))
  (if (>= (Utilities|Array|Length Array) 1)
    (Utilities|FlowControl|Sequence
      (:then_0
        (for _array_element Array
          (bind _asbp_base_pawn (Utilities|Casting|CastToBP_BASE_Pawn (.charter (Utilities|Struct|Breakst_unit_class _array_element))))
          (bind _asbp_unit_class (Utilities|Casting|CastToBP_Unit_class _asbp_base_pawn))
          (bind _asbp_monster_class (Utilities|Casting|CastToBP_Monster_class _asbp_unit_class))
          (if (Math|Boolean|ANDBoolean (Variables|/Game/BP/BP_Battle_Phase/BP_BASE_Pawn.BP_BASE_Pawn_C|Getunit_can_action _asbp_monster_class) (Utilities|Enum|Equal(Enum) (.theunit_Belongs (Utilities|Struct|Breakst_unit_class _array_element)) "NewEnumerator0") (Utilities|Enum|Equal(Enum) (Variables|/Game/BP/BP_Battle_Phase/BP_BASE_Pawn.BP_BASE_Pawn_C|Getgameplay_unit_type _asbp_unit_class) "NewEnumerator0")) ; 单位筛选条件
            (if (Utilities|IsValid (LocalVariables|Getunit_target))
              (Math|Integer|CompareInt (Utilities|Struct|Breakst_the_unit_resource (Variables|/Game/BP/BP_AC/BP_UNIT_AC/BP_AC_unit_attribute.BP_AC_unit_attribute_C|Getunit_resource (Variables|/Game/BP/BP_Battle_Phase/BP_Monster_class.BP_Monster_class_C|GetBP_AC_unit_attribute1 _asbp_monster_class))) (Utilities|Struct|Breakst_the_unit_resource (Variables|/Game/BP/BP_AC/BP_UNIT_AC/BP_AC_unit_attribute.BP_AC_unit_attribute_C|Getunit_resource (Variables|/Game/BP/BP_Battle_Phase/BP_Monster_class.BP_Monster_class_C|GetBP_AC_unit_attribute1 (LocalVariables|Getunit_target)))) ; 选择行动点最大的单位
                (:>
                  _)
                (:==
                  _))
              (LocalVariables|Setunit_target _asbp_monster_class)
              (else
                (LocalVariables|Setunit_target _asbp_monster_class))))))
      (:then_1
        (return (Utilities|IsValid (LocalVariables|Getunit_target)) (LocalVariables|Getunit_target))))
    (else
      (return false (LocalVariables|Getunit_target)))))

(fn CheckActionpointEnough
  (if (> (- (Variables|Default|GetCurrent%20Action%20Point) 1) 0) ; 检查行动点是否足够
    (Variables|Default|SetCurrent%20Action%20Point (- (Variables|Default|GetCurrent%20Action%20Point) 1))
    (return false) ; 足够
    (else
      (return true) ; 不足够
    )))

(fn ReduceActionPoints
  (Variables|Default|SetCurrent%20Action%20Point (- (Variables|Default|GetCurrent%20Action%20Point) 1)))

(fn FilterUnitsThatCanTakeAction
  (params (Array :type Array%20of%20St%20Unit%20Class%20Structures))
  (Utilities|FlowControl|Sequence
    (:then_0
      (for _array_element Array
        (bind _asbp_base_pawn (Utilities|Casting|CastToBP_BASE_Pawn (.charter (Utilities|Struct|Breakst_unit_class _array_element))))
        (bind _asbp_unit_class (Utilities|Casting|CastToBP_Unit_class _asbp_base_pawn))
        (bind _asbp_monster_class (Utilities|Casting|CastToBP_Monster_class _asbp_unit_class))
        (LocalVariables|SetMonster _asbp_monster_class)
        (if (Math|Boolean|ANDBoolean (Variables|/Game/BP/BP_Battle_Phase/BP_BASE_Pawn.BP_BASE_Pawn_C|Getunit_can_action _asbp_unit_class) (Utilities|Enum|Equal(Enum) (.theunit_Belongs (Utilities|Struct|Breakst_unit_class _array_element)) "NewEnumerator0") (Utilities|Enum|Equal(Enum) (Variables|/Game/BP/BP_Battle_Phase/BP_BASE_Pawn.BP_BASE_Pawn_C|Getgameplay_unit_type _asbp_monster_class) "NewEnumerator0")) ; 初级筛选
          (for _array_element_2 (Variables|/Game/BP/BP_Battle_Phase/BP_Monster_class.BP_Monster_class_C|Getunit_skill (LocalVariables|GetMonster))
            (if (== (.infinite (Utilities|Struct|Breakst_unitclass_skilldata _array_element_2)) false) ; 技能是否是永久
              (if (<= (.actionpoint (Utilities|Struct|Breakst_unitclass_skilldata _array_element_2)) (Utilities|Struct|BreakST_UNIT_Current_resource_AA (Variables|/Game/BP/BP_AC/BP_Generic_attributes_AC/AC_Generic_attributes.AC_Generic_attributes_C|GetCurrent_resource (Variables|/Game/BP/BP_Battle_Phase/BP_BASE_Pawn.BP_BASE_Pawn_C|GetAC_Generic_attributes (LocalVariables|GetMonster))))) :!label _label ; 技能行动点是否小于单位的行动点
                (Utilities|Array|Add (LocalVariables|GetFilter) _array_element))
              (elif (> (.use_number (Utilities|Struct|Breakst_unitclass_skilldata _array_element_2)) 0) ; 次数大于1
                (goto _label)))))))
    (:then_1
      (return (LocalVariables|GetFilter)))))

(fn UseUnitSkill
  (params (unit :type BP%20BASE%20Pawn%20Object%20Reference))
  (Utilities|FlowControl|Sequence
    (:then_0
      (Utilities|Casting|CastToBP_Monster_class unit)
      (LocalVariables|Setmonster 0))
    (:then_1
      (bind _unit_skill (Default|SelectUnitSkill (Variables|/Game/BP/BP_Battle_Phase/BP_Monster_class.BP_Monster_class_C|GetAC_unit_Skill (LocalVariables|Getmonster)) (LocalVariables|Getmonster))) ; 选择单位的技能
      (LocalVariables|Setskill_name (.skill_name (Utilities|Struct|Breakst_unitclass_skilldata _unit_skill)))
      (bind (_skill_mind_target _returnvalue) (Default|FindMainObjective (Variables|/Game/BP/BP_Battle_Phase/BP_Monster_class.BP_Monster_class_C|GetAC_unit_Skill (LocalVariables|Getmonster)) (LocalVariables|Getskill_name) (LocalVariables|Getmonster) "NewEnumerator1"))
      (if _returnvalue
        (LocalVariables|Setskill_target _skill_mind_target)
        (bind _targetdata1 (Default|FindTargetsBasedonMainObjectives (Variables|/Game/BP/BP_Battle_Phase/BP_Monster_class.BP_Monster_class_C|GetAC_unit_Skill (LocalVariables|Getmonster)) (LocalVariables|Getmonster) (LocalVariables|Getskill_target) (LocalVariables|Getskill_name) "NewEnumerator1")) ; 问题
        (bind _action_type (Default|UseUnitSkill (Variables|/Game/BP/BP_Battle_Phase/BP_Monster_class.BP_Monster_class_C|GetAC_unit_Skill (LocalVariables|Getmonster)) (LocalVariables|Getskill_name) "NewEnumerator1" (LocalVariables|Getmonster) _targetdata1))
        (LocalVariables|Setaction _action_type)
        (action|ReduceActionPoints)
        (Default|ActionUnitResponse (Variables|/Game/BP/BP_Battle_Phase/BP_land_spaner.BP_land_spaner_C|GetAC_player_buff_C (Variables|Default|Getland)) "NewEnumerator7" "NewEnumerator1" "NewEnumerator2" "NewEnumerator4" "NewEnumerator3" "NewEnumerator0" (LocalVariables|Getmonster) (LocalVariables|Getskill_target) 0.0)
        (return true (LocalVariables|Getmonster) (LocalVariables|Getskill_target) (LocalVariables|Getaction))))))

(fn NewFunction
  (params (Action_typexxc :type E_skill_action_type%20Enum :default "NewEnumerator3") (action_object :type BP%20BASE%20Pawn%20Object%20Reference) (target_object :type BP%20BASE%20Pawn%20Object%20Reference))
  (Utilities|FlowControl|Sequence
    (:then_0
      (LocalVariables|Sett_action_type (CallFunction|SkillTypeActionSwitch Action_typexxc (Variables|Default|Getland))))
    (:then_1
      (Variables|/Game/BP/BP_Battle_Phase/BP_land_spaner.BP_land_spaner_C|Setbattle_overall (Variables|Default|Getland) (Utilities|Struct|Makest_Battlefield_Inspector "NewEnumerator4" "NewEnumerator1" "NewEnumerator2" "NewEnumerator4" "NewEnumerator3" (LocalVariables|Gett_action_type) action_object target_object)))))