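; BP_gamechear_class is a selectable "chear" actor used in the battle phase, with a Cube mesh as its visual.
; Its Beselect event checks the turn state and player action on the global character, then registers itself as SelectedChear and fires that character's PlayerEvent.
; SetChearMaterial swaps a material slot on the Cube.
; Tick, click and construction script are empty, so selection relies on Beselect being called.
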(event EventBeginPlay)

(event Collision|EventActorBeginOverlap
  (params (OtherActor :type Actor%20Object%20Reference)))

(event EventTick
  (params (DeltaSeconds :type Float%20%28single-precision%29)))

(event MouseInput|EventActorOnClicked
  (params (ButtonPressed :type Key%20Structure :default "None")))

(event EventBeselect
  (bind _as_bp_global_charater (Variables|Default|GetAs%20BP%20GLOBAL%20CHARATER))
  (bind _as_bp_global_charater_2 (Variables|Default|GetAs%20BP%20GLOBAL%20CHARATER))
  (if (and (Utilities|Enum|Equal(Enum) (Variables|/Game/BP/BP_Battle_Phase/BP_GLOBAL_CHARACTER.BP_GLOBAL_CHARACTER_C|GetTurn_GAME_state _as_bp_global_charater_2) "NewEnumerator8") (Utilities|Enum|Equal(Enum) (Variables|/Game/BP/BP_Battle_Phase/BP_GLOBAL_CHARACTER.BP_GLOBAL_CHARACTER_C|Getplayer_action _as_bp_global_charater_2) "NewEnumerator1"))
    (Variables|/Game/BP/BP_Battle_Phase/BP_GLOBAL_CHARACTER.BP_GLOBAL_CHARACTER_C|SetSelected%20chear _as_bp_global_charater self)
    (Default|CallPlayerEvent _as_bp_global_charater)))

(fn ConstructionScript)

(fn SetChearMaterial
  (params (ElementIndex :type Integer) (Material :type Material%20Interface%20Object%20Reference))
  (Rendering|Material|SetMaterial (Variables|Default|GetCube) ElementIndex Material))