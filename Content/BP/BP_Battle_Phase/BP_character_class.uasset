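; Battle-phase character unit Blueprint that sets up a character's skills and stats and handles its selection.
; On spawn it builds the skill list from CharacterCoreData plus the current finisher, then initializes the widget and attributes from the level data table.
; Selection checks the global character's action and game flow, then registers the target and updates either battle UI or decal.
; Tick runs a health check.
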(event Custom|character_be_spawn
  (CallFunction|CharacterDataBegin)
  (CallFunction|UnitInitializationFunction)
  (CallFunction|SetWidget)
  (bind _newparam (CallFunction|DataDocking (Variables|Default|GetLevel)))
  (bind _output_get (Default|TickAttributes (Variables|Default|GetAC_Generic_attributes) (Variables|Default|Getunit_bonus) _newparam))
  (Default|InitializetheProperty (Variables|Default|GetAC_Generic_attributes) _output_get))

(event EventBeginPlay
  (|CallParentFunction))

(event EventTick
  (params (DeltaSeconds :type Float%20%28single-precision%29))
  (CallFunction|CheakHealth（NG）))

(event EventBeselect
  (Utilities|FlowControl|Sequence
    (:then_0
      (bind _output_get (CallFunction|GetPlayer))
      (Variables|Default|SetAs%20BP%20GLOBAL%20CHARATER _output_get)
      (if (and (Utilities|Enum|Equal(Enum) (Variables|/Game/BP/BP_Battle_Phase/BP_GLOBAL_CHARACTER.BP_GLOBAL_CHARACTER_C|Getplayer_action (Variables|Default|GetAs%20BP%20GLOBAL%20CHARATER)) "NewEnumerator5") (Utilities|Enum|Equal(Enum) (Variables|/Game/BP/BP_Battle_Phase/BP_land_spaner.BP_land_spaner_C|GetGame%20flow (Variables|/Game/BP/BP_Battle_Phase/BP_GLOBAL_CHARACTER.BP_GLOBAL_CHARACTER_C|Getland (Variables|Default|GetAs%20BP%20GLOBAL%20CHARATER))) "NewEnumerator1")) ; 检查回合
        (CallFunction|StelectTarget (Variables|Default|GetAs%20BP%20GLOBAL%20CHARATER))
        (CallFunction|UpdataBattleWidget)
        (CallFunction|CallPlayer)
        (Default|WhenCharacterBeselect (Variables|Default|GetAs%20BP%20GLOBAL%20CHARATER))
        (elif (and (Utilities|Enum|NotEqual(Enum) (Variables|/Game/BP/BP_Battle_Phase/BP_GLOBAL_CHARACTER.BP_GLOBAL_CHARACTER_C|Getplayer_action (Variables|Default|GetAs%20BP%20GLOBAL%20CHARATER)) "NewEnumerator0") (Utilities|Enum|NotEqual(Enum) (Variables|/Game/BP/BP_Battle_Phase/BP_GLOBAL_CHARACTER.BP_GLOBAL_CHARACTER_C|Getplayer_action (Variables|Default|GetAs%20BP%20GLOBAL%20CHARATER)) "NewEnumerator1"))
          (CallFunction|StelectTarget (Variables|Default|GetAs%20BP%20GLOBAL%20CHARATER))
          (Variables|/Game/BP/BP_Battle_Phase/BP_GLOBAL_CHARACTER.BP_GLOBAL_CHARACTER_C|SetTurn_GAME_state (Variables|Default|GetAs%20BP%20GLOBAL%20CHARATER) "NewEnumerator2")
          (CallFunction|CallPlayer)
          (CallFunction|UpdataDecal "NewEnumerator1" true))))
    (:then_1
      (CallFunction|IsClickedEvent)
      (Default|SelectUnitSkillTargetAfter (Variables|Default|GetAs%20BP%20GLOBAL%20CHARATER))
      (CallFunction|CallPlayer))))

(fn ConstructionScript)

(fn GetPlayer
  (bind _asbp_global_character (Utilities|Casting|CastToBP_GLOBAL_CHARACTER (Game|Player|GetPlayerPawn 0)))
  (return _asbp_global_character))

(fn TakeEffects
  (params (Effects :type St%20Child%20Base%20Attributes%20Structure)))

(fn DataDocking
  (params (RowName :type Name :default "None"))
  (bind _ac_level (Variables|组件|GetAC_level))
  (bind _pawn_fix_attributes (Variables|/Game/BP/BP_AC/BP_Player_level_AC/AC_level_exp.AC_level_exp_C|Getpawn_fix_attributes _ac_level))
  (bind (_speedcap _overloadroundcap _maximumshield _overloadcap _energycap _unit_actionpointcap _element_tag_number_max _initialvelocity _initial_unit_actionpoint) (Utilities|Struct|BreakST_Fixed_attributes_A _pawn_fix_attributes))
  (bind _returnvalue (Utilities|GetDataTableRow "/Game/Struct/rank_table/T_character_level_data.T_character_level_data" RowName)
    (:then
      (bind _output_get (Variables|/Game/BP/BP_AC/BP_Generic_attributes_AC/AC_Generic_attributes.AC_Generic_attributes_C|SetUNIT_Fixed%20attributes (Variables|Default|GetAC_Generic_attributes) (Utilities|Struct|MakeST_Attribute_collection_AA (Utilities|Struct|MakeST_Base_attributes_A (.Health (Utilities|Struct|Breakst_character_bese_level_data _returnvalue)) (.Attack (Utilities|Struct|Breakst_character_bese_level_data _returnvalue)) (.defense (Utilities|Struct|Breakst_character_bese_level_data _returnvalue)) 50 (Math|Float|Truncate 5.0) (Math|Float|Truncate 1.5e+02)) (Utilities|Struct|MakeST_Edge_attributes_A 0.0 0.0) (Utilities|Struct|MakeST_Fixed_attributes_A _speedcap _overloadroundcap _maximumshield _overloadcap _energycap _unit_actionpointcap _element_tag_number_max _initialvelocity _initial_unit_actionpoint) "(element_bonus_3_7E47476240021223A27EB1B15F25B237=((),(element_type_2_A382164746729B1F7E90C0B960DFA649=NewEnumerator1),(element_type_2_A382164746729B1F7E90C0B960DFA649=NewEnumerator2),(element_type_2_A382164746729B1F7E90C0B960DFA649=NewEnumerator4),(element_type_2_A382164746729B1F7E90C0B960DFA649=NewEnumerator3)),Finaldamagebonus_7_C0F6EFE54D0D41C34BEE3BA503A9A25C=0.000000,Damagereductionbonus_9_9010B5E8408BD39C6EABC9BBEBF850BC=0.000000)")))
      (return _output_get))))

(fn StelectTarget
  (params (global :type BP%20GLOBAL%20CHARACTER%20Object%20Reference))
  (Variables|/Game/BP/BP_Battle_Phase/BP_GLOBAL_CHARACTER.BP_GLOBAL_CHARACTER_C|SetSelected%20Widget global self)
  (Variables|/Game/BP/BP_Battle_Phase/BP_GLOBAL_CHARACTER.BP_GLOBAL_CHARACTER_C|SetAs%20BP%20Base%20Pawn%20Class global self))

(fn UpdataBattleWidget
  (bind _as2dplayer_contrller (Utilities|Casting|CastTo2DplayerContrller (Game|GetPlayerController 0)))
  (bind _aswbp_main (Utilities|Casting|CastToWBP_Main (Variables|/Game/BP/BP_AC/BP_UIManager/AC_UI_ManagerComponent.AC_UI_ManagerComponent_C|GetMain%20Menu (Variables|/Game/gamemode/2DplayerContrller.2DplayerContrller_C|GetAC_UI_ManagerComponent _as2dplayer_contrller))))
  (bind _aswbp_main_battle (Utilities|Casting|CastToWBP_Main_battle (Variables|/Game/WBP_common_ui/Parentcontrol_widget/WBP_Main.WBP_Main_C|GetUnderlying%20stack_widget _aswbp_main)))
  (Default|UpdataMainCharacter _aswbp_main_battle self))

(fn CharacterDataBegin
  (bind _character_core_data (Variables|Default|Getcharacter_core_data))
  (Utilities|Array|Clear (Variables|pawn_Data|GetThe_final_skill))
  (Variables|pawn_Data|Setlocal_Regular_skill (Variables|/Game/BP/BP_AC/BP_Player_level_AC/BP_character_object.BP_character_object_C|GetG_skill_%20Data _character_core_data))
  (Variables|pawn_Data|Setlocal_finsher_array (Variables|/Game/BP/BP_AC/BP_Player_level_AC/BP_character_object.BP_character_object_C|GetG_Finish%20Skill _character_core_data))
  (Variables|Default|SetLevel (Variables|/Game/BP/BP_AC/BP_Player_level_AC/BP_character_object.BP_character_object_C|Getlevel _character_core_data))
  (Variables|pawn_Data|Setname (Utilities|Struct|Breakst_character_info (Utilities|Struct|Breakst_player_character_data (Variables|/Game/BP/BP_AC/BP_Player_level_AC/BP_character_object.BP_character_object_C|Getcharacter_data _character_core_data))))
  (for _array_element (Variables|pawn_Data|Getlocal_Regular_skill)
    (Utilities|Array|Add (Variables|pawn_Data|GetThe_final_skill) _array_element))
  (Utilities|Array|Add (Variables|pawn_Data|GetThe_final_skill) (Utilities|Struct|Makest_role_skill "NewEnumerator1" (.Asset_skill_name (Utilities|Struct|Breakst_Finisher (Utilities|Array|Get(acopy) (Variables|pawn_Data|Getlocal_finsher_array) (Variables|Playercontrol|Getcurrent_finisher_index)))) (.rowname (Utilities|Struct|Breakst_Finisher (Utilities|Array|Get(acopy) (Variables|pawn_Data|Getlocal_finsher_array) (Variables|Playercontrol|Getcurrent_finisher_index))))))
  (return))