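; Base pawn for units in a turn-based board battle, handling player selection, damage, healing, shields and buffs.
; BeginPlay caches the global character pawn, sets the mesh and initializes ACGenericAttributes; clicks write skill target selection to that pawn.
; Damage passes through ACBuff effects at first or second priority before reaching attributes, and actions notify the Land's player buff component for reactions.
; Quarantine arrays compare and swap area buffs by board cell.
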(event Custom|beselect
  (bind _as_bp_global_charater (Variables|Other|GetAs%20BP%20GLOBAL%20CHARATER))
  (bind _as_bp_global_charater_2 (Variables|Other|GetAs%20BP%20GLOBAL%20CHARATER))
  (if (and (Utilities|Enum|Equal(Enum) (Variables|/Game/BP/BP_Battle_Phase/BP_GLOBAL_CHARACTER.BP_GLOBAL_CHARACTER_C|GetTurn_GAME_state _as_bp_global_charater) "NewEnumerator2") (Utilities|Enum|Equal(Enum) (Variables|/Game/BP/BP_Battle_Phase/BP_GLOBAL_CHARACTER.BP_GLOBAL_CHARACTER_C|Getplayer_action _as_bp_global_charater) "NewEnumerator0")) ; 检查是否处于我方回合
    (if (== (Variables|/Game/BP/BP_Battle_Phase/BP_GLOBAL_CHARACTER.BP_GLOBAL_CHARACTER_C|GetSelect%20skill%20object (Variables|Other|GetAs%20BP%20GLOBAL%20CHARATER)) self) ; 角色是否等于自身
      (Variables|/Game/BP/BP_Battle_Phase/BP_GLOBAL_CHARACTER.BP_GLOBAL_CHARACTER_C|SetSelect%20the%20target _as_bp_global_charater_2 true)
      (CallFunction|CallPlayer)
      (else
        (Variables|/Game/BP/BP_Battle_Phase/BP_GLOBAL_CHARACTER.BP_GLOBAL_CHARACTER_C|SetSelect%20the%20target _as_bp_global_charater_2 false)
        (Variables|/Game/BP/BP_Battle_Phase/BP_GLOBAL_CHARACTER.BP_GLOBAL_CHARACTER_C|SetSelect%20skill%20object (Variables|Other|GetAs%20BP%20GLOBAL%20CHARATER) self)
        (CallFunction|CallPlayer)))
    (else
      (Development|PrintText "不执行"))))

(event EventBeginPlay
  ;[1 1 1] 初始化
  (Utilities|FlowControl|Sequence
    (:then_0
      (|CallParentFunction)
      (bind _as2dplayer_contrller (Utilities|Casting|CastTo2DplayerContrller (Game|GetPlayerController 0)))
      (Variables|Default|Settemp_player_contrllo _as2dplayer_contrller))
    (:then_1
      (A1|UnitInitializationFunction))
    (:then_2
      (bind _attributs (Default|AttributeDetermination (Variables|Default|GetAC_Generic_attributes) (Variables|pawn_team|GetTable%20Switch) (Variables|pawn_team|GetLevel) (Variables|pawn_team|GetFix) (Variables|pawn_team|GetFix%20Attributs)))
      (bind _output_get (Default|TickAttributes (Variables|Default|GetAC_Generic_attributes) (Variables|Default|Getunit_bonus) (Utilities|Struct|MakeST_Attribute_collection_AA (Utilities|Struct|MakeST_Base_attributes_A (.hp_max (Utilities|Struct|Breakst_the_unit_attribute _attributs)) (.attack (Utilities|Struct|Breakst_the_unit_attribute _attributs)) (.defense (Utilities|Struct|Breakst_the_unit_attribute _attributs))) "(element_bonus_3_7E47476240021223A27EB1B15F25B237=((),(element_type_2_A382164746729B1F7E90C0B960DFA649=NewEnumerator1),(element_type_2_A382164746729B1F7E90C0B960DFA649=NewEnumerator2),(element_type_2_A382164746729B1F7E90C0B960DFA649=NewEnumerator4),(element_type_2_A382164746729B1F7E90C0B960DFA649=NewEnumerator3)),Finaldamagebonus_7_C0F6EFE54D0D41C34BEE3BA503A9A25C=0.000000,Damagereductionbonus_9_9010B5E8408BD39C6EABC9BBEBF850BC=0.000000)")))
      (Default|InitializetheProperty (Variables|Default|GetAC_Generic_attributes) _output_get))))

(fn ConstructionScript
  (Input|EnableInput (Variables|Default|Gettemp_player_contrllo)))

(fn BuffImmunityCheak
  (params (Execution%20of%20the%20immune%20phase :type e_buff_Immunity%20Enum :default "NewEnumerator1") (element_type :type E_element_type%20Enum :default "NewEnumerator5") (element_type_level :type E_element_advance%20Enum :default "NewEnumerator2") (buff_nature_type :type E_buff_Nature_type%20Enum :default "NewEnumerator0") (buff_type :type E_BUFF_type%20Enum :default "NewEnumerator0"))
  (LocalVariables|Setimmunity Execution%20of%20the%20immune%20phase)
  (for _array_element (Variables|/Game/BP/BP_AC/BP_BUFF_AC/AC_buff.AC_buff_C|Getcurrent_buff (Variables|Default|GetAC_buff))
    (for _array_element_2 (Variables|/Game/BP/BP_AC/BP_BUFF_AC/BP_buff_class.BP_buff_class_C|Getimmunity_info _array_element)
      (if (Utilities|Enum|Equal(Enum) (LocalVariables|Getimmunity) (.immunity_type (Utilities|Struct|Breakst_buff_immunity _array_element_2)))
        (if (Math|Boolean|ANDBoolean (Utilities|Enum|Equal(Enum) buff_type (.buff_type (Utilities|Struct|Breakst_buff_search_criteria (.buff_search_info (Utilities|Struct|Breakst_buff_immunity _array_element_2))))) (Utilities|Enum|Equal(Enum) buff_nature_type (.buff_nature_type (Utilities|Struct|Breakst_buff_search_criteria (.buff_search_info (Utilities|Struct|Breakst_buff_immunity _array_element_2))))) (Utilities|Enum|Equal(Enum) (.element_type (Utilities|Struct|Breakst_buff_search_criteria (.buff_search_info (Utilities|Struct|Breakst_buff_immunity _array_element_2)))) element_type) (Utilities|Enum|Equal(Enum) (.element_level (Utilities|Struct|Breakst_buff_search_criteria (.buff_search_info (Utilities|Struct|Breakst_buff_immunity _array_element_2)))) element_type_level))
          (return true _array_element)
          (else
            (return false 0)))))))

(fn DataDocking
  (params (RowName :type Name))
  (bind _returnvalue (Utilities|GetDataTableRow "/Game/Struct/rank_table/T_character_level_data.T_character_level_data" RowName)
    (:then
      (return (Utilities|Struct|MakeST_Attribute_collection_AA (Utilities|Struct|MakeST_Base_attributes_A (.Health (Utilities|Struct|Breakst_character_bese_level_data _returnvalue)) (.Attack (Utilities|Struct|Breakst_character_bese_level_data _returnvalue)) (.defense (Utilities|Struct|Breakst_character_bese_level_data _returnvalue))) "(element_bonus_3_7E47476240021223A27EB1B15F25B237=((),(element_type_2_A382164746729B1F7E90C0B960DFA649=NewEnumerator1),(element_type_2_A382164746729B1F7E90C0B960DFA649=NewEnumerator2),(element_type_2_A382164746729B1F7E90C0B960DFA649=NewEnumerator4),(element_type_2_A382164746729B1F7E90C0B960DFA649=NewEnumerator3)),Finaldamagebonus_7_C0F6EFE54D0D41C34BEE3BA503A9A25C=0.000000,Damagereductionbonus_9_9010B5E8408BD39C6EABC9BBEBF850BC=0.000000)")))))

(fn SetUnitdata
  (params (unit_area :type E_area%20Enum :default "NewEnumerator0") (unit_faction :type E_unitfaction%20Enum :default "NewEnumerator0") (gameplay_unit_type :type E_unit_type%20Enum :default "NewEnumerator0"))
  (Variables|unit_info|Setunit_area unit_area)
  (Variables|unit_info|Setunit_faction unit_faction)
  (Variables|unit_info|Setgameplay_unit_type gameplay_unit_type))

(fn UnitInitializationFunction
  (bind _asbp_global_character (Utilities|Casting|CastToBP_GLOBAL_CHARACTER (Game|Player|GetPlayerPawn 0)))
  (if (Utilities|IsValid _asbp_global_character)
    (Variables|Other|SetAs%20BP%20GLOBAL%20CHARATER _asbp_global_character)
    (Components|SkeletalMesh|SetSkeletalMeshAsset (Variables|Default|GetSkeletalMesh_C) (Variables|Default|GetUNITSkeletal%20Mesh))))

(fn IsClickedEvent
  (bind _as_bp_global_charater (Variables|Other|GetAs%20BP%20GLOBAL%20CHARATER))
  (bind _as_bp_global_charater_2 (Variables|Other|GetAs%20BP%20GLOBAL%20CHARATER))
  (if (Utilities|Enum|Equal(Enum) (Variables|/Game/BP/BP_Battle_Phase/BP_GLOBAL_CHARACTER.BP_GLOBAL_CHARACTER_C|Getplayer_action _as_bp_global_charater) "NewEnumerator0") ; 检查是否处于我方回合
    (switch Utilities|FlowControl|Switch|Switchone_game_state (Variables|/Game/BP/BP_Battle_Phase/BP_GLOBAL_CHARACTER.BP_GLOBAL_CHARACTER_C|GetTurn_GAME_state _as_bp_global_charater)
      (:NewEnumerator2
        (if (== (Variables|/Game/BP/BP_Battle_Phase/BP_GLOBAL_CHARACTER.BP_GLOBAL_CHARACTER_C|GetSelect%20skill%20object (Variables|Other|GetAs%20BP%20GLOBAL%20CHARATER)) self) ; 角色是否等于自身
          (Variables|/Game/BP/BP_Battle_Phase/BP_GLOBAL_CHARACTER.BP_GLOBAL_CHARACTER_C|SetSelect%20the%20target (Variables|Other|GetAs%20BP%20GLOBAL%20CHARATER) true)
          (Development|PrintString "BP_base_unit_select_target")
          (else
            (Variables|/Game/BP/BP_Battle_Phase/BP_GLOBAL_CHARACTER.BP_GLOBAL_CHARACTER_C|SetSelect%20skill%20object (Variables|Other|GetAs%20BP%20GLOBAL%20CHARATER) self))))
      (:NewEnumerator8
        (if (== (Variables|/Game/BP/BP_Battle_Phase/BP_GLOBAL_CHARACTER.BP_GLOBAL_CHARACTER_C|GetSelect%20skill%20object (Variables|Other|GetAs%20BP%20GLOBAL%20CHARATER)) self) ; 角色是否等于自身
          (Variables|/Game/BP/BP_Battle_Phase/BP_GLOBAL_CHARACTER.BP_GLOBAL_CHARACTER_C|SetSelect%20the%20target _as_bp_global_charater_2 true)
          (else
            (Variables|/Game/BP/BP_Battle_Phase/BP_GLOBAL_CHARACTER.BP_GLOBAL_CHARACTER_C|SetSelect%20the%20target _as_bp_global_charater_2 false)
            (Variables|/Game/BP/BP_Battle_Phase/BP_GLOBAL_CHARACTER.BP_GLOBAL_CHARACTER_C|SetSelect%20skill%20object (Variables|Other|GetAs%20BP%20GLOBAL%20CHARATER) self)))))))

(fn CheakHealth（NG）
  (bind _is_dead (Default|CheckLifeAttributes (Variables|Default|GetAC_Generic_attributes)))
  (if _is_dead
    (Default|WhentheUnitDies (Variables|/Game/BP/BP_Battle_Phase/BP_GLOBAL_CHARACTER.BP_GLOBAL_CHARACTER_C|Getland (Variables|Other|GetAs%20BP%20GLOBAL%20CHARATER)) self)))

(fn GainAShield
  (params (shield_type :type E_shield_type%20Enum :default "NewEnumerator0") (Shield :type Float%20%28double-precision%29))
  (Variables|/Game/BP/BP_AC/BP_Generic_attributes_AC/AC_Generic_attributes.AC_Generic_attributes_C|SetCurrent_resource (Variables|Default|GetAC_Generic_attributes) (Utilities|Struct|MakeST_UNIT_Current_resource_AA (Utilities|Struct|MakeST_unit_shield shield_type (+ Shield (Utilities|Struct|BreakST_unit_shield (Utilities|Struct|BreakST_UNIT_Current_resource_AA (Variables|/Game/BP/BP_AC/BP_Generic_attributes_AC/AC_Generic_attributes.AC_Generic_attributes_C|GetCurrent_resource (Variables|Default|GetAC_Generic_attributes))))))))
  (Default|ActionUnitResponse (Variables|/Game/BP/BP_Battle_Phase/BP_land_spaner.BP_land_spaner_C|GetAC_player_buff_C (Variables|/Game/BP/BP_Battle_Phase/BP_GLOBAL_CHARACTER.BP_GLOBAL_CHARACTER_C|Getland (Variables|Other|GetAs%20BP%20GLOBAL%20CHARATER))) "NewEnumerator35" "NewEnumerator0" "NewEnumerator3" "NewEnumerator4" "NewEnumerator3" "NewEnumerator2" self 0 0.0 (CallFunction|FormShieldTypetoIndex shield_type)))

(fn GetBuff
  (params (buff_rowname :type Name) (target :type Actor%20Object%20Reference) (create :type Actor%20Object%20Reference) (buff_index :type Integer) (buff_type :type E_BUFF_type%20Enum :default "NewEnumerator0") (buff_nature :type E_buff_Nature_type%20Enum :default "NewEnumerator0") (buff_Updata :type E_BuffTimeUpdataEnum%20Enum :default "NewEnumerator0") (element_type :type E_element_type%20Enum :default "NewEnumerator5") (element_type_level :type E_element_advance%20Enum :default "NewEnumerator2") (immunity :type Array%20of%20St%20Buff%20Immunity%20Structures))
  (bind _ac_buff (Variables|Default|GetAC_buff))
  (bind _newparam (Default|Addbuff0 _ac_buff buff_rowname target create))
  (LocalVariables|Setcurrent_buff _newparam)
  (Game|SpawnActorfromClass "/Game/BP/BP_actor/bp_battle_effect_widget.bp_battle_effect_widget_C" (Math|Transform|MakeTransform (Transformation|GetActorLocation self)) "Undefined" "MultiplyWithRoot" 0 "buff" 0)
  (Emptyfunction|AfterReceivingtheBuff _newparam)
  (Default|BuffTick _ac_buff)
  (CallFunction|UpdataUnitElementBuff)
  (Default|ActionUnitResponse (Variables|/Game/BP/BP_Battle_Phase/BP_land_spaner.BP_land_spaner_C|GetAC_player_buff_C (Variables|/Game/BP/BP_Battle_Phase/BP_GLOBAL_CHARACTER.BP_GLOBAL_CHARACTER_C|Getland (Variables|Other|GetAs%20BP%20GLOBAL%20CHARATER))) "NewEnumerator35" "NewEnumerator0" "NewEnumerator3" "NewEnumerator4" "NewEnumerator3" "NewEnumerator1" self 0 0.0))

(fn BeTreaed
  (params (tread_v :type Float%20%28double-precision%29))
  (Default|InTreaed (Variables|Default|GetAC_Generic_attributes) tread_v)
  (Default|ActionUnitResponse (Variables|/Game/BP/BP_Battle_Phase/BP_land_spaner.BP_land_spaner_C|GetAC_player_buff_C (Variables|/Game/BP/BP_Battle_Phase/BP_GLOBAL_CHARACTER.BP_GLOBAL_CHARACTER_C|Getland (Variables|Other|GetAs%20BP%20GLOBAL%20CHARATER))) "NewEnumerator35" "NewEnumerator0" "NewEnumerator3" "NewEnumerator4" "NewEnumerator3" "NewEnumerator3" self 0 tread_v))

(fn MoveAfter
  (Default|ActionUnitResponse (Variables|/Game/BP/BP_Battle_Phase/BP_land_spaner.BP_land_spaner_C|GetAC_player_buff_C (Variables|/Game/BP/BP_Battle_Phase/BP_GLOBAL_CHARACTER.BP_GLOBAL_CHARACTER_C|Getland (Variables|Other|GetAs%20BP%20GLOBAL%20CHARATER))) "NewEnumerator7" "NewEnumerator0" "NewEnumerator3" "NewEnumerator4" "NewEnumerator3" "NewEnumerator14" self 0 0.0))

(fn BeAttack
  (params (damage :type Float%20%28double-precision%29) (Critical%20hit :type Boolean) (Critical%20hit%20volume :type Float%20%28double-precision%29) (element_type :type E_element_type%20Enum :default "NewEnumerator5") (damage_type :type e_damage_type%20Enum :default "NewEnumerator1") (element_damage_type :type e_element_damage_type%20Enum :default "NewEnumerator1") (Damage%20final%20bonus :type Float%20%28double-precision%29))
  (LocalVariables|Setnext_damage damage)
  (LocalVariables|Setbuff_effect "NewEnumerator3")
  (LocalVariables|SetHierarchical%20Interrupt false)
  (LocalVariables|Seteffect_prioity 1)
  (if (LocalVariables|GetHierarchical%20Interrupt)
    (Default|InAttack (Variables|Default|GetAC_Generic_attributes) (LocalVariables|Getnext_damage) Critical%20hit Critical%20hit%20volume element_type damage_type element_damage_type Damage%20final%20bonus)
    (Default|ActionUnitResponse (Variables|/Game/BP/BP_Battle_Phase/BP_land_spaner.BP_land_spaner_C|GetAC_player_buff_C (Variables|/Game/BP/BP_Battle_Phase/BP_GLOBAL_CHARACTER.BP_GLOBAL_CHARACTER_C|Getland (Variables|Other|GetAs%20BP%20GLOBAL%20CHARATER))) "NewEnumerator35" "NewEnumerator0" "NewEnumerator3" "NewEnumerator4" "NewEnumerator3" "NewEnumerator7" self 0 (LocalVariables|Getnext_damage) (CallFunction|FormDamgeTypetoIndex damage_type))
    (else
      (bind (_array_element _find) (Default|FindBuffsThatHaveActiveEffects (Variables|Default|GetAC_buff) (LocalVariables|Getbuff_effect) (LocalVariables|Geteffect_prioity)))
      (if _find
        (for _array_element_2 _array_element
          (bind (_excurt _newparam _interrupt) (Default|ExecuteBuffEffect (Variables|Default|GetAC_buff) (LocalVariables|Getbuff_effect) (LocalVariables|Geteffect_prioity) _array_element_2 (LocalVariables|Getnext_damage)))
          (LocalVariables|SetHierarchical%20Interrupt _interrupt)
          (LocalVariables|Setnext_damage _newparam)
          (Default|InAttack (Variables|Default|GetAC_Generic_attributes) (LocalVariables|Getnext_damage) Critical%20hit Critical%20hit%20volume element_type damage_type element_damage_type Damage%20final%20bonus)
          (Game|SpawnActorfromClass "/Game/BP/BP_actor/bp_battle_effect_widget.bp_battle_effect_widget_C" (Math|Transform|MakeTransform (Transformation|GetActorLocation)) "Undefined" "MultiplyWithRoot" 0 (Utilities|Text|ToText(Float) (LocalVariables|Getnext_damage) "HalfToEven") 0)
          (Default|ActionUnitResponse (Variables|/Game/BP/BP_Battle_Phase/BP_land_spaner.BP_land_spaner_C|GetAC_player_buff_C (Variables|/Game/BP/BP_Battle_Phase/BP_GLOBAL_CHARACTER.BP_GLOBAL_CHARACTER_C|Getland (Variables|Other|GetAs%20BP%20GLOBAL%20CHARATER))) "NewEnumerator35" "NewEnumerator0" "NewEnumerator3" "NewEnumerator4" "NewEnumerator3" "NewEnumerator7" self 0 (LocalVariables|Getnext_damage) (CallFunction|FormDamgeTypetoIndex damage_type)))
        (else
          (bind _output_get (LocalVariables|Seteffect_prioity (+ (LocalVariables|Geteffect_prioity) 1)))
          (bind (_array_element_3 _find_2) (Default|FindBuffsThatHaveActiveEffects (Variables|Default|GetAC_buff) (LocalVariables|Getbuff_effect) _output_get))
          (if _find_2
            (for _array_element_4 _array_element_3
              (bind (_excurt_2 _newparam_2 _interrupt_2) (Default|ExecuteBuffEffect (Variables|Default|GetAC_buff) (LocalVariables|Getbuff_effect) (LocalVariables|Geteffect_prioity) _array_element_4 damage))
              (LocalVariables|Setnext_damage _newparam_2)
              (LocalVariables|SetHierarchical%20Interrupt _interrupt_2)
              (Default|InAttack (Variables|Default|GetAC_Generic_attributes) (LocalVariables|Getnext_damage) Critical%20hit Critical%20hit%20volume element_type damage_type element_damage_type Damage%20final%20bonus)
              (Game|SpawnActorfromClass "/Game/BP/BP_actor/bp_battle_effect_widget.bp_battle_effect_widget_C" (Math|Transform|MakeTransform (Transformation|GetActorLocation)) "Undefined" "MultiplyWithRoot" 0 (Utilities|Text|ToText(Float) (LocalVariables|Getnext_damage) "HalfToEven") 0)
              (Default|ActionUnitResponse (Variables|/Game/BP/BP_Battle_Phase/BP_land_spaner.BP_land_spaner_C|GetAC_player_buff_C (Variables|/Game/BP/BP_Battle_Phase/BP_GLOBAL_CHARACTER.BP_GLOBAL_CHARACTER_C|Getland (Variables|Other|GetAs%20BP%20GLOBAL%20CHARATER))) "NewEnumerator35" "NewEnumerator0" "NewEnumerator3" "NewEnumerator4" "NewEnumerator3" "NewEnumerator7" self 0 (LocalVariables|Getnext_damage) (CallFunction|FormDamgeTypetoIndex damage_type)))
            (else
              (LocalVariables|Setnext_damage damage)
              (Default|InAttack (Variables|Default|GetAC_Generic_attributes) (LocalVariables|Getnext_damage) Critical%20hit Critical%20hit%20volume element_type damage_type element_damage_type Damage%20final%20bonus)
              (Game|SpawnActorfromClass "/Game/BP/BP_actor/bp_battle_effect_widget.bp_battle_effect_widget_C" (Math|Transform|MakeTransform (Transformation|GetActorLocation)) "Undefined" "MultiplyWithRoot" 0 (Utilities|Text|ToText(Float) (LocalVariables|Getnext_damage) "HalfToEven") 0)
              (Default|ActionUnitResponse (Variables|/Game/BP/BP_Battle_Phase/BP_land_spaner.BP_land_spaner_C|GetAC_player_buff_C (Variables|/Game/BP/BP_Battle_Phase/BP_GLOBAL_CHARACTER.BP_GLOBAL_CHARACTER_C|Getland (Variables|Other|GetAs%20BP%20GLOBAL%20CHARATER))) "NewEnumerator35" "NewEnumerator0" "NewEnumerator3" "NewEnumerator4" "NewEnumerator3" "NewEnumerator7" self 0 (LocalVariables|Getnext_damage) (CallFunction|FormDamgeTypetoIndex damage_type)))))))))

(fn ChearAreabuffDockingPawnBuff
  (bind (_xindex _yindex) (Default|GetactorLocationIndex (Variables|Other|GetAs%20BP%20GLOBAL%20CHARATER) (Transformation|GetActorLocation)))
  (bind _asactor (Default|FindChearinBoard (Variables|Other|GetAs%20BP%20GLOBAL%20CHARATER) _xindex _yindex))
  (bind _asbp_base_pawn (Utilities|Casting|CastToBP_BASE_Pawn _asactor))
  (Variables|/Game/BP/BP_AC/BP_BUFF_AC/AC_buff.AC_buff_C|SetQuarantine%20AreaA (Variables|Default|GetAC_buff) (Variables|/Game/BP/BP_AC/BP_BUFF_AC/AC_buff.AC_buff_C|Getarea_buff (Variables|BP_BASE_Pawn_C|GetAC_buff _asbp_base_pawn))))

(fn BuffDataComparison
  (bind _ac_buff (Variables|Default|GetAC_buff))
  (for _array_element (Variables|/Game/BP/BP_AC/BP_BUFF_AC/AC_buff.AC_buff_C|GetQuarantine%20AreaA _ac_buff)
    (for _array_element_2 (Variables|/Game/BP/BP_AC/BP_BUFF_AC/AC_buff.AC_buff_C|GetQuarantine%20AreaB _ac_buff)
      (if (== _array_element_2 _array_element) ; 检查buff是否一致
        (return false)
        (else
          (return true))))))

(fn UpdateBuff
  (params (Condition :type Boolean))
  (if Condition
    (for _array_element (Variables|/Game/BP/BP_AC/BP_BUFF_AC/AC_buff.AC_buff_C|GetQuarantine%20AreaB (Variables|Default|GetAC_buff))
      (Utilities|Array|RemoveItem (Variables|/Game/BP/BP_AC/BP_BUFF_AC/AC_buff.AC_buff_C|Getcurrent_buff (Variables|Default|GetAC_buff)) _array_element) ; 在当前buff数组移除隔离区
      (Utilities|Array|Clear (Variables|/Game/BP/BP_AC/BP_BUFF_AC/AC_buff.AC_buff_C|GetQuarantine%20AreaB (Variables|Default|GetAC_buff))) ; 清除隔离区B
      (bind _output_get (Variables|/Game/BP/BP_AC/BP_BUFF_AC/AC_buff.AC_buff_C|SetQuarantine%20AreaB (Variables|Default|GetAC_buff) (Variables|/Game/BP/BP_AC/BP_BUFF_AC/AC_buff.AC_buff_C|GetQuarantine%20AreaA (Variables|Default|GetAC_buff))))
      (for _array_element_2 _output_get
        (Utilities|Array|Add (Variables|/Game/BP/BP_AC/BP_BUFF_AC/AC_buff.AC_buff_C|Getwait_add_buff (Variables|Default|GetAC_buff)) _array_element_2)))))

(fn AfterReceivingtheBuff
  (params (buff :type BP%20Buff%20Class%20Object%20Reference)))

(fn CallPlayer
  (Default|CallPlayerEvent (Variables|Other|GetAs%20BP%20GLOBAL%20CHARATER)))

(fn UpdataUnitElementBuff)

(fn SetSighalMat
  (params (ElementIndex :type Integer) (Material :type Material%20Interface%20Object%20Reference))
  (Rendering|Material|SetMaterial (Variables|Default|GetSignal) ElementIndex Material))

(fn CallGlobalReaction
  (params (Trigger%20timing :type E_TriggerTiming%20Enum :default "NewEnumerator0") (action_type :type E_TriggerAction_type%20Enum :default "NewEnumerator0") (role_skill_type :type E_SKILL_TYPE%20Enum :default "NewEnumerator3") (Action_skill_mode :type E_TriggerAction_skill_mode%20Enum :default "NewEnumerator4") (Action_effect_type :type E_TriggerActionEffectType%20Enum :default "NewEnumerator0") (common_Variable :type Float%20%28double-precision%29))
  (Variables|/Game/BP/BP_Battle_Phase/BP_land_spaner.BP_land_spaner_C|Setbattle_overall (Variables|/Game/BP/BP_Battle_Phase/BP_GLOBAL_CHARACTER.BP_GLOBAL_CHARACTER_C|Getland (Variables|Other|GetAs%20BP%20GLOBAL%20CHARATER)) (Utilities|Struct|Makest_Battlefield_Inspector Trigger%20timing action_type role_skill_type Action_skill_mode "NewEnumerator3" Action_effect_type self 0 common_Variable))
  (Default|CallGlobalReaction))