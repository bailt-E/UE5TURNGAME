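; Game manager for a turn-based grid tactics battle, handling battle setup and round phases.
; On BeginPlay it creates the UI, spawns two 5x5 random-tile boards, places enemy and party units from team data, then switches to the player round.
; Events store the selected tile and character, with helpers converting world positions to grid coordinates.
; Round switching only prints the phase; action points, repositioning and battle checks are stubs.
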(event EventBeginPlay
  (switch Utilities|FlowControl|Switch|Switchone_game_Gameflow "NewEnumerator0"
    (:NewEnumerator0
      (CallFunction|游戏开始：创建UI)
      (CallFunction|游戏开始：生成棋盘)
      (CallFunction|游戏开始：生成敌方单位)
      (CallFunction|游戏开始：生成我方队伍)
      (CallFunction|游戏开始：初始化行动点)
      (CallFunction|切换回合 "NewEnumerator1"))
    (:NewEnumerator1
      (CallFunction|我方回合：获得行动点))
    (:NewEnumerator2
      (Utilities|FlowControl|Delay 0.2))
    (:NewEnumerator3
      (Utilities|FlowControl|Delay 0.2))))

(event Collision|EventActorBeginOverlap
  (params (OtherActor :type Actor%20Object%20Reference)))

(event EventTick
  (params (DeltaSeconds :type Float%20%28single-precision%29)))

(event Event棋盘传输
  (params (棋盘 :type BP%20Gamechear%20Class%20Object%20Reference))
  ;[1 1 1] 获得棋盘以及其位置
  (bind _output_get (Variables|Default|Set当前棋格 棋盘))
  (Variables|Default|Set棋盘位置 (Transformation|GetActorLocation _output_get)))

(event Event角色传输
  (params (角色 :type BP%20Character%20Class%20Object%20Reference))
  ;[1 1 1] 获得角色的相关信息
  (Variables|Default|Set当前角色 角色)
  (Development|PrintText "选中角色"))

(fn ConstructionScript)

(fn 检查战斗情况
  (for _array_element (Variables|固定属性|Get敌人队伍)
    (for _array_element_2 (Variables|固定属性|Get我方队伍)
      _)))

(fn 游戏开始：生成棋盘
  (bind _returnvalue (Transformation|GetActorLocation))
  (bind _returnvalue_2 (Transformation|GetActorLocation))
  (bind _距离 (Variables|固定属性|Get距离))
  (bind (_x _y _z) (Math|Vector|BreakVector _returnvalue_2))
  (bind (_x_2 _y_2 _z_2) (Math|Vector|BreakVector _returnvalue))
  (Utilities|FlowControl|Sequence
    (:then_0
      (for _index (range 1 5)
        (for _index_2 (range 1 5)
          (Game|SpawnActorfromClass :Class (.Value (Utilities|Map|Find (Variables|固定属性|Get棋格字典) (Math|Random|RandomIntegerinRange 1 3))) :SpawnTransform (Math|Transform|MakeTransform (Math|Vector|MakeVector (+ (* _index (Variables|固定属性|Get敌方距离)) _x_2) (+ (* _index_2 (Variables|固定属性|Get距离)) _y_2) _z_2)) :CollisionHandlingOverride "Undefined" :TransformScaleMethod "MultiplyWithRoot" :UNITSkeletal%20Mesh 0 :Instigator 0))))
    (:then_1
      (for _index_3 (range 1 5)
        (for _index_4 (range 1 5)
          (Game|SpawnActorfromClass :Class (.Value (Utilities|Map|Find (Variables|固定属性|Get棋格字典) (Math|Random|RandomIntegerinRange 1 3))) :SpawnTransform (Math|Transform|MakeTransform (Math|Vector|MakeVector (+ (Math|Conversions|ToFloat(Integer) (* _index_4 _距离)) _x) (+ (Math|Conversions|ToFloat(Integer) (* _index_3 _距离)) _y) _z)) :CollisionHandlingOverride "Undefined" :TransformScaleMethod "MultiplyWithRoot" :UNITSkeletal%20Mesh 0 :Instigator 0))))))

(fn 游戏开始：初始化行动点)

(fn 游戏开始：生成敌方单位
  (bind _returnvalue (Transformation|GetActorLocation))
  (bind (_x _y _z) (Math|Vector|BreakVector _returnvalue))
  (for _array_element (Variables|固定属性|Getemeny_team)
    (bind _returnvalue_2 (Game|SpawnActorfromClass :Class (Variables|固定属性|Get单位) :SpawnTransform (Math|Transform|MakeTransform (Math|Vector|MakeVector (+ _x (* (.X-axis (Utilities|Struct|Breakst_team _array_element)) (Variables|固定属性|Get敌方距离))) (+ (* (.Y-axis (Utilities|Struct|Breakst_team _array_element)) (Variables|固定属性|Get距离)) _y) _z)) :CollisionHandlingOverride "Undefined" :TransformScaleMethod "MultiplyWithRoot" :UNITSkeletal%20Mesh 0 :Instigator 0))
    (Variables|固定属性|Set敌人队伍 (Utilities|Array|MakeArray _returnvalue_2))))

(fn 游戏开始：生成我方队伍
  (bind _returnvalue (Transformation|GetActorLocation))
  (bind _距离 (Variables|固定属性|Get距离))
  (bind (_x _y _z) (Math|Vector|BreakVector _returnvalue))
  (for _array_element (Variables|固定属性|Getparty_team)
    (bind _returnvalue_2 (Game|SpawnActorfromClass :Class (Variables|固定属性|Get单位) :SpawnTransform (Math|Transform|MakeTransform (Math|Vector|MakeVector (+ (* (.X-axis (Utilities|Struct|Breakst_team _array_element)) _距离) _x) (+ (* (.Y-axis (Utilities|Struct|Breakst_team _array_element)) _距离) _y) _z)) :CollisionHandlingOverride "Undefined" :TransformScaleMethod "MultiplyWithRoot" :UNITSkeletal%20Mesh 0 :Instigator 0))
    (Variables|固定属性|Set我方队伍 (Utilities|Array|MakeArray _returnvalue_2))))

(fn 我方回合：获得行动点)

(fn 我方回合：调整位置)

(fn 更新当前角色的坐标
  (params (目标 :type Actor%20Object%20Reference))
  (bind _returnvalue (Transformation|GetActorLocation))
  (bind _returnvalue_2 (Transformation|GetActorLocation 目标))
  (bind _距离 (Variables|固定属性|Get距离))
  (bind _returnvalue_3 (- _returnvalue_2 _returnvalue))
  (bind (_x _y) (Math|Vector|BreakVector _returnvalue_3))
  (bind _output_get (Variables|Default|Set角色坐标 (Math|Vector|MakeVector (/ _x _距离) (/ _y _距离) 0.0)))
  (return _output_get))

(fn 更新棋盘的坐标
  (bind _returnvalue (Transformation|GetActorLocation))
  (bind _当前棋格 (Variables|Default|Get当前棋格))
  (bind _距离 (Variables|固定属性|Get距离))
  (bind _returnvalue_2 (Transformation|GetActorLocation _当前棋格))
  (bind _returnvalue_3 (- _returnvalue_2 _returnvalue))
  (bind (_x _y) (Math|Vector|BreakVector _returnvalue_3))
  (Variables|Default|Set棋盘坐标 (Math|Vector|MakeVector (/ _x _距离) (/ _y _距离) 0.0)))

(fn 切换回合
  (params (游戏流程 :type e_game_Gameflow%20Enum :default "NewEnumerator0"))
  (bind _output_get (Variables|固定属性|Set游戏流程 游戏流程))
  (if (Utilities|Enum|Equal(Enum) _output_get "NewEnumerator0")
    (Development|PrintText "游戏开始")
    (elif (Utilities|Enum|Equal(Enum) _output_get "NewEnumerator1")
      (Development|PrintText "我方回合")
      (elif (Utilities|Enum|Equal(Enum) "NewEnumerator2" _output_get)
        (Development|PrintText "敌方回合")
        (elif (Utilities|Enum|Equal(Enum) _output_get "NewEnumerator3")
          (Development|PrintText "中立回合"))))))

(fn 游戏开始：创建UI
  (bind _returnvalue (UserInterface|CreateWidget (Variables|Default|GetUI控件)))
  (UserInterface|Viewport|AddtoViewport _returnvalue 0))