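; Pre-battle formation manager that lets the player's team be placed on a tile board before a fight.
; It spawns the tile grid and formation pieces from team data and the character table, then links them by grid index into unit data.
; Helpers reposition pieces, swap members and write positions back to the team.
; BattleOpen destroys board and pieces and passes team, mode, bonuses and level row to the player controller's battle stage.
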(event Custom|formtion_class_begin
  (A1|SpawnBoard)
  (A1|GenerateChessPiecesBasedontheTeam (Utilities|Struct|Breakst_team_Assembly (Variables|F1|GetFIX_TEAM)))
  ;[1 1 1] 更新队伍
  (bind _level_unit (A1|IntegratetheBoardandPieces (Variables|Rawdata|Getboard) (Variables|Rawdata|Getchess_pieces)))
  (bind _output_get (Variables|level_unit_data|Setfixed_level_unit_data _level_unit))
  (bind _unit_class (CallFunction|UpdateUnitClass _output_get))
  (Variables|level_unit_data|Setfixed_level_unit_data _unit_class))

(event EventBeginPlay
  (bind _asbp_global_character (Utilities|Casting|CastToBP_GLOBAL_CHARACTER (Game|Player|GetPlayerPawn 0)))
  (Variables|A1|SetAs%20BP%20GLOBAL%20CHARATER _asbp_global_character)
  (Utilities|Array|Resize (Utilities|Struct|Breakst_team_Assembly (Variables|level_unit_data|Getteam)) 5)
  (bind _as2dplayer_contrller (Utilities|Casting|CastTo2DplayerContrller (Game|GetPlayerController 0)))
  (Variables|A1|SetAs%202Dplayer%20Contrller _as2dplayer_contrller)
  (Variables|/Game/gamemode/2DplayerContrller.2DplayerContrller_C|Setfortmion _as2dplayer_contrller self))

(fn ConstructionScript)

(fn IntegrateChear
  (params (chear :type Array%20of%20Actor%20Object%20References))
  (for _array_element chear
    (if (Utilities|IsValid _array_element)
      (Utilities|Array|Add (LocalVariables|Gettemp_unit) (Utilities|Struct|Makest_unit_class (CallFunction|GetUnitIndex _array_element) _array_element 0 "NewEnumerator1" "NewEnumerator3" 0 0))))
  (return (LocalVariables|Gettemp_unit)))

(fn IntegratePIE
  (params (OLD_UNIT :type Array%20of%20St%20Unit%20Class%20Structures) (ACTORX :type Array%20of%20Actor%20Object%20References))
  (LocalVariables|SetTEMP_UNIT OLD_UNIT)
  (for _array_element ACTORX
    (for _array_element_2 (LocalVariables|GetTEMP_UNIT)
      (if (Utilities|IsValid _array_element)
        (if (== (CallFunction|GetUnitIndex _array_element) (.unit_location_index (Utilities|Struct|Breakst_unit_class _array_element_2)))
          (Utilities|Array|SetArrayElem (LocalVariables|GetTEMP_UNIT) 0 (Utilities|Struct|Makest_unit_class (.unit_location_index (Utilities|Struct|Breakst_unit_class _array_element_2)) (.chear (Utilities|Struct|Breakst_unit_class _array_element_2)) _array_element (.theunitarea (Utilities|Struct|Breakst_unit_class _array_element_2)) (.theunit_Belongs (Utilities|Struct|Breakst_unit_class _array_element_2)) (.unit_chear_class (Utilities|Struct|Breakst_unit_class _array_element_2)) (.unit_charter_class (Utilities|Struct|Breakst_unit_class _array_element_2)) (.gameplay_unit_type (Utilities|Struct|Breakst_unit_class _array_element_2))))))))
  (return (LocalVariables|GetTEMP_UNIT)))

(fn IntegratetheBoardandPieces
  (params (boardX :type Array%20of%20BP%20Gamechear%20Class%20Object%20References) (piecesX :type Array%20of%20BP%20Formation%20Pieces%20Object%20References))
  (Utilities|Array|Clear (LocalVariables|Getunit))
  (Utilities|FlowControl|Sequence
    (:then_0
      (bind _unit (A1|IntegrateChear boardX))
      (LocalVariables|Setunit _unit))
    (:then_1
      (bind _new_unit (A1|IntegratePIE (LocalVariables|Getunit) piecesX))
      (bind _output_get (LocalVariables|Setunit _new_unit))
      (return _output_get))))

(fn GenerateChessPiecesBasedontheTeam
  (params (Team :type Array%20of%20St%20Team%20Structures))
  (Utilities|Array|Clear (Variables|Rawdata|Getchess_pieces))
  (for _array_element Team
    (bind _returnvalue (Utilities|GetDataTableRow "/Game/Struct/character/T_character_library.T_character_library" (.rowname (Utilities|Struct|Breakst_team _array_element)))
      (:then
        (bind _character_object (Default|FindCharacterbyRowname (Variables|/Game/gamemode/2DplayerContrller.2DplayerContrller_C|GetAC_RoleUpgradeManager (Variables|A1|GetAs%202Dplayer%20Contrller)) (.rowname (Utilities|Struct|Breakst_team _array_element))))
        (bind _returnvalue_2 (Game|SpawnActorfromClass "/Game/BP/BP_Before_the_battle_begins/BP_Formation_Pieces.BP_Formation_Pieces_C" (CallFunction|UnitsLocationCompute "NewEnumerator1" (.X-axis (Utilities|Struct|Breakst_team _array_element)) (.Y-axis (Utilities|Struct|Breakst_team _array_element))) "Undefined" "MultiplyWithRoot" 0 self (Utilities|Struct|Breakst_character_info (.character_index (Utilities|Struct|BreakST_Character_library _returnvalue))) (.index (Utilities|Struct|Breakst_team _array_element)) (.skill_data (Utilities|Struct|BreakST_Character_library _returnvalue)) (.Finsher_skill_ (Utilities|Struct|BreakST_Character_library _returnvalue)) (.Finisherindex (Utilities|Struct|Breakst_team _array_element)) _character_object 0))
        (Utilities|Array|Add (Variables|Rawdata|Getchess_pieces) _returnvalue_2)))))

(fn SpawnBoard
  (Utilities|Array|Clear (Variables|Rawdata|Getboard))
  (for _index (range 0 (- (Variables|borde_info|GetW) 1))
    (Variables|borde_info|Set2dx21d _index)
    (Variables|borde_info|SetX (+ (* (Variables|borde_info|Getpadding) _index) _index))
    (for _index_2 (range 0 (- (Variables|borde_info|GetH) 1))
      (Variables|borde_info|Set2dx21d _index_2)
      (Variables|borde_info|SetY (+ (* (Variables|borde_info|Getpadding) _index_2) _index_2))
      (bind _returnvalue (Game|SpawnActorfromClass :Class "/Game/BP/BP_Battle_Phase/BP_gamechear_class.BP_gamechear_class_C" :SpawnTransform (CallFunction|ChearLocationCompute (Variables|borde_info|GetX) (Variables|borde_info|GetY)) :CollisionHandlingOverride "Undefined" :TransformScaleMethod "MultiplyWithRoot" :UNITSkeletal%20Mesh 0 :Instigator 0))
      (Utilities|Array|Add (Variables|Rawdata|Getboard) _returnvalue))))

(fn ResetUnitLocation
  (for _array_element (Variables|level_unit_data|Getfixed_level_unit_data)
    (if (Utilities|IsValid (.charter (Utilities|Struct|Breakst_unit_class _array_element)))
      (Transformation|SetActorLocation (.charter (Utilities|Struct|Breakst_unit_class _array_element)) (.Location (Math|Transform|BreakTransform (CallFunction|UnitsLocationCompute "NewEnumerator1" (.AXIS%20X (CallFunction|FormAXISbyINDEX (.unit_location_index (Utilities|Struct|Breakst_unit_class _array_element)))) (.AXIS%20Y (CallFunction|FormAXISbyINDEX (.unit_location_index (Utilities|Struct|Breakst_unit_class _array_element))))))) false false))))

(fn SetUnitNewlocation
  (params (target_actor :type Actor%20Object%20Reference))
  (bind _asbp_global_character (Utilities|Casting|CastToBP_GLOBAL_CHARACTER (Game|Player|GetPlayerPawn 0)))
  (bind _empty_unit (Default|CaculateDirectionYouCanWalkV2(Chear)V3 _asbp_global_character (Transformation|GetActorLocation target_actor) (Variables|level_unit_data|Getfixed_level_unit_data)))
  (Transformation|SetActorLocation target_actor (.Location (Math|Transform|BreakTransform (CallFunction|UnitsLocationCompute "NewEnumerator1" (.AXIS%20X (CallFunction|FormAXISbyINDEX (Utilities|Struct|Breakst_unit_class _empty_unit))) (.AXIS%20Y (CallFunction|FormAXISbyINDEX (Utilities|Struct|Breakst_unit_class _empty_unit)))))) false false))

(fn CountLevelDatatoTeamData
  (Utilities|Array|Clear (Utilities|Struct|Breakst_team_Assembly (Variables|level_unit_data|Getteam)))
  (for _array_element (Variables|level_unit_data|Getfixed_level_unit_data)
    (bind _asbp_formation_pieces (Utilities|Casting|CastToBP_Formation_Pieces (.charter (Utilities|Struct|Breakst_unit_class _array_element))))
    (Variables|level_unit_data|Setteam (Utilities|Struct|Makest_team_Assembly (Utilities|Array|MakeArray (Utilities|Struct|Makest_team (Variables|/Game/BP/BP_Before_the_battle_begins/BP_Formation_Pieces.BP_Formation_Pieces_C|Getname _asbp_formation_pieces) (.AXIS%20X (CallFunction|FormAXISbyINDEX (.unit_location_index (Utilities|Struct|Breakst_unit_class _array_element)))) (.AXIS%20Y (CallFunction|FormAXISbyINDEX (.unit_location_index (Utilities|Struct|Breakst_unit_class _array_element)))) "100"))))))

(fn DebugFunction
  (Utilities|FlowControl|Sequence
    (:then_0
      (for _array_element (Variables|Rawdata|Getboard)
        (Utilities|Array|Add (Variables|F1|GetOpen_temp_unit_data) (Utilities|Struct|MakeST_unit_data_temp (CallFunction|GetUnitIndex _array_element) _array_element 0 (Transformation|GetActorLocation _array_element)))))
    (:then_1
      (for _array_element_2 (Variables|Rawdata|Getchess_pieces)
        (for _array_element_3 (Variables|F1|GetOpen_temp_unit_data)
          (if (Utilities|Operators|EqualEqual (Transformation|GetActorLocation _array_element_2) (.chear_location (Utilities|Struct|BreakST_unit_data_temp _array_element_3)) 1e+01)
            (Utilities|Array|SetArrayElem (Variables|F1|GetOpen_temp_unit_data) 0 (Utilities|Struct|MakeST_unit_data_temp (.index (Utilities|Struct|BreakST_unit_data_temp _array_element_3)) (.chear (Utilities|Struct|BreakST_unit_data_temp _array_element_3)) _array_element_2 (.chear_location (Utilities|Struct|BreakST_unit_data_temp _array_element_3)) (.chear_location (Utilities|Struct|BreakST_unit_data_temp _array_element_3))))))))))

(fn ANewCharacterJoinstheTeam
  (params (index :type Integer) (Item :type St%20Team%20Structure%20%28by%20ref%29) (team :type Array%20of%20St%20Team%20Structures))
  (bind (_rowname _index _x_axis _y_axis _unit _finisherindex) (Utilities|Struct|Breakst_team Item))
  (bind (_rowname_2 _index_2 _unit_2 _finisherindex_2) (Utilities|Struct|Breakst_team Item))
  (LocalVariables|SetFtemp_team (.team_number (Utilities|Struct|Breakst_team_Assembly (Variables|level_unit_data|Getteam))))
  (Utilities|FlowControl|Sequence
    (:then_0
      (if (Utilities|IsValidClass (.unit (Utilities|Struct|Breakst_team Item)))
        (if (Utilities|IsValidClass (.unit (Utilities|Struct|Breakst_team (Utilities|Array|Get(acopy) (LocalVariables|GetFtemp_team) index)))) ; 检查特定位置上的角色是否存在
          (Utilities|Array|SetArrayElem (LocalVariables|GetFtemp_team) index (Utilities|Struct|Makest_team _rowname_2 _index_2 (.X-axis (Utilities|Struct|Breakst_team (Utilities|Array|Get(acopy) (LocalVariables|GetFtemp_team) index))) (.Y-axis (Utilities|Struct|Breakst_team (Utilities|Array|Get(acopy) (LocalVariables|GetFtemp_team) index))) _unit_2 _finisherindex_2))
          (else
            (Utilities|Array|SetArrayElem (.team_number (Utilities|Struct|Breakst_team_Assembly (Variables|level_unit_data|Getteam))) index Item)))
        (else
          (Utilities|Array|SetArrayElem :TargetArray (LocalVariables|GetFtemp_team) :Index index))))
    (:then_1
      ;[1 1 1] 注释
      (for _array_element (LocalVariables|GetFtemp_team)
        (for _array_element_2 (.team_number (Utilities|Struct|Breakst_team_Assembly (Variables|level_unit_data|Getteam)))
          (if (Math|Boolean|ANDBoolean (== (.rowname (Utilities|Struct|Breakst_team _array_element)) (.rowname (Utilities|Struct|Breakst_team _array_element_2))) (== (.index (Utilities|Struct|Breakst_team _array_element)) (.index (Utilities|Struct|Breakst_team _array_element_2))) (== (.unit (Utilities|Struct|Breakst_team _array_element_2)) (.unit (Utilities|Struct|Breakst_team _array_element)))) ; 检查队伍是否一致
            (if (not (== (.Finisherindex (Utilities|Struct|Breakst_team _array_element_2)) (.Finisherindex (Utilities|Struct|Breakst_team _array_element))))
              (for _array_element_3 (Variables|Rawdata|Getchess_pieces)
                (if (== (Variables|/Game/BP/BP_Before_the_battle_begins/BP_Formation_Pieces.BP_Formation_Pieces_C|Getrole_ID _array_element_3) (.index (Utilities|Struct|Breakst_team _array_element_2)))
                  (Variables|/Game/BP/BP_Before_the_battle_begins/BP_Formation_Pieces.BP_Formation_Pieces_C|Setfinsher_index _array_element_3 (.Finisherindex (Utilities|Struct|Breakst_team _array_element_2))))))
            (else
              (for _array_element_4 (Variables|Rawdata|Getchess_pieces)
                (if (== (Variables|/Game/BP/BP_Before_the_battle_begins/BP_Formation_Pieces.BP_Formation_Pieces_C|Getrole_ID _array_element_4) (.index (Utilities|Struct|Breakst_team _array_element_2)))
                  (Actor|DestroyActor _array_element_4)
                  ;[1 1 1] 生成新的角色到特定位置上
                  (bind _returnvalue (Utilities|GetDataTableRow "/Game/Struct/character/T_character_library.T_character_library" _rowname)
                    (:then
                      (bind _returnvalue_2 (Game|SpawnActorfromClass "/Game/BP/BP_Before_the_battle_begins/BP_Formation_Pieces.BP_Formation_Pieces_C" (CallFunction|UnitsLocationCompute "NewEnumerator1" _x_axis _y_axis) "Undefined" "MultiplyWithRoot" 0 self _rowname _index (.skill_data (Utilities|Struct|BreakST_Character_library _returnvalue)) (.Finsher_skill_ (Utilities|Struct|BreakST_Character_library _returnvalue)) _finisherindex 0 0))
                      (Utilities|Array|Add (Variables|Rawdata|Getchess_pieces) _returnvalue_2)
                      (for _array_element_5 (Variables|level_unit_data|Getfixed_level_unit_data)
                        (if (== (.unit_location_index (Utilities|Struct|Breakst_unit_class _array_element_5)) (CallFunction|GetUnitIndex _returnvalue_2))
                          (Utilities|Array|SetArrayElem (Variables|level_unit_data|Getfixed_level_unit_data) 0 (Utilities|Struct|Makest_unit_class (.unit_location_index (Utilities|Struct|Breakst_unit_class _array_element_5)) (.chear (Utilities|Struct|Breakst_unit_class _array_element_5)) _returnvalue_2 (.theunitarea (Utilities|Struct|Breakst_unit_class _array_element_5)) (.theunit_Belongs (Utilities|Struct|Breakst_unit_class _array_element_5)) (.unit_chear_class (Utilities|Struct|Breakst_unit_class _array_element_5)) (.unit_charter_class (Utilities|Struct|Breakst_unit_class _array_element_5)) (.gameplay_unit_type (Utilities|Struct|Breakst_unit_class _array_element_5))))
                          (bind _unit_class (CallFunction|UpdateUnitClass (Variables|level_unit_data|Getfixed_level_unit_data)))
                          (Variables|level_unit_data|Setfixed_level_unit_data _unit_class))))))))))))))

(fn UpdataTeam
  (params (Team_unit_data :type Array%20of%20St%20Team%20Structures))
  (bind _output_get (Variables|level_unit_data|Setteam (Utilities|Struct|Makest_team_Assembly Team_unit_data)))
  (for _array_element (Variables|Rawdata|Getchess_pieces)
    (Actor|DestroyActor _array_element)
    (Utilities|Array|Clear (Variables|level_unit_data|Getlevel_unit_data_NEW))
    (Utilities|Array|Clear (Variables|level_unit_data|Getfixed_level_unit_data)))
  (A1|GenerateChessPiecesBasedontheTeam (Utilities|Struct|Breakst_team_Assembly _output_get))
  (bind _level_unit (A1|IntegratetheBoardandPieces (Variables|Rawdata|Getboard) (Variables|Rawdata|Getchess_pieces)))
  (Variables|level_unit_data|Setlevel_unit_data_NEW _level_unit))

(fn EndtheFormation
  (bind _chess_pieces (Variables|Rawdata|Getchess_pieces))
  (bind _board (Variables|Rawdata|Getboard))
  (for _array_element _board
    (if (Utilities|IsValid _array_element)
      (Actor|DestroyActor _array_element)))
  (Utilities|Array|Clear _board)
  (for _array_element_2 _chess_pieces
    (Actor|DestroyActor _array_element_2))
  (Utilities|Array|Clear _chess_pieces)
  (return))

(fn BattleOpen
  (params (level_Row%20NameZ :type Name))
  (D1|EndtheFormation)
  (Default|BattleStage (Variables|A1|GetAs%202Dplayer%20Contrller) (Variables|F1|GetOpen_Gamemode%20C) (Utilities|Struct|Breakst_team_Assembly (Variables|F1|GetFIX_TEAM)) (Variables|F1|GetOpen%20Player%20Bonus) (Variables|F1|GetOpen%20Unit%20Bonus) (Variables|F1|GetOpen%20Enemy%20Unit%20Bonus) level_Row%20NameZ))

(fn LoadingFormtionData
  (params (Open_Gamemode%20CX :type E_level_game_mode%20Enum :default "NewEnumerator3") (Open_temp_unit_dataX :type Array%20of%20ST%20Unit%20Data%20Temp%20Structures) (Open%20Enemy%20Unit%20BonusX :type St%20Rougelike%20Unit%20Bonus%20Structure) (Open%20%20Unit%20BonusX :type St%20Rougelike%20Unit%20Bonus%20Structure) (Open%20Player%20BonusX :type ST%20Battle%20Data%20Structure) (LEVEL_FIX_team :type St%20Team%20Assembly%20Structure) (level_rownameXA :type Name))
  (Variables|F1|SetOpen_Gamemode%20C Open_Gamemode%20CX)
  (Variables|F1|SetOpen_temp_unit_data Open_temp_unit_dataX)
  (Variables|F1|SetOpen%20Enemy%20Unit%20Bonus Open%20Enemy%20Unit%20BonusX)
  (Variables|F1|SetOpen%20Unit%20Bonus Open%20%20Unit%20BonusX)
  (Variables|F1|SetOpen%20Player%20Bonus Open%20Player%20BonusX)
  (Variables|F1|SetFIX_TEAM LEVEL_FIX_team)
  (Variables|F1|Setlevel_rowname level_rownameXA))

(fn LoadTeam
  (params (Selection :type E_level_game_mode%20Enum :default "NewEnumerator3"))
  (switch Utilities|FlowControl|Switch|SwitchonE_level_game_mode Selection
    (:NewEnumerator0
      _)
    (:NewEnumerator5
      _)
    (:NewEnumerator4
      _)
    (:NewEnumerator1
      (return (Variables|F1|GetFIX_TEAM))))
  (bind _asbp_game_instance (Utilities|Casting|CastToBP_GameInstance (Game|GetGameInstance)))
  (return (Utilities|Array|Get(acopy) (Variables|/Game/gamemode/BP_GameInstance.BP_GameInstance_C|Getteam_data _asbp_game_instance) 1)))

(fn UpdateUnitClass
  (params (team_unit_class :type Array%20of%20St%20Unit%20Class%20Structures))
  (bind _output_get (LocalVariables|Setteam_unit team_unit_class))
  (for (_array_element _array_index) _output_get
    (Utilities|Array|SetArrayElem (LocalVariables|Getteam_unit) _array_index (Utilities|Struct|Makest_unit_class (.unit_location_index (Utilities|Struct|Breakst_unit_class _array_element)) (.chear (Utilities|Struct|Breakst_unit_class _array_element)) 0 (.theunitarea (Utilities|Struct|Breakst_unit_class _array_element)) (.theunit_Belongs (Utilities|Struct|Breakst_unit_class _array_element)) (.unit_chear_class (Utilities|Struct|Breakst_unit_class _array_element)) (.unit_charter_class (Utilities|Struct|Breakst_unit_class _array_element)) (.gameplay_unit_type (Utilities|Struct|Breakst_unit_class _array_element)))))
  (for _array_element_2 (Variables|Rawdata|Getchess_pieces)
    (if (Utilities|IsValid _array_element_2)
      (for _array_element_3 (LocalVariables|Getteam_unit)
        (if (== (CallFunction|GetUnitIndex _array_element_2) (.unit_location_index (Utilities|Struct|Breakst_unit_class _array_element_3)))
          (Utilities|Array|SetArrayElem (LocalVariables|Getteam_unit) 0 (Utilities|Struct|Makest_unit_class (.unit_location_index (Utilities|Struct|Breakst_unit_class _array_element_3)) (.chear (Utilities|Struct|Breakst_unit_class _array_element_3)) _array_element_2 (.theunitarea (Utilities|Struct|Breakst_unit_class _array_element_3)) (.theunit_Belongs (Utilities|Struct|Breakst_unit_class _array_element_3)) (.unit_chear_class (Utilities|Struct|Breakst_unit_class _array_element_3)) (.unit_charter_class (Utilities|Struct|Breakst_unit_class _array_element_3)) (.gameplay_unit_type (Utilities|Struct|Breakst_unit_class _array_element_3))))))))
  (return (LocalVariables|Getteam_unit)))

(fn UpdataTeamData
  (params (unit_class :type Array%20of%20St%20Unit%20Class%20Structures))
  (for _array_element unit_class
    (bind _asbp_formation_pieces (Utilities|Casting|CastToBP_Formation_Pieces (Utilities|Struct|Breakst_unit_class _array_element)))
    (for _array_element_2 (Utilities|Struct|Breakst_team_Assembly (Variables|F1|GetFIX_TEAM))
      (if (== (.rowname (Utilities|Struct|Breakst_character_info (Utilities|Struct|Breakst_player_character_data (Variables|/Game/BP/BP_AC/BP_Player_level_AC/BP_character_object.BP_character_object_C|Getcharacter_data (Variables|/Game/BP/BP_Before_the_battle_begins/BP_Formation_Pieces.BP_Formation_Pieces_C|Getcharacter_object _asbp_formation_pieces))))) (.rowname (Utilities|Struct|Breakst_team _array_element_2)))
        (Utilities|Array|SetArrayElem (Utilities|Struct|Breakst_team_Assembly (Variables|F1|GetFIX_TEAM)) 0 (Utilities|Struct|Makest_team (.rowname (Utilities|Struct|Breakst_team _array_element_2)) (.index (Utilities|Struct|Breakst_team _array_element_2)) (.AXIS%20X (CallFunction|FormAXISbyINDEX (CallFunction|GetUnitIndex (Utilities|Struct|Breakst_unit_class _array_element)))) (.AXIS%20Y (CallFunction|FormAXISbyINDEX (CallFunction|GetUnitIndex (Utilities|Struct|Breakst_unit_class _array_element)))) (.unit (Utilities|Struct|Breakst_team _array_element_2)) (.Finisherindex (Utilities|Struct|Breakst_team _array_element_2)) (.ture_level (Utilities|Struct|Breakst_team _array_element_2)))))))
  (return))