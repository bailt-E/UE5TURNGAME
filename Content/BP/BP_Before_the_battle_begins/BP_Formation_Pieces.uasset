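; Draggable chess piece for arranging the team formation before battle.
; While clicked, it follows the cursor each Tick, converts its position to a board index stored as NewIndex, and has Formation relocate any piece found there.
; On release it snaps to that cell, then rebuilds Formation's board-and-piece data and updates the team data.
; An older line-trace cell detection remains as unconnected logic.
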(event Custom|updata_pieces_location_team_data
  (CallFunction|SetthePiecestoNewLocation (Variables|Default|Getnew%20index))
  (bind _level_unit (Default|IntegratetheBoardandPieces (Variables|Base|Getformation) (Variables|/Game/BP/BP_Before_the_battle_begins/BP_Level_formation_class.BP_Level_formation_class_C|Getboard (Variables|Base|Getformation)) (Variables|/Game/BP/BP_Before_the_battle_begins/BP_Level_formation_class.BP_Level_formation_class_C|Getchess_pieces (Variables|Base|Getformation))))
  (bind _output_get (Variables|/Game/BP/BP_Before_the_battle_begins/BP_Level_formation_class.BP_Level_formation_class_C|Setlevel_unit_data_NEW (Variables|Base|Getformation) _level_unit))
  (bind _output_get_2 (Variables|/Game/BP/BP_Before_the_battle_begins/BP_Level_formation_class.BP_Level_formation_class_C|Setfixed_level_unit_data (Variables|Base|Getformation) _output_get))
  (Default|UpdataTeamData (Variables|Base|Getformation) _output_get_2))

(event EventTick
  (params (DeltaSeconds :type Float%20%28single-precision%29))
  (bind _returnvalue (Game|GetPlayerController 0))
  (bind _returnvalue_2 (Transformation|GetActorLocation))
  (bind _hitresult (Game|Player|GetHitResultUnderCursorbyChannel _returnvalue "TraceTypeQuery1" true))
  (bind (_x_axis _y_axis) (CallFunction|AXIS-InverseCompute _returnvalue_2))
  (bind _location (Collision|BreakHitResult _hitresult))
  (bind (_xxaxis _yyaxis) (CallFunction|AdjustmentFunction _x_axis _y_axis))
  (bind (_x _y) (Math|Vector|BreakVector _location))
  (bind _returnvalue_3 (Math|Conversions|ToFloat(Integer) _xxaxis))
  (bind _returnvalue_4 (Math|Conversions|ToFloat(Integer) _yyaxis))
  (bind _returnvalue_5 (CallFunction|2d21d _returnvalue_3 _returnvalue_4))
  (if (Variables|Default|GetIS_onclicked)
    (Transformation|SetActorLocation (Math|Vector|MakeVector (- _x 5e+01) (- _y 5e+01) 5e+01) false false) ; 拖拽棋子
    (for _array_element (Variables|/Game/BP/BP_Before_the_battle_begins/BP_Level_formation_class.BP_Level_formation_class_C|Getlevel_unit_data_NEW (Variables|Base|Getformation))
      (if (== _returnvalue_5 (.unit_location_index (Utilities|Struct|Breakst_unit_class _array_element))) ; 当前角色与所处位置的棋子是否相符
        (if (Utilities|IsValid (.charter (Utilities|Struct|Breakst_unit_class _array_element))) ; 该位置是否存在棋子
          (Default|SetUnitNewlocation (Variables|Base|Getformation) (.charter (Utilities|Struct|Breakst_unit_class _array_element))) ; 将改棋子移动到新的位置上
          (Variables|Default|Setnew%20index _returnvalue_5)
          (else
            (Variables|Default|Setnew%20index (.unit_location_index (Utilities|Struct|Breakst_unit_class _array_element)))))))))

(event MouseInput|EventActorOnClicked
  (params (ButtonPressed :type Key%20Structure))
  (Variables|Default|SetIS_onclicked true))

(event EventActorOnReleased
  (params (ButtonReleased :type Key%20Structure))
  (Variables|Default|SetIS_onclicked false)
  (CallFunction|UpdataPiecesLocationTeamData))

(fn ConstructionScript)

(fn SetthePiecestoNewLocation
  (params (index :type Integer))
  (bind (_axis_x _axis_y) (CallFunction|FormAXISbyINDEX index))
  (bind _returnvalue (CallFunction|UnitsLocationCompute "NewEnumerator1" _axis_x _axis_y))
  (bind _location (Math|Transform|BreakTransform _returnvalue))
  (bind (_x _y) (Math|Vector|BreakVector _location))
  (if (not (Variables|Default|GetIS_onclicked))
    (Transformation|SetActorLocation (Math|Vector|MakeVector _x _y 0.0) false false)))