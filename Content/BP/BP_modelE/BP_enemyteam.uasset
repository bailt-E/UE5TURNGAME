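; BP_enemyteam manages an action point pool for what appears to be the enemy team's turn.
; An init function refills current points to the maximum, and a spend function runs unit selection and deducts one point while the count is zero or above.
; Selection, named for picking the unit with most action points, only filters units by owner and major type, then casts to BP_base_enemy_class without comparing or returning anything.
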(fn TheNumberOfInitializationActions
  (Variables|Default|SetCurrent%20Action%20Point (Variables|Default|Getactionpoint_max)))

(fn 选择单位行动点最多的单位
  (params (unit_class :type Array%20of%20St%20Unit%20Class%20Structures))
  (for _array_element unit_class
    (if (Utilities|Enum|Equal(Enum) (.theunit_Belongs (Utilities|Struct|Breakst_unit_class _array_element)) "NewEnumerator0")
      (switch Utilities|FlowControl|Switch|SwitchonE_unit_type (.gameplay_unit_type (Utilities|Struct|Breakst_unit_class _array_element))
        (:NewEnumerator0
          (Utilities|Casting|CastToBP_base_enemy_class (.charter (Utilities|Struct|Breakst_unit_class _array_element))))))))

(fn 新函数
  (params (unit_class :type Array%20of%20St%20Unit%20Class%20Structures))
  (if (>= (Variables|Default|GetCurrent%20Action%20Point) 0)
    (CallFunction|选择单位行动点最多的单位 unit_class)
    (Variables|Default|SetCurrent%20Action%20Point (- (Variables|Default|GetCurrent%20Action%20Point) 1))))