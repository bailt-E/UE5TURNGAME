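; Clickable character unit for a turn-based game that registers itself as the global player pawn's selected target.
; BeginPlay initializes the unit, its skills and its widget; clicks check player action and game flow before selecting and, in some cases, changing turn state.
; DataDocking copies level component stats into the generic attributes component.
; TakeEffects is an empty stub, and the skill filter's contradictory type check never adds anything.
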(event EventBeginPlay
  (Utilities|FlowControl|Sequence
    (:then_0
      (CallFunction|UnitInitializationFunction)
      (CallFunction|PawnSkillInitalize (Variables|pawn_Data|Getname)))
    (:then_1
      (CallFunction|SetWidget))))

(event MouseInput|EventActorOnClicked
  (params (ButtonPressed :type Key%20Structure :default "None"))
  (Utilities|FlowControl|Sequence
    (:then_0
      (bind _output_get (CallFunction|Initialize)) ; 获得玩家
      (if (and (Utilities|Enum|Equal(Enum) (Variables|/Game/BP/BP_modelE/BP_GLOBAL_CHARATER.BP_GLOBAL_CHARATER_C|Getplayer_action _output_get) "NewEnumerator5") (Utilities|Enum|Equal(Enum) (Variables|/Game/BP/BP_modelE/BP_land_spaner.BP_land_spaner_C|GetGame%20flow (Variables|/Game/BP/BP_modelE/BP_GLOBAL_CHARATER.BP_GLOBAL_CHARATER_C|Getland _output_get)) "NewEnumerator1")) ; 检查回合
        (CallFunction|StelectTarget)
        (elif (and (Utilities|Enum|NotEqual(Enum) (Variables|/Game/BP/BP_modelE/BP_GLOBAL_CHARATER.BP_GLOBAL_CHARATER_C|Getplayer_action _output_get) "NewEnumerator0") (Utilities|Enum|NotEqual(Enum) (Variables|/Game/BP/BP_modelE/BP_GLOBAL_CHARATER.BP_GLOBAL_CHARATER_C|Getplayer_action _output_get) "NewEnumerator1"))
          (CallFunction|StelectTarget)
          (Variables|/Game/BP/BP_modelE/BP_GLOBAL_CHARATER.BP_GLOBAL_CHARATER_C|SetTurn_GAME_state (Variables|gamecheck|GetAs%20BP%20GLOBAL%20CHARATER_0) "NewEnumerator2"))))
    (:then_1
      (CallFunction|IsClickedEvent))))

(fn ConstructionScript)

(fn Initialize
  (bind _asbp_global_charater (Utilities|Casting|CastToBP_GLOBAL_CHARATER (Game|Player|GetPlayerPawn 0)))
  (bind _output_get (Variables|gamecheck|SetAs%20BP%20GLOBAL%20CHARATER_0 _asbp_global_charater))
  (return _output_get))

(fn TakeEffects
  (params (Effects :type St%20Child%20Base%20Attributes%20Structure)))

(fn DataDocking
  (bind _ac_level (Variables|组件|GetAC_level))
  (bind _pawn_fix_attributes (Variables|/Game/BP/BP_AC/BP_Player_level_AC/AC_level_exp.AC_level_exp_C|Getpawn_fix_attributes _ac_level))
  (bind _full_attributes (Variables|/Game/BP/BP_AC/BP_Player_level_AC/AC_level_exp.AC_level_exp_C|GetFull%20attributes _ac_level))
  (bind (_hp _attatk _defense _speed _speed_max _overlord_max _criticalrate _critchance) (Utilities|Struct|BreakST_Full_attributes _full_attributes))
  (bind (_speedcap _overloadroundcap _maximumshield _overloadcap _energycap _unit_actionpointcap _element_tag_number_max _initialvelocity _initial_unit_actionpoint) (Utilities|Struct|BreakST_Fixed_attributes_A _pawn_fix_attributes))
  (bind _output_get (Variables|/Game/BP/BP_AC/BP_Generic_attributes_AC/AC_Generic_attributes.AC_Generic_attributes_C|SetUNIT_Fixed%20attributes (Variables|Default|GetAC_Generic_attributes) (Utilities|Struct|MakeST_Attribute_collection_AA (Utilities|Struct|MakeST_Base_attributes_A _hp _attatk _defense _speed (Math|Float|Truncate _criticalrate) (Math|Float|Truncate _critchance)) (Utilities|Struct|MakeST_Edge_attributes_A 0.0 0.0) (Utilities|Struct|MakeST_Fixed_attributes_A _speedcap _overloadroundcap _maximumshield _overloadcap _energycap _unit_actionpointcap _element_tag_number_max _initialvelocity _initial_unit_actionpoint) "(element_bonus_3_7E47476240021223A27EB1B15F25B237=((element_type_2_A382164746729B1F7E90C0B960DFA649=NewEnumerator0),(element_type_2_A382164746729B1F7E90C0B960DFA649=NewEnumerator1),(element_type_2_A382164746729B1F7E90C0B960DFA649=NewEnumerator2),(element_type_2_A382164746729B1F7E90C0B960DFA649=NewEnumerator4),(element_type_2_A382164746729B1F7E90C0B960DFA649=NewEnumerator3)),Finaldamagebonus_7_C0F6EFE54D0D41C34BEE3BA503A9A25C=0.000000,Damagereductionbonus_9_9010B5E8408BD39C6EABC9BBEBF850BC=0.000000)")))
  (return _output_get))

(fn PawnSkillInitalize
  (params (RowName :type Name))
  (Utilities|FlowControl|Sequence
    (:then_0
      (for _array_element (Variables|pawn_Data|Getskill)
        (if (and (Utilities|Enum|Equal(Enum) (Utilities|Struct|Breakst_role_skill _array_element) "NewEnumerator2") (Utilities|Enum|Equal(Enum) (Utilities|Struct|Breakst_role_skill _array_element) "NewEnumerator0"))
          (Utilities|Array|Add (Variables|pawn_Data|Getskill) _array_element))))
    (:then_1
      (Variables|pawn_Data|SetXXX (Math|Random|RandomInteger 100)))))

(fn StelectTarget
  (Variables|/Game/BP/BP_modelE/BP_GLOBAL_CHARATER.BP_GLOBAL_CHARATER_C|SetSelected%20Widget (Variables|gamecheck|GetAs%20BP%20GLOBAL%20CHARATER_0) self)
  (Variables|/Game/BP/BP_modelE/BP_GLOBAL_CHARATER.BP_GLOBAL_CHARATER_C|SetAs%20BP%20Base%20Pawn%20Class (Variables|gamecheck|GetAs%20BP%20GLOBAL%20CHARATER_0) self))