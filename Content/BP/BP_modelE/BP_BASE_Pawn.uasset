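; BP_BASE_Pawn is the base unit pawn for turn-based board battles, handling selection, damage, healing, shields and buffs.
; BeginPlay sets the mesh and initializes attributes; clicks update selection on the cached BP_GLOBAL_CHARATER.
; Attacks pass through prioritized ACBuff effects that can alter damage before reaching ACGenericAttributes, then spawn battle-effect widgets.
; Area buffs sync through quarantine arrays; immunity logic in GetBuff and healing's buff hook never execute.
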(event MouseInput|EventActorOnClicked
  (params (ButtonPressed :type Key%20Structure))
  (bind _as_bp_global_charater (Variables|Other|GetAs%20BP%20GLOBAL%20CHARATER))
  (bind _as_bp_global_charater_2 (Variables|Other|GetAs%20BP%20GLOBAL%20CHARATER))
  (if (and (Utilities|Enum|Equal(Enum) (Variables|/Game/BP/BP_modelE/BP_GLOBAL_CHARATER.BP_GLOBAL_CHARATER_C|GetTurn_GAME_state _as_bp_global_charater) "NewEnumerator2") (Utilities|Enum|Equal(Enum) (Variables|/Game/BP/BP_modelE/BP_GLOBAL_CHARATER.BP_GLOBAL_CHARATER_C|Getplayer_action _as_bp_global_charater) "NewEnumerator0")) ; 检查是否处于我方回合
    (if (== (Variables|/Game/BP/BP_modelE/BP_GLOBAL_CHARATER.BP_GLOBAL_CHARATER_C|GetSelect%20skill%20object (Variables|Other|GetAs%20BP%20GLOBAL%20CHARATER)) self) ; 角色是否等于自身
      (Variables|/Game/BP/BP_modelE/BP_GLOBAL_CHARATER.BP_GLOBAL_CHARATER_C|SetSelect%20the%20target _as_bp_global_charater_2 true)
      (CallFunction|CallPlayer)
      (else
        (Variables|/Game/BP/BP_modelE/BP_GLOBAL_CHARATER.BP_GLOBAL_CHARATER_C|SetSelect%20the%20target _as_bp_global_charater_2 false)
        (Variables|/Game/BP/BP_modelE/BP_GLOBAL_CHARATER.BP_GLOBAL_CHARATER_C|SetSelect%20skill%20object (Variables|Other|GetAs%20BP%20GLOBAL%20CHARATER) self)
        (CallFunction|CallPlayer)))
    (else
      (Development|PrintText "不执行"))))

(event EventBeginPlay
  ;[1 1 1] 初始化
  (Utilities|FlowControl|Sequence
    (:then_0
      (|CallParentFunction))
    (:then_1
      (A1|UnitInitializationFunction))
    (:then_2
      (bind _attributs (Default|AttributeDetermination (Variables|Default|GetAC_Generic_attributes) (Variables|pawn_team|GetTable%20Switch) (Variables|pawn_team|GetLevel) (Variables|pawn_team|GetFix) (Variables|pawn_team|GetFix%20Attributs)))
      (bind _output_get (Default|TickAttributes (Variables|Default|GetAC_Generic_attributes) (Variables|Default|Getunit_bonus) (Utilities|Struct|MakeST_Attribute_collection_AA (Utilities|Struct|MakeST_Base_attributes_A (.hp_max (Utilities|Struct|Breakst_the_unit_attribute _attributs)) (.attack (Utilities|Struct|Breakst_the_unit_attribute _attributs)) (.defense (Utilities|Struct|Breakst_the_unit_attribute _attributs))))))
      (Default|InitializetheProperty (Variables|Default|GetAC_Generic_attributes) _output_get))))

(fn ConstructionScript)

(fn BuffImmunityCheak
  (params (Execution%20of%20the%20immune%20phase :type e_buff_Immunity%20Enum :default "NewEnumerator1") (element_type :type E_element_type%20Enum :default "NewEnumerator5") (element_type_level :type E_element_advance%20Enum :default "NewEnumerator2") (buff_nature_type :type E_buff_Nature_type%20Enum :default "NewEnumerator0") (buff_type :type E_BUFF_type%20Enum :default "NewEnumerator0"))
  (LocalVariables|Setimmunity Execution%20of%20the%20immune%20phase)
  (for _array_element (Variables|/Game/BP/BP_AC/BP_BUFF_AC/AC_buff.AC_buff_C|Getcurrent_buff (Variables|Default|GetAC_buff))
    (for _array_element_2 (Variables|/Game/BP/BP_AC/BP_BUFF_AC/BP_buff_class.BP_buff_class_C|Getimmunity_info _array_element)
      (if (Utilities|Enum|Equal(Enum) (LocalVariables|Getimmunity) (.immunity_type (Utilities|Struct|Breakst_buff_immunity _array_element_2)))
        (if (Math|Boolean|ANDBoolean (Utilities|Enum|Equal(Enum) buff_type (.buff_type (Utilities|Struct|Breakst_buff_search_criteria (.buff_search_info (Utilities|Struct|Breakst_buff_immunity _array_element_2))))) (Utilities|Enum|Equal(Enum) buff_nature_type (.buff_nature_type (Utilities|Struct|Breakst_buff_search_criteria (.buff_search_info (Utilities|Struct|Breakst_buff_immunity _array_element_2))))) (Utilities|Enum|Equal(Enum) (.element_type (Utilities|Struct|Breakst_buff_search_criteria (.buff_search_info (Utilities|Struct|Breakst_buff_immunity _array_element_2)))) element_type) (Utilities|Enum|Equal(Enum) (.element_level (Utilities|Struct|Breakst_buff_search_criteria (.buff_search_info (Utilities|Struct|Breakst_buff_immunity _array_element_2)))) element_type_level))
          (return true _array_element)
          (else
            (return false 0)))))))

(fn DataDocking
  (params (RowName :type Name))
  (bind _returnvalue (Utilities|GetDataTableRow "/Game/Struct/rank_table/T_leveltand.T_leveltand" RowName)
    (:then
      (return (Utilities|Struct|MakeST_Attribute_collection_AA (Utilities|Struct|MakeST_Base_attributes_A (.Health (Utilities|Struct|Breakst_levelrand _returnvalue)) (.Attack (Utilities|Struct|Breakst_levelrand _returnvalue)) (.defense (Utilities|Struct|Breakst_levelrand _returnvalue))))))))

(fn SetUnitdata
  (params (unit_area :type E_area%20Enum :default "NewEnumerator0") (unit_faction :type E_unitfaction%20Enum :default "NewEnumerator0") (gameplay_unit_type :type E_unit_type%20Enum :default "NewEnumerator0"))
  (Variables|unit_info|Setunit_area unit_area)
  (Variables|unit_info|Setunit_faction unit_faction)
  (Variables|unit_info|Setgameplay_unit_type gameplay_unit_type))

(fn UnitInitializationFunction
  (bind _asbp_global_charater (Utilities|Casting|CastToBP_GLOBAL_CHARATER (Game|Player|GetPlayerPawn 0)))
  (if (Utilities|IsValid _asbp_global_charater)
    (Variables|Other|SetAs%20BP%20GLOBAL%20CHARATER _asbp_global_charater)
    (Components|SkeletalMesh|SetSkeletalMeshAsset (Variables|Default|GetSkeletalMesh_C) (Variables|Default|GetUNITSkeletal%20Mesh))))

(fn IsClickedEvent
  (bind _as_bp_global_charater (Variables|Other|GetAs%20BP%20GLOBAL%20CHARATER))
  (bind _as_bp_global_charater_2 (Variables|Other|GetAs%20BP%20GLOBAL%20CHARATER))
  (if (Utilities|Enum|Equal(Enum) (Variables|/Game/BP/BP_modelE/BP_GLOBAL_CHARATER.BP_GLOBAL_CHARATER_C|Getplayer_action _as_bp_global_charater) "NewEnumerator0") ; 检查是否处于我方回合
    (switch Utilities|FlowControl|Switch|Switchonenum_game_state (Variables|/Game/BP/BP_modelE/BP_GLOBAL_CHARATER.BP_GLOBAL_CHARATER_C|GetTurn_GAME_state _as_bp_global_charater)
      (:NewEnumerator2
        (if (== (Variables|/Game/BP/BP_modelE/BP_GLOBAL_CHARATER.BP_GLOBAL_CHARATER_C|GetSelect%20skill%20object (Variables|Other|GetAs%20BP%20GLOBAL%20CHARATER)) self) ; 角色是否等于自身
          (Variables|/Game/BP/BP_modelE/BP_GLOBAL_CHARATER.BP_GLOBAL_CHARATER_C|SetSelect%20the%20target (Variables|Other|GetAs%20BP%20GLOBAL%20CHARATER) true)
          (Development|PrintString "BP_base_unit_select_target")
          (else
            (Variables|/Game/BP/BP_modelE/BP_GLOBAL_CHARATER.BP_GLOBAL_CHARATER_C|SetSelect%20skill%20object (Variables|Other|GetAs%20BP%20GLOBAL%20CHARATER) self))))
      (:NewEnumerator8
        (if (== (Variables|/Game/BP/BP_modelE/BP_GLOBAL_CHARATER.BP_GLOBAL_CHARATER_C|GetSelect%20skill%20object (Variables|Other|GetAs%20BP%20GLOBAL%20CHARATER)) self) ; 角色是否等于自身
          (Variables|/Game/BP/BP_modelE/BP_GLOBAL_CHARATER.BP_GLOBAL_CHARATER_C|SetSelect%20the%20target _as_bp_global_charater_2 true)
          (else
            (Variables|/Game/BP/BP_modelE/BP_GLOBAL_CHARATER.BP_GLOBAL_CHARATER_C|SetSelect%20the%20target _as_bp_global_charater_2 false)
            (Variables|/Game/BP/BP_modelE/BP_GLOBAL_CHARATER.BP_GLOBAL_CHARATER_C|SetSelect%20skill%20object (Variables|Other|GetAs%20BP%20GLOBAL%20CHARATER) self)))))))

(fn CheakHealth（NG）
  (bind _is_dead (Default|CheckLifeAttributes (Variables|Default|GetAC_Generic_attributes)))
  (if _is_dead
    (Default|WhentheUnitDies (Variables|/Game/BP/BP_modelE/BP_GLOBAL_CHARATER.BP_GLOBAL_CHARATER_C|Getland (Variables|Other|GetAs%20BP%20GLOBAL%20CHARATER)) self)))

(fn GainAShield
  (params (shield_type :type E_shield_type%20Enum :default "NewEnumerator0") (B :type Float%20%28double-precision%29))
  (Variables|/Game/BP/BP_AC/BP_Generic_attributes_AC/AC_Generic_attributes.AC_Generic_attributes_C|SetCurrent_resource (Variables|Default|GetAC_Generic_attributes) (Utilities|Struct|MakeST_UNIT_Current_resource_AA (Utilities|Struct|MakeST_unit_shield shield_type (+ B (Utilities|Struct|BreakST_unit_shield (Utilities|Struct|BreakST_UNIT_Current_resource_AA (Variables|/Game/BP/BP_AC/BP_Generic_attributes_AC/AC_Generic_attributes.AC_Generic_attributes_C|GetCurrent_resource (Variables|Default|GetAC_Generic_attributes)))))))))

(fn GetBuff
  (params (buff_rowname :type Name) (target :type Actor%20Object%20Reference) (create :type Actor%20Object%20Reference) (buff_index :type Integer) (buff_type :type E_BUFF_type%20Enum :default "NewEnumerator0") (buff_nature :type E_buff_Nature_type%20Enum :default "NewEnumerator0") (buff_Updata :type E_BuffTimeUpdataEnum%20Enum :default "NewEnumerator0") (element_type :type E_element_type%20Enum :default "NewEnumerator5") (element_type_level :type E_element_advance%20Enum :default "NewEnumerator2"))
  (bind _newparam (Default|Addbuff0 (Variables|Default|GetAC_buff) buff_rowname target create))
  (bind _returnvalue (Game|SpawnActorfromClass "/Game/BP/BP_actor/bp_battle_effect_widget.bp_battle_effect_widget_C" (Math|Transform|MakeTransform (Transformation|GetActorLocation self)) "Undefined" "MultiplyWithRoot" 0 "buff" 0))
  (Emptyfunction|AfterReceivingtheBuff _newparam))

(fn BeTreaed
  (params (tread_v :type Float%20%28double-precision%29))
  (Utilities|FlowControl|Sequence
    (:then_0
      (Default|InTreaed (Variables|Default|GetAC_Generic_attributes) tread_v))
    (:then_1
      (LocalVariables|Seteffect_prioity 1)
      (LocalVariables|Setinterupt false)
      (if (LocalVariables|Getinterupt)
        (bind (_array_element _find) (Default|FindBuffsThatHaveActiveEffects (Variables|Default|GetAC_buff) (LocalVariables|Geteffect_type) (LocalVariables|Geteffect_prioity)))
        (if _find
          (for _array_element_2 _array_element
            (bind _interrupt (Default|ExecuteBuffEffect (Variables|Default|GetAC_buff) (LocalVariables|Geteffect_type) (LocalVariables|Geteffect_prioity) _array_element_2 0.0))
            (LocalVariables|Setinterupt _interrupt))
          (else
            (LocalVariables|Seteffect_prioity (+ (LocalVariables|Geteffect_prioity) 1))
            (bind (_array_element_3 _find_2) (Default|FindBuffsThatHaveActiveEffects (Variables|Default|GetAC_buff) (LocalVariables|Geteffect_type) (LocalVariables|Geteffect_prioity)))
            (if _find_2
              (for _array_element_4 _array_element_3
                (bind _interrupt_2 (Default|ExecuteBuffEffect (Variables|Default|GetAC_buff) (LocalVariables|Geteffect_type) (LocalVariables|Geteffect_prioity) _array_element_4 0.0))
                (LocalVariables|Setinterupt _interrupt_2)))))))))

(fn BeAttack
  (params (damage :type Float%20%28double-precision%29) (Critical%20hit :type Boolean) (Critical%20hit%20volume :type Float%20%28double-precision%29) (element_type :type E_element_type%20Enum :default "NewEnumerator5") (damage_type :type e_damage_type%20Enum :default "NewEnumerator1") (element_damage_type :type e_element_damage_type%20Enum :default "NewEnumerator1") (Damage%20final%20bonus :type Float%20%28double-precision%29))
  (LocalVariables|Setnext_damage damage)
  (LocalVariables|Setbuff_effect "NewEnumerator3")
  (LocalVariables|SetHierarchical%20Interrupt false)
  (LocalVariables|Seteffect_prioity 1)
  (if (LocalVariables|GetHierarchical%20Interrupt)
    (Default|InAttack (Variables|Default|GetAC_Generic_attributes) (LocalVariables|Getnext_damage) Critical%20hit Critical%20hit%20volume element_type damage_type element_damage_type Damage%20final%20bonus)
    (else
      (bind (_array_element _find) (Default|FindBuffsThatHaveActiveEffects (Variables|Default|GetAC_buff) (LocalVariables|Getbuff_effect) (LocalVariables|Geteffect_prioity)))
      (if _find
        (for _array_element_2 _array_element
          (bind (_excurt _newparam _interrupt) (Default|ExecuteBuffEffect (Variables|Default|GetAC_buff) (LocalVariables|Getbuff_effect) (LocalVariables|Geteffect_prioity) _array_element_2 (LocalVariables|Getnext_damage)))
          (LocalVariables|SetHierarchical%20Interrupt _interrupt)
          (LocalVariables|Setnext_damage _newparam)
          (Default|InAttack (Variables|Default|GetAC_Generic_attributes) (LocalVariables|Getnext_damage) Critical%20hit Critical%20hit%20volume element_type damage_type element_damage_type Damage%20final%20bonus)
          (Game|SpawnActorfromClass "/Game/BP/BP_actor/bp_battle_effect_widget.bp_battle_effect_widget_C" (Math|Transform|MakeTransform (Transformation|GetActorLocation)) "Undefined" "MultiplyWithRoot" 0 (Utilities|Text|ToText(Float) (LocalVariables|Getnext_damage) "HalfToEven") 0))
        (else
          (bind _output_get (LocalVariables|Seteffect_prioity (+ (LocalVariables|Geteffect_prioity) 1)))
          (bind (_array_element_3 _find_2) (Default|FindBuffsThatHaveActiveEffects (Variables|Default|GetAC_buff) (LocalVariables|Getbuff_effect) _output_get))
          (if _find_2
            (for _array_element_4 _array_element_3
              (bind (_excurt_2 _newparam_2 _interrupt_2) (Default|ExecuteBuffEffect (Variables|Default|GetAC_buff) (LocalVariables|Getbuff_effect) (LocalVariables|Geteffect_prioity) _array_element_4 damage))
              (LocalVariables|Setnext_damage _newparam_2)
              (LocalVariables|SetHierarchical%20Interrupt _interrupt_2)
              (Default|InAttack (Variables|Default|GetAC_Generic_attributes) (LocalVariables|Getnext_damage) Critical%20hit Critical%20hit%20volume element_type damage_type element_damage_type Damage%20final%20bonus)
              (Game|SpawnActorfromClass "/Game/BP/BP_actor/bp_battle_effect_widget.bp_battle_effect_widget_C" (Math|Transform|MakeTransform (Transformation|GetActorLocation)) "Undefined" "MultiplyWithRoot" 0 (Utilities|Text|ToText(Float) (LocalVariables|Getnext_damage) "HalfToEven") 0))
            (else
              (LocalVariables|Setnext_damage damage)
              (Default|InAttack (Variables|Default|GetAC_Generic_attributes) (LocalVariables|Getnext_damage) Critical%20hit Critical%20hit%20volume element_type damage_type element_damage_type Damage%20final%20bonus)
              (Game|SpawnActorfromClass "/Game/BP/BP_actor/bp_battle_effect_widget.bp_battle_effect_widget_C" (Math|Transform|MakeTransform (Transformation|GetActorLocation)) "Undefined" "MultiplyWithRoot" 0 (Utilities|Text|ToText(Float) (LocalVariables|Getnext_damage) "HalfToEven") 0))))))))

(fn ChearAreabuffDockingPawnBuff
  (bind (_xindex _yindex) (Default|GetactorLocationIndex (Variables|Other|GetAs%20BP%20GLOBAL%20CHARATER) (Transformation|GetActorLocation)))
  (bind _asactor (Default|FindChearinBoard (Variables|Other|GetAs%20BP%20GLOBAL%20CHARATER) _xindex _yindex))
  (bind _asbp_base_pawn (Utilities|Casting|CastToBP_BASE_Pawn _asactor))
  (Variables|/Game/BP/BP_AC/BP_BUFF_AC/AC_buff.AC_buff_C|SetQuarantine%20AreaA (Variables|Default|GetAC_buff) (Variables|/Game/BP/BP_AC/BP_BUFF_AC/AC_buff.AC_buff_C|Getarea_buff (Variables|BP_BASE_Pawn_C|GetAC_buff _asbp_base_pawn))))

(fn BuffDataComparison
  (bind _ac_buff (Variables|Default|GetAC_buff))
  (for _array_element (Variables|/Game/BP/BP_AC/BP_BUFF_AC/AC_buff.AC_buff_C|GetQuarantine%20AreaA _ac_buff)
    (for _array_element_2 (Variables|/Game/BP/BP_AC/BP_BUFF_AC/AC_buff.AC_buff_C|GetQuarantine%20AreaB _ac_buff)
      (if (== _array_element_2 _array_element) ; 检查buff是否一致
        (return false)
        (else
          (return true))))))

(fn UpdateBuff
  (params (Condition :type Boolean))
  (if Condition
    (for _array_element (Variables|/Game/BP/BP_AC/BP_BUFF_AC/AC_buff.AC_buff_C|GetQuarantine%20AreaB (Variables|Default|GetAC_buff))
      (Utilities|Array|RemoveItem (Variables|/Game/BP/BP_AC/BP_BUFF_AC/AC_buff.AC_buff_C|Getcurrent_buff (Variables|Default|GetAC_buff)) _array_element) ; 在当前buff数组移除隔离区
      (Utilities|Array|Clear (Variables|/Game/BP/BP_AC/BP_BUFF_AC/AC_buff.AC_buff_C|GetQuarantine%20AreaB (Variables|Default|GetAC_buff))) ; 清除隔离区B
      (bind _output_get (Variables|/Game/BP/BP_AC/BP_BUFF_AC/AC_buff.AC_buff_C|SetQuarantine%20AreaB (Variables|Default|GetAC_buff) (Variables|/Game/BP/BP_AC/BP_BUFF_AC/AC_buff.AC_buff_C|GetQuarantine%20AreaA (Variables|Default|GetAC_buff))))
      (for _array_element_2 _output_get
        (Utilities|Array|Add (Variables|/Game/BP/BP_AC/BP_BUFF_AC/AC_buff.AC_buff_C|Getwait_add_buff (Variables|Default|GetAC_buff)) _array_element_2)))))

(fn AfterReceivingtheBuff
  (params (buff :type BP%20Buff%20Class%20Object%20Reference)))

(fn CallPlayer
  (Default|CallPlayerEvent (Variables|Other|GetAs%20BP%20GLOBAL%20CHARATER))
  (Development|PrintString "call_player"))