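; Base pawn for selectable characters in a turn-based game, holding level, XP and combat attributes.
; Clicking it registers it as the selection on the BP_GLOBAL_CHARATER player pawn and updates turn state, while Tick passes valid Result entries to that pawn's GetactorNumber.
; Functions handle XP, level-ups from a fixed Level_data row, effects, and summing base and synthesis attributes.
; Event-graph leveling and walkable-tile highlighting chains are disconnected.
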(event EventTick
  (params (DeltaSeconds :type Float%20%28single-precision%29))
  ;[1 1 1] 获取所有的数字，并形成数组
  (for _array_element (Variables|Gamecheck|GetResult)
    (Utilities|IsValid _array_element
      (:Is%20Valid
        (Default|GetactorNumber (Variables|gamecheck|GetAs%20BP%20GLOBAL%20CHARATER) _array_element)))))

(event MouseInput|EventActorOnClicked
  (params (ButtonPressed :type Key%20Structure :default "None"))
  (bind _as_bp_global_charater (Variables|gamecheck|GetAs%20BP%20GLOBAL%20CHARATER))
  (bind _output_get (CallFunction|Initialize))
  (if (Utilities|Enum|Equal(Enum) (Variables|/Game/BP/BP_modelE/BP_GLOBAL_CHARATER.BP_GLOBAL_CHARATER_C|GetTurn_GAME_state _output_get) "NewEnumerator1")
    (Variables|/Game/BP/BP_modelE/BP_GLOBAL_CHARATER.BP_GLOBAL_CHARATER_C|SetSelected%20Widget (Variables|gamecheck|GetAs%20BP%20GLOBAL%20CHARATER) self)
    (else
      (Variables|/Game/BP/BP_modelE/BP_GLOBAL_CHARATER.BP_GLOBAL_CHARATER_C|SetTurn_GAME_state _as_bp_global_charater "NewEnumerator1")
      (Variables|/Game/BP/BP_modelE/BP_GLOBAL_CHARATER.BP_GLOBAL_CHARATER_C|Setplayer_action _as_bp_global_charater "NewEnumerator1")
      (Variables|/Game/BP/BP_modelE/BP_GLOBAL_CHARATER.BP_GLOBAL_CHARATER_C|SetSelected%20Widget (Variables|gamecheck|GetAs%20BP%20GLOBAL%20CHARATER) self))))

(fn ConstructionScript)

(fn LevelUp
  (bind _returnvalue (Utilities|GetDataTableRow "/Game/Struct/table/level_data.level_data" "19")
    (:then
      (Variables|level|SetlevelandXP (Utilities|Struct|Makest_child_levelXP (+ (.level (Utilities|Struct|Breakst_child_levelXP (Variables|level|GetlevelandXP))) 1) (- (.XP (Utilities|Struct|Breakst_child_levelXP (Variables|level|GetlevelandXP))) (.Experiencerequired (Utilities|Struct|Breakst_child_levelXP (Variables|level|GetlevelandXP)))) (Math|Float|Truncate (Utilities|Struct|Breakst_child_beseleveldate _returnvalue)))))))

(fn Getxp
  (params (newxp :type Integer))
  (Variables|level|SetlevelandXP (Utilities|Struct|Makest_child_levelXP (+ newxp (.XP (Utilities|Struct|Breakst_child_levelXP (Variables|level|GetlevelandXP))))))
  (return (> (+ newxp (.XP (Utilities|Struct|Breakst_child_levelXP (Variables|level|GetlevelandXP)))) (.Experiencerequired (Utilities|Struct|Breakst_child_levelXP (Variables|level|GetlevelandXP))))))

(fn LevelNAIYIWU
  (bind _kaleta_synthesis_attributes (Variables|attributes|Getkaleta_synthesis_attributes))
  (bind _levelattributes (Variables|level|GetlevelAttributes))
  (bind (_health _currentlife _lifedebt _anomalouslife _amountofshield _attack _defense _critical _criticaldamage _speed _speedcap _overload _oneturn_overloadcap) (Utilities|Struct|Breakst_child_base_attributes _kaleta_synthesis_attributes))
  (bind (_health_2 _attack_2 _defense_2) (Utilities|Struct|Breakst_child_beseleveldate _levelattributes))
  (Variables|attributes|Setkaleta_base_attributes (Utilities|Struct|Makest_child_base_attributes _health_2 _attack_2 _defense_2))
  (Variables|attributes|Setkaleta_final_attributes (Utilities|Struct|Makest_child_base_attributes (+ _health (.health (Utilities|Struct|Breakst_child_base_attributes (Variables|attributes|Getkaleta_base_attributes)))) (+ _currentlife (.Currentlife (Utilities|Struct|Breakst_child_base_attributes (Variables|attributes|Getkaleta_base_attributes)))) 0.0 (+ _anomalouslife (.Anomalouslife (Utilities|Struct|Breakst_child_base_attributes (Variables|attributes|Getkaleta_base_attributes)))) 0.0 (+ _attack (.Attack (Utilities|Struct|Breakst_child_base_attributes (Variables|attributes|Getkaleta_base_attributes)))) (+ _defense (.defense (Utilities|Struct|Breakst_child_base_attributes (Variables|attributes|Getkaleta_base_attributes)))) (+ _critical (.Critical (Utilities|Struct|Breakst_child_base_attributes (Variables|attributes|Getkaleta_base_attributes)))) (+ _criticaldamage (.Criticaldamage (Utilities|Struct|Breakst_child_base_attributes (Variables|attributes|Getkaleta_base_attributes)))) (+ _speed (.speed (Utilities|Struct|Breakst_child_base_attributes (Variables|attributes|Getkaleta_base_attributes)))) (+ _speedcap (.Speedcap (Utilities|Struct|Breakst_child_base_attributes (Variables|attributes|Getkaleta_base_attributes)))) (+ _overload (.overload (Utilities|Struct|Breakst_child_base_attributes (Variables|attributes|Getkaleta_base_attributes)))) (+ _oneturn_overloadcap (.oneturn_Overloadcap (Utilities|Struct|Breakst_child_base_attributes (Variables|attributes|Getkaleta_base_attributes)))))))

(fn Initialize
  (bind _asbp_global_charater (Utilities|Casting|CastToBP_GLOBAL_CHARATER (Game|Player|GetPlayerPawn 0)))
  (bind _output_get (Variables|gamecheck|SetAs%20BP%20GLOBAL%20CHARATER _asbp_global_charater))
  (return _output_get))

(fn TakeEffects
  (params (Effects :type St%20Child%20Base%20Attributes%20Structure))
  (bind (_health _currentlife _lifedebt _anomalouslife _amountofshield _attack _defense _critical _criticaldamage _speed _speedcap _overload _oneturn_overloadcap) (Utilities|Struct|Breakst_child_base_attributes Effects))
  (bind _kaleta_final_attributes (Variables|attributes|Getkaleta_final_attributes))
  (bind (_health_2 _currentlife_2 _lifedebt_2 _anomalouslife_2 _amountofshield_2 _attack_2 _defense_2 _critical_2 _criticaldamage_2 _speed_2 _speedcap_2 _overload_2 _oneturn_overloadcap_2) (Utilities|Struct|Breakst_child_base_attributes _kaleta_final_attributes))
  (Variables|attributes|Setkaleta_synthesis_attributes (Utilities|Struct|Makest_child_base_attributes (- _health _health_2) (- _currentlife _currentlife_2) (- _lifedebt _lifedebt_2) (- _anomalouslife _anomalouslife_2) (- _amountofshield _amountofshield_2) (- _attack _attack_2) (- _defense _defense_2) (- _critical _critical_2) (- _criticaldamage _criticaldamage_2) (- _speed _speed_2) (- _speedcap _speedcap_2) (- _overload _overload_2) (- _oneturn_overloadcap _oneturn_overloadcap_2))))

(fn Cheaklevelxp
  (bind _levelandxp (Variables|level|GetlevelandXP))
  (bind (_xp _experiencerequired) (Utilities|Struct|Breakst_child_levelXP _levelandxp))
  (if (>= _xp _experiencerequired)
    (return true)))