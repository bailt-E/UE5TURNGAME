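; BP_unit_class is a unit actor that builds its stats and can be clicked as a target.
; BeginPlay runs initialization, then feeds type, grade, level and attributes into BPACUnitAttribute.
; Clicking sets the unit as the player character's TargetActor, then fires its clicked event (被点击事件).
; DataDocking copies health, attack, defense and action points from BPACUnitAttribute into ACGenericAttributes, but is not called in these graphs.
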(event EventTick
  (params (DeltaSeconds :type Float%20%28single-precision%29)))

(event EventBeginPlay
  (bind _initialize_unit_information (Variables|Default|GetInitialize%20unit%20information))
  (bind (_unit_name _unit_type _fixedgrade _the_unit_level _the_unitfaction _unit_attribute) (Utilities|Struct|Breakst_level_unit_Initialize_DATA _initialize_unit_information))
  (CallFunction|InitializationFunction)
  (Default|InitializationOfAttributes (Variables|Default|GetBP_AC_unit_attribute) _unit_type _fixedgrade _the_unit_level _unit_attribute))

(event MouseInput|EventActorOnClicked
  (params (ButtonPressed :type Key%20Structure))
  (Utilities|FlowControl|Sequence
    (:then_0
      (bind _asbp_global_charater (Utilities|Casting|CastToBP_GLOBAL_CHARATER (Game|Player|GetPlayerPawn 0)))
      (Variables|/Game/BP/BP_modelE/BP_GLOBAL_CHARATER.BP_GLOBAL_CHARATER_C|Settarget_actor _asbp_global_charater self))
    (:then_1
      (CallFunction|被点击事件))))

(fn ConstructionScript)

(fn DataDocking
  (bind _bp_ac_unit_attribute (Variables|Default|GetBP_AC_unit_attribute))
  (bind _unit_attributes (Variables|/Game/BP/BP_AC/BP_UNIT_AC/BP_AC_unit_attribute.BP_AC_unit_attribute_C|Getunit_attributes _bp_ac_unit_attribute))
  (bind (_hp_max _attack _defense _growthactionpoints) (Utilities|Struct|Breakst_the_unit_attribute _unit_attributes))
  (Variables|/Game/BP/BP_AC/BP_Generic_attributes_AC/AC_Generic_attributes.AC_Generic_attributes_C|SetUNIT_Fixed%20attributes (Variables|Default|GetAC_Generic_attributes) (Utilities|Struct|MakeST_Attribute_collection_AA (Utilities|Struct|MakeST_Base_attributes_A _hp_max _attack _defense 0 0 0 _growthactionpoints) "(Healingbonus_2_3E1CBC5547F1D7BB6CA4EEB39461C4F9=0.000000,Healbonus_4_405BD1E640E508570CF5639AC2D96CF7=0.000000,Shieldedbonus_6_C15C311E4485322B9C5CB78DAE9E85F0=0.000000,Shieldbonus_8_B343CC88453336528D5A24B00172ED2A=0.000000,aggro_bonus_13_12C01A6C4813ECCDE9637191B4452CEB=0.000000)" (Utilities|Struct|MakeST_Fixed_attributes_A) "(element_bonus_3_7E47476240021223A27EB1B15F25B237=,Finaldamagebonus_7_C0F6EFE54D0D41C34BEE3BA503A9A25C=0.000000,Damagereductionbonus_9_9010B5E8408BD39C6EABC9BBEBF850BC=0.000000)")))