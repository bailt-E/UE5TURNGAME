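; Base Blueprint for monster units, which the player clicks to select as a target.
; On BeginPlay it runs the parent logic, sets up its widget and sets its level to a fixed value.
; A click makes it the player character's TargetActor, then triggers the clicked event and post-target skill selection.
; DataDocking copies max HP, attack and defense from the unit attribute component into the generic attributes component, ignoring its RowName input.
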(event EventTick
  (params (DeltaSeconds :type Float%20%28single-precision%29)))

(event EventBeginPlay
  (Utilities|FlowControl|Sequence
    (:then_0
      (|CallParentFunction))
    (:then_1
      (CallFunction|SetWidget)
      (Variables|Default|SetLevel "100"))))

(event MouseInput|EventActorOnClicked
  (params (ButtonPressed :type Key%20Structure :default "None"))
  (Utilities|FlowControl|Sequence
    (:then_0
      (bind _asbp_global_charater (Utilities|Casting|CastToBP_GLOBAL_CHARATER (Game|Player|GetPlayerPawn 0)))
      (Variables|/Game/BP/BP_modelE/BP_GLOBAL_CHARATER.BP_GLOBAL_CHARATER_C|Settarget_actor _asbp_global_charater self))
    (:then_1
      (CallFunction|IsClickedEvent)
      (Default|SelectUnitSkillTargetAfter (Variables|Default|GetAs%20BP%20GLOBAL%20CHARATER))
      (CallFunction|CallPlayer))))

(fn ConstructionScript)

(fn DataDocking
  (params (RowName :type Name :default "None"))
  (bind _bp_ac_unit_attribute1 (Variables|Default|GetBP_AC_unit_attribute1))
  (bind _unit_attributes (Variables|/Game/BP/BP_AC/BP_UNIT_AC/BP_AC_unit_attribute.BP_AC_unit_attribute_C|Getunit_attributes _bp_ac_unit_attribute1))
  (bind (_hp_max _attack _defense) (Utilities|Struct|Breakst_the_unit_attribute _unit_attributes))
  (bind _output_get (Variables|/Game/BP/BP_AC/BP_Generic_attributes_AC/AC_Generic_attributes.AC_Generic_attributes_C|SetUNIT_Fixed%20attributes (Variables|Default|GetAC_Generic_attributes) (Utilities|Struct|MakeST_Attribute_collection_AA (Utilities|Struct|MakeST_Base_attributes_A _hp_max _attack _defense))))
  (return _output_get))