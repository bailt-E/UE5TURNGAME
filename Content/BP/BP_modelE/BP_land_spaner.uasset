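; Battlefield spawner and turn-flow manager that builds the player and enemy boards for a grid-based, turn-based battle.
; At BeginPlay it registers with BP_GLOBAL_CHARATER, spawns both tile grids, and places units from TeamData and UnityData.
; Tiles and units go into flattened arrays on that character, then UnitRecords pairs them by index into UnitClass records.
; TheGameBegins switches on GameFlow to handle setup and player, enemy and neutral rounds.
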(event Custom|The%20game%20begins
  (bind _as_bp_global_charater (Variables|data|GetAs%20BP%20GLOBAL%20CHARATER))
  (Utilities|FlowControl|Sequence
    (:then_0
      (switch Utilities|FlowControl|Switch|Switchonenum_game_Gameflow (Variables|Processcontrol|GetGame%20flow)
        (:NewEnumerator0
          (beginplay|SpawnEnemyBoardsandUnits)
          (beginplay|GenerateYourBoardandCharacters)
          (Auxiliarycontrol|CountAllActors(map)) ; 检查
          (Processcontrol|ToggleRounds "NewEnumerator1")
          (Variables|/Game/BP/BP_modelE/BP_GLOBAL_CHARATER.BP_GLOBAL_CHARATER_C|Setplayer_action _as_bp_global_charater "NewEnumerator5")
          (Variables|/Game/BP/BP_modelE/BP_GLOBAL_CHARATER.BP_GLOBAL_CHARATER_C|SetTurn_GAME_state _as_bp_global_charater "NewEnumerator2")
          (bind _unit_class (CallFunction|UnitRecords))
          (for _array_element _unit_class
            (if (and (Utilities|Enum|Equal(Enum) (.theunitarea (Utilities|Struct|Breakst_unit_class _array_element)) "NewEnumerator0") (Utilities|Enum|Equal(Enum) (.theunit_Belongs (Utilities|Struct|Breakst_unit_class _array_element)) "NewEnumerator0"))
              (Development|PrintString (Utilities|String|Append "编号/" (Utilities|String|ToString(Integer) (.unit_index (Utilities|Struct|Breakst_unit_class _array_element))) "/棋子-" (Utilities|GetDisplayName (.chear (Utilities|Struct|Breakst_unit_class _array_element))) "单位/" (Utilities|GetDisplayName (.charter (Utilities|Struct|Breakst_unit_class _array_element))) "/" (Utilities|GetClassDisplayName (.unit_chear_class (Utilities|Struct|Breakst_unit_class _array_element))) (Utilities|GetClassDisplayName (.unit_charter_class (Utilities|Struct|Breakst_unit_class _array_element)))) true true "(R=0.000000,G=0.660000,B=1.000000,A=1.000000)" 1e+02))))
        (:NewEnumerator1
          (Default|初始化行动点 (Variables|data|Getenemyteam))
          (if (Variables|ProcessControl|GetConfirm%20the%20switch%20round)
            (Processcontrol|ToggleRounds "NewEnumerator2")
            (bind _output_get (Variables|ProcessControl|SetConfirm%20the%20switch%20round false))
            (if _output_get
              (Variables|/Game/BP/BP_modelE/BP_GLOBAL_CHARATER.BP_GLOBAL_CHARATER_C|SetTurn_GAME_state (Variables|data|GetAs%20BP%20GLOBAL%20CHARATER) "NewEnumerator2"))))
        (:NewEnumerator2
          (Utilities|FlowControl|Delay 1e+02)
          (Processcontrol|ToggleRounds "NewEnumerator3"))
        (:NewEnumerator3
          (Processcontrol|ToggleRounds "NewEnumerator1")
          (Variables|/Game/BP/BP_modelE/BP_GLOBAL_CHARATER.BP_GLOBAL_CHARATER_C|SetTurn_GAME_state (Variables|data|GetAs%20BP%20GLOBAL%20CHARATER) "NewEnumerator2")
          (Default|CallTurnCheak))))))

(event EventBeginPlay
  (Utilities|FlowControl|Sequence
    (:then_0
      (beginplay|DataInitialize)
      (CallFunction|TheGameBegins))))

(event EventTick
  (params (DeltaSeconds :type Float%20%28single-precision%29)))

(fn ConstructionScript)

(fn ToggleRounds
  (params (Game%20flow :type enum_game_Gameflow%20Enum :default "NewEnumerator0"))
  (Variables|Processcontrol|SetGame%20flow Game%20flow))

(fn SpawnNewRoundsOfEnemiesontheBattlefield)

(fn SpawnNewRoundsOfEnemiesontheMap)

(fn ChecktheCombatSituation(win/lost))

(fn DataIntegration(NG)
  (bind _as_bp_global_charater (Variables|data|GetAs%20BP%20GLOBAL%20CHARATER))
  (Utilities|FlowControl|Sequence
    (:then_0
      (bind _asbp_gamechear_class (CallFunction|Getmygamechear))
      (Utilities|Array|Add (Variables|/Game/BP/BP_modelE/BP_GLOBAL_CHARATER.BP_GLOBAL_CHARATER_C|Getunit_class (Variables|data|GetAs%20BP%20GLOBAL%20CHARATER)) (Utilities|Struct|Makest_unit_class (Default|GetactorNumber (Variables|data|GetAs%20BP%20GLOBAL%20CHARATER) 0 _asbp_gamechear_class) _asbp_gamechear_class 0 "NewEnumerator0" "NewEnumerator0" 0)))
    (:then_1
      (bind _asbp_base_pawn_class (CallFunction|GetAllPawn))
      (bind _asbp_gamechear_class_2 (CallFunction|Getmygamechear))
      (if (== (Default|GetactorNumber _as_bp_global_charater 0 _asbp_base_pawn_class) (Default|GetactorNumber _as_bp_global_charater 0 _asbp_gamechear_class_2))
        (Utilities|Array|SetArrayElem (Variables|/Game/BP/BP_modelE/BP_GLOBAL_CHARATER.BP_GLOBAL_CHARATER_C|Getunit_class (Variables|data|GetAs%20BP%20GLOBAL%20CHARATER)) 0 (Utilities|Struct|Makest_unit_class (Default|GetactorNumber _as_bp_global_charater 0 _asbp_base_pawn_class) _asbp_gamechear_class_2 _asbp_base_pawn_class 0))))
    (:then_2
      (Utilities|FlowControl|Sequence
        (:then_0
          (return (Variables|/Game/BP/BP_modelE/BP_GLOBAL_CHARATER.BP_GLOBAL_CHARATER_C|Getunit_class (Variables|data|GetAs%20BP%20GLOBAL%20CHARATER))))))))

(fn CountAllActors(map)
  (bind _as_bp_global_charater (Variables|data|GetAs%20BP%20GLOBAL%20CHARATER))
  (for _array_element (Variables|/Game/BP/BP_modelE/BP_GLOBAL_CHARATER.BP_GLOBAL_CHARATER_C|GetPlayers _as_bp_global_charater)
    (if (Utilities|IsValid _array_element)
      (Utilities|Map|Add (Variables|/Game/BP/BP_modelE/BP_GLOBAL_CHARATER.BP_GLOBAL_CHARATER_C|Getteam _as_bp_global_charater) (Default|2d21d _as_bp_global_charater (.X (Default|LocationNormalization _as_bp_global_charater (Transformation|GetActorLocation _array_element))) (.Y (Default|LocationNormalization _as_bp_global_charater (Transformation|GetActorLocation _array_element)))) _array_element))))

(fn GenerateYourBoardandCharacters
  (bind _w (Variables|棋盘信息|Getw))
  (bind _h (Variables|棋盘信息|Geth))
  (bind _returnvalue (* _w _h))
  ;[1 1 1] 初始化棋盘
  (Utilities|FlowControl|Sequence
    (:then_0
      (bind _asbp_global_charater (Utilities|Casting|CastToBP_GLOBAL_CHARATER (Game|GetPlayerCharacter 0)))
      (Variables|data|SetAs%20BP%20GLOBAL%20CHARATER _asbp_global_charater)
      (Utilities|Array|Resize (Variables|/Game/BP/BP_modelE/BP_GLOBAL_CHARATER.BP_GLOBAL_CHARATER_C|Getplayer_select_Widgets _asbp_global_charater) _returnvalue)
      (Utilities|Array|Resize (Variables|/Game/BP/BP_modelE/BP_GLOBAL_CHARATER.BP_GLOBAL_CHARATER_C|GetPlayers _asbp_global_charater) _returnvalue)
      (for _index (range 0 (- (Variables|棋盘信息|Getw) 1))
        (Variables|棋盘信息|Set2dx21d _index)
        (Variables|棋盘信息|Setx (+ (* (Variables|棋盘信息|Getpadding) _index) _index))
        (for _index_2 (range 0 (- (Variables|棋盘信息|Geth) 1))
          (Variables|棋盘信息|Set2dy21d _index_2)
          (Variables|棋盘信息|Sety (+ (* (Variables|棋盘信息|Getpadding) _index_2) _index_2))
          (Utilities|FlowControl|Sequence
            (:then_0
              (bind _returnvalue_2 (Game|SpawnActorfromClass "/Game/BP/BP_modelE/BP_gamechear_class.BP_gamechear_class_C" (Math|Transform|MakeTransform (Math|Vector|MakeVector (Math|Conversions|ToFloat(Integer) (* (Variables|棋盘信息|Getx) 100)) (Math|Conversions|ToFloat(Integer) (* (Variables|棋盘信息|Gety) 100)) 0.0)) "Undefined" "MultiplyWithRoot" 0 0)) ; 生成我方棋盘
              (Variables|棋盘信息|SetPLAYERCHUNK _returnvalue_2))
            (:then_1
              (bind _asbp_global_charater_2 (Utilities|Casting|CastToBP_GLOBAL_CHARATER (Game|GetPlayerCharacter 0)))
              (Utilities|Array|SetArrayElem (Variables|/Game/BP/BP_modelE/BP_GLOBAL_CHARATER.BP_GLOBAL_CHARATER_C|Getplayer_select_Widgets _asbp_global_charater_2) (+ (* (Variables|棋盘信息|Getw) (Variables|棋盘信息|Get2dx21d)) (Variables|棋盘信息|Get2dy21d)) (Variables|棋盘信息|GetPLAYERCHUNK)) ; 将棋盘变为数组
              (Utilities|Array|SetArrayElem (Variables|/Game/BP/BP_modelE/BP_GLOBAL_CHARATER.BP_GLOBAL_CHARATER_C|GetPlayers _asbp_global_charater_2) (+ (* (Variables|棋盘信息|Getw) (Variables|棋盘信息|Get2dx21d)) (Variables|棋盘信息|Get2dy21d)) (Variables|棋盘信息|Getplayer)) ; 将角色变量转变为数组
            )))))
    (:then_1
      (for _array_element (Variables|data|Getteam_data)
        (bind _returnvalue_3 (Game|SpawnActorfromClass :Class "/Game/BP/BP_modelE/BP_base_pawn_class.BP_base_pawn_class_C" :SpawnTransform (Math|Transform|MakeTransform (Math|Vector|MakeVector (Math|Conversions|ToFloat(Integer) (* (- (.X坐标 (Utilities|Struct|Breakst_team _array_element)) 1) 200)) (Math|Conversions|ToFloat(Integer) (* (- (.Y坐标 (Utilities|Struct|Breakst_team _array_element)) 1) 200)) 0.0)) :CollisionHandlingOverride "Undefined" :TransformScaleMethod "MultiplyWithRoot" :Instigator 0)) ; 生成角色
        (bind _output_get (Variables|棋盘信息|Setplayer _returnvalue_3))
        (Utilities|Array|Add (Variables|/Game/BP/BP_modelE/BP_GLOBAL_CHARATER.BP_GLOBAL_CHARATER_C|GetPlayers (Variables|data|GetAs%20BP%20GLOBAL%20CHARATER)) _output_get)))))

(fn SpawnEnemyBoardsandUnits
  (bind _w (Variables|棋盘信息|Getw))
  (bind _h (Variables|棋盘信息|Geth))
  (bind _returnvalue (* _w _h))
  ;[1 1 1] 初始化棋盘
  (Utilities|FlowControl|Sequence
    (:then_0
      (bind _asbp_global_charater (Utilities|Casting|CastToBP_GLOBAL_CHARATER (Game|GetPlayerCharacter 0)))
      (Utilities|Array|Resize (Variables|/Game/BP/BP_modelE/BP_GLOBAL_CHARATER.BP_GLOBAL_CHARATER_C|Getenemy_widets _asbp_global_charater) _returnvalue)
      (Utilities|Array|Resize (Variables|/Game/BP/BP_modelE/BP_GLOBAL_CHARATER.BP_GLOBAL_CHARATER_C|Getenemys _asbp_global_charater) _returnvalue)
      (for _index (range 0 (- (Variables|棋盘信息|Getw) 1))
        (Variables|棋盘信息|Set2dx21d _index)
        (Variables|棋盘信息|Setx (+ (* (Variables|棋盘信息|Getpadding) _index) _index))
        (for _index_2 (range 0 (- (Variables|棋盘信息|Geth) 1))
          (Variables|棋盘信息|Set2dy21d _index_2)
          (Variables|棋盘信息|Sety (+ (* (Variables|棋盘信息|Getpadding) _index_2) _index_2))
          (Utilities|FlowControl|Sequence
            (:then_0
              (bind _returnvalue_2 (Game|SpawnActorfromClass "/Game/BP/BP_modelE/BP_gamechear_class.BP_gamechear_class_C" (Math|Transform|MakeTransform (Math|Vector|MakeVector (Math|Conversions|ToFloat(Integer) (+ (* (Variables|棋盘信息|Getx) 100) (Variables|棋盘信息|Getenemy_juli))) (Math|Conversions|ToFloat(Integer) (* (Variables|棋盘信息|Gety) 100)) 0.0)) "Undefined" "MultiplyWithRoot" 0 0)) ; 生成敌方棋盘棋盘
              (Variables|棋盘信息|SetENEMYCHUNK _returnvalue_2)
              (bind _returnvalue_3 (Game|ConstructObjectfromClass "/Game/BP/BP_modelE/BP_enemyteam.BP_enemyteam_C"))
              (Variables|data|Setenemyteam _returnvalue_3))
            (:then_1
              (Utilities|FlowControl|Sequence
                (:then_0
                  (Utilities|Array|SetArrayElem (Variables|/Game/BP/BP_modelE/BP_GLOBAL_CHARATER.BP_GLOBAL_CHARATER_C|Getenemy_widets (Variables|data|GetAs%20BP%20GLOBAL%20CHARATER)) (+ (* (Variables|棋盘信息|Getw) (Variables|棋盘信息|Get2dx21d)) (Variables|棋盘信息|Get2dy21d)) (Variables|棋盘信息|GetENEMYCHUNK)) ; 将敌方棋盘加入棋盘
                )
                (:then_1
                  (Utilities|Array|SetArrayElem (Variables|/Game/BP/BP_modelE/BP_GLOBAL_CHARATER.BP_GLOBAL_CHARATER_C|Getenemys (Variables|data|GetAs%20BP%20GLOBAL%20CHARATER)) (+ (* (Variables|棋盘信息|Getw) (Variables|棋盘信息|Get2dx21d)) (Variables|棋盘信息|Get2dy21d)) (Variables|棋盘信息|Getenemy)) ; 将敌方单位变量转变为数组
                )))))))
    (:then_1
      (for _array_element (Variables|data|Getunity_data)
        (bind _returnvalue_4 (Game|SpawnActorfromClass "/Game/BP/BP_modelE/BP_base_enemy_class.BP_base_enemy_class_C" (Math|Transform|MakeTransform (Math|Vector|MakeVector (Math|Conversions|ToFloat(Integer) (+ (* (- (.X坐标 (Utilities|Struct|Breakst_team _array_element)) 1) 200) (Variables|棋盘信息|Getenemy_juli))) (Math|Conversions|ToFloat(Integer) (* (- (.Y坐标 (Utilities|Struct|Breakst_team _array_element)) 1) 200)) 0.0)) "Undefined" "MultiplyWithRoot" 0 0)) ; 生成角色
        (bind _output_get (Variables|棋盘信息|Setenemy _returnvalue_4))
        (Utilities|Array|Add (Variables|/Game/BP/BP_modelE/BP_GLOBAL_CHARATER.BP_GLOBAL_CHARATER_C|Getenemys (Variables|data|GetAs%20BP%20GLOBAL%20CHARATER)) _output_get)))))

(fn GetAllPawn
  (for (_array_element _array_index) (Variables|/Game/BP/BP_modelE/BP_GLOBAL_CHARATER.BP_GLOBAL_CHARATER_C|GetPlayers (Variables|data|GetAs%20BP%20GLOBAL%20CHARATER))
    (bind _asbp_base_unit (Utilities|Casting|CastToBP_BASE_UNIT _array_element))
    (bind _asbp_base_pawn_class (Utilities|Casting|CastToBP_base_pawn_class _asbp_base_unit))
    (return _asbp_base_pawn_class _array_index)))

(fn Getmygamechear
  (for (_array_element _array_index) (Variables|/Game/BP/BP_modelE/BP_GLOBAL_CHARATER.BP_GLOBAL_CHARATER_C|Getplayer_select_Widgets (Variables|data|GetAs%20BP%20GLOBAL%20CHARATER))
    (Development|PrintText "Hello")
    (bind _asactor (Utilities|Casting|CastToActor _array_element))
    (bind _asbp_base_unit (Utilities|Casting|CastToBP_BASE_UNIT _asactor))
    (bind _asbp_gamechear_class (Utilities|Casting|CastToBP_gamechear_class _asbp_base_unit))
    (return _asbp_gamechear_class _array_index)))

(fn UnitRecords
  (Utilities|Array|Clear (Variables|/Game/BP/BP_modelE/BP_GLOBAL_CHARATER.BP_GLOBAL_CHARATER_C|Getunit_class (Variables|data|GetAs%20BP%20GLOBAL%20CHARATER)))
  (Utilities|FlowControl|Sequence
    (:then_0
      ;[1 1 1] 我方单位统计
      (CallFunction|UnitChearStatistics (Variables|/Game/BP/BP_modelE/BP_GLOBAL_CHARATER.BP_GLOBAL_CHARATER_C|Getplayer_select_Widgets (Variables|data|GetAs%20BP%20GLOBAL%20CHARATER)) "NewEnumerator1" "NewEnumerator1")
      (CallFunction|UnitStatistics (Variables|/Game/BP/BP_modelE/BP_GLOBAL_CHARATER.BP_GLOBAL_CHARATER_C|GetPlayers (Variables|data|GetAs%20BP%20GLOBAL%20CHARATER)) "NewEnumerator1" "NewEnumerator1"))
    (:then_1
      ;[1 1 1] 敌方单位统计
      (CallFunction|UnitChearStatistics (Variables|/Game/BP/BP_modelE/BP_GLOBAL_CHARATER.BP_GLOBAL_CHARATER_C|Getenemy_widets (Variables|data|GetAs%20BP%20GLOBAL%20CHARATER)) "NewEnumerator0" "NewEnumerator0")
      (CallFunction|UnitStatistics (Variables|/Game/BP/BP_modelE/BP_GLOBAL_CHARATER.BP_GLOBAL_CHARATER_C|Getenemys (Variables|data|GetAs%20BP%20GLOBAL%20CHARATER)) "NewEnumerator1" "NewEnumerator0"))
    (:then_2
      (Utilities|FlowControl|Sequence
        (:then_0
          (return (Variables|/Game/BP/BP_modelE/BP_GLOBAL_CHARATER.BP_GLOBAL_CHARATER_C|Getunit_class (Variables|data|GetAs%20BP%20GLOBAL%20CHARATER))))))))

(fn DataInitialize
  (bind _asbp_global_charater (Utilities|Casting|CastToBP_GLOBAL_CHARATER (Game|Player|GetPlayerPawn 0)))
  (bind _output_get (Variables|data|SetAs%20BP%20GLOBAL%20CHARATER _asbp_global_charater))
  (Variables|/Game/BP/BP_modelE/BP_GLOBAL_CHARATER.BP_GLOBAL_CHARATER_C|Setland _output_get self))

(fn UnitStatistics
  (params (THEUNIT :type Array%20of%20Actor%20Object%20References) (the%20unitarea :type E_area%20Enum :default "NewEnumerator0") (the%20unit%20belongs :type E_unitfaction%20Enum :default "NewEnumerator0"))
  ;[1 1 1] 获得单位数字
  (for _array_element THEUNIT
    (for (_array_element_2 _array_index) (Variables|/Game/BP/BP_modelE/BP_GLOBAL_CHARATER.BP_GLOBAL_CHARATER_C|Getunit_class (Variables|data|GetAs%20BP%20GLOBAL%20CHARATER))
      (bind _asbp_base_unit (Utilities|Casting|CastToBP_BASE_UNIT _array_element))
      (bind _asbp_base_unit_2 (Utilities|Casting|CastToBP_BASE_UNIT (.chear (Utilities|Struct|Breakst_unit_class _array_element_2))))
      (if (and (Utilities|Enum|Equal(Enum) (.theunitarea (Utilities|Struct|Breakst_unit_class _array_element_2)) the%20unitarea) (Utilities|Enum|Equal(Enum) (.theunit_Belongs (Utilities|Struct|Breakst_unit_class _array_element_2)) the%20unit%20belongs))
        (if (== (.unit_index (Utilities|Struct|Breakst_unit_class _array_element_2)) (Default|GetactorNumber1 (Variables|data|GetAs%20BP%20GLOBAL%20CHARATER) _array_element))
          (Utilities|Array|SetArrayElem (Variables|/Game/BP/BP_modelE/BP_GLOBAL_CHARATER.BP_GLOBAL_CHARATER_C|Getunit_class (Variables|data|GetAs%20BP%20GLOBAL%20CHARATER)) _array_index (Utilities|Struct|Makest_unit_class (.unit_index (Utilities|Struct|Breakst_unit_class _array_element_2)) (.chear (Utilities|Struct|Breakst_unit_class _array_element_2)) _array_element (Utilities|GetClass _asbp_base_unit_2) (Utilities|GetClass _asbp_base_unit))))))))

(fn UnitChearStatistics
  (params (Array :type Array%20of%20Object%20Object%20References) (the%20unit%20area :type E_area%20Enum :default "NewEnumerator0") (the%20unit_Belongs :type E_unitfaction%20Enum :default "NewEnumerator0"))
  (for _array_element Array
    (bind _asactor (Utilities|Casting|CastToActor _array_element))
    (bind _asbp_base_unit (Utilities|Casting|CastToBP_BASE_UNIT _asactor))
    (bind _asbp_gamechear_class (Utilities|Casting|CastToBP_gamechear_class _asbp_base_unit))
    (Utilities|Array|Add (Variables|/Game/BP/BP_modelE/BP_GLOBAL_CHARATER.BP_GLOBAL_CHARATER_C|Getunit_class (Variables|data|GetAs%20BP%20GLOBAL%20CHARATER)) (Utilities|Struct|Makest_unit_class (Default|GetactorNumber1 (Variables|data|GetAs%20BP%20GLOBAL%20CHARATER) _asactor) _asbp_gamechear_class the%20unit%20area the%20unit_Belongs (Utilities|GetClass _asbp_gamechear_class)))))