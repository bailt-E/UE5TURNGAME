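; BP_gamechear_class is a clickable actor, apparently a game chair, that the player can select.
; On click it casts the player character to BP_GLOBAL_CHARATER and checks its TurnGAMEState and PlayerAction enum values.
; When both match, it stores itself in that character's SelectedChear variable.
; Tick and construction are empty, and a PlayerAction assignment is left unconnected.
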(event EventBeginPlay)

(event Collision|EventActorBeginOverlap
  (params (OtherActor :type Actor%20Object%20Reference)))

(event EventTick
  (params (DeltaSeconds :type Float%20%28single-precision%29)))

(event MouseInput|EventActorOnClicked
  (params (ButtonPressed :type Key%20Structure :default "None"))
  (bind _asbp_global_charater (Utilities|Casting|CastToBP_GLOBAL_CHARATER (Game|GetPlayerCharacter 0)))
  (Variables|Default|SetAs%20BP%20GLOBAL%20CHARATER_0 _asbp_global_charater)
  (if (and (Utilities|Enum|Equal(Enum) (Variables|/Game/BP/BP_modelE/BP_GLOBAL_CHARATER.BP_GLOBAL_CHARATER_C|GetTurn_GAME_state _asbp_global_charater) "NewEnumerator8") (Utilities|Enum|Equal(Enum) (Variables|/Game/BP/BP_modelE/BP_GLOBAL_CHARATER.BP_GLOBAL_CHARATER_C|Getplayer_action _asbp_global_charater) "NewEnumerator1"))
    (Variables|/Game/BP/BP_modelE/BP_GLOBAL_CHARATER.BP_GLOBAL_CHARATER_C|SetSelected%20chear (Variables|Default|GetAs%20BP%20GLOBAL%20CHARATER_0) self)))

(fn ConstructionScript)