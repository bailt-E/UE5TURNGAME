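; Base Blueprint for turn-based units, holding area, faction and type data and handling click selection.
; BeginPlay caches the BP_GLOBAL_CHARATER player pawn and initializes attributes when the unit is a BP_unit_class.
; Clicks write the selected unit to that pawn, gated by action and turn state; re-clicking confirms the target.
; A comment notes child units override ActorOnClicked; a separate click function repeats the logic, while DataDocking is empty.
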(event MouseInput|EventActorOnClicked
  (params (ButtonPressed :type Key%20Structure :default "None"))
  (bind _as_bp_global_charater (Variables|other|GetAs%20BP%20GLOBAL%20CHARATER))
  (bind _as_bp_global_charater_2 (Variables|other|GetAs%20BP%20GLOBAL%20CHARATER))
  (if (and (Utilities|Enum|Equal(Enum) (Variables|/Game/BP/BP_modelE/BP_GLOBAL_CHARATER.BP_GLOBAL_CHARATER_C|GetTurn_GAME_state _as_bp_global_charater) "NewEnumerator2") (Utilities|Enum|Equal(Enum) (Variables|/Game/BP/BP_modelE/BP_GLOBAL_CHARATER.BP_GLOBAL_CHARATER_C|Getplayer_action _as_bp_global_charater) "NewEnumerator0")) ; 检查是否处于我方回合
    (if (== (Variables|/Game/BP/BP_modelE/BP_GLOBAL_CHARATER.BP_GLOBAL_CHARATER_C|GetSelect%20skill%20object (Variables|other|GetAs%20BP%20GLOBAL%20CHARATER)) self) ; 角色是否等于自身
      (Variables|/Game/BP/BP_modelE/BP_GLOBAL_CHARATER.BP_GLOBAL_CHARATER_C|SetSelect%20the%20target _as_bp_global_charater_2 true)
      (else
        (Variables|/Game/BP/BP_modelE/BP_GLOBAL_CHARATER.BP_GLOBAL_CHARATER_C|SetSelect%20the%20target _as_bp_global_charater_2 false)
        (Variables|/Game/BP/BP_modelE/BP_GLOBAL_CHARATER.BP_GLOBAL_CHARATER_C|SetSelect%20skill%20object (Variables|other|GetAs%20BP%20GLOBAL%20CHARATER) self)))
    (else
      (Development|PrintText "不执行"))))

(event EventBeginPlay
  ;[1 1 1] 初始化
  (CallFunction|InitializationFunction)
  (bind _asbp_unit_class (Utilities|Casting|CastToBP_unit_class self))
  (Default|InitializationOfAttributes (Variables|/Game/BP/BP_modelE/BP_unit_class.BP_unit_class_C|GetBP_AC_unit_attribute _asbp_unit_class) "None" false))

(fn ConstructionScript)

(fn 被点击事件
  (bind _as_bp_global_charater (Variables|other|GetAs%20BP%20GLOBAL%20CHARATER))
  (bind _as_bp_global_charater_2 (Variables|other|GetAs%20BP%20GLOBAL%20CHARATER))
  (if (Utilities|Enum|Equal(Enum) (Variables|/Game/BP/BP_modelE/BP_GLOBAL_CHARATER.BP_GLOBAL_CHARATER_C|Getplayer_action _as_bp_global_charater) "NewEnumerator0") ; 检查是否处于我方回合
    (switch Utilities|FlowControl|Switch|Switchonenum_game_state (Variables|/Game/BP/BP_modelE/BP_GLOBAL_CHARATER.BP_GLOBAL_CHARATER_C|GetTurn_GAME_state _as_bp_global_charater)
      (:NewEnumerator2
        (if (== (Variables|/Game/BP/BP_modelE/BP_GLOBAL_CHARATER.BP_GLOBAL_CHARATER_C|GetSelect%20skill%20object (Variables|other|GetAs%20BP%20GLOBAL%20CHARATER)) self) ; 角色是否等于自身
          (Variables|/Game/BP/BP_modelE/BP_GLOBAL_CHARATER.BP_GLOBAL_CHARATER_C|SetSelect%20the%20target (Variables|other|GetAs%20BP%20GLOBAL%20CHARATER) true)
          (Development|PrintString "the unit_target")
          (else
            (Variables|/Game/BP/BP_modelE/BP_GLOBAL_CHARATER.BP_GLOBAL_CHARATER_C|SetSelect%20skill%20object (Variables|other|GetAs%20BP%20GLOBAL%20CHARATER) self))))
      (:NewEnumerator8
        (if (== (Variables|/Game/BP/BP_modelE/BP_GLOBAL_CHARATER.BP_GLOBAL_CHARATER_C|GetSelect%20skill%20object (Variables|other|GetAs%20BP%20GLOBAL%20CHARATER)) self) ; 角色是否等于自身
          (Variables|/Game/BP/BP_modelE/BP_GLOBAL_CHARATER.BP_GLOBAL_CHARATER_C|SetSelect%20the%20target _as_bp_global_charater_2 true)
          (else
            (Variables|/Game/BP/BP_modelE/BP_GLOBAL_CHARATER.BP_GLOBAL_CHARATER_C|SetSelect%20the%20target _as_bp_global_charater_2 false)
            (Variables|/Game/BP/BP_modelE/BP_GLOBAL_CHARATER.BP_GLOBAL_CHARATER_C|SetSelect%20skill%20object (Variables|other|GetAs%20BP%20GLOBAL%20CHARATER) self)))))))

(fn InitializationFunction
  (bind _asbp_global_charater (Utilities|Casting|CastToBP_GLOBAL_CHARATER (Game|Player|GetPlayerPawn 0)))
  (if (Utilities|IsValid _asbp_global_charater)
    (Variables|other|SetAs%20BP%20GLOBAL%20CHARATER _asbp_global_charater)))

(fn SetUnitdata
  (params (unit_area :type E_area%20Enum :default "NewEnumerator0") (unit_faction :type E_unitfaction%20Enum :default "NewEnumerator0") (gameplay_unit_type :type E_unit_type%20Enum :default "NewEnumerator0"))
  (Variables|unit_info|Setunit_area unit_area)
  (Variables|unit_info|Setunit_faction unit_faction)
  (Variables|unit_info|Setgameplay_unit_type gameplay_unit_type))

(fn DataDocking)