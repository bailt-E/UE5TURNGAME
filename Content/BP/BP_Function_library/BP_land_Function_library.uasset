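; Function library of grid helpers for a chessboard-style battle with enemy and player areas.
; Converts between world locations, X/Y cells and flat indices, and builds cell transforms per area.
; FindUnit applies 2D offsets to a target cell and collects movable characters found there through the battle's global character lookup.
; The two board-spawn functions return inside their nested loops, so they yield only the first padded cell.
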(fn GetUnitIndex
  (params (Object :type Actor%20Object%20Reference))
  (bind _unit_distance (LocalVariables|Getunit%20distance))
  (bind _object_spacing (LocalVariables|GetObject%20spacing))
  (bind _returnvalue (Transformation|GetActorLocation Object))
  (bind _returnvalue_2 (/ _returnvalue _unit_distance))
  (bind (_x _y _z) (Math|Vector|BreakVector _returnvalue_2))
  (bind _returnvalue_3 (Math|Float|Floor _x))
  (bind _returnvalue_4 (Math|Float|Floor _y))
  (bind _returnvalue_5 (Math|Float|Floor _z))
  (bind _returnvalue_6 (Math|Conversions|ToFloat(Integer) _returnvalue_3))
  (bind _returnvalue_7 (Math|Conversions|ToFloat(Integer) _returnvalue_4))
  (bind _returnvalue_8 (Math|Conversions|ToFloat(Integer) _returnvalue_5))
  (bind _returnvalue_9 (Math|Vector|MakeVector _returnvalue_6 _returnvalue_7 _returnvalue_8))
  (bind _returnvalue_10 (/ _returnvalue_9 _object_spacing))
  (bind (_x_2 _y_2) (Math|Vector|BreakVector _returnvalue_10))
  (if (Utilities|IsValid Object)
    (return (Math|Float|Truncate (+ (* _x_2 (LocalVariables|GetWW)) _y_2)))))

(fn BoradSpawn
  (for _index (range 0 (- (LocalVariables|GetW) 1))
    (LocalVariables|Set2dx21d _index)
    (bind _output_get (LocalVariables|SetX (+ (* (LocalVariables|Getpadding) _index) _index)))
    (for _index_2 (range 0 (- (LocalVariables|GetH) 1))
      (LocalVariables|Set2dx21d _index_2)
      (bind _output_get_2 (LocalVariables|SetY (+ (* (LocalVariables|Getpadding) _index_2) _index_2)))
      (return _output_get _output_get_2))))

(fn UnitsLocationCompute
  (params (area :type E_area%20Enum :default "NewEnumerator0") (x_axis :type Integer) (Y_axis :type Integer))
  (bind _padding (LocalVariables|Getpadding))
  (switch Utilities|FlowControl|Switch|SwitchonE_area area
    (:NewEnumerator0
      (return (Math|Transform|MakeTransform (Math|Vector|MakeVector (Math|Conversions|ToFloat(Integer) (+ (* x_axis 100) (LocalVariables|Getenemy%20juli))) (Math|Conversions|ToFloat(Integer) (* Y_axis 100)) 0.0))))
    (:NewEnumerator1
      (return (Math|Transform|MakeTransform (Math|Vector|MakeVector (Math|Conversions|ToFloat(Integer) (* (- x_axis _padding) 200)) (Math|Conversions|ToFloat(Integer) (* (- Y_axis _padding) 200)) 0.0))))))

(fn ChearLocationCompute
  (params (X :type Integer) (Y :type Integer))
  (return (Math|Transform|MakeTransform (Math|Vector|MakeVector (Math|Conversions|ToFloat(Integer) (* X 100)) (Math|Conversions|ToFloat(Integer) (* Y 100)) 0.0))))

(fn FormAXISbyINDEX
  (params (NewParam :type Integer))
  (return (/ NewParam 5) (+ (Math|Integer|%(Integer) NewParam 5) 1)))

(fn GetPC
  (bind _as2dplayer_contrller (Utilities|Casting|CastTo2DplayerContrller (Game|GetPlayerController 0)))
  (return _as2dplayer_contrller))

(fn AXIS-InverseCompute
  (params (location :type Vector))
  (bind (_x _y) (Math|Vector|BreakVector location))
  (return (+ (Math|Float|Floor (/ _x 2e+02)) 1) (Math|Float|Floor (/ _y 2e+02))))

(fn 2d21d
  (params (X :type Float%20%28double-precision%29) (Y :type Float%20%28double-precision%29))
  (return (Math|Float|Truncate (+ (* X (LocalVariables|GetW)) Y))))

(fn AdjustmentFunction
  (params (XAXIS :type Integer) (YAXIS :type Integer))
  (Utilities|FlowControl|Sequence
    (:then_0
      (if (<= XAXIS 0)
        (LocalVariables|SetXX (+ XAXIS 1))
        (else
          (LocalVariables|SetXX XAXIS))))
    (:then_1
      (LocalVariables|SetYY YAXIS))
    (:then_2
      (return (LocalVariables|GetXX) (LocalVariables|GetYY)))))

(fn ChessboardFunction
  (params (WS :type Integer) (HS :type Integer) (padding :type Integer))
  (for _index (range 0 (- WS 1))
    (LocalVariables|Set2DDX _index)
    (LocalVariables|SetXC (+ (* padding _index) _index))
    (for _index_2 (range 0 (- HS 1))
      (LocalVariables|Set2DDX _index_2)
      (LocalVariables|SetYC (+ (* padding _index_2) _index_2))
      (return (LocalVariables|GetXC) (LocalVariables|GetYC) (LocalVariables|Get2DDX)))))

(fn FindUnit
  (params (target_2D :type Vector%202D%20Structure) (2D :type Array%20of%20Vector%202D%20Structures) (battle :type BP%20Land%20Spaner%20Object%20Reference))
  (bind (_x _y) (Math|Vector2D|BreakVector2D target_2D))
  (for _array_element 2D
    (bind (_chear _returnvalue _character) (Default|CheckiftheActorIsValidV2-1(chear)0 (Variables|/Game/BP/BP_Battle_Phase/BP_land_spaner.BP_land_spaner_C|GetAs%20BP%20GLOBAL%20CHARATER battle) (- _x (.X (Math|Vector2D|BreakVector2D _array_element))) (- _y (.Y (Math|Vector2D|BreakVector2D _array_element)))))
    (if (Utilities|IsValid _chear)
      (if (Utilities|IsValid _character)
        (bind _asbp_character_class (Utilities|Casting|CastToBP_character_class _character))
        (if (Utilities|Struct|Breakst_unit_status (Variables|/Game/BP/BP_AC/BP_Generic_attributes_AC/AC_Generic_attributes.AC_Generic_attributes_C|Getthe_final_status (Variables|/Game/BP/BP_Battle_Phase/BP_BASE_Pawn.BP_BASE_Pawn_C|GetAC_Generic_attributes _asbp_character_class)))
          (Utilities|Array|Add (LocalVariables|Gettarget) _character)))))
  (return (LocalVariables|Gettarget)))