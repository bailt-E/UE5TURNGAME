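; Blueprint function library that calculates character attributes and level-up experience requirements.
; CalculateRoleAttributes builds attributes from a character level data table row, with constant speed and crit values.
; UpdataRoleAtt sums two attribute collections field by field, adding a third input for edge and fixed attributes only.
; The experience function totals remaining XP within a rank stage, using level ranges from the rank table, minus current XP.
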(fn CalculateRoleAttributes
  (params (RowName :type Name))
  (bind _returnvalue (Utilities|GetDataTableRow "/Game/Struct/rank_table/T_character_level_data.T_character_level_data" RowName)
    (:then
      (return (Utilities|Struct|MakeST_Attribute_collection_AA (Utilities|Struct|MakeST_Base_attributes_A (.Health (Utilities|Struct|Breakst_character_bese_level_data _returnvalue)) (.Attack (Utilities|Struct|Breakst_character_bese_level_data _returnvalue)) (.defense (Utilities|Struct|Breakst_character_bese_level_data _returnvalue)) 50 (Math|Float|Truncate 5.0) (Math|Float|Truncate 1.5e+02)) (Utilities|Struct|MakeST_Edge_attributes_A 0.0 0.0) (Utilities|Struct|MakeST_Fixed_attributes_A 300 25) "(element_bonus_3_7E47476240021223A27EB1B15F25B237=((),(element_type_2_A382164746729B1F7E90C0B960DFA649=NewEnumerator1),(element_type_2_A382164746729B1F7E90C0B960DFA649=NewEnumerator2),(element_type_2_A382164746729B1F7E90C0B960DFA649=NewEnumerator4),(element_type_2_A382164746729B1F7E90C0B960DFA649=NewEnumerator3)),Finaldamagebonus_7_C0F6EFE54D0D41C34BEE3BA503A9A25C=0.000000,Damagereductionbonus_9_9010B5E8408BD39C6EABC9BBEBF850BC=0.000000)")))))

(fn UpdataRoleAtt
  (params (NewParam1 :type St%20Character%20Bese%20Level%20Data%20Structure) (F1 :type ST%20Attribute%20Collection%20AA%20Structure%20%28by%20ref%29) (FIX :type ST%20Attribute%20Collection%20AA%20Structure%20%28by%20ref%29) (A2 :type St%20Rougelike%20Unit%20Bonus%20Structure%20%28by%20ref%29))
  (bind _secondary_attributes (Utilities|Struct|BreakST_Attribute_collection_AA FIX))
  (bind _secondary_attributes_2 (Utilities|Struct|BreakST_Attribute_collection_AA F1))
  (bind _edgeattrobutes (Utilities|Struct|Breakst_rougelike_unit_bonus A2))
  (bind _fixed_attributes (Utilities|Struct|BreakST_Attribute_collection_AA FIX))
  (bind _fixed_attributes_2 (Utilities|Struct|BreakST_Attribute_collection_AA F1))
  (bind _fixedattrobutes (Utilities|Struct|Breakst_rougelike_unit_bonus A2))
  (bind (_base_attributes _edge_attributes) (Utilities|Struct|BreakST_Attribute_collection_AA FIX))
  (bind (_base_attributes_2 _edge_attributes_2) (Utilities|Struct|BreakST_Attribute_collection_AA F1))
  (bind (_element_bonus _finaldamagebonus _damagereductionbonus) (Utilities|Struct|BreakST_Secondary_attributes_A _secondary_attributes_2))
  (bind (_healingbonus _healbonus _shieldedbonus _shieldbonus _aggro_bonus) (Utilities|Struct|BreakST_Edge_attributes_A _edgeattrobutes))
  (bind (_speedcap _overloadroundcap _maximumshield _overloadcap _energycap _unit_actionpointcap _element_tag_number_max _initialvelocity) (Utilities|Struct|BreakST_Fixed_attributes_A _fixedattrobutes))
  (bind (_healthy _attack _defense _velocity _criticalhits _criticaldamage _unit_actionpoints) (Utilities|Struct|BreakST_Base_attributes_A _base_attributes))
  (bind (_healthy_2 _attack_2 _defense_2 _velocity_2 _criticalhits_2 _criticaldamage_2 _unit_actionpoints_2) (Utilities|Struct|BreakST_Base_attributes_A _base_attributes_2))
  (bind (_healingbonus_2 _healbonus_2 _shieldedbonus_2 _shieldbonus_2 _aggro_bonus_2) (Utilities|Struct|BreakST_Edge_attributes_A _edge_attributes_2))
  (bind (_healingbonus_3 _healbonus_3 _shieldedbonus_3 _shieldbonus_3 _aggro_bonus_3) (Utilities|Struct|BreakST_Edge_attributes_A _edge_attributes))
  (bind (_speedcap_2 _overloadroundcap_2 _maximumshield_2 _overloadcap_2 _energycap_2 _unit_actionpointcap_2 _element_tag_number_max_2 _initialvelocity_2) (Utilities|Struct|BreakST_Fixed_attributes_A _fixed_attributes))
  (bind (_speedcap_3 _overloadroundcap_3 _maximumshield_3 _overloadcap_3 _energycap_3 _unit_actionpointcap_3 _element_tag_number_max_3 _initialvelocity_3) (Utilities|Struct|BreakST_Fixed_attributes_A _fixed_attributes_2))
  (bind (_element_bonus_2 _finaldamagebonus_2 _damagereductionbonus_2) (Utilities|Struct|BreakST_Secondary_attributes_A _secondary_attributes))
  (return (Utilities|Struct|MakeST_Attribute_collection_AA (Utilities|Struct|MakeST_Base_attributes_A (+ _healthy_2 _healthy) (+ _attack_2 _attack) (+ _defense_2 _defense) (+ _velocity_2 _velocity) (+ _criticalhits_2 _criticalhits) (+ _criticaldamage_2 _criticaldamage) (+ _unit_actionpoints_2 _unit_actionpoints)) (Utilities|Struct|MakeST_Edge_attributes_A (+ _healingbonus (+ _healingbonus_2 _healingbonus_3)) (+ _healbonus (+ _healbonus_2 _healbonus_3)) (+ _shieldedbonus (+ _shieldedbonus_2 _shieldedbonus_3)) (+ (+ _shieldbonus_2 _shieldbonus_3) _shieldbonus) (+ _aggro_bonus (+ _aggro_bonus_2 _aggro_bonus_3))) (Utilities|Struct|MakeST_Fixed_attributes_A (+ (+ _speedcap_3 _speedcap_2) _speedcap) (+ (+ _overloadroundcap_3 _overloadroundcap_2) _overloadroundcap) (+ (+ _maximumshield_3 _maximumshield_2) _maximumshield) (+ (+ _overloadcap_3 _overloadcap_2) _overloadcap) (+ (+ _energycap_3 _energycap_2) _energycap) (+ (+ _unit_actionpointcap_3 _unit_actionpointcap_2) _unit_actionpointcap) (+ (+ _element_tag_number_max_3 _element_tag_number_max_2) _element_tag_number_max) (+ (+ _initialvelocity_3 _initialvelocity_2) _initialvelocity)) (Utilities|Struct|MakeST_Secondary_attributes_A 0 (+ _finaldamagebonus _finaldamagebonus_2) (+ _damagereductionbonus _damagereductionbonus_2)))))

(fn CounttheExperienceNeededfortheCurrentStage
  (params (current_state :type Integer) (currentlevel :type Integer) (current_exp :type Integer))
  (bind _returnvalue (CallFunction|GetcharacterRand current_state))
  (for _index (range (+ (+ currentlevel 1) (.Initial (Utilities|Struct|Breakst_character_rank_info _returnvalue))) (.End (Utilities|Struct|Breakst_character_rank_info _returnvalue)))
    (bind _returnvalue_2 (Utilities|GetDataTableRow "/Game/Struct/rank_table/T_character_level_data.T_character_level_data" (Utilities|String|StringToName (Utilities|String|ToString(Integer) _index)))
      (:then
        (LocalVariables|Setneed_exp (+ (Utilities|Struct|Breakst_character_bese_level_data _returnvalue_2) (LocalVariables|Getneed_exp))))))
  (bind _returnvalue_3 (CallFunction|GetcharacterRand current_state))
  (bind _returnvalue_4 (Utilities|GetDataTableRow "/Game/Struct/rank_table/T_character_level_data.T_character_level_data" (Utilities|String|StringToName (Utilities|String|ToString(Integer) (+ currentlevel (.Initial (Utilities|Struct|Breakst_character_rank_info _returnvalue_3))))))
    (:then
      (bind _output_get (LocalVariables|Setneed_exp (+ (- (Utilities|Struct|Breakst_character_bese_level_data _returnvalue_4) current_exp) (LocalVariables|Getneed_exp))))
      (return _output_get))))

(fn GetcharacterRand
  (params (current_state :type Integer))
  (switch int current_state
    (:0
      (bind _returnvalue (Utilities|GetDataTableRow "/Game/Struct/common_Character_data/T_characer_rank_level_max.T_characer_rank_level_max" "rand0")
        (:then
          (return _returnvalue))))
    (:1
      (bind _returnvalue_2 (Utilities|GetDataTableRow "/Game/Struct/common_Character_data/T_characer_rank_level_max.T_characer_rank_level_max" "rand1")
        (:then
          (return _returnvalue_2))))
    (:2
      (bind _returnvalue_3 (Utilities|GetDataTableRow "/Game/Struct/common_Character_data/T_characer_rank_level_max.T_characer_rank_level_max" "rand2")
        (:then
          (return _returnvalue_3))))
    (:3
      (bind _returnvalue_4 (Utilities|GetDataTableRow "/Game/Struct/common_Character_data/T_characer_rank_level_max.T_characer_rank_level_max" "rand3")
        (:then
          (return _returnvalue_4))))))