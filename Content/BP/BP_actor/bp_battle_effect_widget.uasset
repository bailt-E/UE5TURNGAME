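; Floating combat text actor that displays a Damage value in battle through a widget component.
; On BeginPlay it picks a random horizontal drift, creates a Wbp_effect widget with Damage as its text and assigns it to the component.
; The Up timeline then moves the actor upward and sideways each update, lerping from its current location by the curve's alpha.
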(event EventBeginPlay
  (bind _returnvalue (Transformation|GetActorLocation))
  (bind (_x _y _z) (Math|Vector|BreakVector _returnvalue))
  (Utilities|FlowControl|Sequence
    (:then_0
      (Variables|Default|SetX (Math|Random|RandomFloatinRange -2.0 2.0))
      (Variables|Default|SetY (Math|Random|RandomFloatinRange -2.0 2.0)))
    (:then_1
      (bind _returnvalue_2 (UserInterface|CreateWidget "/Game/WBP/effect_widget/wbp_effect.wbp_effect_C" 0 (Variables|Default|Getdamage)))
      (UserInterface|SetWidget (Variables|Default|GetWidget) _returnvalue_2)
      (bind _新建轨道_0 (Timeline|up Play)
        (:Update
          (Transformation|SetActorLocation (Math|Vector|Lerp(Vector) _returnvalue (Math|Vector|MakeVector (+ _x (Variables|Default|GetX)) (+ _y (Variables|Default|GetY)) (+ _z 1.5)) _新建轨道_0) false false))))))

(fn ConstructionScript)