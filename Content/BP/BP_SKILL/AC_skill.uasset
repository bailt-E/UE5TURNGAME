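; Skill component that activates skills and shows selectable targets and hit range, driven by rows in TB_skill.
; Activation constructs the row's DirectSkills class and calls Activation with creator and target.
; Targeting marks all actors of the row's class as chosen; hit preview repositions units returned by the player pawn's row/column grid calculation.
; Cooldown, per-turn and use-count logic is unwired, and Tick's queue loop is empty.
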(event EventBeginPlay)

(event EventTick
  (params (DeltaSeconds :type Float%20%28single-precision%29))
  (for _array_element (Variables|Default|GetWAITADDskill_array)
    _))

(fn ActivationSkill
  (params (RowName :type Name) (create :type Actor%20Object%20Reference) (tager :type Actor%20Object%20Reference))
  (bind _returnvalue (Utilities|GetDataTableRow "/Game/Struct/st_skill/TB_skill.TB_skill" RowName)
    (:then
      (bind _returnvalue_2 (Game|ConstructObjectfromClass (Utilities|Struct|Breakst_skill_beseinfo _returnvalue)))
      (Default|Activation _returnvalue_2 create tager) ; 技能的激活
    )))

(fn DisplaystheRangeOfSkills
  (params (RowName :type Name))
  (bind _returnvalue (Utilities|GetDataTableRow "/Game/Struct/st_skill/TB_skill.TB_skill" RowName)
    (:then
      ;[1 1 1] 获得所有能选择的单位
      (bind _outactors (Actor|GetAllActorsOfClass (Utilities|Struct|Breakst_skill_beseinfo _returnvalue)))
      (bind _output_get (LocalVariables|Setskill_range _outactors))
      (for _array_element _output_get
        (Default|IsChosen _array_element) ; 为什么只有一个单位响应了
        (Utilities|Array|Add (LocalVariables|GetEligible%20actors) _array_element))
      (return (LocalVariables|GetEligible%20actors)))))

(fn 显示命中范围以及结果
  (params (base_unit :type BP%20BASE%20UNIT%20Object%20Reference) (RowName :type Name))
  (bind _asbp_global_charater (Utilities|Casting|CastToBP_GLOBAL_CHARATER (Game|Player|GetPlayerPawn 0)))
  (bind _returnvalue (Utilities|GetDataTableRow "/Game/Struct/st_skill/TB_skill.TB_skill" RowName)
    (:then
      (bind _result (Default|CaculateDirectionYouCanWalkV2(skill) _asbp_global_charater (.Skillcolumn (Utilities|Struct|Breakst_skill_beseinfo _returnvalue)) (Transformation|GetActorLocation base_unit) (.skill_row (Utilities|Struct|Breakst_skill_beseinfo _returnvalue)))) ; 获得技能的数组，并基于数组
      (for _array_element _result
        (bind _asbp_base_unit (Utilities|Casting|CastToBP_BASE_UNIT _array_element))
        (Default|Reposition _asbp_base_unit))
      (return))))