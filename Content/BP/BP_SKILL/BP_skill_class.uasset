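; BP_skill_class is a skill class for what appears to be a turn-based game, with empty stubs for activation and turn control (Huihekongzhi).
; 初始化 looks up a TB_skill row by name and caches persistent turns, action count and countdown.
; Decrease rebuilds the pawn's KaletaFinalAttributes from SkillInfo, adding debt, erosion and overload.
; For health and speed it computes the depletion value minus the current value, not the reverse.
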(fn Activation
  (params (create :type Actor%20Object%20Reference) (tager :type Actor%20Object%20Reference)))

(fn Decrease
  (params (pawn :type BP%20Base%20Pawn%20Class%20Object%20Reference))
  (bind _skill_info (Variables|Default|Getskill_info))
  (bind (_deplete_speed _overload_speed _deplete_life _deplete_overlordspeed _lifeerosion _lifedebt) (Utilities|Struct|Breakst_skill_beseinfo _skill_info))
  (Variables|/Game/BP/BP_modelE/BP_base_pawn_class.BP_base_pawn_class_C|Setkaleta_final_attributes pawn (Utilities|Struct|Makest_child_base_attributes (- _deplete_life (.Currentlife (Utilities|Struct|Breakst_child_base_attributes (Variables|/Game/BP/BP_modelE/BP_base_pawn_class.BP_base_pawn_class_C|Getkaleta_final_attributes pawn)))) (+ _lifedebt (.Lifedebt (Utilities|Struct|Breakst_child_base_attributes (Variables|/Game/BP/BP_modelE/BP_base_pawn_class.BP_base_pawn_class_C|Getkaleta_final_attributes pawn)))) (+ _lifeerosion (.Anomalouslife (Utilities|Struct|Breakst_child_base_attributes (Variables|/Game/BP/BP_modelE/BP_base_pawn_class.BP_base_pawn_class_C|Getkaleta_final_attributes pawn)))) (- _deplete_speed (.speed (Utilities|Struct|Breakst_child_base_attributes (Variables|/Game/BP/BP_modelE/BP_base_pawn_class.BP_base_pawn_class_C|Getkaleta_final_attributes pawn)))) (+ _overload_speed (.overload (Utilities|Struct|Breakst_child_base_attributes (Variables|/Game/BP/BP_modelE/BP_base_pawn_class.BP_base_pawn_class_C|Getkaleta_final_attributes pawn)))))))

(fn 初始化
  (params (RowName :type Name))
  (bind _returnvalue (Utilities|GetDataTableRow "/Game/Struct/st_skill/TB_skill.TB_skill" RowName)
    (:then
      (Variables|Default|SetSkill%20Persistent%20Turn (.skill_persistent_turn (Utilities|Struct|Breakst_skill_beseinfo _returnvalue)))
      (Variables|Default|SetSkill%20Number%20Of%20Actions (.skill_Numberofactions (Utilities|Struct|Breakst_skill_beseinfo _returnvalue)))
      (Variables|Default|SetSkill%20Countdown (.skill_countdown (Utilities|Struct|Breakst_skill_beseinfo _returnvalue))))))

(fn Huihekongzhi)