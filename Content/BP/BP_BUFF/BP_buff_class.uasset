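; Buff base class that tracks a turn-based duration for an effect on a target.
; Initialize stores the target, the Create argument and the starting round count, while Create and InTheEnd are empty hooks.
; Tick returns true without decrementing when a non-forever buff has enough turns left for the given amount; otherwise it subtracts that amount and returns false.
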(fn Create)

(fn IntheEnd)

(fn Tick
  (params (B :type Integer))
  (if (and (>= (- (Variables|Default|GetRemaining_turn) B) 0) (not (Utilities|Struct|Breakst_buff_attribute_info (Variables|Default|Getbuffinfo))))
    (return true)
    (else
      (Variables|Default|SetRemaining_turn (- (Variables|Default|GetRemaining_turn) B))
      (return false))))

(fn Initialize
  (params (st_buff_attribute_info :type St%20Buff%20Attribute%20Info%20Structure%20%28by%20ref%29) (target :type Actor%20Object%20Reference) (create :type Actor%20Object%20Reference))
  (Variables|Default|SetTarget target)
  (Variables|Default|SetCreate_0 create)
  (Variables|Default|SetRemaining_turn (Utilities|Struct|Breakst_buff_attribute_info st_buff_attribute_info)))