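; AC_buff is a buff manager, apparently an actor component, that creates buff effect objects from rows in T_buff_table and runs their lifecycle.
; Addbuff constructs and initializes the row's effect class, then queues it in WaitAddBuff.
; Each Tick passes truncated integer delta seconds to BuffTick, which activates queued buffs, ticks current ones, and calls InTheEnd on those reporting finished.
; A turn-check event binding exists but never runs.
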(event Custom|自定义事件)

(event EventBeginPlay)

(event EventTick
  (params (DeltaSeconds :type Float%20%28single-precision%29))
  (CallFunction|BuffTick (Math|Float|Truncate DeltaSeconds)))

(fn Addbuff
  (params (RowName :type Name) (target :type Actor%20Object%20Reference) (create :type Actor%20Object%20Reference))
  (bind _returnvalue (Utilities|GetDataTableRow "/Game/Struct/st_buff/T_buff_table.T_buff_table" RowName)
    (:then
      (bind _returnvalue_2 (Game|ConstructObjectfromClass (Utilities|Struct|Breakst_buff_attribute_info _returnvalue)))
      (Default|Initialize _returnvalue_2 _returnvalue target create)
      (Utilities|Array|Add (Variables|Default|Getwait_add_buff) _returnvalue_2))))

(fn BuffTick
  (params (B :type Integer))
  (Utilities|FlowControl|Sequence
    (:then_0
      (for _array_element (Variables|Default|Getwait_add_buff)
        (Utilities|Array|Add (Variables|Default|Getcurrent_buff) _array_element)
        (Default|Create _array_element) ; point
        (Utilities|Array|RemoveItem (Variables|Default|Getwait_add_buff) _array_element)))
    (:then_1
      (for _array_element_2 (Variables|Default|Getcurrent_buff)
        (bind _newparam (Default|Tick _array_element_2 B)) ; point
        (if _newparam
          (Utilities|Array|Add (Variables|Default|Getwait_remove_buff) _array_element_2)))
      (Utilities|Array|RemoveItem (Variables|Default|Getcurrent_buff) _array_element_2))
    (:then_2
      (for _array_element_3 (Variables|Default|Getwait_remove_buff)
        (Default|IntheEnd _array_element_3) ; point
        (Utilities|Array|RemoveItem (Variables|Default|Getwait_remove_buff) _array_element_3)))))